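; BP_SaveGameData holds per-faction save data: character rosters, diplomacy and town camps.
; On new game it takes the team faction list from game metadata and fills arrays parallel to that list from each preset's defaults, writing modified structs back by index.
; Continue only reloads the faction list, with checkpoints marked todo.
; Interface functions append missing factions and return the list, rosters and diplomacy, but not town camps.
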(event EventSGDISaveGameData-NewGameMetaDataSETI
  (params (NewMetaGameData :type Primary%20Data%20Asset%20Object%20Reference))
  (bind _teamfactionpresetid_logindexer (Class|BPIMetaDataPresetInterfaceI|SGIMetaGameDataGETI(Message) NewMetaGameData))
  (bind _output_get (Variables|Default|SetTeamFactionPresetID_LogIndexerx _teamfactionpresetid_logindexer))
  (CallFunction|NewGame-DataSetupF _output_get))

(event EventSGDISaveGameData-ContinueGameLoadedDataETI
  (params (CheckptMetaGameData :type Primary%20Data%20Asset%20Object%20Reference) (MetaProgression :type Array%20of%20Booleans))
  ;[1 1 1] Todolater: ZeroTimeDelima style checkpoints
  (bind _teamfactionpresetid_logindexer (Class|BPIMetaDataPresetInterfaceI|SGIMetaGameDataGETI(Message) CheckptMetaGameData))
  (Variables|Default|SetTeamFactionPresetID_LogIndexerx _teamfactionpresetid_logindexer))

(fn NewGame-DataSetupF
  (params (TeamFactionPresetIDLogIndexer :type Array%20of%20Primary%20Data%20Asset%20Object%20References))
  (for (_array_element _array_index) TeamFactionPresetIDLogIndexer
    (CallFunction|NewGame-DataSetupHiearchyRosterF _array_index _array_element)
    (CallFunction|NewGame-DataSetupDiplomacyAlignmentF _array_index _array_element)
    (CallFunction|NewGame-DataSetupTownCampsF _array_index _array_element)))

(fn NewGame-DataSetupHiearchyRosterF
  (params (TeamFactionPresetID-Index :type Integer) (TeamFactionPresetID-Pda :type Primary%20Data%20Asset%20Object%20Reference))
  (LocalVariables|SetTeamFactionPresetID_Local TeamFactionPresetID-Pda)
  (LocalVariables|SetTeamFactionPresetIDIndex_Local TeamFactionPresetID-Index)
  ;[1 1 1] SingleTeam
  (bind _output_get (LocalVariables|SetHierarhcyRoster-SingleTeam_Local (Utilities|Array|Get(acopy) (Variables|Default|GetHierarchyRoster) TeamFactionPresetID-Index)))
  (LocalVariables|SetCharacterPresetIDLogIndexer-SingleTeam_Local (.CharacterPresetIndexer (Utilities|Struct|BreakS_HierarchyRoster01TeamRoster _output_get)))
  (LocalVariables|SetCharacterInfoArray-SingleTeam_Local (.CharacterInfoArray (Utilities|Struct|BreakS_HierarchyRoster01TeamRoster _output_get)))
  (bind _hierarchyrosterdefault (Class|BPITeamFactionPresetInterfaceI|TFPITeamFactionPresetInfoGETI(Message) (LocalVariables|GetTeamFactionPresetID_Local)))
  (for (_array_element _array_index) _hierarchyrosterdefault
    ;[1 1 1] Character Entry
    (LocalVariables|SetCharacterPresetIDEntry_Local _array_element)
    (LocalVariables|SetCharacterPresetIDEntryIndex_local _array_index)
    (Utilities|Array|SetArrayElem (LocalVariables|GetCharacterPresetIDLogIndexer-SingleTeam_Local) (LocalVariables|GetCharacterPresetIDEntryIndex_local) (LocalVariables|GetCharacterPresetIDEntry_Local) true)
    ;[1 1 1] HierarchyRoster
    (bind _structout (Utilities|Struct|SetmembersinS_HierarchyRoster01TeamRoster (LocalVariables|GetHierarhcyRoster-SingleTeam_Local) (LocalVariables|GetCharacterPresetIDLogIndexer-SingleTeam_Local) (LocalVariables|GetCharacterInfoArray-SingleTeam_Local)))
    (bind _output_get_2 (LocalVariables|SetHierarhcyRoster-SingleTeam_Local _structout))
    (Utilities|Array|SetArrayElem (Variables|Default|GetHierarchyRoster) (LocalVariables|GetTeamFactionPresetIDIndex_Local) _output_get_2 true)))

(fn NewGame-DataSetupDiplomacyAlignmentF
  (params (TeamFactionPresetID-Index :type Integer) (TeamFactionPresetID-Pda :type Primary%20Data%20Asset%20Object%20Reference))
  (bind _diplomacyalignment (Variables|Default|GetDiplomacyAlignment))
  (bind _output (Utilities|Array|Get(acopy) _diplomacyalignment TeamFactionPresetID-Index))
  (bind (_teamfactionpresetid_replacedbyindexer ___ _enemylogindexer _enemy_factionshated_war _alliedlogindexer _allied_factionsliked_alliance _nuetrallogindexer _nuetral_factions) (Utilities|Struct|BreakS_DiplomacyAlignment01 _output))
  (LocalVariables|SetTeamFactionPresetID_Local TeamFactionPresetID-Pda)
  (LocalVariables|SetTeamFactionPresetIDIndex_Local TeamFactionPresetID-Index)
  ;[1 1 1] SingleTeam
  (LocalVariables|SetDiplomacyAlignment-OfSingleTeam_Local _output)
  (LocalVariables|SetEnemyIDLogIndexer_Local _enemylogindexer)
  (LocalVariables|SetEnemyInfoArray_Local _enemy_factionshated_war)
  (LocalVariables|SetAlliedIDLogIndexer_Local _alliedlogindexer)
  (LocalVariables|SetAlliedInfoArray_local _allied_factionsliked_alliance)
  (LocalVariables|SetNuetralIdLogIndexer_Local _nuetrallogindexer)
  (LocalVariables|SetNuetralInfoArray_Local _nuetral_factions)
  ;[1 1 1] TeamFraction
  (bind (_towncamps _hierarchyrosterdefault _diplomaticalignment_enemiesstartdefault _diplomaticalignment_alliesstartdefault _diplomaticalignment_nuetralstartdefault) (Class|BPITeamFactionPresetInterfaceI|TFPITeamFactionPresetInfoGETI(Message) (LocalVariables|GetTeamFactionPresetID_Local)))
  (Utilities|FlowControl|Sequence
    (:then_0
      (for (_array_element _array_index) _diplomaticalignment_enemiesstartdefault
        (LocalVariables|SetEntry_Local _array_element)
        (LocalVariables|SetEntryIndex_local _array_index)
        (Utilities|Array|SetArrayElem (LocalVariables|GetEnemyIDLogIndexer_Local) (LocalVariables|GetEntryIndex_local) (LocalVariables|GetEntry_Local) true)
        ;[1 1 1] Enemy
        (bind _structout (Utilities|Struct|SetmembersinS_DiplomacyAlignment01 (LocalVariables|GetDiplomacyAlignment-OfSingleTeam_Local) (LocalVariables|GetTeamFactionPresetID_Local) (LocalVariables|GetEnemyIDLogIndexer_Local) (LocalVariables|GetEnemyInfoArray_Local)))
        (bind _output_get (LocalVariables|SetDiplomacyAlignment-OfSingleTeam_Local _structout))
        (Utilities|Array|SetArrayElem (Variables|Default|GetDiplomacyAlignment) (LocalVariables|GetTeamFactionPresetIDIndex_Local) _output_get true)))
    (:then_1
      (for (_array_element_2 _array_index_2) _diplomaticalignment_alliesstartdefault
        (LocalVariables|SetEntry_Local _array_element_2)
        (LocalVariables|SetEntryIndex_local _array_index_2)
        (Utilities|Array|SetArrayElem (LocalVariables|GetAlliedIDLogIndexer_Local) (LocalVariables|GetEntryIndex_local) (LocalVariables|GetEntry_Local) true)
        ;[1 1 1] Ally
        (bind _structout_2 (Utilities|Struct|SetmembersinS_DiplomacyAlignment01 (LocalVariables|GetDiplomacyAlignment-OfSingleTeam_Local) (LocalVariables|GetTeamFactionPresetID_Local) (LocalVariables|GetAlliedIDLogIndexer_Local) (LocalVariables|GetAlliedInfoArray_local)))
        (bind _output_get_2 (LocalVariables|SetDiplomacyAlignment-OfSingleTeam_Local _structout_2))
        (Utilities|Array|SetArrayElem (Variables|Default|GetDiplomacyAlignment) (LocalVariables|GetTeamFactionPresetIDIndex_Local) _output_get_2 true)))
    (:then_2
      (for (_array_element_3 _array_index_3) _diplomaticalignment_nuetralstartdefault
        (LocalVariables|SetEntry_Local _array_element_3)
        (LocalVariables|SetEntryIndex_local _array_index_3)
        (Utilities|Array|SetArrayElem (LocalVariables|GetNuetralIdLogIndexer_Local) (LocalVariables|GetEntryIndex_local) (LocalVariables|GetEntry_Local) true)
        ;[1 1 1] Nuetral
        (bind _structout_3 (Utilities|Struct|SetmembersinS_DiplomacyAlignment01 (LocalVariables|GetDiplomacyAlignment-OfSingleTeam_Local) (LocalVariables|GetTeamFactionPresetID_Local) (LocalVariables|GetNuetralIdLogIndexer_Local) (LocalVariables|GetNuetralInfoArray_Local)))
        (bind _output_get_3 (LocalVariables|SetDiplomacyAlignment-OfSingleTeam_Local _structout_3))
        (Utilities|Array|SetArrayElem (Variables|Default|GetDiplomacyAlignment) (LocalVariables|GetTeamFactionPresetIDIndex_Local) _output_get_3 true)))))

(fn NewGame-DataSetupTownCampsF
  (params (TeamFactionPresetID-Index :type Integer) (TeamFactionPresetID-Pda :type Primary%20Data%20Asset%20Object%20Reference))
  (LocalVariables|SetTeamFactionPresetID_Local TeamFactionPresetID-Pda)
  (LocalVariables|SetTeamFactionPresetIDIndex_Local TeamFactionPresetID-Index)
  ;[1 1 1] SingleTeam
  (bind _output_get (LocalVariables|SetCampTownsOfSingleTeam_Local (Utilities|Array|Get(acopy) (Variables|Default|GetTownCamps) TeamFactionPresetID-Index)))
  (LocalVariables|SetCampTownIDLogIndexer-OfSingleTeam_Local (.CampTownLogIndexer (Utilities|Struct|BreakS_CampTown01FactionMangement _output_get)))
  (LocalVariables|SetCampTownInfoArray-OfSingleTeam_Local (.CampTownInfoArray (Utilities|Struct|BreakS_CampTown01FactionMangement _output_get)))
  ;[1 1 1] Character Entry
  (bind _towncamps (Class|BPITeamFactionPresetInterfaceI|TFPITeamFactionPresetInfoGETI(Message) (LocalVariables|GetTeamFactionPresetID_Local)))
  (for (_array_element _array_index) _towncamps
    (LocalVariables|SetCampTownPresetIDEntry_Local _array_element)
    (LocalVariables|SetCampTownPresetIDEntryIndex_local _array_index)
    (Utilities|Array|SetArrayElem (LocalVariables|GetCampTownIDLogIndexer-OfSingleTeam_Local) (LocalVariables|GetCampTownPresetIDEntryIndex_local) (LocalVariables|GetCampTownPresetIDEntry_Local) true)
    ;[1 1 1] HierarchyRoster
    (bind _structout (Utilities|Struct|SetmembersinS_CampTown01FactionMangement (LocalVariables|GetCampTownsOfSingleTeam_Local) (LocalVariables|GetTeamFactionPresetID_Local) (LocalVariables|GetCampTownIDLogIndexer-OfSingleTeam_Local) (LocalVariables|GetCampTownInfoArray-OfSingleTeam_Local)))
    (bind _output_get_2 (LocalVariables|SetCampTownsOfSingleTeam_Local _structout))
    (Utilities|Array|SetArrayElem (Variables|Default|GetTownCamps) (LocalVariables|GetTeamFactionPresetIDIndex_Local) _output_get_2 true)))

(fn SGDISaveGameDataInfoADDMissingTeamFactionI
  (params (TeamFactionPresetID :type Primary%20Data%20Asset%20Object%20Reference))
  (bind _returnvalue (Utilities|Array|Add (Variables|Default|GetTeamFactionPresetID_LogIndexerx) TeamFactionPresetID))
  (return _returnvalue))

(fn SGDISaveGameDataInfoGETI
  (return (Variables|Default|GetTeamFactionPresetID_LogIndexerx) (Variables|Default|GetHierarchyRoster) (Variables|Default|GetDiplomacyAlignment) 0))