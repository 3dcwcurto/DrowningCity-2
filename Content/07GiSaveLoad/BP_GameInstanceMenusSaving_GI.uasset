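; Game instance that creates the current save-data object on Init and exposes it through an interface getter.
; It always seeds a new game from the Drowning City meta-data preset, then caches team index, hierarchy roster, diplomacy and town camp data.
; Slot loading and saving nodes are unwired.
; A roster update function marked "dontNeed" records character alive state per faction, but its faction lookup is stubbed to return invalid.
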(event EventInit
  ;[1 1 1] Load All Settings Vs CreateNewGame
  (CallFunction|DataSetup01LoadGameVsNewGameSetup-MainF))

(fn DataSetup01LoadGameVsNewGameSetup-MainF
  (bind _returnvalue (SaveGame|CreateSaveGameObject "/Game/07GiSaveLoad/SaveData/BP_SaveGameData.BP_SaveGameData_C"))
  (bind _output_get (Variables|Default|SetData_SaveGameDataCurrent _returnvalue))
  ;[1 1 1] New Game
  (CallFunction|DataSetup01NewGameDataF "/Game/xDc07GiSaveloadGame/DA_MetaDataPreset01NewGameDrowAgoge_xDrowningCity.DA_MetaDataPreset01NewGameDrowAgoge_xDrowningCity" _output_get))

(fn DataSetup01NewGameDataF
  (params (MetaGameDataPreset :type Primary%20Data%20Asset%20Object%20Reference) (SaveGameDataObject :type Save%20Game%20Object%20Reference))
  (Class|BPISaveGameDataInterfaceI|SGDISaveGameData-NewGameMetaDataSETI(Message) SaveGameDataObject MetaGameDataPreset)
  (bind (_teamfactionpresetid_logindexerx _hierarchyroster _diplomaticstance _towncamp) (Class|BPISaveGameDataInterfaceI|SGDISaveGameDataInfoGETI(Message) (Variables|Default|GetData_SaveGameDataCurrent)))
  (Variables|Default|SetTeamFactionPreset-IDLogIndexer-Runtime _teamfactionpresetid_logindexerx)
  (Variables|Default|SetHierarchy%20Roster _hierarchyroster)
  (Variables|Default|SetDiplomatic%20Stance _diplomaticstance)
  (Variables|Default|SetTown%20Camp _towncamp))

(fn HierarchyRosterSetupCharacterFv2-dontNeed
  (params (CharacterRuntime :type Character%20Object%20Reference))
  ;[1 1 1] CharacterRuntime
  (bind _output_get (LocalVariables|SetCharacterRuntime_Local CharacterRuntime))
  ;[1 1 1] CharacterPreset
  (bind _pdacharacterpreset (Class|BPICharacterBaseInterface|CBICharacterPresetPdaGETI(Message) _output_get))
  (bind _output_get_2 (LocalVariables|SetCharacterPresetID_Local _pdacharacterpreset))
  ;[1 1 1] Character's Team
  (bind _teamfactionpresetid (Class|BPICharacterPresetInterface|HCPICharacterPresetInfoGETI(Message) _output_get_2))
  (bind _output_get_3 (LocalVariables|SetTeamFactionPresetID_LOcal _teamfactionpresetid))
  (LocalVariables|SetTeamFactionLogIndexer_Local (.TeamFactionIDIndex (CallFunction|TeamFaction-LogIndexFindCreatePureFv2-dontNeed _output_get_3)))
  (if (.Valid (CallFunction|TeamFaction-LogIndexFindCreatePureFv2-dontNeed _output_get_3))
    (bind _output_get_4 (LocalVariables|SetHierachyRoster01TeamRoster_OfSingleFaction_local (Utilities|Array|Get(acopy) (Variables|Default|GetHierarchy%20Roster) (LocalVariables|GetTeamFactionLogIndexer_Local))))
    (LocalVariables|SetCharacterPresetLogIndexer_local (.CharacterPresetIndexer (Utilities|Struct|BreakS_HierarchyRoster01TeamRoster _output_get_4)))
    (LocalVariables|SetHierachyRoster02CharacterInfoArray_Local (.CharacterInfoArray (Utilities|Struct|BreakS_HierarchyRoster01TeamRoster _output_get_4)))
    (if (Utilities|Array|ContainsItem (LocalVariables|GetCharacterPresetLogIndexer_local) (LocalVariables|GetCharacterPresetID_Local))
      ;[1 1 1] Update Alive&RealtimeCharacter
      ;;[1 1 1] Indexer
      (LocalVariables|SetHierachyRoster02CharacterRosterIndex_Local (Utilities|Array|FindItem (LocalVariables|GetCharacterPresetLogIndexer_local) (LocalVariables|GetCharacterPresetID_Local)))
      ;;[1 1 1] CharacterEntry
      (LocalVariables|SetHierachyRoster02CharacterRosterEntry_Local (Utilities|Array|Get(acopy) (LocalVariables|GetHierachyRoster02CharacterInfoArray_Local) (Utilities|Array|FindItem (LocalVariables|GetCharacterPresetLogIndexer_local) (LocalVariables|GetCharacterPresetID_Local))))
      (bind _bisalive (Class|BPCharacterStatsInterfaceI|CSIAliveGETCheckI(Message) (LocalVariables|GetCharacterRuntime_Local)))
      (bind _structout (Utilities|Struct|SetmembersinS_HierarchyRoster02CharactersRoster (Utilities|Struct|MakeS_HierarchyRoster02CharactersRoster (LocalVariables|GetCharacterRuntime_Local) _bisalive)))
      (bind _output_get_5 (LocalVariables|SetHierachyRoster02CharacterRosterEntry_Local _structout))
      (Utilities|Array|SetArrayElem (LocalVariables|GetHierachyRoster02CharacterInfoArray_Local) (LocalVariables|GetHierachyRoster02CharacterRosterIndex_Local) _output_get_5 true)
      ;;[1 1 1] Single TeamFaction's CharactersArray
      (bind _structout_2 (Utilities|Struct|SetmembersinS_HierarchyRoster01TeamRoster (LocalVariables|GetHierachyRoster01TeamRoster_OfSingleFaction_local) (LocalVariables|GetHierachyRoster02CharacterInfoArray_Local)))
      (LocalVariables|SetHierachyRoster01TeamRoster_OfSingleFaction_local _structout_2)
      (Utilities|Array|SetArrayElem (Variables|Default|GetHierarchy%20Roster) (LocalVariables|GetTeamFactionLogIndexer_Local) (LocalVariables|GetHierachyRoster01TeamRoster_OfSingleFaction_local) true)
      (else
        ;[1 1 1] NewFallback
        (Development|PrintString "BPGameInstanceMenusSavingGI>HierarchyRosterSetupCharacterF== Character not contained in Data")
        ;;[1 1 1] CharacterEntry
        (Utilities|Array|Add (LocalVariables|GetCharacterPresetLogIndexer_local) (LocalVariables|GetCharacterPresetID_Local))
        (bind _bisalive_2 (Class|BPCharacterStatsInterfaceI|CSIAliveGETCheckI(Message) (LocalVariables|GetCharacterRuntime_Local)))
        (Utilities|Array|Add (LocalVariables|GetHierachyRoster02CharacterInfoArray_Local) (Utilities|Struct|MakeS_HierarchyRoster02CharactersRoster (LocalVariables|GetCharacterRuntime_Local) _bisalive_2))
        ;;[1 1 1] Single TeamFaction's CharactersArray
        (LocalVariables|SetHierachyRoster01TeamRoster_OfSingleFaction_local (Utilities|Struct|MakeS_HierarchyRoster01TeamRoster (LocalVariables|GetCharacterPresetLogIndexer_local) (LocalVariables|GetHierachyRoster02CharacterInfoArray_Local)))
        ;;[1 1 1] TeamFactionArray
        (Utilities|Array|SetArrayElem (Variables|Default|GetHierarchy%20Roster) (LocalVariables|GetTeamFactionLogIndexer_Local) (LocalVariables|GetHierachyRoster01TeamRoster_OfSingleFaction_local) true)))))

(fn TeamFaction-LogIndexFindCreatePureFv2-dontNeed
  (params (TeamFactionPreset :type Primary%20Data%20Asset%20Object%20Reference))
  (return 0 false))

(fn GIISaveGameDataCurrentGetI
  (return (Variables|Default|GetData_SaveGameDataCurrent)))