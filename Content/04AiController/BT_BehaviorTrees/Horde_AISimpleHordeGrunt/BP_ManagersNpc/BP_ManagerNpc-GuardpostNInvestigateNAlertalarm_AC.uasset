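; Manager component for horde grunt NPCs that tracks patrol-route progress and guard-post patrol/protect state.
; It lazily caches the owning controller's pawn and pulls its route actor, path points and settings through interface calls.
; Functions set the start index by direction, step it, resolve world locations from route-local points, and either loop or reverse at lap end.
; Most return validity or patrol state; despite the name, no investigate or alarm logic is present.
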(fn ReferenceCharacterRefPureF
  (Utilities|IsValid (Variables|Default|GetOwningActorRef)
    (:Is%20Valid
      (return (Variables|Default|GetOwningActorRef)))
    (:Is%20Not%20Valid
      (bind _ascontroller (Utilities|Casting|CastToController (Components|GetOwner)))
      (bind _output_get (Variables|Default|SetOwningControllerRef _ascontroller))
      (bind _output_get_2 (Variables|Default|SetOwningActorRef (Pawn|GetControlledPawn _output_get)))
      (return _output_get_2))))

(fn PatrolRouteStart-DirectionNIndexUPDATEF
  (bind _patrol_routeactorref (Variables|Default|GetPatrol%20RouteActorRef))
  (Utilities|IsValid _patrol_routeactorref
    (:Is%20Valid
      (bind (_patrolpath2 _patrollapcompletion_circleorreverse _patrolstartdirection_forwardbackward) (Class|BPIPatrolRouteInterfaceI|PRIPatrolRouteInfoGETI(Message) _patrol_routeactorref))
      (bind _output_get (Variables|Default|SetPatrolRouteDirection _patrolstartdirection_forwardbackward))
      (switch Utilities|FlowControl|Switch|SwitchonE_GenericDirectionSimple-ForwardVsBackwards _output_get
        (:NewEnumerator0
          (Development|PrintString "BTTaskPatrolRouteStartSetDirectionnIndex>EG== Patrol Actor Direction is null" true true "(R=1.000000,G=0.042986,B=0.000000,A=1.000000)" 22.0)
          (Variables|Default|SetPatolRouteIndex 0 :!label _label))
        (:NewEnumerator1
          (goto _label))
        (:NewEnumerator2
          (Variables|Default|SetPatolRouteIndex (- (Utilities|Array|Length _patrolpath2) 1))))
      (if (Utilities|Array|IsValidIndex _patrolpath2 (Variables|Default|GetPatolRouteIndex))
        (Variables|Default|SetPatrolRouteLocation (Utilities|Array|Get(acopy) _patrolpath2 (Variables|Default|GetPatolRouteIndex)))
        (return true)
        (else
          (Development|PrintString "BPInfoNpcPatrolStateAC>PatrolRouteStart== PatrolRoutePath Array Index is not valid" true true "(R=1.000000,G=0.366009,B=0.000000,A=1.000000)" 22.0)
          (return false))))
    (:Is%20Not%20Valid
      (Development|PrintString "BPInfoNpcPatrolStateAC>PatrolRouteStart== PatrolRoute is not valid" true true "(R=1.000000,G=0.366009,B=0.000000,A=1.000000)" 22.0)
      (return false))))

(fn PatrolRouteLocationUPDATEF
  (bind _patrol_routeactorref (Variables|Default|GetPatrol%20RouteActorRef))
  (bind _patolrouteindex (Variables|Default|GetPatolRouteIndex))
  (Utilities|IsValid _patrol_routeactorref
    (:Is%20Valid
      (bind _patrolpath2 (Class|BPIPatrolRouteInterfaceI|PRIPatrolRouteInfoGETI(Message) _patrol_routeactorref))
      (if (Utilities|Array|IsValidIndex _patrolpath2 _patolrouteindex)
        (bind _output_get (Variables|Default|SetPatrolRouteLocation (Math|Transform|TransformLocation (Transformation|GetActorTransform _patrol_routeactorref) (Utilities|Array|Get(acopy) _patrolpath2 _patolrouteindex))))
        (return _output_get true)
        (else
          (Development|PrintString "BPManagerNpcPatrolStateAC>PatrolRouteLocationUpdateF== PatrolValid index is not valid" true true "(R=1.000000,G=0.235961,B=0.000000,A=1.000000)" 22.0))))
    (:Is%20Not%20Valid
      (Development|PrintString "BPManagerNpcPatrolStateAC>PatrolRouteLocationUpdateF==PatrolRoute not valid" true true "(R=1.000000,G=0.217986,B=0.000000,A=1.000000)" 22.0)))
  (return "0, 0, 0" false))

(fn PatrolRouteIndex-DecrementorIncrementUPDATEF
  (Development|PrintString (Utilities|String|ToString(Integer) (Variables|Default|GetPatolRouteIndex)) true true "(R=1.000000,G=0.252429,B=0.000000,A=1.000000)" 22.0)
  (Utilities|IsValid (Variables|Default|GetPatrol%20RouteActorRef)
    (:Is%20Valid
      (switch Utilities|FlowControl|Switch|SwitchonE_GenericDirectionSimple-ForwardVsBackwards (Variables|Default|GetPatrolRouteDirection)
        (:NewEnumerator0
          (Development|PrintString "BPManagerNpcGuardPostPatrolNProtect== PatrolDirection is null" true true "(R=1.000000,G=0.252429,B=0.000000,A=1.000000)" 22.0))
        (:NewEnumerator1
          _)
        (:NewEnumerator2
          (if (< (- (Variables|Default|GetPatolRouteIndex) 1) 0)
            (return "NewEnumerator2" true)
            (else
              (Variables|Default|SetPatolRouteIndex (- (Variables|Default|GetPatolRouteIndex) 1))
              ;[1 1 1] Unchanged
              (return "NewEnumerator1" true)))))
      (bind _patrolpath2 (Class|BPIPatrolRouteInterfaceI|PRIPatrolRouteInfoGETI(Message) (Variables|Default|GetPatrol%20RouteActorRef)))
      (if (> (+ (Variables|Default|GetPatolRouteIndex) 1) (- (Utilities|Array|Length _patrolpath2) 1))
        (return "NewEnumerator2" true)
        (else
          (Variables|Default|SetPatolRouteIndex (+ (Variables|Default|GetPatolRouteIndex) 1))
          ;[1 1 1] Unchanged
          (return "NewEnumerator1" true))))
    (:Is%20Not%20Valid
      (Development|PrintString "BTTask_PatrolRouteIncrementIndex>EG== PatrolActor is not valid" true true "(R=1.000000,G=0.252429,B=0.000000,A=1.000000)" 22.0)
      (return "NewEnumerator4" false))))

(fn PatrolRouteActorUPDATEF
  (bind _owningactorrefout (CallFunction|ReferenceCharacterRefPureF))
  (Utilities|IsValid _owningactorrefout
    (:Is%20Valid
      (bind _patrolroute (Class|BPICharacterAIMasterInterfaceI|ChAIPatrolRouteActorStaringGETI(Message) _owningactorrefout))
      (Utilities|IsValid _patrolroute
        (:Is%20Valid
          (Variables|Default|SetPatrol%20RouteActorRef _patrolroute)
          (return true))
        (:Is%20Not%20Valid
          _)))
    (:Is%20Not%20Valid
      _))
  (Development|PrintString "BPManagerNpcPatrolStateAc>PatrolRouteActorUpdate== patrolROuteActor is not valid" true true "(R=1.000000,G=0.209541,B=0.000000,A=1.000000)" 22.0)
  (return false))

(fn PatrolRouteLapCompleteF
  (bind _patrol_routeactorref (Variables|Default|GetPatrol%20RouteActorRef))
  (Utilities|IsValid _patrol_routeactorref
    (:Is%20Valid
      (bind (_patrolpath2 _patrollapcompletion_circleorreverse _patrolstartdirection_forwardbackward) (Class|BPIPatrolRouteInterfaceI|PRIPatrolRouteInfoGETI(Message) _patrol_routeactorref))
      (LocalVariables|SetPatrolRouteLength (Utilities|Array|Length _patrolpath2))
      ;[1 1 1] Direction
      (switch Utilities|FlowControl|Switch|SwitchonE_GenericRepeat-LoopVsLine _patrollapcompletion_circleorreverse
        (:NewEnumerator0
          (Development|PrintString "BTTaskPatrolRouteLoopComplete>EG==PatrolLapComplete is null" true true "(R=1.000000,G=0.186159,B=0.000000,A=1.000000)" 22.0)
          ;;[1 1 1] StartingDirection
          (bind _output_get (Variables|Default|SetPatrolRouteDirection _patrolstartdirection_forwardbackward :!label _label))
          (switch Utilities|FlowControl|Switch|SwitchonE_GenericDirectionSimple-ForwardVsBackwards _output_get
            (:NewEnumerator0
              (Development|PrintString "BTTaskPatrolRouteLoopComplete>EG== PatrolRouteDirection is null ")
              ;[1 1 1] Index
              ;;[1 1 1] Reset
              (Variables|Default|SetPatolRouteIndex 0 :!label _label_2))
            (:NewEnumerator1
              (goto _label_2))
            (:NewEnumerator2
              (Variables|Default|SetPatolRouteIndex (- (LocalVariables|GetPatrolRouteLength) 1)))))
        (:NewEnumerator1
          (goto _label))
        (:NewEnumerator2
          ;;[1 1 1] Flip direction from currentDirection
          (switch Utilities|FlowControl|Switch|SwitchonE_GenericDirectionSimple-ForwardVsBackwards (Variables|Default|GetPatrolRouteDirection)
            (:NewEnumerator0
              (Variables|Default|SetPatrolRouteDirection (Utilities|Enum|LiteralenumE_GenericDirectionSimple-ForwardVsBackwards "NewEnumerator2") :!label _label_3)
              ;;[1 1 1] Reset
              (Variables|Default|SetPatolRouteIndex (- (- (LocalVariables|GetPatrolRouteLength) 1) 1)))
            (:NewEnumerator1
              (goto _label_3))
            (:NewEnumerator2
              (Variables|Default|SetPatrolRouteDirection (Utilities|Enum|LiteralenumE_GenericDirectionSimple-ForwardVsBackwards "NewEnumerator1"))
              ;;[1 1 1] Reset
              (Variables|Default|SetPatolRouteIndex 0)))))
      ;[1 1 1] State
      (return (Utilities|Enum|LiteralenumE_GuardDutyPatrolProtectState-StartVsOngoingVsCompletelap "NewEnumerator3") true))
    (:Is%20Not%20Valid
      (Development|PrintString "BPManagerNpcGuardPostPatrolNProtectAc>PatrolRouteLapComplete== PatrolRouteActor is not valid" true true "(R=1.000000,G=0.208814,B=0.000000,A=1.000000)" 22.0)
      (return "NewEnumerator4" false))))

(fn GuardPostPatrolProtectStateUpdateF
  (params (GuardDutyPatrolProtect_StateCurrent :type E_GuardDutyPatrolProtectState-StartVsOngoingVsCompletelap%20Enum :default "NewEnumerator4"))
  (Variables|Default|SetGuardDutyPatrolProtect_StateCurrent GuardDutyPatrolProtect_StateCurrent))

(fn GuardPostPatrolProtectStateGETF
  (return (Variables|Default|GetGuardDutyPatrolProtect_StateCurrent)))