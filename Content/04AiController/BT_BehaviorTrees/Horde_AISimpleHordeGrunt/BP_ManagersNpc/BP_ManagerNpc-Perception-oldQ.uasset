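; NPC perception manager for an AI controller that turns sight perception into combat targeting.
; On possess it caches the perception component and polls known sight actors on a looping timer.
; It takes the first actor, with enemy, alive and closest checks still unimplemented.
; Interface messages handle battle-circle membership and hard-lock target, alongside controller focus updates; last-known-location tracking is disconnected.
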(event Custom|OnPossesses_CE
  (params (AIController :type AI%20Controller%20Object%20Reference))
  ;[0 1 0.4249] OnPossess
  (bind _output_get (Variables|Default|SetAIControllerRef AIController))
  (Utilities|IsValid (Class|AIController|GetAIPerceptionComponent _output_get)
    (:Is%20Valid
      (Variables|Default|SetAIPerceptionComponentRef (Class|AIController|GetAIPerceptionComponent _output_get)))
    (:Is%20Not%20Valid
      _))
  (Utilities|Time|SetTimerbyEvent (delegate Custom|UpdateTargeting_CE) 0.25 true))

(event Custom|UpdateTargeting_CE
  (bind _aiperceptioncomponentref (Variables|Default|GetAIPerceptionComponentRef))
  ;[0 1 0.4249] OnPossess
  (Utilities|IsValid _aiperceptioncomponentref
    (:Is%20Valid
      (CallFunction|SightSenseUpdateF _aiperceptioncomponentref))))

(event Custom|ClearPreviousTarget_CE
  ;[0 1 0.4249] OnPossess
)

(event Custom|AddNewTarget_CE
  ;[0 1 0.4249] OnPossess
)

(fn ReferenceCharacterRefPureF
  (Utilities|IsValid (Variables|Default|GetOwningActor%20Ref)
    (:Is%20Valid
      (return (Variables|Default|GetOwningActor%20Ref)))
    (:Is%20Not%20Valid
      (bind _output_get (Variables|Default|SetOwningActor%20Ref (Pawn|GetControlledPawn (CallFunction|ReferenceAiControllerRefPureF))))
      (return _output_get))))

(fn ReferenceAiControllerRefPureF
  (Utilities|IsValid (Variables|Default|GetAIControllerRef)
    (:Is%20Valid
      (return (Variables|Default|GetAIControllerRef)))
    (:Is%20Not%20Valid
      (bind _asaicontroller (Utilities|Casting|CastToAIController (Components|GetOwner)))
      (bind _output_get (Variables|Default|SetAIControllerRef _asaicontroller))
      (return _output_get))))

(fn SightSenseUpdateF
  (params (AIPerceptionComponent :type AI%20Perception%20Component%20Object%20Reference))
  (for _array_element (Class|AIPerceptionComponent|GetKnownPerceivedActors AIPerceptionComponent "/Script/AIModule.AISense_Sight")
    ;[1 1 1] Check if actor is alive. Dont want to continue targeting dead characters
    (Utilities|Array|Add (LocalVariables|GetPercievedActors_Local) _array_element))
  ;[1 1 1] Choose only enemy actors and set closest one as a target
  (if (> (Utilities|Array|Length (LocalVariables|GetPercievedActors_Local)) 0)
    (bind _output_get (LocalVariables|SetEnemyActors_Local_0 (LocalVariables|GetPercievedActors_Local)))
    (if (> (Utilities|Array|Length _output_get) 0)
      ;;[1 1 1] setTargetNBattleCircle
      (CallFunction|TargetNBattleCircleUpdateF (Utilities|Array|Get(acopy) (LocalVariables|GetEnemyActors_Local_0)))
      ;;[1 0.4769 0.7844 1 14] NEED this SETFOCUS for SightSense to stick on character. Every Sight update without focus the target location will stop updating.
      (AI|SetFocus (Variables|Default|GetAIControllerRef))
      (else
        ;[1 1 1] Clear- No enemies to target
        ;;[1 1 1] Clear targetNBattleCircleNSearch
        (CallFunction|TargetNBattleCircleClearF :!label _label)
        (AI|ClearFocus (Variables|Default|GetAIControllerRef))))
    (else
      (goto _label))))

(fn TargetNBattleCircleUpdateF
  (params (NewEnemyTarget :type Actor%20Object%20Reference))
  ;[1 1 1] Not the same target?
  (if (and (Utilities|IsValid NewEnemyTarget) (!= NewEnemyTarget (Variables|Default|GetTargetActor_F)))
    ;[1 1 1] BattleCircle: Add self to the enemies battleCircle
    ;;[1 1 1 1 14] Targets battleCircle
    (Class|BPICharacterBaseInterface|CPILockonBattleCircleAddxI(Message) (Pawn|GetControlledPawn (Variables|Default|GetAIControllerRef)) NewEnemyTarget)
    ;[1 1 1] LockonHardLockTargetActor
    (Class|BPICharacterBaseInterface|CPILockonPerceptionHardLockSETxI(Message) (Pawn|GetControlledPawn (Variables|Default|GetAIControllerRef)) NewEnemyTarget)
    (AI|Navigation|StopMovement (Variables|Default|GetAIControllerRef))))

(fn TargetNBattleCircleClearF
  (bind _targetactor_f (Variables|Default|GetTargetActor_F))
  (Utilities|IsValid _targetactor_f
    (:Is%20Valid
      ;[1 1 1] BattleCircle: Add self to the enemies battleCircle
      ;;[1 1 1 1 14] Targets battleCircle
      (Class|BPICharacterBaseInterface|CPILockonBattleCircleRemovexI(Message) _targetactor_f (Pawn|GetControlledPawn (Variables|Default|GetAIControllerRef))))))

(fn TargetLastKnownLocationF
  (Utilities|IsValid (Variables|Default|GetTargetActor_F)
    (:Is%20Not%20Valid
      (Development|PrintString "AICNPCControllerMasterBP>TargetLastSpottedLcoationVectorF=NPCref is not valid" true true "(R=1.000000,G=0.363357,B=0.000000,A=1.000000)" 22.0))))