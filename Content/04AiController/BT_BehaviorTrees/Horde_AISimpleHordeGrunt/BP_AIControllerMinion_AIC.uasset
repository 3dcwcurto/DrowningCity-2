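; AI controller for horde minion grunts, with perception and guard-post patrol logic that is mostly unwired.
; On possess it only caches the pawn as a Character.
; A patrol graph steps a state machine through the guard-post manager component, setting walk gait and using AIMoveTo along route points.
; Its caller, the looping sight-update timer, perception setup and alert-to-hostile transitions are all disconnected, so none currently run.
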(event Custom|UpdateTargeting_CE
  (bind _aiperception (Variables|Default|GetAIPerception))
  ;[0 1 0.4249] Possess
  (Utilities|IsValid _aiperception
    (:Is%20Valid
      (Default|SightSenseUpdateF (Variables|Default|GetBP_ManagerNpc-Perception-SightNHearing) _aiperception))))

(event EventTick
  (params (DeltaSeconds :type Float%20%28single-precision%29)))

(event EventPossess
  (params (PossessedPawn :type Pawn%20Object%20Reference))
  ;[0 1 0.4249] Possess
  (|PossessedPawn_CG PossessedPawn))

(fn ConstructionScript)