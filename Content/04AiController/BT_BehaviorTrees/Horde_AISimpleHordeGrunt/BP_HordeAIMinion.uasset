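; BP_HordeAIMinion is a horde minion Blueprint that exposes AI setup data through ChAI interface functions.
; It reports a fixed AI type and returns its patrol route actor.
; The behavior tree, camp town and leash getters return nothing, and all setters return false without storing their input.
; BeginPlay and the construction script are empty, and the BehaviorTreeNpcHeroDontNeeDQ variable is unused.
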(event EventBeginPlay
  ;[0.2507 1 0] BeginPlay
)

(fn ConstructionScript)

(fn ChAIAITypeGETI
  (return "NewEnumerator0"))

(fn ChAIBehaviorTreeObjectGetI
  (return 0))

(fn ChAICampTownActorStartingGETI
  (params (Location :type Name :default "None"))
  (return 0))

(fn ChAICampTownActorStartingSETI
  (params (CampTownActor :type Actor%20Object%20Reference))
  (return false))

(fn ChAILeashActorStartingGETI
  (return 0))

(fn ChAILeashActorStartingSETI
  (params (LeashActorStarting :type Actor%20Object%20Reference))
  (return false))

(fn ChAIPatrolRouteActorStaringGETI
  (return (Variables|Default|GetPatrolRouteActor)))

(fn ChAIPatrolRouteActorStartingSETI
  (params (PatrolRouteActor :type Actor%20Object%20Reference))
  (return false))