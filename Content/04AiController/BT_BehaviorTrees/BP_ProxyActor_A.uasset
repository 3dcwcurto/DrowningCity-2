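; BP_ProxyActor_A is an AI proxy actor that attaches to and detaches from other actors through interface events.
; Attaching fetches the target's designated scene component via interface, then snaps the proxy to it at a relative offset.
; That component is switched to absolute rotation, so it ignores its parent's rotation.
; Detaching keeps the world transform and clears the AttatchedToActor reference, acting only when that reference is valid.
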(event EventPAIDetatchProxyActortoActorAutomaticifValidI
  (CallFunction|DetatchfromActorF))

(event EventPAIAttatchProxyActortoActorI
  (params (Actor :type Actor%20Object%20Reference) (Offset :type Vector :default "0, 0, 0"))
  (CallFunction|AttatchtoActorF Actor Offset))

(fn ConstructionScript)

(fn AttatchtoActorF
  (params (AttatchedToActor :type Actor%20Object%20Reference) (Offset :type Vector))
  (bind _scenecomponent (Class|BPICharacterAIMasterInterfaceI|ChAISceneComponentRelativeRotationAttatchGETI(Message) AttatchedToActor))
  (Utilities|IsValid _scenecomponent
    (:Is%20Valid
      (Transformation|SetAbsolute _scenecomponent false true false)
      (Transformation|AttachComponentToComponent (Variables|Transformation|GetRootComponent) _scenecomponent "None" "SnapToTarget" "KeepRelative" "KeepRelative" true)
      (Transformation|SetRelativeLocation (Variables|Transformation|GetRootComponent) Offset false false))))

(fn DetatchfromActorF
  (Utilities|IsValid (Variables|Default|GetAttatchedToActor)
    (:Is%20Valid
      (Transformation|DetachFromActor self "KeepWorld" "KeepWorld" "KeepWorld")
      ;[1 1 1] Clear
      (Variables|Default|SetAttatchedToActor 0))))