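; Retired AI controller Blueprint for player-side RTS squad units, kept in an old folder and meant to receive squad orders.
; Its add-to-queue and override-queue order events are empty, with a todo to replace them with a queue system and manager service.
; Unreachable leftover nodes show an earlier approach that wrote order state, move location, direction and squad size to Blackboard keys for a behavior tree.
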(event EventAICISquadOrderNewOrderAddtoStackQueI
  (params (SquadOrderInfo :type S%20Order%20Info%20Structure))
  ;[0.9437 1 0.5609] Todo: replace with queSystem and queManagerService. Setup task that will wipe que and try to execute right away or add itself as a single que
  ;;[1 1 1] Orders
)

(event EventAICSquadOrderNewOrderOverideStackQueI
  (params (OrderInfo :type S%20Order%20Info%20Structure))
  ;[0.9437 1 0.5609] Todo: replace with queSystem and queManagerService. Setup task that will wipe que and try to execute right away or add itself as a single que
  ;;[1 1 1] Orders
)

(fn ConstructionScript)