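; Character Blueprint that manages inventory and weapon-set loadouts, adding container components from a hard-coded test loadout and async-loading the preset's mesh.
; Weapon-set animation classes supply abilities to grant, with attack combos found by following each ability's next-ability links.
; Draw/sheath state drives weapon socket attachment and the animation set on a linked anim graph, while equip notifies become gameplay events.
; Item bumping and trophy receiving are stubs.
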(event Custom|WeaponSet-HoldingCurrent_CE
  (params (new-WeaponSetHoldingCurrent :type Integer))
  ;[1 1 1] HoldingCurrent
  (Variables|03Inventory|SetWeaponSetPairHoldingCurrent new-WeaponSetHoldingCurrent))

(event Custom|WeaponSet-SocketAttatchUpdate_CE
  (params (Interupt :type Boolean))
  ;[1 0.007843 0] Socket Change-phase4
  (05InventoryChar|EquipSheath|WeaponSetWeaponPairSocketAttachUpdateF Interupt))

(event Custom|DrawSheathState-WeaponSetAnimationSetFightStyle_CE
  (params (DrawSheathState :type S%20Draw%20Sheath%20State%20Info%20Structure))
  ;[1 0.009744 0] EquipUnequip_StateNAnimSet
  (05InventoryChar|EquipSheath|DrawSheathState-WeaponSetAnimationSetFightStyleF DrawSheathState))

(event EventBeginPlay
  (|CallParentFunction))

(event EventCIIAnUnequipSheathEventI
  ;[1 0.007843 0] AN_UnequipSheath
  (Ability|SendGameplayEventtoActor self "(TagName=\"GameplayEvent.DrawSheathEvent.AN_UnequipSheathEvent\")"))

(event EventCIIWeaponSetWeaponPairGrantAbilitiesI
  (params (WeaponSetWeaponPair :type S%20Weapon%20Set%20Weapon%20Pair%20Structure))
  ;[1 1 1] LoadoutWeaponSet GrantAbilities
  (05InventoryChar|Abilities|GrantAbilitiesAutoMainF WeaponSetWeaponPair)
  (05InventoryChar|EquipSheath|WeaponPairExtraSetupF-todo WeaponSetWeaponPair))

(event EventCSIStoryChangeNpcCharacterSetupInventoryI
  (params (dataAsset-NewInventory :type Boolean))
  ;[1 1 1 1 12] Note: a story event might cause a Npc to change thier clothing and equipment.
)

(event EventCIIWeaponSet-HoldingCurrentSETI
  (params (WeaponSet-HoldingCurrent :type Integer))
  ;[1 1 1] HoldingCurrent
  (CallFunction|WeaponSet-HoldingCurrentCE WeaponSet-HoldingCurrent))

(event EventTick
  (params (DeltaSeconds :type Float%20%28single-precision%29))
  ;[0.03766 0.3229 0] Tick
  (|CallParentFunction DeltaSeconds))

(event EventCIIAnEquipHoldEventI
  ;[1 0.009744 0] AN_EquipHold
  (Ability|SendGameplayEventtoActor self "(TagName=\"GameplayEvent.DrawSheathEvent.AN_EquipNHoldEvent\")"))

(event EventCSIBeginPlayLoadCharacterSetupInventoryI
  (params (LoadedInventory-todo :type Boolean)))

(event EventCharacterPresetSetup-InheritableCE
  (params (CharacterPreset :type Primary%20Data%20Asset%20Object%20Reference) (SpawnTrueVsSceneFalse :type Boolean))
  ;[0 1 0.4249] Possessed
  (|CallParentFunction CharacterPreset SpawnTrueVsSceneFalse)
  (05InventoryChar|BeginPlay|BeginPlaySetupInventoryMainF)
  (05InventoryChar|BeginPlay|Beginplay-InventoryCharacterPresetF)
  (|SkeletalMeshAsyncLoad_CG_2 CharacterPreset))

(event EventCIIDrawSheathStateSETI
  (params (DrawSheathState :type S%20Draw%20Sheath%20State%20Info%20Structure))
  ;[1 0.009744 0] EquipUnequip_StateNAnimSet
  (CallFunction|DrawSheathState-WeaponSetAnimationSetFightStyleCE DrawSheathState))

(event EventCIIWeaponSetSocketAttatchUpdateI
  (params (Interupt :type Boolean))
  ;[1 0.007843 0] Socket Change-phase4
  (CallFunction|WeaponSet-SocketAttatchUpdateCE Interupt))

(event EventCIIInventoryItemBumpingI
  (params (InventoryItem_ :type S%20Inventory%20Item%20Structure))
  ;[1 1 1] InventoryItemBumping
  ;;[1 1 1 1 14] Find generalInventoryPockets slot or backpackInventory slot to bump item into
  (05InventoryChar|ContainersItems|InventoryItemBumpF InventoryItem_))

(event EventCSIBeginPlayNewCharacterSetupInventoryI)

(fn ConstructionScript)

(fn BeginPlayLoadCreateInventoryContainerF
  (bind _s_inventoryitem (Utilities|Struct|MakeS_InventoryItem "/Game/02CharacterBP/004InvChar/Items/01Weapons/01FallbackFists/DrowFists/BP_WeaponItemFallbackFists_A.BP_WeaponItemFallbackFists_A_C" 0 0 0 false 1))
  ;[1 1 1] SpecialItem(questItems)
  ;;[1 1 1] Index 0
  (Utilities|Array|SetArrayElem (LocalVariables|GetInventoryContainer_Local) 0 (Utilities|Struct|MakeS_InventoryContainerInfo "/Game/02CharacterBP/004InvChar/Container/BP_InventoryContainer00Master_AC.BP_InventoryContainer00Master_AC_C" 0 (Utilities|Array|MakeArray (Utilities|Struct|MakeS_InventoryItem))) true)
  ;[1 1 1] WeaponEquipment
  ;;[1 1 1] Index 1
  (Utilities|Array|SetArrayElem (LocalVariables|GetInventoryContainer_Local) 1 (Utilities|Struct|MakeS_InventoryContainerInfo "/Game/02CharacterBP/004InvChar/Container/Loadout01WeaponSets/BP_InventoryContainer01Weapon_AC.BP_InventoryContainer01Weapon_AC_C" 0 (Utilities|Array|MakeArray _s_inventoryitem _s_inventoryitem (Utilities|Struct|MakeS_InventoryItem) (Utilities|Struct|MakeS_InventoryItem "/Game/02CharacterBP/004InvChar/Items/01Weapons/05SubParentTwohandedGreatWeapon/TwoHandedAxe/BP_WeaponItemAxeTwoHanded_A.BP_WeaponItemAxeTwoHanded_A_C" 0 0 0 false 1) (Utilities|Struct|MakeS_InventoryItem "/Game/02CharacterBP/004InvChar/Items/01Weapons/02SubParentBowsCrossbows/BowShort/BP_WeaponItem_BowShort.BP_WeaponItem_BowShort_C" 0 0 0 false 1) (Utilities|Struct|MakeS_InventoryItem 0 0 0 0 false 1))) true)
  (return (LocalVariables|GetInventoryContainer_Local)))

(fn BeginPlayAddInventoryContainersF
  (params (InventoryContainer :type Array%20of%20S%20Inventory%20Container%20Info%20Structures))
  ;[1 1 1] Add New Cotnainer
  (for (_array_element _array_index) InventoryContainer
    (if (Utilities|IsValidClass (.Container (Utilities|Struct|BreakS_InventoryContainerInfo _array_element)))
      (bind _returnvalue (Game|AddComponentbyClass self (.Container (Utilities|Struct|BreakS_InventoryContainerInfo _array_element))))
      (Utilities|Array|SetArrayElem (Variables|03Inventory|GetInventoryContainer) _array_index _returnvalue true)
      (Variables|/Game/02CharacterBP/004InvChar/Container/BP_InventoryContainer00Master_AC.BP_InventoryContainer00Master_AC_C|SetInventoryItem _returnvalue (.InventoryItems (Utilities|Struct|BreakS_InventoryContainerInfo _array_element)))
      ;;[1 1 1] Loadout Containers overide code. Weapons spawn actors in weaponSet pairs, armor adds skeletal meshes, consumables add staticMeshes?
      (Default|LoadoutSetupOverideableF _returnvalue self))))

(fn Beginplay-InventoryCharacterPresetF)

(fn BeginPlaySetupInventoryMainF
  (bind _inventorycontainersavefile (05InventoryChar|BeginPlay|BeginPlayLoadCreateInventoryContainerF))
  (05InventoryChar|BeginPlay|BeginPlayAddInventoryContainersF _inventorycontainersavefile))

(fn ItemCollectDispatcherF
  (params (TropheItemReceiveTake :type Primary%20Data%20Asset%20Object%20Reference))
  (Class|BPIPlayerControllerStoryInterfaceI|PcSIObjectiveItemCollectDispatchI(Message) (Game|GetPlayerController 0) "NewEnumerator2" (Variables|/Game/02CharacterBP/004InvChar/00ItemPresets/PDA_ItemPreset00Parent.PDA_ItemPreset00Parent_C|GetItemNameID (.AsPDA%20Item%20Preset%2000Parent (Utilities|Casting|CastToPDA_ItemPreset00Parent TropheItemReceiveTake)))))

(fn InventoryItemBumpF
  (params (InventoryItem :type S%20Inventory%20Item%20Structure))
  (Development|PrintString "BPCharacterInventory>EG== InventoryItemBumping is not set up  yet" true true "(R=1.000000,G=0.415079,B=0.000000,A=1.000000)" 22.0))

(fn SpecificContainerFindF
  (params (ContainerClass :type BP%20Inventory%20Container%2000%20Master%20AC%20Class%20Reference))
  (bind _array_element (Utilities|Array|ForEachLoopwithBreak (Variables|03Inventory|GetInventoryContainer))
    (:LoopBody
      (if (== (Utilities|GetClass _array_element) ContainerClass)
        (LocalVariables|SetFoundContainer_Local true)
        (LocalVariables|SetContainer_Local _array_element)))
    (:Completed
      (return (LocalVariables|GetContainer_Local) (LocalVariables|GetFoundContainer_Local)))))

(fn WeaponPairExtraSetupF-todo
  (params (NewWeaponSetWEaponPair :type S%20Weapon%20Set%20Weapon%20Pair%20Structure)))

(fn DrawSheathState-WeaponSetAnimationSetFightStyleF
  (params (S_DrawSheathStateInfo :type S%20Draw%20Sheath%20State%20Info%20Structure%20%28by%20ref%29))
  (bind (_drawsheathstate _nextweaponsetanimset) (Utilities|Struct|BreakS_DrawSheathStateInfo S_DrawSheathStateInfo))
  (bind (_weaponlefthand _weaponrighthand _weapontypelefthand _weapontyperighthand _weaponsetanimationset _weaponsetanimationsetobjectclass) (Utilities|Struct|BreakS_WeaponSetWeaponPair _nextweaponsetanimset))
  (Variables|03Inventory|SetDrawSheathState S_DrawSheathStateInfo)
  (switch Utilities|FlowControl|Switch|SwitchonE_DrawSheathState _drawsheathstate
    (:NewEnumerator0
      _)
    (:NewEnumerator1
      _)
    (:NewEnumerator2)
    (:NewEnumerator3)
    (:NewEnumerator4))
  (Class|BPICharacterInvWeaponSetAnimationSetI|CIWSASWeaponSetAnimationSetSETI(Message) (Class|AnimInstance|GetLinkedAnimGraphInstancebyTag (Components|SkeletalMesh|GetAnimInstance (Variables|Character|GetMesh)) "WeaponSet") _weaponsetanimationset _weapontypelefthand _weapontyperighthand _weaponsetanimationsetobjectclass))

(fn WeaponSetWeaponPairNewGETF
  (params (WeaponSet :type Integer))
  (bind _container (05InventoryChar|ContainersItems|SpecificContainerFindF "/Game/02CharacterBP/004InvChar/Container/Loadout01WeaponSets/BP_InventoryContainer01Weapon_AC.BP_InventoryContainer01Weapon_AC_C"))
  (bind _asbp_inventory_container_01weapon_ac (Utilities|Casting|CastToBP_InventoryContainer01Weapon_AC _container)
    (:then
      _)
    (:CastFailed
      (Development|PrintString "BPCharacterInventory>WeaponSetNewGetF== inventoryContainer01WeaponAC Cast Failed" true true "(R=1.000000,G=0.662674,B=0.000000,A=1.000000)" 22.0)))
  (return (Utilities|Array|Get(acopy) (Variables|/Game/02CharacterBP/004InvChar/Container/Loadout01WeaponSets/BP_InventoryContainer01Weapon_AC.BP_InventoryContainer01Weapon_AC_C|GetWeaponSetPair _asbp_inventory_container_01weapon_ac) WeaponSet)))

(fn WeaponSetWeaponPairCurrentHoldingGETF
  (bind _container (05InventoryChar|ContainersItems|SpecificContainerFindF "/Game/02CharacterBP/004InvChar/Container/Loadout01WeaponSets/BP_InventoryContainer01Weapon_AC.BP_InventoryContainer01Weapon_AC_C"))
  (bind _asbp_inventory_container_01weapon_ac (Utilities|Casting|CastToBP_InventoryContainer01Weapon_AC _container)
    (:then
      _)
    (:CastFailed
      (Development|PrintString "BPCharacterInventory>WeaponSetNewGetF== inventoryContainer01WeaponAC Cast Failed" true true "(R=1.000000,G=0.662674,B=0.000000,A=1.000000)" 22.0)))
  (return (Utilities|Array|Get(acopy) (Variables|/Game/02CharacterBP/004InvChar/Container/Loadout01WeaponSets/BP_InventoryContainer01Weapon_AC.BP_InventoryContainer01Weapon_AC_C|GetWeaponSetPair _asbp_inventory_container_01weapon_ac) (Variables|03Inventory|GetWeaponSetPairHoldingCurrent))))

(fn DrawHoldnSheathHolsterStateUpdateF
  (params (Interupt :type Boolean))
  (return ""))

(fn WeaponSetWeaponPairSocketAttachUpdateF
  (params (Interupt :type Boolean))
  (bind _drawsheathstate (Variables|03Inventory|GetDrawSheathState))
  (bind (_drawsheathstate_2 _nextweaponsetanimset _previousweaponsetanimset) (Utilities|Struct|BreakS_DrawSheathStateInfo _drawsheathstate))
  (bind (_weaponlefthand _weaponrighthand) (Utilities|Struct|BreakS_WeaponSetWeaponPair _nextweaponsetanimset))
  (bind (_weaponlefthand_2 _weaponrighthand_2) (Utilities|Struct|BreakS_WeaponSetWeaponPair _previousweaponsetanimset))
  (if Interupt
    ;[1 1 1 1 14] Update previous first then new to prevent issues with tracenodes
    ;;[1 1 1 1 14] If interupting then set both mainHandAndOffHand NewSet  and the PreviousSet
    (Utilities|FlowControl|Sequence
      (:then_0
        ;[1 1 1] Previous WeaponSet
        (LocalVariables|SetLeftHand_Local (.InventoryItemActor-RuntimeLoadout (Utilities|Struct|BreakS_InventoryItem _weaponlefthand_2)) :!label _label)
        (LocalVariables|SetRightHand_Local (.InventoryItemActor-RuntimeLoadout (Utilities|Struct|BreakS_InventoryItem _weaponrighthand_2)))
        (Utilities|IsValid (LocalVariables|GetLeftHand_Local)
          (:Is%20Valid
            (Default|ActorAttachSocketingSheathF (LocalVariables|GetLeftHand_Local) self))
          (:Is%20Not%20Valid
            _))
        (Utilities|IsValid (LocalVariables|GetRightHand_Local)
          (:Is%20Valid
            (Default|ActorAttachSocketingSheathF (LocalVariables|GetRightHand_Local) self))
          (:Is%20Not%20Valid)))
      (:then_1
        ;[1 1 1] New WeaponSet
        (LocalVariables|SetLeftHand_Local (.InventoryItemActor-RuntimeLoadout (Utilities|Struct|BreakS_InventoryItem _weaponlefthand)) :!label _label_2)
        (LocalVariables|SetRightHand_Local (.InventoryItemActor-RuntimeLoadout (Utilities|Struct|BreakS_InventoryItem _weaponrighthand)))
        (Utilities|IsValid (LocalVariables|GetLeftHand_Local)
          (:Is%20Valid
            (Default|ActorAttatchSocketingHoldingF (LocalVariables|GetLeftHand_Local) self "NewEnumerator1"))
          (:Is%20Not%20Valid
            _))
        (Utilities|IsValid (LocalVariables|GetRightHand_Local)
          (:Is%20Valid
            (Default|ActorAttatchSocketingHoldingF (LocalVariables|GetRightHand_Local) self "NewEnumerator2"))
          (:Is%20Not%20Valid))))
    (else
      (switch Utilities|FlowControl|Switch|SwitchonE_DrawSheathState _drawsheathstate_2
        (:NewEnumerator0
          (goto _label_2))
        (:NewEnumerator1
          (goto _label_2))
        (:NewEnumerator2
          (goto _label))
        (:NewEnumerator3
          (goto _label))
        (:NewEnumerator4
          (goto _label_2))))))

(fn AnUnequipSheathEventF)

(fn AnEquipHoldEventF)

(fn RemoveAbilitiesF
  (params (WeaponSetWeaponPair :type S%20Weapon%20Set%20Weapon%20Pair%20Structure))
  (bind _array_element (Utilities|Array|ForEachLoopwithBreak (Variables|03Inventory|GetGrantedAbilitiesHoldingCurrent))
    (:LoopBody
      (if (Utilities|IsValidClass _array_element)
        (Class|DCCharacterBase|RemoveAbilityMy _array_element)))
    (:Completed
      (Utilities|Array|Clear (Variables|03Inventory|GetGrantedAbilitiesHoldingCurrent)))))

(fn GrantAbilitiesNormalAttackLoopF
  (params (Array :type Array%20of%20GA%20Ability%20Master%20Class%20References))
  (bind _nextabilities (LocalVariables|GetNextAbilities))
  (Utilities|Array|Clear (LocalVariables|GetNextAbilities))
  (bind _array_element (Utilities|Array|ForEachLoopwithBreak Array)
    (:LoopBody
      (if (Utilities|IsValidClass _array_element)
        (if (not (Utilities|Array|ContainsItem (Variables|03Inventory|GetGrantedAbilitiesHoldingCurrent) _array_element))
          (Class|DCCharacterBase|AquireAbility _array_element)
          (Utilities|Array|AddUnique (Variables|03Inventory|GetGrantedAbilitiesHoldingCurrent) _array_element)
          (for _array_element_2 (.NextGaAbility (Utilities|GetClassDefaults _array_element))
            (if (Utilities|IsValidClass _array_element_2)
              (if (not (Utilities|Array|ContainsItem _nextabilities _array_element_2))
                (Utilities|Array|AddUnique _nextabilities _array_element_2)))))))
    (:Completed
      (return (LocalVariables|GetNextAbilities)))))

(fn GrantAbilitiesAutoMainF
  (params (New_WeaponSetWeaponPair :type S%20Weapon%20Set%20Weapon%20Pair%20Structure))
  (bind _weaponsetanimationsetobjectclass (Utilities|Struct|BreakS_WeaponSetWeaponPair New_WeaponSetWeaponPair))
  (bind _ga_drawequipsheathputup (Utilities|GetClassDefaults _weaponsetanimationsetobjectclass))
  (if (Utilities|IsValidClass _weaponsetanimationsetobjectclass)
    (Utilities|FlowControl|Sequence
      (:then_0
        (LocalVariables|SetAttackAbilities_Local (.GA_InputAction (Utilities|GetClassDefaults _weaponsetanimationsetobjectclass)))
        (if (> (Utilities|Array|Length (LocalVariables|GetAttackAbilities_Local)) 0) :!label _label
          (for _index (range 0 99)
            ;[1 1 1] Combo length 1
            (bind _nextgaability (05InventoryChar|Abilities|GrantAbilitiesNormalAttackLoopF (LocalVariables|GetAttackAbilities_Local)))
            (LocalVariables|SetAttackAbilities_Local _nextgaability)
            (goto _label))))
      (:then_1
        ;[1 1 1] Reaction
        (bind _array_element (Utilities|Array|ForEachLoopwithBreak (.GA_ReactionAction (Utilities|GetClassDefaults _weaponsetanimationsetobjectclass)))
          (:LoopBody
            (if (Utilities|IsValidClass _array_element)
              (Class|DCCharacterBase|AquireAbility _array_element)))))
      (:then_2
        ;[0 0 0] Move to Array. Use an array so reactions can be scalable and have multiple with different modifiers
        ;;[1 1 1] Draw Sheath
        (if (Utilities|IsValidClass _ga_drawequipsheathputup)
          (Class|DCCharacterBase|AquireAbility _ga_drawequipsheathputup)
          (else
            (Development|PrintString "BPCharacterInventory>WeaponSetAnimationSet_GrantAbilities==GADrawSheath not valid" true true "(R=1.000000,G=0.510844,B=0.000000,A=1.000000)" 22.0)))))))

(fn CIIComponentCharacterInventoryGETI
  (return))

(fn CIIDrawSheathStateGETI
  (return (Variables|03Inventory|GetDrawSheathState)))

(fn CIISpecificContainerClassGETI
  (params (ContainerClass :type BP%20Inventory%20Container%2000%20Master%20AC%20Class%20Reference))
  (bind (_container _valid) (05InventoryChar|ContainersItems|SpecificContainerFindF ContainerClass))
  (if _valid
    _
    (else
      (Development|PrintString "BPInventoryCharacter>CIILoadoutContainerWeaponGetI== Container Not Found" true true "(R=1.000000,G=0.297250,B=0.000000,A=1.000000)" 22.0)))
  (return _container))

(fn CIIWeaponSet-DesiredNewGETI
  (params (WeaponSet-DesiredNew :type Integer))
  (bind _new_weaponsetcontainerloadout (05InventoryChar|EquipSheath|WeaponSetWeaponPairNewGETF WeaponSet-DesiredNew))
  (return _new_weaponsetcontainerloadout))

(fn CIIWeaponSet-HoldingCurrentGETI
  (bind _current_weaponsetcontainerloadout (05InventoryChar|EquipSheath|WeaponSetWeaponPairCurrentHoldingGETF))
  (return (Variables|03Inventory|GetWeaponSetPairHoldingCurrent) _current_weaponsetcontainerloadout))

(fn CSIInventoryTropheCollectAttackerRecieveItemI
  (params (TropheItemRecieveTake :type Primary%20Data%20Asset%20Object%20Reference))
  (return))

(fn CSIInventoryTropheCollectedStatusCheckI-dontNeed
  (return (Variables|Default|GetbIsTropheCollected)))

(fn CSIInventoryTropheCollectVictimRemoveItemI
  (bind _tropheitem_todoreplacebymanualchoppingheadoff (Variables|Default|GetTropheItem-todoReplaceByManualChoppingHeadOff))
  (if (Variables|Default|GetbIsTropheCollected)
    ;[1 1 1] Purposefully set null
    (return 0)
    (else
      (Variables|Default|SetbIsTropheCollected true)
      (Utilities|IsValid _tropheitem_todoreplacebymanualchoppingheadoff
        (:Is%20Valid
          (return _tropheitem_todoreplacebymanualchoppingheadoff))
        (:Is%20Not%20Valid
          (Development|PrintString "CharacterInventory>CSIInventoryTropheColectVictimeRemoveItemI== TropheItem is null" true true "(R=1.000000,G=0.799738,B=0.000000,A=1.000000)" 22.0)
          ;[1 1 1] TodoSetupFallback???
          (return 0))))))