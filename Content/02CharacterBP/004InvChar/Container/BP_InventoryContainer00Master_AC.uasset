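; Master inventory container component that turns a character's loadout items into visible gear, with an empty overridable setup hook for children.
; Loops validate each slot, then spawn item actors attached sheathed or add master-posed skeletal meshes for armor, storing references back into the item array.
; Validation only checks that classes are set; the child-class test is unwired.
; Helpers bump items via interface message, check the held weapon set and attach to hands.
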(event EventBeginPlay)

(event EventTick
  (params (DeltaSeconds :type Float%20%28single-precision%29)))

(fn LoadoutSetupOverideableF
  (params (Owner_Character :type Character%20Object%20Reference))
  ;[1 1 1] LoadoutWeapon,LoadoutArmor, LoadoutConsumable overides
  (return))

(fn LoadoutValidationF
  (params (InventoryItems :type S%20Inventory%20Item%20Structure) (SlotIndexs :type Integer))
  (bind _inventoryitem_classid (Utilities|Struct|BreakS_InventoryItem InventoryItems))
  (if (Utilities|IsValidClass _inventoryitem_classid)
    (LocalVariables|SetInventoryItemToValidate_Local _inventoryitem_classid)
    (LocalVariables|SetSlotIndex_Local SlotIndexs)
    ;[1 1 1] Validation
    (if (Utilities|IsValidClass (Variables|Default|GetLoadoutAllowed-ParentItemClassWeaponArmor))
      (if (Utilities|IsValidClass (Utilities|Array|Get(acopy) (Variables|Default|GetLoadoutDestination-ParentItemClassPerSlotIndex) (LocalVariables|GetSlotIndex_Local)))
        (return true)
        (else
          (Development|PrintString "BPInventoryContainer>DestinationValidationF== LoadoutDesintation SlotIndex  does not have a valid or matching Class" true true "(R=1.000000,G=0.258736,B=0.000000,A=1.000000)" 22.0)
          (return false)))
      (elif (Utilities|Array|IsValidIndex (Variables|Default|GetLoadoutDestination-ParentItemClassPerSlotIndex))
        (Development|PrintString "BPInventoryContainer>DestinationValidationF== PROOFING. LoadoutAllowed is null and LoadoutValidation has ValidIndex. Both should be null or both should be set" true true "(R=1.000000,G=0.168185,B=0.000000,A=1.000000)" 22.0)
        (return false)
        (else
          ;;[1 1 1] Success: No Validation required
          (return true))))
    (else
      ;[1 1 1] Item empty
      (return false))))

(fn LoadoutSpawnItemActorsLoopF-todo
  (params (Owner_Character :type Character%20Object%20Reference))
  (bind _inventoryitem (Variables|Default|GetInventoryItem))
  (LocalVariables|SetOwner_Character_Local Owner_Character)
  (bind (_array_element _array_index) (Utilities|Array|ForEachLoopwithBreak _inventoryitem)
    (:LoopBody
      (bind _updatedinvetoryitem (CallFunction|LoadoutSpawnActorF-todo (LocalVariables|GetOwner_Character_Local) _array_index _array_element false))
      (bind _structout (Utilities|Struct|SetmembersinS_InventoryItem _updatedinvetoryitem _array_index))
      (Utilities|Array|SetArrayElem _inventoryitem _array_index _structout true))
    (:Completed
      (return))))

(fn LoadoutSpawnActorF-todo
  (params (Owner_Character :type Character%20Object%20Reference) (SlotIndex :type Integer) (InventoryItem :type S%20Inventory%20Item%20Structure) (HoldingVsSheathed-old :type Boolean))
  (LocalVariables|SetOwner_Character_Localx Owner_Character)
  (LocalVariables|SetSlotIndex_Local SlotIndex)
  (LocalVariables|SetInventoryItem_Local InventoryItem)
  (LocalVariables|SetHoldingVsSheathed_Local-old HoldingVsSheathed-old)
  (bind _validationx (CallFunction|LoadoutValidationF (LocalVariables|GetInventoryItem_Local) (LocalVariables|GetSlotIndex_Local)))
  (if _validationx
    (Utilities|IsValid (.InventoryItemActor-RuntimeLoadout (Utilities|Struct|BreakS_InventoryItem (LocalVariables|GetInventoryItem_Local)))
      (:Is%20Valid
        (Actor|DestroyActor (.InventoryItemActor-RuntimeLoadout (Utilities|Struct|BreakS_InventoryItem (LocalVariables|GetInventoryItem_Local)))))
      (:Is%20Not%20Valid
        _))
    (Utilities|FlowControl|Sequence
      (:then_0
        (bind _returnvalue (Game|SpawnActorfromClass (.InventoryItem-ClassID (Utilities|Struct|BreakS_InventoryItem (LocalVariables|GetInventoryItem_Local))) (Math|Transform|MakeTransform "0, 0, 0" "0, 0, 0" "1.000000,1.000000,1.000000") "Undefined" (LocalVariables|GetOwner_Character_Localx) (LocalVariables|GetOwner_Character_Localx)))
        (bind _output_get (LocalVariables|SetItemActorSpawned_Local _returnvalue))
        ;[1 1 1] StartSheathed
        (Default|ActorAttachSocketingSheathF _output_get (LocalVariables|GetOwner_Character_Localx)))
      (:then_1
        ;[1 1 1] Update InventoryItem with spawnedActor
        (bind _structout (Utilities|Struct|SetmembersinS_InventoryItem (LocalVariables|GetInventoryItem_Local) (LocalVariables|GetItemActorSpawned_Local) :!label _label))
        (return _structout)))
    (else
      (goto _label))))

(fn LoadoutAddSkeletalLoopF-todo
  (params (Owner_Character_ :type Character%20Object%20Reference))
  (bind _inventoryitem (Variables|Default|GetInventoryItem))
  (LocalVariables|SetOwner_Character_Local Owner_Character_)
  (bind (_array_element _array_index) (Utilities|Array|ForEachLoopwithBreak _inventoryitem)
    (:LoopBody
      (bind _updatedinvetoryitem (CallFunction|LoadoutAddItemSkeletalF-todo (LocalVariables|GetOwner_Character_Local) _array_element _array_index))
      (Utilities|Array|SetArrayElem _inventoryitem _array_index _updatedinvetoryitem true))))

(fn LoadoutAddItemSkeletalF-todo
  (params (Owner_Character_ :type Character%20Object%20Reference) (InventoryItem_ :type S%20Inventory%20Item%20Structure) (SlotIndexs :type Integer))
  (bind (_inventoryitem_classid _quickindex _inventoryitemactor_runtimeloadout _inventoryitemsc_runtimeloadout) (Utilities|Struct|BreakS_InventoryItem InventoryItem_))
  (bind _skeletalmesh_var (Utilities|GetClassDefaults _inventoryitem_classid))
  (LocalVariables|SetOwner_Character_Local Owner_Character_)
  (bind _output_get (LocalVariables|SetInventoryItem_Local InventoryItem_))
  (bind _validationx (CallFunction|LoadoutValidationF _output_get SlotIndexs))
  (if _validationx
    (Utilities|IsValid _inventoryitemsc_runtimeloadout
      (:Is%20Valid
        ;[1 1 1] Update InventoryItem with spawnedActor
        (bind _structout (Utilities|Struct|SetmembersinS_InventoryItem (LocalVariables|GetInventoryItem_Local) (LocalVariables|GetSkeletalMeshComponent_local) :!label _label))
        (return _structout))
      (:Is%20Not%20Valid
        ;[1 1 1] Armor&Clothing is always a skeletal mesh
        (Utilities|IsValid _skeletalmesh_var
          (:Is%20Valid
            ;[1 1 1] SceneComponent SkeletalMeshComponent
            (bind _returnvalue (Game|AddComponentbyClass (LocalVariables|GetOwner_Character_Local) "/Script/Engine.SkeletalMeshComponent" false))
            (LocalVariables|SetSkeletalMeshComponent_local _returnvalue)
            (Transformation|AttachComponentToComponent _returnvalue (Variables|/Script/Engine.Character|GetMesh (LocalVariables|GetOwner_Character_Local)) "None" "SnapToTarget" "SnapToTarget" "KeepRelative" true)
            (Class|SkinnedMeshComponent|SetSkeletalMesh _returnvalue _skeletalmesh_var true)
            (Class|SkinnedMeshComponent|SetMasterPoseComponent _returnvalue (Variables|/Script/Engine.Character|GetMesh (LocalVariables|GetOwner_Character_Local)) false))
          (:Is%20Not%20Valid
            (goto _label)))))
    (else
      (goto _label))))

(fn LoadoutWeaponHoldingCheckF
  (params (OwningCharacter :type Character%20Object%20Reference) (WeaponSet :type Integer))
  (bind _weaponsetholding (Class|BPICharacterInventoryInterfaceI|CIIWeaponSet-HoldingCurrentGETI(Message) OwningCharacter))
  (return (== _weaponsetholding WeaponSet)))

(fn LoadoutActorAttatchHoldingF-replacedQ
  (params (HoldingRightVsHoldingLeft :type E_Generic-LeftVsRight%20Enum :default "NewEnumerator0") (ItemActor :type BP%20Item%2000%20Item%20Master%20A%20Object%20Reference) (Character :type Character%20Object%20Reference))
  (bind _returnvalue (Utilities|GetClass ItemActor))
  (bind (_animinstance _skeletalmesh_var _itemicon _stackmax _staticmesh_var _socketdefaultsheath _socketdefaultsheath_transform _socketholdingright_transform _socketholdingleft_tranform) (Utilities|GetClassDefaults _returnvalue))
  (bind (_location _rotation) (Math|Transform|BreakTransform _socketholdingright_transform))
  (bind (_location_2 _rotation_2) (Math|Transform|BreakTransform _socketholdingleft_tranform))
  (Utilities|IsValid ItemActor
    (:Is%20Valid
      (switch Utilities|FlowControl|Switch|SwitchonE_Generic-LeftVsRight HoldingRightVsHoldingLeft
        (:NewEnumerator1
          ;[1 1 1] LEft
          (Transformation|AttachComponentToComponent (Variables|/Script/Engine.Actor|GetRootComponent ItemActor) (Variables|/Script/Engine.Character|GetMesh Character) "Hand_l" "SnapToTarget" "SnapToTarget" "KeepRelative" true)
          (Transformation|SetActorRelativeTransform ItemActor (Math|Transform|MakeTransform _location_2 _rotation_2) false false))
        (:NewEnumerator2
          ;[1 1 1] Right
          (Transformation|AttachComponentToComponent (Variables|/Script/Engine.Actor|GetRootComponent ItemActor) (Variables|/Script/Engine.Character|GetMesh Character) "Hand_r" "SnapToTarget" "SnapToTarget" "KeepRelative" true)
          (Transformation|SetActorRelativeTransform ItemActor (Math|Transform|MakeTransform _location _rotation) false false))))))

(fn LoadoutAllowedDestinationPROOFF
  (if (Utilities|IsValidClass (Variables|Default|GetLoadoutAllowed-ParentItemClassWeaponArmor))
    _
    (else
      (Development|PrintString "BPInventoryContainer00MasterAC>LoadoutAllowedDestinationPROOF== LoadoutAllowed is not valid " true true "(R=1.000000,G=0.599342,B=0.000000,A=1.000000)" 22.0)))
  (if (== (Utilities|Array|Length (Variables|Default|GetLoadoutDestination-ParentItemClassPerSlotIndex)) 0)
    (Development|PrintString "BPInventoryContainer00MasterAC>LoadoutAllowedDestinationPROOF== LDestination len " true true "(R=1.000000,G=0.599342,B=0.000000,A=1.000000)" 22.0)))

(fn ItemBumpF
  (params (Character :type Character%20Object%20Reference) (InventoryItem :type S%20Inventory%20Item%20Structure) (SlotIndex :type Integer))
  (if (Utilities|IsValidClass (.InventoryItem-ClassID (Utilities|Struct|BreakS_InventoryItem InventoryItem)))
    (Class|BPICharacterInventoryInterfaceI|CIIInventoryItemBumpingI(Message) Character InventoryItem)
    ;[1 1 1] Clear
    (Utilities|Array|SetArrayElem :TargetArray (Variables|Default|GetInventoryItem) :Index SlotIndex :bSizeToFit true)
    (return)))