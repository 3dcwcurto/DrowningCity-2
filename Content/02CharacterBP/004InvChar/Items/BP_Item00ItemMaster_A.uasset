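; Master item actor, apparently a base for child items, that can be held in a character's hands or sheathed on the body.
; Construction applies the configured static or skeletal mesh and optional AnimInstance, with a debug warning if neither mesh component is valid.
; Attach functions snap the root to hand, pelvis or spine sockets, then apply per-socket offsets, defaulting to right hand or pelvis.
; EquipmentHoldingOverideable is an empty override hook.
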(event EventBeginPlay)

(event Collision|EventActorBeginOverlap
  (params (OtherActor :type Actor%20Object%20Reference)))

(event EventTick
  (params (DeltaSeconds :type Float%20%28single-precision%29)))

(fn ConstructionScript
  (CallFunction|ConstructStaticVsSkeletalShowHideF))

(fn ConstructStaticVsSkeletalShowHideF
  (bind _animinstance (Variables|ItemInfo|GetAnimInstance))
  ;[1 1 1] PROOFING
  (|SkeletalNStaticValidCheckPROOF_CG
    (:OutputPin
      (Utilities|IsValid (Variables|ItemInfo|GetSkeletalMesh_Var)
        (:Is%20Valid
          (Class|SkinnedMeshComponent|SetSkeletalMesh (Variables|Default|GetSkeletalMesh_Component) (Variables|ItemInfo|GetSkeletalMesh_Var) true)
          (if (Utilities|IsValidClass _animinstance)
            (Class|SkeletalMeshComponent|SetAnimClass (Variables|Default|GetSkeletalMesh_Component) _animinstance)))
        (:Is%20Not%20Valid
          _))
      (Utilities|IsValid (Variables|ItemInfo|GetStaticMesh_Var)
        (:Is%20Valid
          (Components|StaticMesh|SetStaticMesh (Variables|Default|GetStaticMesh_Component) (Variables|ItemInfo|GetStaticMesh_Var)))
        (:Is%20Not%20Valid)))))

(fn ActorAttatchSocketingHoldingF
  (params (Character :type Character%20Object%20Reference) (HoldingRightVsHoldingLeft :type E_Generic-LeftVsRight%20Enum :default "NewEnumerator0"))
  (bind _socketholdingright_transform (Variables|ItemSocketing|GetSocketHoldingRight_Transform))
  (bind _socketholdingleft_tranform (Variables|ItemSocketing|GetSocketHoldingLeft_Tranform))
  (bind (_location _rotation) (Math|Transform|BreakTransform _socketholdingright_transform))
  (bind (_location_2 _rotation_2) (Math|Transform|BreakTransform _socketholdingleft_tranform))
  (Utilities|IsValid Character
    (:Is%20Valid
      (switch Utilities|FlowControl|Switch|SwitchonE_Generic-LeftVsRight HoldingRightVsHoldingLeft
        (:NewEnumerator0
          (Development|PrintString "BPItem00ItemMasterA>ActorAttatchSocketingF== LeftVsRight is null" true true "(R=1.000000,G=0.359367,B=0.000000,A=1.000000)" 22.0)
          ;[1 1 1] Right
          (Transformation|AttachComponentToComponent (Variables|Transformation|GetRootComponent self) (Variables|/Script/Engine.Character|GetMesh Character) "hand_r" "SnapToTarget" "SnapToTarget" "KeepRelative" true :!label _label)
          (Transformation|SetActorRelativeTransform (Math|Transform|MakeTransform _location _rotation) false false))
        (:NewEnumerator1
          ;[1 1 1] Left
          (Transformation|AttachComponentToComponent (Variables|Transformation|GetRootComponent self) (Variables|/Script/Engine.Character|GetMesh Character) "hand_l" "SnapToTarget" "SnapToTarget" "KeepRelative" true)
          (Transformation|SetActorRelativeTransform (Math|Transform|MakeTransform _location_2 _rotation_2) false false))
        (:NewEnumerator2
          (goto _label))))))

(fn ActorAttachSocketingSheathF
  (params (Character :type Character%20Object%20Reference))
  (bind _socketdefaultsheath_transform (Variables|ItemSocketing|GetSocketDefaultSheath_Transform))
  (bind (_location _rotation) (Math|Transform|BreakTransform _socketdefaultsheath_transform))
  (switch Utilities|FlowControl|Switch|SwitchonE_ItemSocketDefaultSheathed (Variables|ItemSocketing|GetSocketDefaultSheath)
    (:NewEnumerator0
      (LocalVariables|SetSocketSheathedName_Local "Pelvis" :!label _label))
    (:NewEnumerator1
      (goto _label))
    (:NewEnumerator2
      (LocalVariables|SetSocketSheathedName_Local "Spine_03")))
  (Transformation|AttachComponentToComponent (Variables|Transformation|GetRootComponent self) (Variables|/Script/Engine.Character|GetMesh Character) (LocalVariables|GetSocketSheathedName_Local) "SnapToTarget" "SnapToTarget" "KeepRelative" true)
  (Transformation|SetActorRelativeTransform self (Math|Transform|MakeTransform _location _rotation) false false))

(fn EquipmentHoldingOverideableF
  (params (Character :type Character%20Object%20Reference) (OtherHand :type BP%20Item%2000%20Item%20Master%20A%20Object%20Reference)))