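; Parent weapon item Blueprint that provides swept box-trace hit detection for a weapon's blade and handle.
; WeaponBoxTraceF sweeps each collision box from its stored previous location to its current one and returns the combined hits.
; WeaponBoxTracePreviousF seeds those stored locations, though both functions set the handle's previous location from the blade box.
; Collision activate and deactivate functions are unused stubs, and the event graph is empty.
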(event EventBeginPlay)

(event Collision|EventActorBeginOverlap
  (params (OtherActor :type Actor%20Object%20Reference)))

(event EventTick
  (params (DeltaSeconds :type Float%20%28single-precision%29)))

(fn ConstructionScript)

(fn WeaponBoxTraceF
  (params (TraceChannel :type ETraceTypeQuery%20Enum :default "TraceTypeQuery1") (ActorsToIgnore :type Array%20of%20Actor%20Object%20References) (DrawDebugType :type EDrawDebugTrace%20Enum :default "None"))
  (bind _boxcollision_weapontraceblade (Variables|Default|GetBoxCollision_WeaponTraceBlade))
  (bind _boxcollision_weapontracehandle (Variables|Default|GetBoxCollision_WeaponTraceHandle))
  (Utilities|FlowControl|Sequence
    (:then_0
      (bind _outhits (Class|KismetSystemLibrary|BoxTraceMulti (Variables|Default|GetTraceBladePrevious_Location) (Transformation|GetWorldLocation _boxcollision_weapontraceblade) (Variables|/Script/Engine.BoxComponent|GetBoxExtent _boxcollision_weapontraceblade) (Transformation|GetWorldRotation _boxcollision_weapontraceblade) TraceChannel false ActorsToIgnore DrawDebugType true))
      ;[1 1 1] Previous Location
      (Variables|Default|SetTraceBladePrevious_Location (Transformation|GetWorldLocation (Variables|Default|GetBoxCollision_WeaponTraceBlade)))
      (LocalVariables|SetHitResults_Local _outhits))
    (:then_1
      (bind _outhits_2 (Class|KismetSystemLibrary|BoxTraceMulti (Variables|Default|GetTraceHandlePrevious_Location) (Transformation|GetWorldLocation _boxcollision_weapontracehandle) (Variables|/Script/Engine.BoxComponent|GetBoxExtent _boxcollision_weapontracehandle) (Transformation|GetWorldRotation _boxcollision_weapontracehandle) TraceChannel false ActorsToIgnore DrawDebugType true))
      ;[1 1 1] Previous Location
      (Variables|Default|SetTraceHandlePrevious_Location (Transformation|GetWorldLocation (Variables|Default|GetBoxCollision_WeaponTraceBlade)))
      (Utilities|Array|AppendArray (LocalVariables|GetHitResults_Local) _outhits_2))
    (:then_2
      (return (LocalVariables|GetHitResults_Local)))))

(fn WeaponCollisionActiveF-DontNeed)

(fn WeaponCollisionDeactivateF-DontNeed)

(fn WeaponBoxTracePreviousF
  ;[1 1 1] Previous Location
  (Variables|Default|SetTraceBladePrevious_Location (Transformation|GetWorldLocation (Variables|Default|GetBoxCollision_WeaponTraceBlade)))
  ;[1 1 1] Previous Location
  (Variables|Default|SetTraceHandlePrevious_Location (Transformation|GetWorldLocation (Variables|Default|GetBoxCollision_WeaponTraceBlade))))