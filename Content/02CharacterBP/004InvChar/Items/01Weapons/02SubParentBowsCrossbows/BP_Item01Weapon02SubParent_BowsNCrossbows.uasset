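; Sub-parent weapon item Blueprint for bows and crossbows that sets which arrow mesh the weapon's fake arrow component uses.
; The static-vs-skeletal show/hide override takes the default mesh from the weapon's projectile class defaults.
; The equipment-holding override swaps in the projectile mesh of a quiver in the other hand, printing errors for most invalid references.
; Event graph events are disabled, and the fake arrow's attachment and visibility nodes are unconnected.
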(event EventBeginPlay
  (|CallParentFunction) ; This node is disabled and will not be called.\nDrag off pins to build functionality.
)

(event Collision|EventActorBeginOverlap
  (params (OtherActor :type Actor%20Object%20Reference))
  (|CallParentFunction OtherActor) ; This node is disabled and will not be called.\nDrag off pins to build functionality.
)

(event EventTick
  (params (DeltaSeconds :type Float%20%28single-precision%29))
  (|CallParentFunction DeltaSeconds) ; This node is disabled and will not be called.\nDrag off pins to build functionality.
)

(fn ConstructionScript
  (|CallParentFunction))

(fn EquipmentHoldingOverideableF
  (params (Character :type Character%20Object%20Reference) (OtherHand :type BP%20Item%2000%20Item%20Master%20A%20Object%20Reference))
  (bind (_asbp_item_01weapon_03sub_parent_quiver _bsuccess) (Utilities|Casting|CastToBP_Item01Weapon03SubParent_Quiver OtherHand))
  (bind _projectileslasharrowect_objectclass (Variables|Default|GetProjectileSlashArrowEct_ObjectClass))
  (bind _projectileslasharrowect_objectclass_2 (Variables|/Game/02CharacterBP/004InvChar/Items/01Weapons/BP_Item01WeaponItem00Parent_A.BP_Item01WeaponItem00Parent_A_C|GetProjectileSlashArrowEct_ObjectClass _asbp_item_01weapon_03sub_parent_quiver))
  (bind _staticmesh (Utilities|GetClassDefaults _projectileslasharrowect_objectclass_2))
  (|CallParentFunction Character OtherHand)
  (if (Utilities|IsValidClass _projectileslasharrowect_objectclass)
    (if (Utilities|IsValid (.StaticMesh (Utilities|GetClassDefaults _projectileslasharrowect_objectclass)))
      (if (Utilities|IsValid OtherHand)
        (if _bsuccess
          (if (Utilities|IsValidClass _projectileslasharrowect_objectclass_2)
            (if (Utilities|IsValid _staticmesh)
              ;[1 1 1] Set StaticMesh to QuiversArrow
              (Components|StaticMesh|SetStaticMesh (Variables|Default|GetStaticMesh_FakeArrow) _staticmesh)
              (else
                ;[1 1 1] Proofing
                (Development|PrintString "BPItem01Weapon02SubParentBowsNCrossBows>SetupEquipmentHoldingOverideable== Quivers PProjectileClass Static mEsh is not valid")))
            (else
              (Development|PrintString "BPItem01Weapon02SubParentBowsNCrossBows>SetupEquipmentHoldingOverideable== Quivers PProjectileClass is not valid")))))
      (else
        ;[1 0.9933 0.9792] Proofing
        (Development|PrintString "BPItem01Weapon02SubParentBowsNCrossBows>SetupEquipmentHoldingOverideable== PProjectileClasses Static mesh is not valid")))
    (else
      (Development|PrintString "BPItem01Weapon02SubParentBowsNCrossBows>SetupEquipmentHoldingOverideable== PProjectileClass is not valid"))))

(fn ConstructStaticVsSkeletalShowHideF
  (bind _projectileslasharrowect_objectclass (Variables|Default|GetProjectileSlashArrowEct_ObjectClass))
  (bind _staticmesh (Utilities|GetClassDefaults _projectileslasharrowect_objectclass))
  (|CallParentFunction)
  ;[1 1 1] Projectile
  (if (Utilities|IsValidClass _projectileslasharrowect_objectclass)
    (if (Utilities|IsValid _staticmesh)
      (Components|StaticMesh|SetStaticMesh (Variables|Default|GetStaticMesh_FakeArrow) _staticmesh))))