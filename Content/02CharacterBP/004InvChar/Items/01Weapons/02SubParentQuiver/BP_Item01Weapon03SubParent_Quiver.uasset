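; Quiver sub-parent Blueprint for weapon items in the inventory character system, currently little more than a pass-through to its parent class.
; The construction script and the equipment-holding override only call their parent versions, and the event graph's default events are disabled.
; Disconnected leftovers hold debug prints, a relative-transform reset and a hand socket lookup, with a note that the bow can handle arrow setup.
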(event EventBeginPlay
  (|CallParentFunction) ; This node is disabled and will not be called.\nDrag off pins to build functionality.
)

(event Collision|EventActorBeginOverlap
  (params (OtherActor :type Actor%20Object%20Reference))
  (|CallParentFunction OtherActor) ; This node is disabled and will not be called.\nDrag off pins to build functionality.
)

(event EventTick
  (params (DeltaSeconds :type Float%20%28single-precision%29))
  (|CallParentFunction DeltaSeconds) ; This node is disabled and will not be called.\nDrag off pins to build functionality.
)

(fn ConstructionScript
  (|CallParentFunction))

(fn EquipmentHoldingOverideableF
  (params (Character :type Character%20Object%20Reference) (OtherHand :type BP%20Item%2000%20Item%20Master%20A%20Object%20Reference))
  (|CallParentFunction Character OtherHand))