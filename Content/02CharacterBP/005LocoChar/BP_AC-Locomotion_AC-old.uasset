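; Older character locomotion component that turns movement input into camera-yaw-relative motion and tracks gait and movement state.
; Its tick derives ALSv4-style velocity, acceleration and aim values, then resolves allowed gait from desired input and cap, limiting sprint on sharp turns.
; Movement-mode changes push grounded or falling state to the AnimInstance through an interface.
; The tired-gait limit is a pass-through, and walk-speed application is never called.
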(event Custom|GaitDesiredInput_AclCE
  (params (GaitDesiredInput :type E_Gait-WalkRunSprint%20Enum :default "NewEnumerator0"))
  ;[1 1 1] GetDesired
  (CallFunction|GaitDesiredInputF GaitDesiredInput))

(event Custom|AcL_EventOnLanding_CE
  ;[1 1 1] OnLanding
  ;;[1 0.9404 0.4792] todo-LandingAction:hard,shallow,prone,Supine
  (CallFunction|EventonLandingF))

(event Custom|Loco-Tick_AclCE
  ;[0.399 1 0] Tick
  (CallFunction|LocomotionTickF))

(event Custom|OnMovementModeChange_CE
  (params (NewMovementMode :type EMovementMode%20Enum :default "MOVE_None"))
  ;[1 1 1] OnMovementModeChange
  (CallFunction|EventonMovementModeChangeF NewMovementMode))

(event Custom|LandingCompressionStart_CE
  ;[1 1 1] LandCompression_Start&Stop
)

(event Custom|LandingCompressionTrick_CE
  (params (LandingCompressionAlpha :type Float%20%28double-precision%29))
  ;[1 1 1] LandCompression_Start&Stop
)

(event Custom|InputMovementForwardBack_AclCE
  (params (InputForwardAxis :type Float%20%28double-precision%29))
  ;[1 1 1] Input
  (CallFunction|Input-MovementForwardBackwardF InputForwardAxis))

(event Custom|InputMovementRightLeft_AclCE
  (params (InputRightAxis :type Float%20%28double-precision%29))
  ;[1 1 1] Input
  (CallFunction|Input-MovementRightLeftF InputRightAxis))

(event Custom|GaitCurrent_%28SERVER%29_CE
  (params (GaitCurrent%20%20 :type Byte :default 0))
  ;[1 1 1] Gait
)

(event Custom|GaitCap-WalkRunSprint_CE
  (params (GaitCap :type Byte :default 0))
  ;[1 1 1] Gait
)

(event Custom|GaitAllowed_%28SERVER%29_CE
  (params (Gait :type E_Gait-WalkRunSprint%20Enum :default "NewEnumerator0"))
  ;[1 1 1] GaitAllowed
  (CallFunction|Loco-GaitAllowedNMoveSettingsF Gait))

(event Custom|LandingCompressionStop_CE
  ;[1 1 1] LandCompression_Start&Stop
)

(fn ReferenceAnimInstancePureF
  (Utilities|IsValid (Variables|Reference|GetAnimInstance_Ref)
    (:Is%20Valid
      (Variables|Reference|SetAnimInstance_Ref (Variables|Reference|GetAnimInstance_Ref)))
    (:Is%20Not%20Valid
      (bind _output_get (Variables|Reference|SetAnimInstance_Ref (Components|SkeletalMesh|GetAnimInstance (Variables|/Script/Engine.Character|GetMesh (Reference|ReferenceCharacterPureF)))))
      (Utilities|IsValid _output_get
        (:Is%20Valid
          (return _output_get))
        (:Is%20Not%20Valid
          (Development|PrintString "BPACLocotionAc>ReferenceAnimInstancePureF==  AnimInstance is not valid" true true "(R=1.000000,G=0.244032,B=0.000000,A=1.000000)" 22.0)
          (return 0))))))

(fn ReferenceCharacterPureF
  (Utilities|IsValid (Variables|Reference|GetCharacter_Ref)
    (:Is%20Valid
      (return (Variables|Reference|GetCharacter_Ref)))
    (:Is%20Not%20Valid
      (bind _ascharacter (Utilities|Casting|CastToCharacter (Components|GetOwner))
        (:then
          (bind _output_get (Variables|Reference|SetCharacter_Ref _ascharacter))
          (return _output_get))
        (:CastFailed
          (Development|PrintString "BPACLocotionAc>ReferenceCharacterPureF== owning character cast failed" true true "(R=1.000000,G=0.102836,B=0.000000,A=1.000000)" 22.0)
          (return 0))))))

(fn ReferenceMovementComponentPureF
  (bind _character (Reference|ReferenceCharacterPureF))
  (bind _movementcomponent_ref (Variables|Reference|GetMovementComponent_Ref))
  (bind _charactermovement (Variables|/Script/Engine.Character|GetCharacterMovement _character))
  (Utilities|IsValid _movementcomponent_ref
    (:Is%20Valid
      (return _movementcomponent_ref))
    (:Is%20Not%20Valid
      (Utilities|IsValid _charactermovement
        (:Is%20Valid
          (return _charactermovement))
        (:Is%20Not%20Valid
          (Development|PrintString "BPACLocotionAc>ReferenceMovementComponentPureF== characterMovementComponent not valid")
          (return 0))))))

(fn LocomotionTickF
  ;[0.18 0.6 0.9] Do Every Frame
  (Utilities|FlowControl|Sequence
    (:then_0
      (CallFunction|LocoCalculateEssentialVariablesALSv4F)
      (switch Utilities|FlowControl|Switch|SwitchonE_MoveModeState (Variables|Default|GetMoveModeStateCurrent_Var)
        (:NewEnumerator0
          _)
        (:NewEnumerator1
          _))
      ;[0.18 0.6 0.9] Do While On Ground
      (CallFunction|LocoCharacterMovement-GaitCalculationF))
    (:then_1
      (CallFunction|LocoCacheValuesALSv4F))))

(fn GaitDesiredInputF
  (params (GaitDesiredInput :type E_Gait-WalkRunSprint%20Enum :default "NewEnumerator0"))
  (Variables|Default|SetGaitDesiredInput_Var GaitDesiredInput))

(fn EventonLandingF
  (bind _character (Reference|ReferenceCharacterPureF))
  (bind _returnvalue (Transformation|GetVelocity _character))
  (bind (_x _y _z) (Math|Vector|BreakVector _returnvalue))
  ;[1 1 1] FallingInAirDownwardLateralSpeedTick_F
  (Variables|Default|SetFallingInAir_SpeedDownwardLastInAirFall_Var _z)
  (Variables|Default|SetFallingInAir_SpeedLateralLastInAirFall_Var (Math|Vector|VectorLength (Math|Vector|MakeVector _x _y 0.0))))

(fn EventonMovementModeChangeF
  (params (NewMovementMode :type EMovementMode%20Enum :default "MOVE_None"))
  (switch Utilities|FlowControl|Switch|SwitchonEMovementMode NewMovementMode
    (:MOVE_None
      (CallFunction|MoveModeStateAnimBpUpdateF "NewEnumerator1" :!label _label))
    (:MOVE_Walking
      (goto _label))
    (:MOVE_NavWalking
      (goto _label))
    (:MOVE_Falling
      (CallFunction|MoveModeStateAnimBpUpdateF "NewEnumerator2")
      (CallFunction|FallingAirCancelF))
    (:MOVE_Swimming
      (Development|PrintString "BPACLocotionAC>EG== Flying&Swimming&Custom Not set up" true true "(R=1.000000,G=0.176580,B=0.000000,A=1.000000)" 22.0 :!label _label_2))
    (:MOVE_Flying
      (goto _label_2))
    (:MOVE_Custom
      (goto _label_2))))

(fn MoveModeStateAnimBpUpdateF
  (params (MoveModeState :type E_MoveModeState%20Enum :default "NewEnumerator0"))
  (bind _animinstance (Reference|ReferenceAnimInstancePureF))
  (bind _aout (Utilities|DoDiffSwitchM MoveModeState (Variables|Default|GetMoveModeStateCurrent_Var))
    (:true
      (bind _output_get (Variables|Default|SetMoveModeStatePrevious_Var (Variables|Default|GetMoveModeStateCurrent_Var)))
      (bind _output_get_2 (Variables|Default|SetMoveModeStateCurrent_Var _aout))
      (Class|BPIAnimationLocomotionInterfaceI|ALIMoveModeStateCurrentSETI(Message) _animinstance _output_get_2)
      (Class|BPIAnimationLocomotionInterfaceI|ALIMoveModeStatePreviousSETI(Message) _animinstance _output_get))))

(fn FallingAirCancelF
  (CallFunction|LandingCompressionStopCE))

(fn LocoCalculateEssentialVariablesALSv4F
  (bind _character (Reference|ReferenceCharacterPureF))
  (bind _movementcomponent_ref (Reference|ReferenceMovementComponentPureF))
  (bind _returnvalue (Pawn|Components|CharacterMovement|GetCurrentAcceleration _movementcomponent_ref))
  (bind _returnvalue_2 (Class|CharacterMovementComponent|GetMaxAcceleration _movementcomponent_ref))
  (bind _returnvalue_3 (Transformation|GetVelocity _character))
  (bind _returnvalue_4 (Math|Vector|VectorLength _returnvalue))
  (bind _returnvalue_5 (Math|Vector|VectorLength (Math|Vector|MakeVector (.x _returnvalue_3) (.y _returnvalue_3) 0.0)))
  (bind _returnvalue_6 (> _returnvalue_5 1.0))
  (bind _returnvalue_7 (/ _returnvalue_4 _returnvalue_2))
  (bind _returnvalue_8 (> _returnvalue_7 0.0))
  (Utilities|FlowControl|Sequence
    (:then_0
      ;[1 1 1] Set the amount of Acceleration.
      (Variables|Default|SetAcceleration_ALSv4 (/ (- (Transformation|GetVelocity (Reference|ReferenceCharacterPureF)) (Variables|Default|GetPreviousVelocity_ALSv4)) (Utilities|Time|GetWorldDeltaSeconds))))
    (:then_1
      ;[1 1 1] Determine if the character is moving by getting it's speed. The Speed equals the length of the horizontal (x y) velocity, so it does not take vertical movement into account. If the character is moving, update the last velocity rotation. This value is saved because it might be useful to know the last orientation of movement even after the character has stopped.
      (Variables|Default|SetSpeed%28XYVeloctiy%29_ALSv4 _returnvalue_5)
      (Variables|Default|SetIsMoving%28&InMoveState%29 _returnvalue_6)
      (if _returnvalue_6
        (Variables|Default|SetLastVelocityRotation (Math|Conversions|RotationFromXVector (Transformation|GetVelocity (Reference|ReferenceCharacterPureF))))))
    (:then_2
      ;[1 1 1] Determine if the character has movement input by getting its movement input amount. The Movement Input Amount is equal to the current acceleration divided by the max acceleration so that it has a range of 0-1, 1 being the maximum possible amount of input, and 0 beiung none. If the character has movement input, update the Last Movement Input Rotation.
      (Variables|Default|SetMovementInputAmount_ALSv4 _returnvalue_7)
      (Variables|Default|SetHasMovementInput%28&InMoveState%29 _returnvalue_8)
      (if _returnvalue_8
        (Variables|Default|SetLastMovementInputRotation (Math|Conversions|RotationFromXVector (Pawn|Components|CharacterMovement|GetCurrentAcceleration (Reference|ReferenceMovementComponentPureF))))))
    (:then_3
      ;[1 1 1] Set the Aim Yaw rate by comparing the current and previous Aim Yaw value, divided by Delta Seconds. This represents the speed the camera is rotating left to right.
      (Variables|Default|SetAimYawRate (Math|Float|Absolute(Float) (/ (- (.yaw (Pawn|GetControlRotation (Reference|ReferenceCharacterPureF) :!class /Script/Engine.Pawn)) (Variables|Default|GetPreviousAimYaw_ALSv4)) (Utilities|Time|GetWorldDeltaSeconds)))))))

(fn LocoCacheValuesALSv4F
  (bind _character (Reference|ReferenceCharacterPureF))
  ;[1 1 1] Cache certain values to be used in calculations on the next frame
  (Utilities|FlowControl|Sequence
    (:then_0
      (Variables|Default|SetPreviousVelocity_ALSv4 (Transformation|GetVelocity _character)))
    (:then_1
      (Variables|Default|SetPreviousAimYaw_ALSv4 (.yaw (Pawn|GetControlRotation _character :!class /Script/Engine.Pawn))))))

(fn LocoCharacterMovement-GaitCalculationF
  (bind _gaitallowedresult (CallFunction|LocoGaitAllowedUpdate-DesiredVsGapNRestrictionF "NewEnumerator0" "NewEnumerator0"))
  (bind _gaitresult (CallFunction|Loco-GaitTiredLimitF _gaitallowedresult "NewEnumerator0"))
  (CallFunction|GaitAllowed(SERVER)CE _gaitresult))

(fn LocoGaitAllowedUpdate-DesiredVsGapNRestrictionF
  (params (SettingsGaitFastest-todo :type E_Gait-WalkRunSprint%20Enum :default "NewEnumerator0") (SettingsStopStyle-todo :type E_Gait-WalkRunSprint%20Enum :default "NewEnumerator0"))
  (switch Utilities|FlowControl|Switch|SwitchonE_Gait-WalkRunSprint (Variables|Default|GetGaitDesiredInput_Var)
    (:NewEnumerator0
      (switch Utilities|FlowControl|Switch|SwitchonE_Gait-WalkRunSprint (Variables|Default|GetGaitCap_Var)
        (:NewEnumerator0
          _)
        (:NewEnumerator1
          _)
        (:NewEnumerator2
          _)
        (:NewEnumerator3
          _))
      (return "NewEnumerator0"))
    (:NewEnumerator1
      (switch Utilities|FlowControl|Switch|SwitchonE_Gait-WalkRunSprint (Variables|Default|GetGaitCap_Var)
        (:NewEnumerator0
          (return "NewEnumerator0"))
        (:NewEnumerator1
          _)
        (:NewEnumerator2
          _)
        (:NewEnumerator3
          _))
      (return "NewEnumerator1"))
    (:NewEnumerator2
      (switch Utilities|FlowControl|Switch|SwitchonE_Gait-WalkRunSprint (Variables|Default|GetGaitCap_Var)
        (:NewEnumerator0
          (return "NewEnumerator0"))
        (:NewEnumerator1
          (return "NewEnumerator1"))
        (:NewEnumerator2
          _)
        (:NewEnumerator3
          _))
      (return "NewEnumerator2"))
    (:NewEnumerator3
      (switch Utilities|FlowControl|Switch|SwitchonE_Gait-WalkRunSprint (Variables|Default|GetGaitCap_Var)
        (:NewEnumerator0
          (return "NewEnumerator0"))
        (:NewEnumerator1
          (return "NewEnumerator1"))
        (:NewEnumerator2
          (return "NewEnumerator2"))
        (:NewEnumerator3
          (bind _movefastest_turnanglenmoveinput_ (CallFunction|Loco-SharpTurnCheckF "NewEnumerator0"))
          (if _movefastest_turnanglenmoveinput_
            (return "NewEnumerator3")
            (else
              (return "NewEnumerator2"))))))))

(fn Loco-SharpTurnCheckF
  (params (SettingsFastRequirement-todo :type E_Gait-WalkRunSprint%20Enum :default "NewEnumerator0"))
  (bind _character (Reference|ReferenceCharacterPureF))
  (return (and (Variables|Default|GetHasMovementInput%28&InMoveState%29) (<= (Math|Float|Absolute(Float) (.yaw (Math|Rotator|Delta(Rotator) (Math|Conversions|RotationFromXVector (Pawn|Components|CharacterMovement|GetCurrentAcceleration (Variables|/Script/Engine.Character|GetCharacterMovement _character))) (Transformation|GetActorRotation _character)))) 55.0))))

(fn Loco-GaitTiredLimitF
  (params (GaitAllowedResult :type E_Gait-WalkRunSprint%20Enum :default "NewEnumerator0") (SettingsTiredGaitLimit-Todo :type E_Gait-WalkRunSprint%20Enum :default "NewEnumerator0"))
  (bind _output_get (LocalVariables|SetGaitAllowedResult_Local GaitAllowedResult))
  (return _output_get))

(fn Loco-GaitAllowedNMoveSettingsF
  (params (Gait :type E_Gait-WalkRunSprint%20Enum :default "NewEnumerator0"))
  (Variables|Default|SetGaitAllowed_Var Gait))

(fn Loco-MovementSettingsF
  (params (SettingsMovement-Todo :type Boolean))
  (switch Utilities|FlowControl|Switch|SwitchonE_Gait-WalkRunSprint (Variables|Default|GetGaitAllowed_Var)
    (:NewEnumerator0
      (LocalVariables|SetSpeed_local 0.0))
    (:NewEnumerator1
      (LocalVariables|SetSpeed_local 175.0))
    (:NewEnumerator2
      (LocalVariables|SetSpeed_local 375.0))
    (:NewEnumerator3
      (LocalVariables|SetSpeed_local 6e+02)))
  (Variables|/Script/Engine.CharacterMovementComponent|SetMaxWalkSpeed (Reference|ReferenceMovementComponentPureF) (LocalVariables|GetSpeed_local)))

(fn Input-MovementForwardBackwardF
  (params (InputForwardAxis :type Float%20%28double-precision%29))
  (bind _character (Reference|ReferenceCharacterPureF))
  (bind _output_get (Variables|Input|SetInputForwardAxis InputForwardAxis))
  (CallFunction|Input-FixDiagonalsF _output_get 0.0)
  (Pawn|Input|AddMovementInput _character (Math|Vector|GetForwardVector (Math|Rotator|MakeRotator 0.0 0.0 (.yaw (Pawn|GetControlRotation _character :!class /Script/Engine.Pawn)))) _output_get false))

(fn Input-MovementRightLeftF
  (params (InputRightAxis :type Float%20%28double-precision%29))
  (bind _character (Reference|ReferenceCharacterPureF))
  (bind _output_get (Variables|Input|SetInputRightAxis InputRightAxis))
  (bind _x_out (CallFunction|Input-FixDiagonalsF 0.0 _output_get))
  (Pawn|Input|AddMovementInput _character (Math|Vector|GetRightVector (Math|Rotator|MakeRotator 0.0 0.0 (.yaw (Pawn|GetControlRotation _character :!class /Script/Engine.Pawn)))) _x_out false))

(fn Input-FixDiagonalsF
  (params (Y%20in :type Float%20%28double-precision%29) (X%20in :type Float%20%28double-precision%29))
  (return (Math|Float|Clamp(Float) (* Y%20in (Math|Float|MapRangeClamped (Math|Float|Absolute(Float) X%20in) 0.0 0.6 1.0 1.2)) -1.0) (Math|Float|Clamp(Float) (* X%20in (Math|Float|MapRangeClamped (Math|Float|Absolute(Float) Y%20in) 0.0 0.6 1.0 1.2)) -1.0)))