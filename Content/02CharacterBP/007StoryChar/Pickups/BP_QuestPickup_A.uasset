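; BP_QuestPickup_A is a quest item pickup for the Narrative quest system.
; When the sphere is overlapped, it completes the NT_FindItem task on the overlapping actor's Narrative component, using TaskNameItemName as the item name, then destroys itself.
; On BeginPlay it binds to the Narrative load-complete event and destroys itself if the loaded save already has that task completed.
; That load check is noted as single-player only.
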(event OnComponentBeginOverlap(Sphere)
  (params (OverlappedComponent :type Primitive%20Component%20Object%20Reference) (OtherActor :type Actor%20Object%20Reference) (OtherComp :type Primitive%20Component%20Object%20Reference) (OtherBodyIndex :type Integer) (bFromSweep :type Boolean) (SweepResult :type Hit%20Result%20Structure%20%28by%20ref%29))
  ;[1 1 1] Pickup Overlap
  (Utilities|IsValid OtherActor
    (:Is%20Valid
      (|CompleteNarrativeTask (Class|NarrativeFunctionLibrary|GetNarrativeComponentfromTarget OtherActor) "/Game/02CharacterBP/007StoryChar/Narrative/06NarrativeTask/NT_FindItem.NT_FindItem" (Utilities|String|ToString(Name) (Variables|00PickupItem|GetTaskName_ItemName)))
      (Development|PrintString "ItemPickup" true true "(R=1.000000,G=0.000000,B=0.822304,A=1.000000)")
      (Actor|DestroyActor))))

(event Custom|OnLoadComplete
  (params (SaveGameName :type String))
  ;[1 1 1] Destroy
  ;;[1 1 1] LoadingSaveFile: already pickup Item so destroy it
  (if (Class|NarrativeComponent|HasCompletedTask (Class|NarrativeFunctionLibrary|GetNarrativeComponent) "/Game/02CharacterBP/007StoryChar/Narrative/06NarrativeTask/NT_FindItem.NT_FindItem" (Utilities|String|ToString(Name) (Variables|00PickupItem|GetTaskName_ItemName)) 1)
    (Development|PrintString (Utilities|String|Append "PickupAlreadyPickedup:Destroy:" (Utilities|String|ToString(Name) (Variables|00PickupItem|GetTaskName_ItemName))))
    (Actor|DestroyActor)))

(event EventBeginPlay
  ;[1 1 1] Destroy
  (Utilities|FlowControl|Sequence
    (:then_1
      ;;[1 1 1] LoadingSaveFile: already pickup Item so destroy it
      (EventDispatchers|BindEventtoOnLoadComplete (Class|NarrativeFunctionLibrary|GetNarrativeComponent) (delegate Custom|OnLoadComplete)))))

(event Collision|EventActorBeginOverlap
  (params (OtherActor :type Actor%20Object%20Reference))
  ;[1 1 1] Destroy
)

(event EventTick
  (params (DeltaSeconds :type Float%20%28single-precision%29))
  ;[1 1 1] Destroy
)

(fn ConstructionScript)