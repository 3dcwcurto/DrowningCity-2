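; Master character Blueprint whose BeginPlay and Tick only call the parent; most other logic is marked as moved there or left unwired.
; Leftover functions combine hover and selection states into custom depth stencil values for mesh outlines, and set third-person spring arm values from the controller's perspective mode.
; A macro sorts active-state gameplay tags into moving or disabled branches, beside an unwired graph of tag-matching tests.
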(event EventTick
  (params (DeltaSeconds :type Float%20%28single-precision%29))
  ;[0.03137 0.4627 0] Tick
  (|CallParentFunction DeltaSeconds))

(event EventBeginPlay
  ;[0.251 1 0] BeginPlay
  (|CallParentFunction))

(fn ConstructionScript)

(fn OutlineSelectionHoverF-oldMoved
  (params (OutlineStateDesired :type E_Generic-OnOpenActiveVsOffClosedDisabled%20Enum :default "NewEnumerator0") (HoveringStateDesired :type E_Generic-OnOpenActiveVsOffClosedDisabled%20Enum :default "NewEnumerator0"))
  (bind _mesh (Variables|Character|GetMesh))
  (bind _mesh_2 (Variables|Character|GetMesh))
  (bind _mesh_3 (Variables|Character|GetMesh))
  (bind _mesh_4 (Variables|Character|GetMesh))
  (bind _mesh_5 (Variables|Character|GetMesh))
  (bind _mesh_6 (Variables|Character|GetMesh))
  (switch Utilities|FlowControl|Switch|SwitchonE_Generic-OnOpenActiveVsOffClosedDisabled OutlineStateDesired
    (:NewEnumerator0
      (switch Utilities|FlowControl|Switch|SwitchonE_Generic-OnOpenActiveVsOffClosedDisabled HoveringStateDesired
        (:NewEnumerator0)
        (:NewEnumerator1
          ;[1 1 1] HoverBegin
          (if (not (Utilities|Enum|Equal(Enum) (Variables|00GameplayTagTestMaster|GetOutlineHoveringStateDesired_Var_0) "NewEnumerator1"))
            ;;[1 1 1] Set
            (Variables|00GameplayTagTestMaster|SetOutlineHoveringStateDesired_Var_0 "NewEnumerator1")
            (switch Utilities|FlowControl|Switch|SwitchonE_Generic-OnOpenActiveVsOffClosedDisabled (Variables|00GameplayTagTestMaster|GetOutlineSelectedStateDesired_Var_0)
              (:NewEnumerator0
                ;;[1 1 1] Hovering
                (Rendering|SetRenderCustomDepth _mesh_5 true :!label _label)
                (Rendering|SetCustomDepthStencilValue _mesh_5 (Variables|00GameplayTagTestMaster|GetSelectedState-Hovered_3Default_0)))
              (:NewEnumerator1
                ;;[1 1 1] Hovering+selected
                (Rendering|SetRenderCustomDepth _mesh_6 true)
                (Rendering|SetCustomDepthStencilValue _mesh_6 6))
              (:NewEnumerator2
                (goto _label)))))
        (:NewEnumerator2
          ;[1 1 1] HoverEnd
          (if (not (Utilities|Enum|Equal(Enum) (Variables|00GameplayTagTestMaster|GetOutlineHoveringStateDesired_Var_0) "NewEnumerator2"))
            ;;[1 1 1] Clear
            (Variables|00GameplayTagTestMaster|SetOutlineHoveringStateDesired_Var_0 "NewEnumerator2")
            (switch Utilities|FlowControl|Switch|SwitchonE_Generic-OnOpenActiveVsOffClosedDisabled (Variables|00GameplayTagTestMaster|GetOutlineSelectedStateDesired_Var_0)
              (:NewEnumerator0
                ;;[1 1 1] Zero is disabled
                (Rendering|SetCustomDepthStencilValue (Variables|Character|GetMesh) 0 :!label _label_2))
              (:NewEnumerator1
                ;;[1 1 1] Still Selected
                (Rendering|SetRenderCustomDepth _mesh_4 true)
                (Rendering|SetCustomDepthStencilValue _mesh_4 (Variables|00GameplayTagTestMaster|GetSelectedState-Active_3Default_0)))
              (:NewEnumerator2
                (goto _label_2)))))))
    (:NewEnumerator1
      ;[1 1 1] Select
      (if (not (Utilities|Enum|Equal(Enum) (Variables|00GameplayTagTestMaster|GetOutlineSelectedStateDesired_Var_0) "NewEnumerator1"))
        ;;[1 1 1] Set
        (Variables|00GameplayTagTestMaster|SetOutlineSelectedStateDesired_Var_0 "NewEnumerator1")
        (switch Utilities|FlowControl|Switch|SwitchonE_Generic-OnOpenActiveVsOffClosedDisabled (Variables|00GameplayTagTestMaster|GetOutlineHoveringStateDesired_Var_0)
          (:NewEnumerator0
            ;;[1 1 1] Selected
            (Rendering|SetRenderCustomDepth _mesh_3 true :!label _label_3)
            (Rendering|SetCustomDepthStencilValue _mesh_3 (Variables|00GameplayTagTestMaster|GetSelectedState-Active_3Default_0)))
          (:NewEnumerator1
            ;;[1 1 1] Hovering+selected
            (Rendering|SetRenderCustomDepth _mesh true)
            (Rendering|SetCustomDepthStencilValue _mesh 6))
          (:NewEnumerator2
            (goto _label_3)))))
    (:NewEnumerator2
      ;[1 1 1] Deselect
      (if (not (Utilities|Enum|Equal(Enum) (Variables|00GameplayTagTestMaster|GetOutlineSelectedStateDesired_Var_0) "NewEnumerator2"))
        ;;[1 1 1] Clear
        (Variables|00GameplayTagTestMaster|SetOutlineSelectedStateDesired_Var_0 "NewEnumerator2")
        (switch Utilities|FlowControl|Switch|SwitchonE_Generic-OnOpenActiveVsOffClosedDisabled (Variables|00GameplayTagTestMaster|GetOutlineHoveringStateDesired_Var_0)
          (:NewEnumerator0
            ;;[1 1 1] Zero is disabled
            (Rendering|SetCustomDepthStencilValue (Variables|Character|GetMesh) 0 :!label _label_4))
          (:NewEnumerator1
            ;;[1 1 1] Still Hovering
            (Rendering|SetRenderCustomDepth _mesh_2 true)
            (Rendering|SetCustomDepthStencilValue _mesh_2 (Variables|00GameplayTagTestMaster|GetSelectedState-Hovered_3Default_0)))
          (:NewEnumerator2
            (goto _label_4)))))))

(fn CameraPerspectiveSetttingsMainF-MovedtoParent
  (bind _returnvalue (Pawn|GetController))
  (Utilities|IsValid _returnvalue
    (:Is%20Valid
      (bind _cameraperspectivemode (Class|BPIPlayerControllerBaseInterfaceI|PcBICameraPerspectiveModeGETI(Message) _returnvalue))
      (switch Utilities|FlowControl|Switch|SwitchonE_CameraPerspectiveMode-Fps3rdIso _cameraperspectivemode
        (:NewEnumerator0
          (Development|PrintString "BPCharacterMasterC>CameraPerspetiveSettingsMainF== CameraPerspectiveMode is null" true true "(R=1.000000,G=0.138182,B=0.247926,A=1.000000)"))
        (:NewEnumerator2
          ;[1 1 1] Settings from AlsV3
          (CallFunction|CameraPerspectiveSettingsSETF-MovedtoParent 275.0 15.0 "0,70.000000,60.000000" 5.0))))))

(fn CameraPerspectiveSettingsSETF-MovedtoParent
  (params (TargetArmLength :type Float%20%28double-precision%29) (CameraLagSpeed :type Float%20%28double-precision%29) (SocketOffset :type Vector) (LerpAlhpa :type Float%20%28double-precision%29))
  (bind _tp_springarm_boon (Variables|Default|GetTP_SpringArm_Boon))
  (Variables|/Script/Engine.SpringArmComponent|SetTargetArmLength _tp_springarm_boon TargetArmLength)
  (Variables|/Script/Engine.SpringArmComponent|SetCameraLagSpeed _tp_springarm_boon CameraLagSpeed)
  (Variables|/Script/Engine.SpringArmComponent|SetSocketOffset _tp_springarm_boon SocketOffset))