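; Character Blueprint layer that gives each character its team faction and diplomatic stance toward other factions.
; On preset setup it caches enemy, allied and neutral lists from the faction preset's starting defaults, then registers with the GameState's faction hierarchy roster.
; Comparison and hit-result filtering functions read that cached copy to classify others or pick out enemies, without refreshing it.
; Interface functions expose the comparison and the cached alignment.
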(event EventBeginPlay
  ;[0.251 1 0] Begin New
  (|CallParentFunction))

(event Collision|EventActorBeginOverlap
  (params (OtherActor :type Actor%20Object%20Reference))
  ;[0.251 1 0] Begin New
)

(event EventTick
  (params (DeltaSeconds :type Float%20%28single-precision%29))
  ;[0.03766 0.3229 0] Tick
)

(event EventCharacterPresetSetup-InheritableCE
  (params (CharacterPreset :type Primary%20Data%20Asset%20Object%20Reference) (SpawnTrueVsSceneFalse :type Boolean))
  ;[0 1 0.4249] Possessed
  (|CallParentFunction CharacterPreset SpawnTrueVsSceneFalse)
  (02TeamFaction|CharacterPreset-TeamFactionF CharacterPreset))

(fn ConstructionScript)

(fn CharacterPreset-TeamFactionF
  (params (CharacterPreset :type Primary%20Data%20Asset%20Object%20Reference))
  ;[1 1 1] DiplomacyAlignment
  (02TeamFaction|TeamFactionDiplomacyAlignmentGsGETF CharacterPreset)
  ;[1 1 1] HierchyRoster
  (Class|BPIGameStateTeamFactionDiplomacyI|GSTFDTeamFactionHierarchyRosterDispatcherI(Message) (Game|GetGameState) self)
  (return))

(fn TeamFactionDiplomacyAlignmentGsGETF
  (params (CharacterPresetId :type Primary%20Data%20Asset%20Object%20Reference))
  (bind _teamfactionpresetid (Class|BPICharacterPresetInterface|HCPICharacterPresetInfoGETI(Message) CharacterPresetId))
  (bind (_towncamps _hierarchyrosterdefault _diplomaticalignment_enemiesstartdefault _diplomaticalignment_alliesstartdefault _diplomaticalignment_nuetralstartdefault) (Class|BPITeamFactionPresetInterfaceI|TFPITeamFactionPresetInfoGETI(Message) _teamfactionpresetid))
  (Variables|Default|SetTeamFactionDiplomacyOfSelf (Utilities|Struct|MakeS_DiplomacyAlignment01 0 false _diplomaticalignment_enemiesstartdefault _diplomaticalignment_alliesstartdefault _diplomaticalignment_nuetralstartdefault)))

(fn TeamFactionCompareTeamsDiplomaticAlignmentF
  (params (SelfCharacterPreset-old :type Boolean) (OtherCharacterPreset :type Primary%20Data%20Asset%20Object%20Reference))
  (bind _teamfactiondiplomacyofself (Variables|Default|GetTeamFactionDiplomacyOfSelf))
  (bind (_teamfactionpresetid_replacedbyindexer ___ _enemylogindexer _enemy_factionshated_war _alliedlogindexer _allied_factionsliked_alliance _nuetrallogindexer) (Utilities|Struct|BreakS_DiplomacyAlignment01 _teamfactiondiplomacyofself))
  ;[1 1 1] Self
  (bind _camptownpresetid (Class|BPICampTownActorInterfaceI|CTGICampTownPresetPdaGETI(Message) self))
  (bind _teamfactionpresetid (Class|BPICharacterPresetInterface|HCPICharacterPresetInfoGETI(Message) _camptownpresetid))
  ;[1 1 1] Other
  (bind _camptownpresetid_2 (Class|BPICampTownActorInterfaceI|CTGICampTownPresetPdaGETI(Message) OtherCharacterPreset))
  (bind _teamfactionpresetid_2 (Class|BPICharacterPresetInterface|HCPICharacterPresetInfoGETI(Message) _camptownpresetid_2))
  (LocalVariables|SetTeamFactonOther_local _teamfactionpresetid_2)
  (if (== _teamfactionpresetid_2 _teamfactionpresetid)
    (LocalVariables|SetAlignment_Local "NewEnumerator6")
    (elif (Utilities|Array|ContainsItem _enemylogindexer (LocalVariables|GetTeamFactonOther_local))
      (LocalVariables|SetAlignment_Local "NewEnumerator3")
      (elif (Utilities|Array|ContainsItem _alliedlogindexer (LocalVariables|GetTeamFactonOther_local))
        (LocalVariables|SetAlignment_Local "NewEnumerator1")
        (else
          (if (Utilities|Array|ContainsItem _nuetrallogindexer (LocalVariables|GetTeamFactonOther_local))
            _
            (else
              (Development|PrintString "TeamFactionCompareMainF--  Faction not found in DiplomacyOfSelf" true true "(R=1.000000,G=0.426837,B=0.000000,A=1.000000)" 22.0)))
          (LocalVariables|SetAlignment_Local "NewEnumerator2")))))
  (return (LocalVariables|GetAlignment_Local)))

(fn TeamFactionHitResultEnemyCheckF
  (params (HitResult :type Array%20of%20Hit%20Result%20Structures))
  (if (> (Utilities|Array|Length (.EnemyLogIndexer (Utilities|Struct|BreakS_DiplomacyAlignment01 (Variables|Default|GetTeamFactionDiplomacyOfSelf)))) 0)
    (for _array_element HitResult
      (bind _ascharacter (Utilities|Casting|CastToCharacter (.HitActor (Collision|BreakHitResult _array_element))))
      (bind _pdacharacterpreset (Class|BPICharacterBaseInterface|CBICharacterPresetPdaGETI(Message) _ascharacter))
      (bind _towncamppresetid (Class|BPICharacterPresetInterface|HCPICharacterPresetInfoGETI(Message) _pdacharacterpreset))
      (if (Utilities|Array|ContainsItem (.EnemyLogIndexer (Utilities|Struct|BreakS_DiplomacyAlignment01 (Variables|Default|GetTeamFactionDiplomacyOfSelf))) _towncamppresetid)
        (Utilities|Array|Add (LocalVariables|GetHitResultEnemyConfimred_Local) _array_element)))
    (else
      (Development|PrintString (Utilities|String|Append "BPCharacterTeamFaction>TeamFactionHitResultEnemyCheckF==" "" "TeamFaction does not have enemies") true true "(R=1.000000,G=0.000000,B=0.044178,A=1.000000)")))
  (return (LocalVariables|GetHitResultEnemyConfimred_Local)))

(fn CTFITeamFactionCompareTeamsDiplomaticAlignmentI
  (params (OtherCharacterPresetID :type Primary%20Data%20Asset%20Object%20Reference))
  (bind _alignment (02TeamFaction|TeamFactionCompareTeamsDiplomaticAlignmentF false OtherCharacterPresetID))
  (return _alignment))

(fn CTFITeamFactionDiplomacticAlignmentOfSelfTeamGETI
  (return (Variables|Default|GetTeamFactionDiplomacyOfSelf)))