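; Master AI character Blueprint that ties NPCs to a town or camp, leash, garrison and patrol route.
; BeginPlay writes those starting actors to the Blackboard using key names fetched from the AI controller by interface.
; Preset setup adds scene-placed characters to their CampTown roster, and a billboard icon shows perception status (Suspicious unfinished).
; Interface functions expose the behavior tree and starting actors, though some setters are stubs, alongside proxy-actor test inputs.
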(event EventBeginPlay
  ;[0.2507 1 0] BeginPlay
  (|CallParentFunction)
  ;;[1 0.8995 0] todo-Rework?
  (CallFunction|StartingBlackBoardValuesF)
  (CallFunction|PerceptionStatusIconUpdateF "NewEnumerator0"))

(event Collision|EventActorBeginOverlap
  (params (OtherActor :type Actor%20Object%20Reference))
  ;[0.03049 0.4635 0] Tick
  (|CallParentFunction OtherActor) ; This node is disabled and will not be called.\nDrag off pins to build functionality.
)

(event EventTick
  (params (DeltaSeconds :type Float%20%28single-precision%29))
  ;[0.03049 0.4635 0] Tick
  (|CallParentFunction DeltaSeconds) ; This node is disabled and will not be called.\nDrag off pins to build functionality.
)

(event EventCharacterPresetSetup-InheritableCE
  (params (CharacterPreset :type Primary%20Data%20Asset%20Object%20Reference) (SpawnTrueVsSceneFalse :type Boolean))
  ;[0 1 0.4249] Possessed
  (|CallParentFunction CharacterPreset SpawnTrueVsSceneFalse)
  (CallFunction|CharacterPresetAi-TownCampCitizenRosterAddF CharacterPreset SpawnTrueVsSceneFalse))

(event EventPossessed
  (params (NewController :type Controller%20Object%20Reference))
  ;[0.2507 1 0] BeginPlay
  ;;[1 0.8269 0.1669] todo: replace in characterBase
  (|CallParentFunction NewController)
  (CallFunction|PossessionAIControllerRefF0-replaced NewController))

(event EventChAIPerceptionStatusIconUpdateI
  (params (PerceptionStatus :type E_PerceptionStatus-IconFeedback%20Enum :default "NewEnumerator0"))
  ;[1 1 1] PerceptionStatus
  (CallFunction|PerceptionStatusIconUpdateF PerceptionStatus))

(event Input|ActionEvents|InputActionTestInputTwo
  (params (Key :type Key%20Structure))
  ;[0.1823 0.1823 0.1823] Test
  (:Pressed
    (Utilities|IsValid (Variables|Default|GetTestProxyActor)
      (:Is%20Valid
        (Transformation|SetAbsolute (Variables|Default|GetSceneComponent_RelativeRotation) false true false)
        (Transformation|AttachComponentToComponent (Variables|/Script/Engine.Actor|GetRootComponent (Variables|Default|GetTestProxyActor)) (Variables|Default|GetSceneComponent_RelativeRotation) "None" "SnapToTarget" "KeepRelative" "KeepRelative" true)
        (Transformation|SetRelativeLocation (Variables|/Script/Engine.Actor|GetRootComponent (Variables|Default|GetTestProxyActor)) "0,111.000000,111.000000" false false))
      (:Is%20Not%20Valid
        (Development|PrintString "SpawingProxyActor")
        (bind _returnvalue (Game|SpawnActorfromClass "/Game/04AiController/BT_BehaviorTrees/BP_ProxyActor_A.BP_ProxyActor_A_C" (Transformation|GetActorTransform) "Undefined" 0 0))
        (Variables|Default|SetTestProxyActor _returnvalue)))))

(event Input|ActionEvents|InputActionTestInputThree
  (params (Key :type Key%20Structure))
  (bind _testproxyactor (Variables|Default|GetTestProxyActor))
  ;[0.1823 0.1823 0.1823] Test
  (:Pressed
    (Utilities|IsValid _testproxyactor
      (:Is%20Valid
        (Transformation|DetachFromActor _testproxyactor "KeepWorld" "KeepWorld" "KeepWorld")))))

(fn ConstructionScript
  (|CallParentFunction))

(fn StartingBlackBoardValuesF
  (bind _self self)
  (bind _self_2 self)
  (bind _self_3 self)
  (bind _self_4 self)
  (bind _startingleashactor (Variables|004AiNpc|GetStartingLeashActor))
  (bind _startinggarrisonactor (Variables|004AiNpc|GetStartingGarrisonActor))
  (bind _camptownactor (Variables|004AiNpc|GetCampTownActor))
  (bind _startingpatrolrouteactor (Variables|004AiNpc|GetStartingPatrolRouteActor))
  (bind _returnvalue (AI|GetAIController _self))
  (bind _returnvalue_2 (AI|GetAIController _self_3))
  (bind _returnvalue_3 (AI|GetAIController _self_4))
  (bind _returnvalue_4 (AI|GetAIController _self_2))
  (Utilities|FlowControl|Sequence
    (:then_0
      ;[1 1 1] CampTown
      (Utilities|IsValid _camptownactor
        (:Is%20Valid
          (if (Utilities|DoesObjectImplementInterface _camptownactor "/Game/05CampTowns/BPI_CampTownActorInterface_I.BPI_CampTownActorInterface_I_C")
            (Utilities|IsValid _returnvalue_2
              (:Is%20Valid
                (bind _camptownactor_key (Class|BPIAIControllerMasterInterfaceI|AICICampTownNAlarmSystemKeyGETI(Message) _returnvalue_2))
                (AI|Components|Blackboard|SetValueasObject (Variables|/Script/AIModule.AIController|GetBlackboard _returnvalue_2) _camptownactor_key _camptownactor)))
            (else
              (Development|PrintString "BPCharacterAiHeroC>StartingBlackboardValuesF== CampTownActor does not implement CampTownInterface"))))))
    (:then_1
      ;[1 1 1] StartingLeash
      (Utilities|IsValid _startingleashactor
        (:Is%20Valid
          (Utilities|IsValid _returnvalue
            (:Is%20Valid
              (bind _leashactor_key (Class|BPIAIControllerMasterInterfaceI|AICILeashKeyGETI(Message) _returnvalue))
              (AI|Components|Blackboard|SetValueasObject (Variables|/Script/AIModule.AIController|GetBlackboard _returnvalue) _leashactor_key _startingleashactor))))))
    (:then_2
      ;[1 1 1] Garrison
      (Utilities|IsValid _startinggarrisonactor
        (:Is%20Valid
          (if (Utilities|DoesObjectImplementInterface _startinggarrisonactor "/Game/05CampTowns/CampTown/DR_GarrisonBarracks/BPI_GarrisonBarracksInterface_I.BPI_GarrisonBarracksInterface_I_C")
            (Utilities|IsValid _returnvalue_3
              (:Is%20Valid
                (bind _garrisonbarracksactor_key (Class|BPIAIControllerMasterInterfaceI|AICIGarrisonKeyGETI(Message) _returnvalue_3))
                (AI|Components|Blackboard|SetValueasObject (Variables|/Script/AIModule.AIController|GetBlackboard _returnvalue_3) _garrisonbarracksactor_key _startinggarrisonactor)))
            (else
              (Development|PrintString "BPCharacterAiHeroC>StartingBlackboardValuesF== GarrisonActor does not implement GarrisonInterface"))))))
    (:then_3
      ;[1 1 1] PatrolRoute
      (Utilities|IsValid _startingpatrolrouteactor
        (:Is%20Valid
          (if (Utilities|DoesObjectImplementInterface _startingpatrolrouteactor "/Game/05CampTowns/CampTown/DR_PartolRoute/BPI_PatrolRouteInterface_I.BPI_PatrolRouteInterface_I_C")
            (Utilities|IsValid _returnvalue_4
              (:Is%20Valid
                (bind _getpatrolrouteactorkey (Class|BPIAIControllerMasterInterfaceI|AICIPatrolRouteKeyGETI(Message) _returnvalue_4))
                (AI|Components|Blackboard|SetValueasObject (Variables|/Script/AIModule.AIController|GetBlackboard _returnvalue_4) _getpatrolrouteactorkey _startingpatrolrouteactor)
                (Development|PrintString "Hpatarllo")))
            (else
              (Development|PrintString "BPCharacterAiHeroC>StartingBlackboardValuesF== GarrisonActor does not implement GarrisonInterface"))))))))

(fn PossessionAIControllerRefF0-replaced
  (params (NewController :type Controller%20Object%20Reference))
  (if (not (Class|Controller|IsPlayerController NewController))
    (Utilities|IsValid (Variables|004AiNpc|GetAIControllerRef_0-duplicate)
      (:Is%20Not%20Valid
        (bind _asaicontroller (Utilities|Casting|CastToAIController NewController))
        (Variables|004AiNpc|SetAIControllerRef_0-duplicate _asaicontroller)))))

(fn CharacterPresetAi-TownCampCitizenRosterAddF
  (params (CharacterPreset :type Primary%20Data%20Asset%20Object%20Reference) (SpawnTrueVsSceneFalse :type Boolean))
  (bind _camptownactor (Variables|004AiNpc|GetCampTownActor))
  ;[1 1 1] If character is spawned from a townCamp then they are automatically added
  (if (not SpawnTrueVsSceneFalse)
    (Utilities|IsValid _camptownactor
      (:Is%20Valid
        (if (Utilities|DoesObjectImplementInterface _camptownactor "/Game/05CampTowns/BPI_CampTownActorInterface_I.BPI_CampTownActorInterface_I_C")
          (Class|BPICampTownActorInterfaceI|CTGICampTownCitizenRosterAddI(Message) _camptownactor self)
          (else
            (Development|PrintString "BPCharacterAIMasterC>CharacterPresetAI-TownCampAddF= townCampActor does not implement interface" true true "(R=1.000000,G=0.368120,B=0.000000,A=1.000000)" 22.0))))
      (:Is%20Not%20Valid
        (Development|PrintString "BPCharacterAIMasterC>CharacterPresetAI-TownCampAddF= townCampActor not set" true true "(R=1.000000,G=0.368120,B=0.000000,A=1.000000)" 22.0)))))

(fn PerceptionStatusIconUpdateF
  (params (PerceptionStatus :type E_PerceptionStatus-IconFeedback%20Enum :default "NewEnumerator0"))
  (bind _billboard_perceptionstatus (Variables|Default|GetBillboard_PerceptionStatus))
  (switch Utilities|FlowControl|Switch|SwitchonE_PerceptionStatus-IconFeedback PerceptionStatus
    (:NewEnumerator0
      (Development|SetHiddeninGame _billboard_perceptionstatus true false))
    (:NewEnumerator1
      (Rendering|Components|Sprite|SetSprite _billboard_perceptionstatus "/Game/10WidgetUIAssets/PerceptionIconsCustom/Icon_PerceptionIcon_Exclamation.Icon_PerceptionIcon_Exclamation")
      (Development|SetHiddeninGame _billboard_perceptionstatus false false))
    (:NewEnumerator2
      (Rendering|Components|Sprite|SetSprite _billboard_perceptionstatus "/Game/10WidgetUIAssets/PerceptionIconsCustom/Icon_PerceptionIcon_WarningOrange.Icon_PerceptionIcon_WarningOrange")
      (Development|SetHiddeninGame _billboard_perceptionstatus false false))
    (:NewEnumerator3
      (Development|PrintString "PercetionStatusIconUpdate_F> suspicious not setup yet"))))

(fn ChAIAITypeGETI
  (return (Variables|004AiNpc|GetCharacterAINpcType-DontNeed)))

(fn ChAIBehaviorTreeObjectGetI
  (return (Variables|004AiNpc|GetBehaviorTreeObject)))

(fn ChAICampTownActorStartingGETI
  (params (Location :type Name :default "None"))
  (bind _camptownactor (Variables|004AiNpc|GetCampTownActor))
  (Utilities|IsValid _camptownactor
    (:Is%20Valid
      _)
    (:Is%20Not%20Valid
      (Development|PrintString (Utilities|String|Append (Utilities|String|ToString(Name) Location) "+vCampTownActor is not valid") true true "(R=1.000000,G=0.333646,B=0.000000,A=1.000000)" 22.0)))
  (return _camptownactor))

(fn ChAICampTownActorStartingSETI
  (params (CampTownActor :type Actor%20Object%20Reference)))

(fn ChAILeashActorStartingGETI
  (bind _startingleashactor (Variables|004AiNpc|GetStartingLeashActor))
  (Utilities|IsValid _startingleashactor
    (:Is%20Valid
      _)
    (:Is%20Not%20Valid
      (Development|PrintString "BPCharacterAIMasterC>ChAiLeashActorStartingGetI== LeashActor is not valid" true true "(R=1.000000,G=0.274334,B=0.000000,A=1.000000)" 22.0)))
  (return _startingleashactor))

(fn ChAILeashActorStartingSETI
  (params (LeashActorStarting :type Actor%20Object%20Reference))
  ;[1 1 1] HomeLeash can be different actors related to daily routine. exBlacksmith station, fishing station,ect
  (bind _output_get (Variables|004AiNpc|SetStartingLeashActor LeashActorStarting))
  (return (Utilities|IsValid _output_get)))

(fn ChAIPatrolRouteActorStaringGETI
  (return (Variables|004AiNpc|GetStartingPatrolRouteActor)))

(fn ChAIPatrolRouteActorStartingSETI
  (params (PatrolRouteActor :type Actor%20Object%20Reference))
  (return false))

(fn ChAISceneComponentRelativeRotationAttatchGETI
  (return (Variables|Default|GetSceneComponent_RelativeRotation)))