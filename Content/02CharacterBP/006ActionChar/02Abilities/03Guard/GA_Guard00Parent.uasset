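; Parent Gameplay Ability for guarding, which puts the character into the Guarding active state.
; On activation it commits, records the buffered action as current, clears the buffer, interrupts the previous active state via gameplay event, and plays a one-direction guard montage.
; The montage is meant to loop, so the ability normally ends on a guard-release or interrupt event.
; A four-direction montage selector is stubbed and unused.
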(event Ability|EventActivateAbility
  (bind _returnvalue (Ability|GetOwningActorfromActorInfo))
  ;[1 1 1] Commit
  (|CallParentFunction)
  (Ability|CommitAbility)
  ;[1 1 1] CurrectAction and InputBuffer
  (bind _inputbufferget (CallFunction|ActionInputBufferGETxF))
  (CallFunction|ActionCurrentMoveAbilitySETxF _inputbufferget)
  ;;[1 1 1] Dont clear guard unless release button
  (CallFunction|ActionInputBufferClearxF)
  ;[1 1 1] StateEvent
  ;;[1 1 1 1 14] Clears/EndsAbility of  all active activeState Abilities. Should only have one active
  (Ability|SendGameplayEventtoActor _returnvalue "(TagName=\"GameplayEvent.StateEvent.PreviousActiveStateInteruptedEvent\")" (Utilities|Struct|MakeGameplayEventData "(TagName=\"\")" _returnvalue))
  ;[1 1 1] Play Montage
  (bind _guardanimmontage (CallFunction|SimpleOneDirectionAnimMontageF))
  (Utilities|IsValid _guardanimmontage
    (:Is%20Valid
      _)
    (:Is%20Not%20Valid
      (Development|PrintString "GaGuard00Parent>EG== Guard animMontage is not valid" true true "(R=1.000000,G=0.516063,B=0.000000,A=1.000000)" 22.0)))
  (|PlayMontageandWaitProxy "None" _guardanimmontage 1.0 "None" true 1.0 0.0
    (:then
      ;[1 1 1] Montage Action
      ;;[1 1 1] Set  ActiveState variable on character
      (CallFunction|ActiveStateSwitchTagSETF "(TagName=\"ActiveState.GuardingAS\")")
      (Utilities|FlowControl|Sequence
        (:then_0
          ;;[1 1 1] PreviousActiveStateInterupted
          (Ability|Tasks|WaitGameplayEvent "(TagName=\"GameplayEvent.StateEvent.PreviousActiveStateInteruptedEvent\")" 0 true
            (:EventReceived
              (Ability|EndAbility))))
        (:then_1
          ;;[1 1 1] Listen for release GuardInput
          (Ability|Tasks|WaitGameplayEvent "(TagName=\"GameplayEvent.CombatEvent.GuardReleaseEvent\")" 0 true
            (:EventReceived
              ;;[1 1 1] handle in characterACtion?
              (CallFunction|ActionInputBufferClearxF)
              (CallFunction|ActionPreviousActiveStateCompletexF)
              (Ability|EndAbility))))))
    (:OnCompleted
      (Development|PrintString "GAGuard00Parent>EG== MontageCompleted")
      ;;[0.06771 0.06771 0.06771] Guard Loops so never Ends
      ;;;[1 1 1 1 14] Attacks,Dodges,HitStun,Ect EndAbility when Montage  plays to the end
      ;;;;[1 1 1 1 14] ReturnTo  (Loco,Prone,Disabled,ec)
      (CallFunction|ActionPreviousActiveStateCompletexF)
      (Ability|EndAbility))
    (:OnInterrupted
      (Ability|EndAbility :!label _label))
    (:OnCancelled
      (goto _label))))

(event Ability|EventOnEndAbility
  (params (bWasCancelled :type Boolean))
  (|CallParentFunction bWasCancelled) ; This node is disabled and will not be called.\nDrag off pins to build functionality.
)

(fn AdvancedFourDirectionAnimMontageF
  (params (ForwardRightPos45 :type Float%20%28double-precision%29) (BackRightPos135 :type Float%20%28double-precision%29) (BackLeftNeg135 :type Float%20%28double-precision%29) (ForwardLeftNeg45 :type Float%20%28double-precision%29))
  (return 0))

(fn SimpleOneDirectionAnimMontageF
  (return (Variables|Default|GetFrontGuardAnimMontageGood)))