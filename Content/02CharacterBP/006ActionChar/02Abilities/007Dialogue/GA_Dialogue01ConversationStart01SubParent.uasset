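; Gameplay ability that starts a dialogue conversation between the owning character and the interactable character from the action input buffer.
; On activation it reads that character's conversation class, interrupts the previous active state, and, for players only, starts the conversation through the player controller.
; It sets an interact lock and the Dialogue active-state tag, then waits for completed or interrupted gameplay events to clear the lock and end.
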(event Ability|EventOnEndAbility
  (params (bWasCancelled :type Boolean))
  (|CallParentFunction bWasCancelled))

(event Ability|EventActivateAbility
  (bind _returnvalue (Ability|GetOwningActorfromActorInfo))
  (|CallParentFunction)
  ;[1 1 1] Cost& Commit & Cooldown
  (Ability|CommitAbility)
  ;[1 1 1] CurrectAction and InputBuffer
  (bind _inputbufferget (CallFunction|ActionInputBufferGETxF))
  (CallFunction|InteractActorDialogueHoldersDialogueNarrativeClassF _inputbufferget)
  (CallFunction|ActionCurrentMoveAbilitySETxF _inputbufferget)
  (CallFunction|ActionInputBufferClearxF)
  ;[1 1 1] StateEvent
  ;;[1 1 1] Clears/EndsAbility of  all active activeState Abilities. Should only have one active
  (Ability|SendGameplayEventtoActor _returnvalue "(TagName=\"GameplayEvent.StateEvent.PreviousActiveStateInteruptedEvent\")" (Utilities|Struct|MakeGameplayEventData "(TagName=\"\")" _returnvalue))
  ;[1 1 1] Dialogue specific
  ;;[1 1 1] Narrative
  ;;;[1 0.7298 0.2011] todolater:Setup fallback dialogueClass
  (CallFunction|StartNarrativeifPlayerF)
  ;;[1 1 1] InteractLock
  (bind _character (CallFunction|OwningCharacterRefGETF))
  (Class|BPICharacterBaseInterface|CPILockonDialogueInteractLockSETI(Message) _character (Variables|Default|GetInteractableCharacter))
  ;[1 1 1] Looping Action
  ;;[1 1 1] Set variable on character
  (CallFunction|ActiveStateSwitchTagSETF "(TagName=\"ActiveState.005DialogueAS\")")
  (Utilities|FlowControl|Sequence
    (:then_0
      ;;[1 1 1] DialogueCompleted
      (Ability|Tasks|WaitGameplayEvent "(TagName=\"GameplayEvent.StateEvent.DialogueCompleted\")" 0 true
        (:EventReceived
          (bind _character_2 (CallFunction|OwningCharacterRefGETF))
          ;;;[1 1 1] Clear
          (Class|BPICharacterBaseInterface|CPILockonDialogueInteractLockSETI(Message) _character_2)
          (CallFunction|ActionPreviousActiveStateCompletexF)
          (Ability|EndAbility))))
    (:then_1
      ;;[1 1 1] PreviousActiveStateInterupted
      (Ability|Tasks|WaitGameplayEvent "(TagName=\"GameplayEvent.StateEvent.PreviousActiveStateInteruptedEvent\")" 0 true
        (:EventReceived
          (bind _character_3 (CallFunction|OwningCharacterRefGETF))
          ;;[1 1 1] Clear
          (Class|BPICharacterBaseInterface|CPILockonDialogueInteractLockSETI(Message) _character_3)
          (Ability|EndAbility))))))

(fn InteractActorDialogueHoldersDialogueNarrativeClassF
  (params (S_InputBuffer :type S%20Input%20Buffer%20Structure%20%28by%20ref%29))
  (bind _ascharacter (Utilities|Casting|CastToCharacter (.InteractableActor (Utilities|Struct|BreakS_InputBuffer S_InputBuffer)))
    (:then
      (bind _output_get (Variables|Default|SetInteractableCharacter _ascharacter))
      (bind _dialogueconversationclass (Class|BPICharacterStoryInterfaceI|CSIDialogueClassGetI(Message) _output_get))
      (bind _output_get_2 (Variables|Default|SetNarrativeDialogueClass-old 0))
      (Variables|Default|SetDialogueConversationClass _dialogueconversationclass))
    (:CastFailed
      _))
  (return))

(fn StartNarrativeifPlayerF
  (bind _character (CallFunction|OwningCharacterRefGETF))
  (if (Pawn|IsPlayerControlled _character)
    ;[1 1 1] Player
    (bind _playercontrollerref (Class|BPICharacterBaseInterface|CBIControllerRefGETI(Message) _character))
    (if (Utilities|IsValidClass (Variables|Default|GetDialogueConversationClass))
      _
      (else
        (Development|PrintString "PlayerStartNarrative== DialogueClass is null" true true "(R=1.000000,G=0.352237,B=0.000000,A=1.000000)" 22.0)
        ;;[1 0.9604 0.4453] Todolater:Fallback dialogue
        (Variables|Default|SetDialogueConversationClass 0)))
    (Class|BPIPlayerControllerStoryInterfaceI|PcSIDialogueConverationStartI(Message) _playercontrollerref _character (Variables|Default|GetInteractableCharacter) (Variables|Default|GetDialogueConversationClass))
    (return)
    (else
      ;[1 1 1] Npc
      (return))))