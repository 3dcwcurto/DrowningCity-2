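; Parent Gameplay Ability for dialogue emotes, playing a montage while the character is in the Dialogue active state.
; On activation it consumes the buffered action, interrupts the previous active-state ability and interact-locks onto the buffered character.
; Montage completion or blend-out sends EmoteCompleted without ending the ability.
; It listens for DialogueCompleted or a later interruption event to complete the action, clear the lock and end.
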(event Ability|EventActivateAbility
  (bind _returnvalue (Ability|GetOwningActorfromActorInfo))
  (bind _montage_to_play (Variables|Default|GetMontage%20to%20Play))
  ;[0.6515 0.1635 1] Emote/FD: Uses dialougeListeFD& dialogueFireFD
  (|CallParentFunction)
  ;[1 1 1] Cost& Commit & Cooldown
  (Ability|CommitAbility)
  ;[1 1 1] CurrectAction and InputBuffer
  (bind _inputbufferget (CallFunction|ActionInputBufferGETxF))
  (CallFunction|InteractActorDialogueHoldersF _inputbufferget)
  (CallFunction|ActionCurrentMoveAbilitySETxF _inputbufferget)
  (CallFunction|ActionInputBufferClearxF)
  ;[1 1 1] StateEvent
  ;;[1 1 1] Clears/EndsAbility of  all active activeState Abilities. Should only have one active
  (Ability|SendGameplayEventtoActor _returnvalue "(TagName=\"GameplayEvent.StateEvent.PreviousActiveStateInteruptedEvent\")" (Utilities|Struct|MakeGameplayEventData "(TagName=\"\")" _returnvalue))
  ;[1 1 1] Dialogue Specific
  ;;[1 1 1] InteractLock
  (bind _character (CallFunction|OwningCharacterRefGETF))
  (Class|BPICharacterBaseInterface|CPILockonDialogueInteractLockSETI(Message) _character (Variables|Default|GetInteractableCharacter))
  ;[1 1 1] MontageLooping
  (Utilities|IsValid _montage_to_play
    (:Is%20Valid
      _)
    (:Is%20Not%20Valid
      (Development|PrintString "GaDialogueEmote>Eg== EmoteMontage is not valid" true true "(R=1.000000,G=0.516063,B=0.000000,A=1.000000)" 22.0)))
  (|PlayMontageandWaitProxy "None" _montage_to_play 1.0 "None" true 1.0 0.0
    (:then
      ;[1 1 1] Looping Action
      ;;[1 1 1] Set variable on character
      (CallFunction|ActiveStateSwitchTagSETF "(TagName=\"ActiveState.005DialogueAS\")")
      (Utilities|FlowControl|Sequence
        (:then_0
          ;;[1 1 1] DialogueCompleted
          (Ability|Tasks|WaitGameplayEvent "(TagName=\"GameplayEvent.StateEvent.DialogueCompleted\")" 0 true
            (:EventReceived
              _)))
        (:then_1
          ;;[1 1 1] PreviousActiveStateInterupted
          (Ability|Tasks|WaitGameplayEvent "(TagName=\"GameplayEvent.StateEvent.PreviousActiveStateInteruptedEvent\")" 0 true
            (:EventReceived
              _))))
      (CallFunction|ActionPreviousActiveStateCompletexF)
      ;;;[1 1 1] Clear
      (bind _character_2 (CallFunction|OwningCharacterRefGETF))
      (Class|BPICharacterBaseInterface|CPILockonDialogueInteractLockSETI(Message) _character_2)
      (Ability|EndAbility))
    (:OnCompleted
      (bind _character_3 (CallFunction|OwningCharacterRefGETF :!label _label))
      (Ability|SendGameplayEventtoActor _character_3 "(TagName=\"GameplayEvent.StateEvent.EmoteCompleted\")" (Utilities|Struct|MakeGameplayEventData "(TagName=\"\")" _character_3)))
    (:OnBlendOut
      (goto _label))))

(event Ability|EventOnEndAbility
  (params (bWasCancelled :type Boolean))
  (|CallParentFunction bWasCancelled) ; This node is disabled and will not be called.\nDrag off pins to build functionality.
)

(fn InteractActorDialogueHoldersF
  (params (S_InputBuffer :type S%20Input%20Buffer%20Structure%20%28by%20ref%29))
  (bind _ascharacter (Utilities|Casting|CastToCharacter (.InteractableActor (Utilities|Struct|BreakS_InputBuffer S_InputBuffer))))
  (Variables|Default|SetInteractableCharacter _ascharacter))