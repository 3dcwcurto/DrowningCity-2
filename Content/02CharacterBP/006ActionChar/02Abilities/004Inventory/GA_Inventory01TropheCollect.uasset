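; Gameplay ability in which the owning character loots a trophy item from an interactable victim character.
; On activation it commits, consumes the buffered action input and sends an event that interrupts the previous active-state ability.
; It transfers the victim's item to the owner, notifies player controller 0's objective system, then plays the collect montage.
; The montage sets the Loot active state; the ability ends on montage completion, interruption, cancellation or a newer state's interrupt event.
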(event Ability|EventActivateAbility
  (bind _returnvalue (Ability|GetOwningActorfromActorInfo))
  (bind _collecttrophemontage (Variables|Default|GetCollectTropheMontage))
  (|CallParentFunction)
  ;[1 1 1] Cost& Commit & Cooldown
  (Ability|CommitAbility)
  ;[1 1 1] CurrectAction and InputBuffer
  (bind _inputbufferget (CallFunction|ActionInputBufferGETxF))
  (CallFunction|InteractActorF _inputbufferget)
  (CallFunction|ActionCurrentMoveAbilitySETxF _inputbufferget)
  (CallFunction|ActionInputBufferClearxF)
  ;[1 1 1] StateEvent
  ;;[1 1 1] Clears/EndsAbility of  all active activeState Abilities. Should only have one active
  (Ability|SendGameplayEventtoActor _returnvalue "(TagName=\"GameplayEvent.StateEvent.PreviousActiveStateInteruptedEvent\")" (Utilities|Struct|MakeGameplayEventData "(TagName=\"\")" _returnvalue))
  ;[1 1 1] CollectingTrophe Specific
  (Utilities|FlowControl|Sequence
    (:then_0
      (bind _tropheitemremovelose (Class|BPICharacterInventoryInterfaceI|CSIInventoryTropheCollectVictimRemoveItemI(Message) (Variables|Default|GetInteractableCharacter)))
      (Utilities|IsValid _tropheitemremovelose
        (:Is%20Valid
          (bind _character (CallFunction|OwningCharacterRefGETF))
          (Class|BPICharacterInventoryInterfaceI|CSIInventoryTropheCollectAttackerRecieveItemI(Message) _character _tropheitemremovelose)
          (bind _itemnameid (Class|BPIItemPresetInterfaceI|IPIItemInfoGETI(Message) _tropheitemremovelose))
          (Class|BPIPlayerControllerStoryInterfaceI|PcSIObjectiveItemCollectDispatchI(Message) (Game|GetPlayerController 0) "NewEnumerator2" _itemnameid))
        (:Is%20Not%20Valid
          _))
      (CallFunction|GaitCapSetF)
      ;[1 1 1] Play Montage
      (Utilities|IsValid _collecttrophemontage
        (:Is%20Valid
          _)
        (:Is%20Not%20Valid
          (Development|PrintString "GaInventoryCollectTrophe>Eg== attackMontage is not valid" true true "(R=1.000000,G=0.516063,B=0.000000,A=1.000000)" 22.0)))
      (|PlayMontageandWaitProxy "None" _collecttrophemontage 1.0 "None" true 1.0 0.0
        (:then
          ;[1 1 1] Montage Action
          ;;[1 1 1] Set variable on character
          (CallFunction|ActiveStateSwitchTagSETF "(TagName=\"ActiveState.003LootAS\")")
          ;;[1 1 1] PreviousActiveStateInterupted
          (Ability|Tasks|WaitGameplayEvent "(TagName=\"GameplayEvent.StateEvent.PreviousActiveStateInteruptedEvent\")" 0 true
            (:EventReceived
              (Ability|EndAbility))))
        (:OnCompleted
          ;;[1 1 1] Attacks,Dodges,HitStun,Ect EndAbility when Montage  plays to the end
          ;;;[1 1 1] ReturnTo  (Loco,Prone,Disabled,ec)
          (CallFunction|ActionPreviousActiveStateCompletexF :!label _label)
          (Ability|EndAbility))
        (:OnInterrupted
          (goto _label))
        (:OnCancelled
          (Ability|EndAbility))))
    (:then_1)))

(event Ability|EventOnEndAbility
  (params (bWasCancelled :type Boolean))
  (|CallParentFunction bWasCancelled) ; This node is disabled and will not be called.\nDrag off pins to build functionality.
)