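; Parent gameplay ability for the character's locomotion active state.
; On activation it commits, broadcasts an interrupt event to end the previous active-state ability, then resets foot-forward, frame-data tags, camera perspective and rotation mode.
; It then sets the gait cap, tags the character as in locomotion, and waits for the same interrupt event to end itself.
; Input-buffer clearing and a duplicate-interrupt debug check are present but disconnected.
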(event Ability|EventActivateAbility
  (bind _returnvalue (Ability|GetOwningActorfromActorInfo))
  ;[1 1 1] Activate Cooldown. Spend Costs
  (Ability|CommitAbility)
  ;[1 1 1] StateEvent
  ;;[1 1 1] Clears/EndsAbility of  all active activeState Abilities. Should only have one active
  (Ability|SendGameplayEventtoActor 0 "(TagName=\"GameplayEvent.StateEvent.PreviousActiveStateInteruptedEvent\")" (Utilities|Struct|MakeGameplayEventData "(TagName=\"\")" _returnvalue _returnvalue))
  ;[1 1 1] Locomotion Specific
  ;;[1 1 1] Return to LeftFootForward?
  (bind _character (CallFunction|OwningCharacterRefGETF))
  (Class|BPICharacterLocomotionInterfaceI|CLIGaFootInfrontSETI(Message) _character "NewEnumerator1")
  (Class|BPICharacterActionInterfaceI|CAIActiveStateFrameDataResetTagsI(Message) _character)
  (Class|BPICharacterBaseInterface|CPICameraPerspecitveResettoDefaultI(Message) _character)
  (Class|BPICharacterLocomotionInterfaceI|CLIRotationModeResettoDefaultI0(Message) _character)
  ;;[1 1 1] GaitCap
  (CallFunction|GaitCapSetF)
  ;[1 1 1] Looping Action
  ;;[1 1 1] Set variable on character
  (CallFunction|ActiveStateSwitchTagSETF "(TagName=\"ActiveState.LocomotionAS\")")
  (Utilities|FlowControl|Sequence
    (:then_0)
    (:then_1
      ;;[1 1 1] PreviousActiveStateInterupted
      (Ability|Tasks|WaitGameplayEvent "(TagName=\"GameplayEvent.StateEvent.PreviousActiveStateInteruptedEvent\")" 0 true
        (:EventReceived
          (Ability|EndAbility))))))

(event Ability|EventOnEndAbility
  (params (bWasCancelled :type Boolean)))