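; Parent attack ability (GAS) that supplies shared charge and projectile helpers for child attack abilities.
; Charge helpers step a clamped level on a looping timer until max and store it in the current action's input-buffer struct.
; Projectiles spawn from the weapon hand's offset with that level, aimed by camera sphere trace (third person) or cursor actor (isometric).
; First-person and RTS aiming are unimplemented, and the montage activation flow is disconnected, leaving activation to its parent.
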(event Ability|EventActivateAbility
  (|CallParentFunction))

(event Ability|EventOnEndAbility
  (params (bWasCancelled :type Boolean))
  (|CallParentFunction bWasCancelled))

(fn ActionCurrentMoveAbilityChargeLevelUpdateF
  (bind _output_get (Variables|Default|SetChargeLevelAmountCurrent_PrivateVar (Math|Integer|Clamp(Integer) (+ (Variables|Default|GetChargeLevelAmountCurrent_PrivateVar) 1) 0 (Variables|Default|GetChargeLevelMaximum_Default3))))
  (if (== (Variables|Default|GetChargeLevelAmountCurrent_PrivateVar) (Variables|Default|GetChargeLevelMaximum_Default3))
    ;[1 1 1] Stop VFX from firing
    (Utilities|Time|ClearandInvalidateTimerbyHandle (Variables|Default|GetChargeTimerHandle_PrivateVar)))
  (bind _actioncurrentmoveability (CallFunction|ActionCurrentMoveAbilityGETxF))
  (bind _structout (Utilities|Struct|SetmembersinS_InputBuffer _actioncurrentmoveability (Variables|Default|GetChargeLevelAmountCurrent_PrivateVar)))
  (CallFunction|ActionCurrentMoveAbilitySETxF _structout))

(fn ChargeLevelReachedEffectsEventVFXSFXF-todo)

(fn ChargeLevelCountingF-oldcombinedinto
  (bind _output_get (Variables|Default|SetChargeLevelAmountCurrent_PrivateVar (Math|Integer|Clamp(Integer) (+ (Variables|Default|GetChargeLevelAmountCurrent_PrivateVar) 1) 0 (Variables|Default|GetChargeLevelMaximum_Default3))))
  (if (== (Variables|Default|GetChargeLevelAmountCurrent_PrivateVar) (Variables|Default|GetChargeLevelMaximum_Default3))
    ;[1 1 1] Stop VFX from firing
    (Utilities|Time|ClearandInvalidateTimerbyHandle (Variables|Default|GetChargeTimerHandle_PrivateVar)))
  (return))

(fn ProjectileSpawnMainF
  (bind _chargelevelamountcurrent_privatevar (Variables|Default|GetChargeLevelAmountCurrent_PrivateVar))
  (if (Utilities|IsValidClass (Variables|Default|GetArrowProjectileSlashProjectile))
    (bind _character (CallFunction|OwningCharacterRefGETF))
    (bind _cameraperspectivemode (Class|BPIPlayerControllerBaseInterfaceI|PcBICameraPerspectiveModeGETI(Message) (Pawn|GetController _character)))
    (switch Utilities|FlowControl|Switch|SwitchonE_CameraPerspectiveMode-Fps3rdIso _cameraperspectivemode
      (:NewEnumerator0
        (Development|PrintString "GAAttackCharge2ReleaseParent>AttackSpawnProjectileOverrideableF== CameraPerspective is null"))
      (:NewEnumerator1
        (Development|PrintString "GAAttackCharge2ReleaseParent>AttackSpawnProjectileOverrideableF== spawn projectile direction CameraPerspective NotSetupYet" true true "(R=1.000000,G=0.272798,B=0.000000,A=1.000000)" 22.0 :!label _label))
      (:NewEnumerator2
        ;[1 1 1] ThirdPerson
        (CallFunction|ProjectileThirdPersonProjectileF _character _chargelevelamountcurrent_privatevar))
      (:NewEnumerator3
        ;[1 1 1] Isometric
        (CallFunction|ProjectileIsometricProjectileF _character _chargelevelamountcurrent_privatevar))
      (:NewEnumerator5
        (goto _label)))
    (else
      (return))))

(fn ProjectileThirdPersonProjectileF
  (params (Character :type Character%20Object%20Reference) (ChargeLevel :type Integer))
  (LocalVariables|SetChargeLevel_Local ChargeLevel)
  (bind (_springarm _camera) (Class|BPICharacterBaseInterface|CBIComponentCharacterParentGETI(Message) Character))
  (bind _weaponsetcontainerloadout (Class|BPICharacterInventoryInterfaceI|CIIWeaponSet-HoldingCurrentGETI(Message) Character))
  (if (Utilities|IsValidClass (.WeaponSetAnimationSetObjectClass (Utilities|Struct|BreakS_WeaponSetWeaponPair _weaponsetcontainerloadout)))
    (switch Utilities|FlowControl|Switch|SwitchonE_Generic-LeftVsRight (.ProjectileSpawnOffsetDefault-LeftVsRight (Utilities|GetClassDefaults (.WeaponSetAnimationSetObjectClass (Utilities|Struct|BreakS_WeaponSetWeaponPair _weaponsetcontainerloadout))))
      (:NewEnumerator0
        (LocalVariables|SetNewLocalVar_0 "0, 0, 0" :!label _label))
      (:NewEnumerator1
        (bind _asbp_item_01weapon_item_00parent_a (Utilities|Casting|CastToBP_Item01WeaponItem00Parent_A (.InventoryItemActor-RuntimeLoadout (Utilities|Struct|BreakS_InventoryItem (.WeaponLeftHand (Utilities|Struct|BreakS_WeaponSetWeaponPair _weaponsetcontainerloadout)))))
          (:then
            (LocalVariables|SetNewLocalVar_0 (Transformation|GetWorldLocation (Variables|/Game/02CharacterBP/004InvChar/Items/01Weapons/BP_Item01WeaponItem00Parent_A.BP_Item01WeaponItem00Parent_A_C|GetScene_ProjectileSpawnOffsetLocation _asbp_item_01weapon_item_00parent_a))))
          (:CastFailed
            (goto _label))))
      (:NewEnumerator2
        (bind _asbp_item_01weapon_item_00parent_a_2 (Utilities|Casting|CastToBP_Item01WeaponItem00Parent_A (.InventoryItemActor-RuntimeLoadout (Utilities|Struct|BreakS_InventoryItem (.WeaponRightHand (Utilities|Struct|BreakS_WeaponSetWeaponPair _weaponsetcontainerloadout)))))
          (:then
            (LocalVariables|SetNewLocalVar_0 (Transformation|GetWorldLocation (Variables|/Game/02CharacterBP/004InvChar/Items/01Weapons/BP_Item01WeaponItem00Parent_A.BP_Item01WeaponItem00Parent_A_C|GetScene_ProjectileSpawnOffsetLocation _asbp_item_01weapon_item_00parent_a_2))))
          (:CastFailed
            (goto _label)))))
    ;[1 1 1] Todolater-projectilePentrating trace channel
    (bind (_outhit _returnvalue) (Collision|SphereTraceByChannel (+ (Transformation|GetWorldLocation _camera) (* (Math|Vector|GetForwardVector _camera) (+ (Math|Vector|VectorLength (- (Transformation|GetWorldLocation _springarm) (Transformation|GetWorldLocation _camera))) 65.0))) (+ (Transformation|GetWorldLocation _camera) (* (Math|Random|RandomUnitVectorinConeinDegrees (Math|Vector|GetForwardVector _camera) 0.0) 5e+03)) 5.0 "TraceTypeQuery1" false (Utilities|Array|MakeArray 0) "ForDuration" true "(R=1.000000,G=0.000000,B=0.000000,A=1.000000)" "(R=0.000000,G=1.000000,B=0.000000,A=1.000000)" 2.0))
    (if _returnvalue
      (Game|SpawnActorfromClass (Variables|Default|GetArrowProjectileSlashProjectile) (Math|Transform|MakeTransform (LocalVariables|GetNewLocalVar_0) (Math|Rotator|FindLookatRotation (LocalVariables|GetNewLocalVar_0) (.ImpactPoint (Collision|BreakHitResult _outhit)))) "Undefined" 0 (LocalVariables|GetChargeLevel_Local) 0)
      (return)
      (else
        ;[1 1 1] Target is based on camera? nothing to hit within ProjecticleSpeed/Max which is the range set between 2k-5k
        (Game|SpawnActorfromClass (Variables|Default|GetArrowProjectileSlashProjectile) (Math|Transform|MakeTransform (LocalVariables|GetNewLocalVar_0) (Math|Rotator|FindLookatRotation (LocalVariables|GetNewLocalVar_0) (+ (Transformation|GetWorldLocation _camera) (* (Math|Random|RandomUnitVectorinConeinDegrees (Math|Vector|GetForwardVector _camera) 0.0) 5e+03)))) "Undefined" 0 (LocalVariables|GetChargeLevel_Local) 0)
        (return)))))

(fn ProjectileIsometricProjectileF
  (params (Character :type Character%20Object%20Reference) (ChargeLevel :type Integer))
  (bind _mesh (Variables|/Script/Engine.Character|GetMesh Character))
  (bind _returnvalue (Transformation|GetWorldLocation _mesh))
  (LocalVariables|SetChargeLevel_Local ChargeLevel)
  (bind _projectilespawnoffsetlocation (CallFunction|ProjectileSpawnOffsetLocatioNF Character))
  (bind _rtsisomousecursoractor (Class|BPIPlayerControllerBaseInterfaceI|PcBIRtsIsoMouseCursorActorGETI(Message) (Pawn|GetController Character)))
  (Utilities|IsValid _rtsisomousecursoractor
    (:Is%20Valid
      (Game|SpawnActorfromClass (Variables|Default|GetArrowProjectileSlashProjectile) (Math|Transform|MakeTransform _projectilespawnoffsetlocation (Math|Rotator|FindLookatRotation (Math|Vector|MakeVector (.x _returnvalue) (.y _returnvalue) (.Z (Math|Vector|BreakVector _projectilespawnoffsetlocation))) (Math|Vector|MakeVector (.x (Transformation|GetActorLocation _rtsisomousecursoractor)) (.y (Transformation|GetActorLocation _rtsisomousecursoractor)) (.Z (Math|Vector|BreakVector _projectilespawnoffsetlocation)))) "1.000000,1.000000,1.000000") "Undefined" 0 (LocalVariables|GetChargeLevel_Local) 0)
      (return))
    (:Is%20Not%20Valid
      (return))))

(fn ChargeLevelInputBufferF
  (params (InputBUffer :type S%20Input%20Buffer%20Structure))
  (bind _output_get (Variables|Default|SetChargeLevelAmountCurrent_PrivateVar (.ChargeLevelAmountCurrent-Tick (Utilities|Struct|BreakS_InputBuffer InputBUffer)))))

(fn ChargeTimerbyEventF
  (params (Delegate :type Delegate))
  (bind _returnvalue (Utilities|Time|SetTimerbyEvent Delegate (Variables|Default|GetChargeLevelTimeLengthTick_Default1) true))
  (Variables|Default|SetChargeTimerHandle_PrivateVar _returnvalue))

(fn ProjectileSpawnOffsetLocatioNF
  (params (Character :type Character%20Object%20Reference))
  (bind _weaponsetcontainerloadout (Class|BPICharacterInventoryInterfaceI|CIIWeaponSet-HoldingCurrentGETI(Message) Character))
  (if (Utilities|IsValidClass (.WeaponSetAnimationSetObjectClass (Utilities|Struct|BreakS_WeaponSetWeaponPair _weaponsetcontainerloadout)))
    (switch Utilities|FlowControl|Switch|SwitchonE_Generic-LeftVsRight (.ProjectileSpawnOffsetDefault-LeftVsRight (Utilities|GetClassDefaults (.WeaponSetAnimationSetObjectClass (Utilities|Struct|BreakS_WeaponSetWeaponPair _weaponsetcontainerloadout))))
      (:NewEnumerator0
        (Development|PrintString "GAAttack00Parent>ProjectileSpawnOffsetLocation== LeftVsRight is null" true true "(R=1.000000,G=0.192062,B=0.000000,A=1.000000)" 22.0))
      (:NewEnumerator1
        (bind _asbp_item_01weapon_item_00parent_a (Utilities|Casting|CastToBP_Item01WeaponItem00Parent_A (.InventoryItemActor-RuntimeLoadout (Utilities|Struct|BreakS_InventoryItem (.WeaponLeftHand (Utilities|Struct|BreakS_WeaponSetWeaponPair _weaponsetcontainerloadout)))))
          (:then
            (return (Transformation|GetWorldLocation (Variables|/Game/02CharacterBP/004InvChar/Items/01Weapons/BP_Item01WeaponItem00Parent_A.BP_Item01WeaponItem00Parent_A_C|GetScene_ProjectileSpawnOffsetLocation _asbp_item_01weapon_item_00parent_a))))
          (:CastFailed
            (Development|PrintString "GAAttack00Parent>ProjectileSpawnOffsetLocation==WeaponL  cast failed" true true "(R=1.000000,G=0.192062,B=0.000000,A=1.000000)" 22.0)
            (return "0, 0, 0"))))
      (:NewEnumerator2
        _))
    (bind _asbp_item_01weapon_item_00parent_a_2 (Utilities|Casting|CastToBP_Item01WeaponItem00Parent_A (.InventoryItemActor-RuntimeLoadout (Utilities|Struct|BreakS_InventoryItem (.WeaponRightHand (Utilities|Struct|BreakS_WeaponSetWeaponPair _weaponsetcontainerloadout)))))
      (:then
        (return (Transformation|GetWorldLocation (Variables|/Game/02CharacterBP/004InvChar/Items/01Weapons/BP_Item01WeaponItem00Parent_A.BP_Item01WeaponItem00Parent_A_C|GetScene_ProjectileSpawnOffsetLocation _asbp_item_01weapon_item_00parent_a_2))))
      (:CastFailed
        (Development|PrintString "GAAttack00Parent>ProjectileSpawnOffsetLocation==WeaponR  cast failed" true true "(R=1.000000,G=0.192062,B=0.000000,A=1.000000)" 22.0)
        (return "0, 0, 0")))))

(event Custom|ChargeingWeaponUpdate_CE
  ;[1 1 1] Charging Timer
  (CallFunction|ChargeLevelCountingF-oldcombinedinto)
  (CallFunction|ActionCurrentMoveAbilityChargeLevelUpdateF)
  (CallFunction|ChargeLevelReachedEffectsEventVFXSFXF-todo))