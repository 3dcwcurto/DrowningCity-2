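; Parent Gameplay Ability, apparently a replaced version, for the release stage of a charged projectile attack.
; On activation it commits, takes charge level from the input buffer, interrupts the previous active state, then plays the attack montage.
; Before the montage, projectile firing branches by camera perspective to third-person or isometric helpers.
; Both helpers' aim-and-spawn logic (camera sphere trace, cursor actor) is disconnected, so no projectile spawns.
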(event Ability|EventActivateAbility
  (bind _returnvalue (Ability|GetOwningActorfromActorInfo))
  (bind _attackmontage (Variables|Default|GetAttackMontage))
  ;[1 1 1] Check Cost . Cooldown. Spend Cost?
  (Ability|CommitAbility)
  ;[1 1 1] CurrectAction and InputBuffer
  (bind _inputbufferget (CallFunction|ActionInputBufferGETxF))
  (Variables|Default|SetInputBuffer_ChargeLevelAmountCurrent-%20Tick (.DesiredIndex_StartBuffer (Utilities|Struct|BreakS_InputBuffer _inputbufferget)))
  (CallFunction|ActionCurrentMoveAbilitySETxF _inputbufferget)
  (CallFunction|ActionInputBufferClearxF)
  ;[1 1 1] StateEvent
  ;;[1 1 1] Clears/EndsAbility of  all active activeState Abilities. Should only have one active
  (Ability|SendGameplayEventtoActor _returnvalue "(TagName=\"GameplayEvent.StateEvent.PreviousActiveStateInteruptedEvent\")" (Utilities|Struct|MakeGameplayEventData "(TagName=\"\")" _returnvalue))
  ;[1 1 1] Release Effects
  ;;[1 1 1] Todo:. Set this function up to get info from abilities supportGems,perks,ect
  (AttackProjectileIfValid|AttackSpawnProjectileMainF)
  ;[1 1 1] Play Montage
  (Utilities|IsValid _attackmontage
    (:Is%20Valid
      _)
    (:Is%20Not%20Valid
      (Development|PrintString "GaAttackParent>Eg== attackMontage is not valid" true true "(R=1.000000,G=0.516063,B=0.000000,A=1.000000)" 22.0)))
  (|PlayMontageandWaitProxy "None" _attackmontage 1.0 "None" true 1.0 0.0
    (:then
      ;[1 1 1] Montage Action
      ;;[1 1 1] Set variable on character
      (CallFunction|ActiveStateSwitchTagSETF "(TagName=\"ActiveState.AttackAS.NormalAS\")")
      ;;[1 1 1] PreviousActiveStateInterupted
      (Ability|Tasks|WaitGameplayEvent "(TagName=\"GameplayEvent.StateEvent.1A\")" 0 true
        (:EventReceived
          (Ability|EndAbility))))
    (:OnCompleted
      ;;[1 1 1] Attacks,Dodges,HitStun,Ect EndAbility when Montage  plays to the end
      ;;;[1 1 1] ReturnTo  (Loco,Prone,Disabled,ec)
      (CallFunction|ActionPreviousActiveStateCompletexF)
      (Ability|EndAbility))
    (:OnInterrupted
      (Ability|EndAbility :!label _label))
    (:OnCancelled
      (goto _label))))

(event Ability|EventOnEndAbility
  (params (bWasCancelled :type Boolean)))

(fn AttackSpawnProjectileMainF
  (if (Utilities|IsValidClass (Variables|Default|GetArrowProjectile))
    (bind _character (CallFunction|OwningCharacterRefGETF))
    (bind _cameraperspectivemode (Class|BPIPlayerControllerBaseInterfaceI|PcBICameraPerspectiveModeGETI(Message) (Pawn|GetController _character)))
    (switch Utilities|FlowControl|Switch|SwitchonE_CameraPerspectiveMode-Fps3rdIso _cameraperspectivemode
      (:NewEnumerator0
        (Development|PrintString "GAAttackCharge2ReleaseParent>AttackSpawnProjectileOverrideableF== CameraPerspective is null"))
      (:NewEnumerator1
        (Development|PrintString "GAAttackCharge2ReleaseParent>AttackSpawnProjectileOverrideableF== spawn projectile direction CameraPerspective NotSetupYet" true true "(R=1.000000,G=0.272798,B=0.000000,A=1.000000)" 22.0 :!label _label))
      (:NewEnumerator2
        ;[1 1 1] ThirdPerson
        (AttackProjectileifValid|ThirdPersonProjectileF _character))
      (:NewEnumerator3
        ;[1 1 1] Isometric
        (AttackProjectileifValid|IsometricProjectileF _character))
      (:NewEnumerator5
        (goto _label)))
    (else
      (return))))

(fn ThirdPersonProjectileF
  (params (Character :type Character%20Object%20Reference))
  (bind (_springarm _camera) (Class|BPICharacterBaseInterface|CBIComponentCharacterParentGETI(Message) Character)))

(fn IsometricProjectileF
  (params (Character :type Character%20Object%20Reference))
  (Class|BPICharacterBaseInterface|CBIComponentCharacterParentGETI(Message) Character))