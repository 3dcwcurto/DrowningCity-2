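; Parent gameplay ability for a character's quick auto attack, stored as an old, replaced version.
; On activation it commits, makes the buffered input the current move, clears the buffer and sends the owner an event to interrupt the previous active state.
; It then plays the attack montage, sets the AttackNormal state and listens for an interrupt event to end itself.
; Montage completion reports the state complete before ending, while interruption or cancellation just ends it.
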(event Ability|EventActivateAbility
  (bind _returnvalue (Ability|GetOwningActorfromActorInfo))
  (bind _attackmontage (Variables|Default|GetAttackMontage))
  ;[1 1 1] CHeck Cooldown. Spend Cost?
  (Ability|CommitAbility)
  ;[1 1 1] CurrectAction and InputBuffer
  (bind _inputbufferget (CallFunction|ActionInputBufferGETxF))
  (CallFunction|ActionCurrentMoveAbilitySETxF _inputbufferget)
  (CallFunction|ActionInputBufferClearxF)
  ;[1 1 1] StateEvent
  ;;[1 1 1] Clears/EndsAbility of  all active activeState Abilities. Should only have one active
  (Ability|SendGameplayEventtoActor _returnvalue "(TagName=\"GameplayEvent.StateEvent.PreviousActiveStateInteruptedEvent\")" (Utilities|Struct|MakeGameplayEventData "(TagName=\"\")" _returnvalue))
  ;[1 1 1] Play Montage
  (Utilities|IsValid _attackmontage
    (:Is%20Valid
      _)
    (:Is%20Not%20Valid
      (Development|PrintString "GaAttackParent>Eg== attackMontage is not valid" true true "(R=1.000000,G=0.516063,B=0.000000,A=1.000000)" 22.0)))
  (|PlayMontageandWaitProxy "None" _attackmontage 1.0 "None" true 1.0 0.0
    (:then
      ;[1 1 1] Montage Action
      ;;[1 1 1] Set variable on character
      (CallFunction|ActiveStateSwitchTagSETF "(TagName=\"ActiveState.AttackNormal\")")
      ;;[1 1 1] PreviousActiveStateInterupted
      (Ability|Tasks|WaitGameplayEvent "(TagName=\"StateEvent.PreviousActiveStateInterupted\")" 0 true
        (:EventReceived
          (Ability|EndAbility))))
    (:OnCompleted
      ;;[1 1 1] Attacks,Dodges,HitStun,Ect EndAbility when Montage  plays to the end
      ;;;[1 1 1] ReturnTo  (Loco,Prone,Disabled,ec)
      (CallFunction|ActionPreviousActiveStateCompletexF)
      (Ability|EndAbility))
    (:OnInterrupted
      (Ability|EndAbility :!label _label))
    (:OnCancelled
      (goto _label))))

(event Ability|EventOnEndAbility
  (params (bWasCancelled :type Boolean)))