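; Gameplay ability sub-parent for instant weapon draw/sheath changes on an action character.
; On activation it consumes the buffered action input and sends a gameplay event interrupting the previous active-state ability.
; The desired index resolves a draw/sheath state: in-progress swap, sheath or equip states run the interrupt function, then hand back to the previous active state.
; Being instant, it ends immediately, leaving its state-switch and interrupt-wait logic disconnected.
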(event Ability|EventActivateAbility
  (bind _returnvalue (Ability|GetOwningActorfromActorInfo))
  (|CallParentFunction)
  ;[1 1 1] CurrectAction and InputBuffer
  (bind _inputbufferget (CallFunction|ActionInputBufferGETxF))
  (Variables|Default|SetDesiredIndexStartBuffer_Private (.DesiredIndex_StartBuffer (Utilities|Struct|BreakS_InputBuffer _inputbufferget)))
  (CallFunction|ActionCurrentMoveAbilitySETxF _inputbufferget)
  (CallFunction|ActionInputBufferClearxF)
  ;[1 1 1] StateEvent
  ;;[1 1 1] Clears/EndsAbility of  all active activeState Abilities. Should only have one active
  (Ability|SendGameplayEventtoActor _returnvalue "(TagName=\"GameplayEvent.StateEvent.PreviousActiveStateInteruptedEvent\")" (Utilities|Struct|MakeGameplayEventData "(TagName=\"\")" _returnvalue))
  (bind (_newvalid _drawsheathstate _newholdingcurrent _drawsheath) (CallFunction|DrawSheathSwapPrevNewResultF (Variables|Default|GetDesiredIndexStartBuffer_Private)))
  (if _newvalid
    (switch Utilities|FlowControl|Switch|SwitchonE_DrawSheathState _drawsheath
      (:NewEnumerator0
        (Development|PrintString "GADrawEquipSheathPutup02InstantSwitchParent>EG== Holding or Sheathed" true true "(R=1.000000,G=0.296756,B=0.000000,A=1.000000)" 22.0 :!label _label)
        (Ability|EndAbility))
      (:NewEnumerator1
        (goto _label))
      (:NewEnumerator2
        ;[1 1 1] Interupt SwapSheath
        (CallFunction|InteruptedF)
        ;[1 1 1] InteruptSwapEquip
        (CallFunction|InteruptedF)
        ;[1 1 1] Completed
        ;;[1 1 1] ReturnTo  (Loco,Prone,Disabled,ec)
        (CallFunction|ActionPreviousActiveStateCompletexF :!label _label_2)
        (Ability|EndAbility))
      (:NewEnumerator3
        ;[1 1 1] Interupt
        (CallFunction|InteruptedF :!label _label_3)
        (goto _label_2))
      (:NewEnumerator4
        (goto _label_3)))
    (else
      ;[1 1 1] Completed
      ;;[1 1 1] ReturnTo  (Loco,Prone,Disabled,ec)
      (CallFunction|ActionPreviousActiveStateCompletexF)
      (Ability|EndAbility))))

(event Ability|EventOnEndAbility
  (params (bWasCancelled :type Boolean))
  (|CallParentFunction false))