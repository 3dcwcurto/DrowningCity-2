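; Parent Gameplay Ability for drawing, sheathing and swapping a character's weapon sets, with index 0 as fallback fists.
; It compares held and desired sets to pick a state and montage, writing both state and held index through character interface messages.
; Draw, sheath and interrupt helpers refresh socket attachment and advance that state.
; The montage flow driven by anim-notify gameplay events is unconnected; activation only calls the parent.
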(event Ability|EventActivateAbility
  (|CallParentFunction))

(event Ability|EventOnEndAbility
  (params (bWasCancelled :type Boolean))
  (|CallParentFunction bWasCancelled))

(fn DrawSheathSwapPrevNewResultF
  (params (WeaponSetDesiredIndex :type Integer))
  (LocalVariables|SetWeaponSetDesiredIndex_Local WeaponSetDesiredIndex)
  (bind _character (CallFunction|OwningCharacterRefGETF))
  (bind (_weaponsetholding _weaponsetcontainerloadout) (Class|BPICharacterInventoryInterfaceI|CIIWeaponSet-HoldingCurrentGETI(Message) _character))
  (bind _weaponsetcontainerloadout_2 (Class|BPICharacterInventoryInterfaceI|CIIWeaponSet-DesiredNewGETI(Message) _character (LocalVariables|GetWeaponSetDesiredIndex_Local)))
  (LocalVariables|SetPrevious_WeaponSet_Local _weaponsetcontainerloadout)
  (bind _output_get (LocalVariables|SetNew_WeaponSet_Local _weaponsetcontainerloadout_2))
  (if (and (== (LocalVariables|GetWeaponSetDesiredIndex_Local) 0) (== _weaponsetholding 0))
    ;[1 1 1] Do nothing.
    (return false "" 0 "NewEnumerator0" 0)
    (else
      ;[1 1 1] New WEaponSet Valid
      (if (or (Utilities|Enum|Equal(Enum) (.WeaponSetAnimationSet (Utilities|Struct|BreakS_WeaponSetWeaponPair _output_get)) "NewEnumerator0") (Utilities|Enum|Equal(Enum) (.WeaponSetAnimationSet (Utilities|Struct|BreakS_WeaponSetWeaponPair _output_get)) "NewEnumerator10"))
        (Development|PrintString "GADrawEquipSheathPutup>DrawSheathSwapPrevNewResult== New WeaponSet not valid" true true "(R=1.000000,G=0.175463,B=0.000000,A=1.000000)")
        (return false "" 0 "NewEnumerator0" 0)
        (else
          ;[1 1 1] Previous Equal New
          (if (== _weaponsetholding (LocalVariables|GetWeaponSetDesiredIndex_Local))
            (if (or (Utilities|Enum|Equal(Enum) (.WeaponSetAnimationSet (Utilities|Struct|BreakS_WeaponSetWeaponPair (LocalVariables|GetPrevious_WeaponSet_Local))) "NewEnumerator10") (Utilities|Enum|Equal(Enum) (.WeaponSetAnimationSet (Utilities|Struct|BreakS_WeaponSetWeaponPair (LocalVariables|GetPrevious_WeaponSet_Local))) "NewEnumerator0"))
              ;[1 1 1] Draw
              (LocalVariables|SetDrawSheatStateResult_Local "NewEnumerator4")
              (LocalVariables|SetNewHoldingCurrent_local (LocalVariables|GetWeaponSetDesiredIndex_Local))
              (LocalVariables|SetAnimMontage_Local (Variables|Default|GetDrawEquipAnimMontage))
              (else
                ;[1 1 1] SheathFallback
                (LocalVariables|SetDrawSheatStateResult_Local "NewEnumerator3")
                ;;[1 1 1] Fallback is 0
                (LocalVariables|SetNewHoldingCurrent_local 0)
                (LocalVariables|SetAnimMontage_Local (Variables|Default|GetSheathPutupAnimMotnage))))
            (elif (or (Utilities|Enum|Equal(Enum) (.WeaponSetAnimationSet (Utilities|Struct|BreakS_WeaponSetWeaponPair (LocalVariables|GetPrevious_WeaponSet_Local))) "NewEnumerator0") (Utilities|Enum|Equal(Enum) (.WeaponSetAnimationSet (Utilities|Struct|BreakS_WeaponSetWeaponPair (LocalVariables|GetPrevious_WeaponSet_Local))) "NewEnumerator10"))
              ;[1 1 1] Draw
              (LocalVariables|SetDrawSheatStateResult_Local "NewEnumerator4")
              (LocalVariables|SetNewHoldingCurrent_local (LocalVariables|GetWeaponSetDesiredIndex_Local))
              (LocalVariables|SetAnimMontage_Local (Variables|Default|GetDrawEquipAnimMontage))
              (else
                ;[1 1 1] Swap
                (LocalVariables|SetDrawSheatStateResult_Local "NewEnumerator2")
                (LocalVariables|SetNewHoldingCurrent_local (LocalVariables|GetWeaponSetDesiredIndex_Local))
                ;;[1 1 1] Sheath First then draw
                (LocalVariables|SetAnimMontage_Local (Variables|Default|GetSheathPutupAnimMotnage)))))
          (bind _character_2 (CallFunction|OwningCharacterRefGETF))
          (Class|BPICharacterInventoryInterfaceI|CIIDrawSheathStateSETI(Message) _character_2 (Utilities|Struct|MakeS_DrawSheathStateInfo (LocalVariables|GetDrawSheatStateResult_Local) (LocalVariables|GetNew_WeaponSet_Local) (LocalVariables|GetPrevious_WeaponSet_Local)))
          (Class|BPICharacterInventoryInterfaceI|CIIWeaponSet-HoldingCurrentSETI(Message) _character_2 (LocalVariables|GetNewHoldingCurrent_local))
          (return true (Utilities|Struct|MakeS_DrawSheathStateInfo (LocalVariables|GetDrawSheatStateResult_Local) (LocalVariables|GetNew_WeaponSet_Local) (LocalVariables|GetPrevious_WeaponSet_Local)) (LocalVariables|GetNewHoldingCurrent_local) (LocalVariables|GetDrawSheatStateResult_Local) (LocalVariables|GetAnimMontage_Local)))))))

(fn DrawHoldnSheath-StateUpdateF
  (params (Interupt :type Boolean) (DrawSheathState :type S%20Draw%20Sheath%20State%20Info%20Structure))
  (bind (_drawsheathstate _nextweaponsetanimset _previousweaponsetanimset) (Utilities|Struct|BreakS_DrawSheathStateInfo DrawSheathState))
  (switch Utilities|FlowControl|Switch|SwitchonE_DrawSheathState (.DrawSheathState (Utilities|Struct|BreakS_DrawSheathStateInfo DrawSheathState))
    (:NewEnumerator0
      ;[1 1 1] Should never happen? Except for instantSheath?
      (LocalVariables|SetDrawSheathState_Local "NewEnumerator0"))
    (:NewEnumerator1
      (LocalVariables|SetDrawSheathState_Local "NewEnumerator1"))
    (:NewEnumerator2
      (if Interupt
        (LocalVariables|SetDrawSheathState_Local "NewEnumerator1")
        (else
          (LocalVariables|SetDrawSheathState_Local "NewEnumerator4"))))
    (:NewEnumerator3
      (LocalVariables|SetDrawSheathState_Local "NewEnumerator0"))
    (:NewEnumerator4
      (LocalVariables|SetDrawSheathState_Local "NewEnumerator1")))
  (return (Utilities|Struct|MakeS_DrawSheathStateInfo (LocalVariables|GetDrawSheathState_Local) _nextweaponsetanimset _previousweaponsetanimset)))

(fn InteruptedF
  (bind _character (CallFunction|OwningCharacterRefGETF))
  (Class|BPICharacterInventoryInterfaceI|CIIWeaponSetSocketAttatchUpdateI(Message) _character false)
  (bind _drawsheathstate (Class|BPICharacterInventoryInterfaceI|CIIDrawSheathStateGETI(Message) _character))
  (bind _drawsheathstateupdated (CallFunction|DrawHoldnSheath-StateUpdateF true _drawsheathstate))
  (Class|BPICharacterInventoryInterfaceI|CIIDrawSheathStateSETI(Message) _character _drawsheathstateupdated))

(fn DrawEquipNHoldF
  (bind _character (CallFunction|OwningCharacterRefGETF))
  (Class|BPICharacterInventoryInterfaceI|CIIWeaponSetSocketAttatchUpdateI(Message) _character false)
  (bind _drawsheathstate (Class|BPICharacterInventoryInterfaceI|CIIDrawSheathStateGETI(Message) _character))
  (bind _drawsheathstateupdated (CallFunction|DrawHoldnSheath-StateUpdateF false _drawsheathstate))
  (Class|BPICharacterInventoryInterfaceI|CIIDrawSheathStateSETI(Message) _character _drawsheathstateupdated))

(fn UnequipSheathNPutputF
  (bind _character (CallFunction|OwningCharacterRefGETF))
  (Class|BPICharacterInventoryInterfaceI|CIIWeaponSetSocketAttatchUpdateI(Message) _character false)
  (bind _drawsheathstate (Class|BPICharacterInventoryInterfaceI|CIIDrawSheathStateGETI(Message) _character))
  (bind _drawsheathstateupdated (CallFunction|DrawHoldnSheath-StateUpdateF false _drawsheathstate))
  (Class|BPICharacterInventoryInterfaceI|CIIDrawSheathStateSETI(Message) _character _drawsheathstateupdated))