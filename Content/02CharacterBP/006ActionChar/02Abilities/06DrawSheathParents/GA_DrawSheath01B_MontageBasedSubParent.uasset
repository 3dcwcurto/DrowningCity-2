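; Montage-based parent Gameplay Ability for drawing, sheathing and swapping weapons.
; On activation it consumes the action input buffer, broadcasts an interrupt to the previous active-state ability, then branches on the draw/sheath result.
; Swaps chain putup and draw montages, while single draws or sheaths play one montage.
; AnimNotify gameplay events trigger hold/putup functions (seemingly crossed in the swap branch); interruptions call InteruptedF, and completion returns to the previous state.
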(event Ability|EventActivateAbility
  (bind _returnvalue (Ability|GetOwningActorfromActorInfo))
  (|CallParentFunction)
  ;[1 1 1] CurrectAction and InputBuffer
  (bind _inputbufferget (CallFunction|ActionInputBufferGETxF))
  (Variables|Default|SetDesiredIndexStartBuffer_Private (.DesiredIndex_StartBuffer (Utilities|Struct|BreakS_InputBuffer _inputbufferget)))
  (CallFunction|ActionCurrentMoveAbilitySETxF _inputbufferget)
  (CallFunction|ActionInputBufferClearxF)
  ;[1 1 1] StateEvent
  ;;[1 1 1] Clears/EndsAbility of  all active activeState Abilities. Should only have one active
  (Ability|SendGameplayEventtoActor _returnvalue "(TagName=\"GameplayEvent.StateEvent.PreviousActiveStateInteruptedEvent\")" (Utilities|Struct|MakeGameplayEventData "(TagName=\"\")" _returnvalue))
  ;[1 1 1] loadoutWeaponSetContainer
  (bind (_newvalid _drawsheathstate _newholdingcurrent _drawsheath _animmontage) (CallFunction|DrawSheathSwapPrevNewResultF))
  (if _newvalid
    (switch Utilities|FlowControl|Switch|SwitchonE_DrawSheathState _drawsheath
      (:NewEnumerator0
        (Development|PrintString "GADrawEquipSheathPutup01MontageBasedParent>EG== Holding or Sheathed" true true "(R=1.000000,G=0.296756,B=0.000000,A=1.000000)" 22.0 :!label _label)
        (Ability|EndAbility))
      (:NewEnumerator1
        (goto _label))
      (:NewEnumerator2
        ;[1 1 1] Play Two AnimMontages
        ;;[1 1 1] Sheathing interuption instantly puts previous on back and new in hands
        (|PlayMontageandWaitProxy "None" (Variables|Default|GetSheathPutupAnimMotnage) 1.0 "None" true 1.0 0.0
          (:then
            ;[1 1 1] MOntageActions
            ;;[1 1 1] SwapSheathing: AN_UnequipSheath
            (Ability|Tasks|WaitGameplayEvent "(TagName=\"GameplayEvent.DrawSheathEvent.AN_UnequipSheathEvent\")" 0 true
              (:EventReceived
                ;;[1 1 1] AN_DrawEquipNHold
                (CallFunction|DrawEquipNHoldF))))
          (:OnCompleted
            ;;[1 1 1] SwapingEquip
            (|PlayMontageandWaitProxy "None" (Variables|Default|GetDrawEquipAnimMontage) 1.0 "None" true 1.0 0.0
              (:then
                ;;[1 1 1] SwapingPArt2Equiping Wait for AN_DrawHold
                (Ability|Tasks|WaitGameplayEvent "(TagName=\"GameplayEvent.DrawSheathEvent.AN_EquipNHoldEvent\")" 0 true
                  (:EventReceived
                    ;;[1 1 1] AN_UnequipSheathNPutup
                    (CallFunction|UnequipSheathNPutputF))))
              (:OnCompleted
                ;;[1 1 1] Completed
                ;;;[1 1 1] ReturnTo  (Loco,Prone,Disabled,ec)
                (CallFunction|ActionPreviousActiveStateCompletexF)
                (Ability|EndAbility))
              (:OnInterrupted
                ;;[1 1 1] InteruptInstant
                (CallFunction|InteruptedF :!label _label_2)
                (Ability|EndAbility))
              (:OnCancelled
                (goto _label_2))))
          (:OnInterrupted
            ;;[1 1 1] InteruptInstant
            ;;;[1 1 1] Interupt SwapSheath
            (CallFunction|InteruptedF :!label _label_3)
            ;;;[1 1 1] InteruptSwapEquip
            (CallFunction|InteruptedF)
            (Ability|EndAbility))
          (:OnCancelled
            (goto _label_3))))
      (:NewEnumerator3
        ;[1 1 1] Play Single AniMontage
        (Utilities|IsValid _animmontage :!label _label_4
          (:Is%20Valid
            _)
          (:Is%20Not%20Valid
            (Development|PrintString "GADrawEquipSheathPutup>EG== animMontageNotValid" true true "(R=1.000000,G=0.319038,B=0.000000,A=1.000000)" 22.0)))
        (|PlayMontageandWaitProxy "None" _animmontage 1.0 "None" true 1.0 0.0
          (:then
            ;[1 1 1] Montage Action
            ;;[1 1 1] Set  ActiveState variable on character
            (CallFunction|ActiveStateSwitchTagSETF "(TagName=\"ActiveState.DrawSheathAS\")")
            ;;[1 1 1] Wait for AN_EquipHold,AN_UnequipSheath,InteruptInstant
            (Utilities|FlowControl|Sequence
              (:then_0
                ;;[1 1 1 1 14] Set variable on character
                (CallFunction|ActiveStateSwitchTagSETF "(TagName=\"ActiveState.AttackNormal\")")
                ;;[1 1 1 1 14] PreviousActiveStateInterupted
                (Ability|Tasks|WaitGameplayEvent "(TagName=\"GameplayEvent.StateEvent.PreviousActiveStateInteruptedEvent\")" 0 true
                  (:EventReceived
                    (CallFunction|InteruptedF)
                    (Ability|EndAbility))))
              (:then_1
                (Ability|Tasks|WaitGameplayEvent "(TagName=\"GameplayEvent.DrawSheathEvent.AN_EquipNHoldEvent\")" 0 true
                  (:EventReceived
                    ;;[1 1 1] AN_DrawEquipNHold
                    (CallFunction|DrawEquipNHoldF))))
              (:then_2
                (Ability|Tasks|WaitGameplayEvent "(TagName=\"GameplayEvent.DrawSheathEvent.AN_UnequipSheathEvent\")" 0 true
                  (:EventReceived
                    ;;[1 1 1] AN_UnequipSheathNPutup
                    (CallFunction|UnequipSheathNPutputF))))))
          (:OnCompleted
            ;;[1 1 1] Completed
            ;;;[1 1 1 1 14] ReturnTo  (Loco,Prone,Disabled,ec)
            (CallFunction|ActionPreviousActiveStateCompletexF)
            (Ability|EndAbility))
          (:OnInterrupted
            ;;[1 1 1] InteruptInstant
            (CallFunction|InteruptedF :!label _label_5)
            (Ability|EndAbility))
          (:OnCancelled
            (goto _label_5))))
      (:NewEnumerator4
        (goto _label_4)))
    (else
      ;[1 1 1] Completed
      ;;[1 1 1] ReturnTo  (Loco,Prone,Disabled,ec)
      (CallFunction|ActionPreviousActiveStateCompletexF)
      (Ability|EndAbility))))

(event Ability|EventOnEndAbility
  (params (bWasCancelled :type Boolean))
  (|CallParentFunction bWasCancelled) ; This node is disabled and will not be called.\nDrag off pins to build functionality.
)