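; Parent Gameplay Ability for a character's block stun, played as a montage reaction.
; On activation it commits, takes the current action from the input buffer, interrupts the previous active-state ability via gameplay event and sets the BlockingStun state.
; It ends on montage completion, interruption or a later state event.
; Montage selection is unfinished: guard break is stubbed false and perfect and good timing both return the good-block montage.
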(event Ability|EventActivateAbility
  (bind _returnvalue (Ability|GetOwningActorfromActorInfo))
  ;[1 1 1] Commit
  (|CallParentFunction)
  (Ability|CommitAbility)
  ;[1 1 1] CurrectAction and InputBuffer
  (bind _inputbufferget (CallFunction|ActionInputBufferGETxF))
  (CallFunction|ActionCurrentMoveAbilitySETxF _inputbufferget)
  (CallFunction|ActionCurrentMoveAbilityPrivateStartWithinGAF)
  (CallFunction|ActionInputBufferClearxF)
  ;[1 1 1] StateEvent
  ;;[1 1 1 1 14] Clears/EndsAbility of  all active activeState Abilities. Should only have one active
  (Ability|SendGameplayEventtoActor _returnvalue "(TagName=\"GameplayEvent.StateEvent.PreviousActiveStateInteruptedEvent\")" (Utilities|Struct|MakeGameplayEventData "(TagName=\"\")" _returnvalue))
  ;[1 1 1] Play Montage
  (bind _blockanimmontage (CallFunction|SimpleBlockAnimMontageF-todoPerfectVsGood))
  (Utilities|IsValid _blockanimmontage
    (:Is%20Valid
      _)
    (:Is%20Not%20Valid
      (Development|PrintString "GaBlockStun00Parent>EG== Hit animMontage is not valid" true true "(R=1.000000,G=0.516063,B=0.000000,A=1.000000)" 22.0)))
  (|PlayMontageandWaitProxy "None" _blockanimmontage 1.0 "None" true 1.0 0.0
    (:then
      ;[1 1 1] Montage Action
      ;;[1 1 1] Set  ActiveState variable on character
      (CallFunction|ActiveStateSwitchTagSETF "(TagName=\"ActiveState.BlockingStunAS\")")
      ;;[1 1 1] PreviousActiveStateInterupted
      (Ability|Tasks|WaitGameplayEvent "(TagName=\"GameplayEvent.StateEvent.PreviousActiveStateInteruptedEvent\")" 0 true
        (:EventReceived
          (Ability|EndAbility))))
    (:OnCompleted
      ;;[1 1 1] Attacks,Dodges,HitStun,Ect EndAbility when Montage  plays to the end
      ;;;[1 1 1 1 14] ReturnTo  (Loco,Prone,Disabled,ec)
      (CallFunction|ActionPreviousActiveStateCompletexF)
      (Ability|EndAbility))
    (:OnInterrupted
      (Ability|EndAbility :!label _label))
    (:OnCancelled
      (goto _label))))

(event Ability|EventOnEndAbility
  (params (bWasCancelled :type Boolean))
  (|CallParentFunction bWasCancelled) ; This node is disabled and will not be called.\nDrag off pins to build functionality.
)

(fn AdvancedFourDirectionAnimMontageF
  (params (ForwardRightPos45 :type Float%20%28double-precision%29) (BackRightPos135 :type Float%20%28double-precision%29) (BackLeftNeg135 :type Float%20%28double-precision%29) (ForwardLeftNeg45 :type Float%20%28double-precision%29)))

(fn SimpleBlockAnimMontageF-todoPerfectVsGood
  (bind _guardguagebroken (CallFunction|GuardGuageBrokenGETF-TodoStatsLater))
  (if _guardguagebroken
    (return (Variables|Default|GetGuardBreakBlockAnimMontage))
    (else
      (CallFunction|BlockTimingProofingF)
      (if (< (- (Utilities|Time|GetGameTimeinSeconds) (.InputPressGameTime-StartBuffer (Utilities|Struct|BreakS_InputBuffer (Variables|Default|GetActionCurrentMoveAbility_Private)))) (Variables|Default|GetBlockPerfectTimeMax))
        (return (Variables|Default|GetFrontGoodBlockAnimMontage))
        (else
          (return (Variables|Default|GetFrontGoodBlockAnimMontage)))))))

(fn BlockTimingProofingF
  (if (> (Variables|Default|GetBlockPerfectTimeMax) 0.0)
    _
    (else
      (Development|PrintString "GABlockStun00Parent>SimpleBlockAnimMontageF==BlockPerfectTimeMax is zero. Should" true true "(R=1.000000,G=0.342601,B=0.000000,A=1.000000)" 22.0)
      (Variables|Default|SetBlockPerfectTimeMax 2.0)))
  (return))

(fn GuardGuageBrokenGETF-TodoStatsLater
  ;[1 1 1] TEmp set to false
  (return false))