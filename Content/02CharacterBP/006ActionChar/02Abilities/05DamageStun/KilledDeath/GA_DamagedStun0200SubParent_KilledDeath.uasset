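; Parent gameplay ability for killed deaths, a damage-stun variant that marks the owning character dead and reports the death to objective tracking.
; DeathDispatcherNDeathStatF runs only while the owner is alive, setting its dead state through interface messages, then sending the victim and its name tag to player controller 0.
; The activate and end events are disabled, and a quest-leader controller lookup is left unwired as a todo.
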(event Ability|EventActivateAbility
  (|CallParentFunction) ; This node is disabled and will not be called.\nDrag off pins to build functionality.
)

(event Ability|EventOnEndAbility
  (params (bWasCancelled :type Boolean))
  (|CallParentFunction bWasCancelled) ; This node is disabled and will not be called.\nDrag off pins to build functionality.
)

(fn DeathDispatcherNDeathStatF
  ;[1 1 1] Todolater:Create GAkilledParent that has dispatcher function
  (bind _character (CallFunction|OwningCharacterRefGETF))
  (bind _bisalive (Class|BPCharacterStatsInterfaceI|CSIAliveGETCheckI(Message) _character))
  (if _bisalive
    ;;[1 1 1] DeathStat
    (Class|BPCharacterStatsInterfaceI|CSIKilledDeadSETI(Message) _character)
    ;;[1 1 1] DeathDispatcher
    (bind _characternameidgameplaytag (Class|BPCharacterStatsInterfaceI|CSICharacterNameIdPortriatIconGETI-todoReplace(Message) _character))
    (Class|BPIPlayerControllerStoryInterfaceI|PcSIObjectiveCharacterDeathDispatchI(Message) (Game|GetPlayerController 0) _character _characternameidgameplaytag))
  (return))