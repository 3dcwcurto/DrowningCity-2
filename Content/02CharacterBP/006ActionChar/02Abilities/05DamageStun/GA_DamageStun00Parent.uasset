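; Parent gameplay ability for damage stun, providing helper functions for directional hit reactions; its own activate and end events only call the parent.
; Stored hit angle, locations and swing direction drive two- or four-way montage selection and prone/supine state.
; Other helpers switch root motion versus impulse launch, fake landing and find the bone nearest the hit.
; An unwired Stun_CG graph sketches commit, montage playback and interruption by gameplay event.
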(event Ability|EventActivateAbility
  (|CallParentFunction))

(event Ability|EventOnEndAbility
  (params (bWasCancelled :type Boolean))
  (|CallParentFunction bWasCancelled))

(fn AdvancedFourDirectionSty;eAnimMontageF
  (switch Utilities|FlowControl|Switch|SwitchonE_GenericDirectionAdvanced-FrontLeftRightBack (Variables|Default|GetDirectionAdvanced)
    (:NewEnumerator0
      (Development|PrintString "GAHitReactionStun00Parent>FourDirectionAnimMontageF== Direction is null"))
    (:NewEnumerator1
      _)
    (:NewEnumerator2
      (return (Variables|Default|GetLeftHitReactionAnimMontage)))
    (:NewEnumerator3
      (return (Variables|Default|GetRightHitReactionAnimMontage)))
    (:NewEnumerator4
      (return (Variables|Default|GetBackHitReactionAnimMontage))))
  (return (Variables|Default|GetFrontHitReactionAnimMontage)))

(fn AdvancedFourDirectionalStyleHitReactionCalculationF
  (params (ForwardRightPos45 :type Float%20%28double-precision%29) (BackRightPos135 :type Float%20%28double-precision%29) (BackLeftNeg135 :type Float%20%28double-precision%29) (ForwardLeftNeg45 :type Float%20%28double-precision%29))
  (LocalVariables|SetForwardRightPos45_Localx ForwardRightPos45)
  (LocalVariables|SetBackRightPos135_Local BackRightPos135)
  (LocalVariables|SetBackLeftNeg135_Local BackLeftNeg135)
  (LocalVariables|SetForwardLeftNeg45_Local ForwardLeftNeg45)
  (LocalVariables|SetAngleFloat_local (Variables|HitInfoPrivate|GetHitDirectionAngle_Private))
  (if (and (>= (LocalVariables|GetAngleFloat_local) (LocalVariables|GetForwardLeftNeg45_Local)) (<= (LocalVariables|GetAngleFloat_local) (LocalVariables|GetForwardRightPos45_Localx)))
    (Variables|Default|SetDirectionAdvanced "NewEnumerator1")
    (return)
    (elif (and (> (LocalVariables|GetAngleFloat_local) (LocalVariables|GetForwardRightPos45_Localx)) (< (LocalVariables|GetAngleFloat_local) (LocalVariables|GetBackRightPos135_Local)))
      (Variables|Default|SetDirectionAdvanced "NewEnumerator3")
      (return)
      (elif (and (> (LocalVariables|GetAngleFloat_local) (LocalVariables|GetBackLeftNeg135_Local)) (< (LocalVariables|GetAngleFloat_local) (LocalVariables|GetForwardLeftNeg45_Local)))
        (Variables|Default|SetDirectionAdvanced "NewEnumerator2")
        (return)
        (elif (or (and (>= (LocalVariables|GetAngleFloat_local) (LocalVariables|GetBackLeftNeg135_Local)) (<= (LocalVariables|GetAngleFloat_local) 1.8e+02)) (and (<= (LocalVariables|GetAngleFloat_local) (LocalVariables|GetBackLeftNeg135_Local)) (>= (LocalVariables|GetAngleFloat_local) -1.8e+02)))
          (Variables|Default|SetDirectionAdvanced "NewEnumerator4")
          (return)
          (else
            (Development|PrintString "GAHitReactionStun00Parent>FourDirectionHitReactionF==Direction Calculation Failed" true true "(R=0.890625,G=0.385938,B=0.000000,A=1.000000)" 22.0)
            (Variables|Default|SetDirectionAdvanced "NewEnumerator4")
            (return)))))))

(fn SimpleTwoDirectionStyleAnimMontageF
  (switch Utilities|FlowControl|Switch|SwitchonE_GenericDirectionSimple-ForwardVsBackwards (Variables|Default|GetDirectionSimple)
    (:NewEnumerator0
      (Development|PrintString "GAHitReactionStun00Parent>AnimMontageTwoDirectionF== FrontVsBack is null" true true "(R=1.000000,G=0.390478,B=0.000000,A=1.000000)" 22.0))
    (:NewEnumerator1
      _)
    (:NewEnumerator2
      (return (Variables|Default|GetBackHitReactionAnimMontage))))
  (return (Variables|Default|GetFrontHitReactionAnimMontage)))

(fn SimpleTwoDirectionStyleHitReactionCalculationF
  (params (LeftSideNeg :type Float%20%28double-precision%29) (RightSidePos :type Float%20%28double-precision%29))
  (LocalVariables|SetLeftSideNeg_Local LeftSideNeg)
  (LocalVariables|SetRightSidePos_Local RightSidePos)
  (LocalVariables|SetAngleFloat_Local (Variables|HitInfoPrivate|GetHitDirectionAngle_Private))
  (if (and (>= (LocalVariables|GetAngleFloat_Local) (LocalVariables|GetLeftSideNeg_Local)) (<= (LocalVariables|GetAngleFloat_Local) (LocalVariables|GetRightSidePos_Local)))
    (Variables|Default|SetDirectionSimple "NewEnumerator1")
    (return)
    (else
      (Variables|Default|SetDirectionSimple "NewEnumerator2")
      (return))))

(fn HitLocationDirectionAngleInfoF
  (params (Info :type S%20Input%20Buffer%20Structure%20%28by%20ref%29))
  (bind (_gaability _inputtag _inputaction_enchancedinput _inputdirection_startbuffer _floatdirection_startbuffer _hasinputdirection_startbuffer _inputpressgametime_startbuffer _desiredindex_startbuffer _stancefootinfront_startfire_oldq _inputdirectionprevious_tick _floatdirection_tick _hasinputdirection_tick _chargelevelamountcurrent_tick _hitconfirm_todolater _modifier_enchanedinput _trigger_enhancedinput _hitresultlocation _hitresultangle _hitattackerlocation _hitswingdirection _hitlaunchdirection _attackerstats _attackercharacter) (Utilities|Struct|BreakS_InputBuffer Info))
  (Variables|HitInfoPrivate|SetHitResultLocation_Private _hitresultlocation)
  (Variables|HitInfoPrivate|SetHitDirectionAngle_Private _hitresultangle)
  (Variables|HitInfoPrivate|SetHitAttackerLocation_Private _hitattackerlocation)
  (Variables|HitInfoPrivate|SetHitSwingDirection_Private _hitswingdirection)
  (Variables|HitInfoPrivate|SetHitLaunchDirection_Private _hitlaunchdirection)
  (Variables|HitInfoPrivate|SetAttackerCharacter_Private _attackercharacter))

(fn RootMotionModeF
  (bind _character (CallFunction|OwningCharacterRefGETF))
  (switch Utilities|FlowControl|Switch|SwitchonE_StunRootMotionVsImpulseForce (Variables|Default|GetRootMotionVsImpulseForce)
    (:NewEnumerator0
      (Development|PrintString "GAhitReactionStun00Parent>RootMotionModeF== RootmotionVsImpulseForce is null" true true "(R=1.000000,G=0.176017,B=0.000000,A=1.000000)" 22.0)
      (return))
    (:NewEnumerator1
      (Class|AnimInstance|SetRootMotionMode (Components|SkeletalMesh|GetAnimInstance (Variables|/Script/Engine.Character|GetMesh _character)) "RootMotionFromMontagesOnly")
      (return))
    (:NewEnumerator2
      (Class|AnimInstance|SetRootMotionMode (Components|SkeletalMesh|GetAnimInstance (Variables|/Script/Engine.Character|GetMesh _character)) "NoRootMotionExtraction")
      (return))))

(fn StopMomentumStopMovementF0
  (bind _character (CallFunction|OwningCharacterRefGETF))
  (Components|Movement|StopMovementImmediately (Variables|/Script/Engine.Character|GetCharacterMovement _character))
  (Class|NavMovementComponent|StopActiveMovement (Variables|/Script/Engine.Character|GetCharacterMovement _character))
  (return))

(fn LaunchImpulseF
  (switch Utilities|FlowControl|Switch|SwitchonE_StunRootMotionVsImpulseForce (Variables|Default|GetRootMotionVsImpulseForce)
    (:NewEnumerator0
      (Development|PrintString "GaHitReactionStun00Parent>LaunchImpulseF==RootMotionVsImpulseForce== " true true "(R=1.000000,G=0.156591,B=0.000000,A=1.000000)" 22.0))
    (:NewEnumerator1
      _)
    (:NewEnumerator2
      (bind _character (CallFunction|OwningCharacterRefGETF))
      (Physics|AddImpulse (Variables|/Script/Engine.Character|GetCharacterMovement _character) (+ (* (Math|Vector|Normalize (Math|Vector|MakeVector (.X (Math|Vector|BreakVector (* (Math|Vector|GetForwardVector (Math|Rotator|FindLookatRotation (Transformation|GetActorLocation _character) (Variables|HitInfoPrivate|GetHitAttackerLocation_Private))) -1.0))) (.Y (Math|Vector|BreakVector (* (Math|Vector|GetForwardVector (Math|Rotator|FindLookatRotation (Transformation|GetActorLocation _character) (Variables|HitInfoPrivate|GetHitAttackerLocation_Private))) -1.0))) 0.0)) 333.0) (* (Math|Vector|MakeVector 0.0 0.0 1.0) 333.0)) true)))
  (return))

(fn SimpleTwoDirectionLaunchProneSupineF
  (bind _character (CallFunction|OwningCharacterRefGETF))
  (switch Utilities|FlowControl|Switch|SwitchonE_GenericDirectionSimple-ForwardVsBackwards (Variables|Default|GetDirectionSimple)
    (:NewEnumerator0
      (LocalVariables|SetStanceProneSupine_Local "NewEnumerator1" :!label _label))
    (:NewEnumerator1
      (goto _label))
    (:NewEnumerator2
      (LocalVariables|SetStanceProneSupine_Local "NewEnumerator0")))
  (Class|BPICharacterActionInterfaceI|CAIHandleDamageLaunchProneSupineI(Message) _character "NewEnumerator1" (LocalVariables|GetStanceProneSupine_Local)))

(fn AdvancedFourDirectionLaunchProneSupineF
  (bind _character (CallFunction|OwningCharacterRefGETF))
  (switch Utilities|FlowControl|Switch|SwitchonE_GenericDirectionAdvanced-FrontLeftRightBack (Variables|Default|GetDirectionAdvanced)
    (:NewEnumerator0
      (LocalVariables|SetStanceProneSupine_Local "NewEnumerator0" :!label _label))
    (:NewEnumerator1
      (goto _label))
    (:NewEnumerator2
      (goto _label))
    (:NewEnumerator3
      (goto _label))
    (:NewEnumerator4
      (LocalVariables|SetStanceProneSupine_Local "NewEnumerator1")))
  (Class|BPICharacterActionInterfaceI|CAIHandleDamageLaunchProneSupineI(Message) _character "NewEnumerator1" (LocalVariables|GetStanceProneSupine_Local)))

(fn RoototionResetF
  (bind _character (CallFunction|OwningCharacterRefGETF))
  ;[1 1 1] Rest to rootmotion from montages
  (Class|AnimInstance|SetRootMotionMode (Components|SkeletalMesh|GetAnimInstance (Variables|/Script/Engine.Character|GetMesh _character)) "RootMotionFromMontagesOnly")
  (return))

(fn LaunchMontageEndFakeLandingCheckF
  (bind _character (CallFunction|OwningCharacterRefGETF))
  (bind _movemodestate (Class|BPICharacterLocomotionInterfaceI|CLIMoveModeStateGETI(Message) _character))
  (return (Utilities|Enum|Equal(Enum) _movemodestate "NewEnumerator1") _movemodestate))

(fn LaunchMontageEndFakeLandingEventF
  (bind _character (CallFunction|OwningCharacterRefGETF))
  (Class|BPICharacterActionInterfaceI|CAILandingMontageEndEventFakefromGaI(Message) _character)
  (return))

(fn SimpleFrontBackSwingDirectionResultF
  (bind _directionsimple (Variables|Default|GetDirectionSimple))
  (Development|PrintString (Utilities|String|EnumtoString _directionsimple) true true "(R=1.000000,G=0.000000,B=0.257265,A=1.000000)")
  (switch Utilities|FlowControl|Switch|SwitchonE_GenericDirectionSimple-ForwardVsBackwards _directionsimple
    (:NewEnumerator0
      _)
    (:NewEnumerator1
      _)
    (:NewEnumerator2
      (switch Utilities|FlowControl|Switch|SwitchonE_HitAttackSwingDirectionVFX (Variables|HitInfoPrivate|GetHitSwingDirection_Private)
        (:NewEnumerator0
          _)
        (:NewEnumerator1
          (return (Variables|Default|GetLeftHitReactionAnimMontage)))
        (:NewEnumerator2
          (return (Variables|Default|GetRightHitReactionAnimMontage)))
        (:NewEnumerator3
          _)
        (:NewEnumerator4
          (return (Variables|Default|GetFrontHitReactionAnimMontage)))
        (:NewEnumerator5
          (return (Variables|Default|GetBackHitReactionAnimMontage))))
      (return (Variables|Default|GetFrontHitReactionAnimMontage))))
  (switch Utilities|FlowControl|Switch|SwitchonE_HitAttackSwingDirectionVFX (Variables|HitInfoPrivate|GetHitSwingDirection_Private)
    (:NewEnumerator0
      _)
    (:NewEnumerator1
      (return (Variables|Default|GetRightHitReactionAnimMontage)))
    (:NewEnumerator2
      (return (Variables|Default|GetLeftHitReactionAnimMontage)))
    (:NewEnumerator3
      _)
    (:NewEnumerator4
      (return (Variables|Default|GetBackHitReactionAnimMontage)))
    (:NewEnumerator5
      (return (Variables|Default|GetFrontHitReactionAnimMontage))))
  (return (Variables|Default|GetFrontHitReactionAnimMontage)))

(fn AttackMeleeHitResultClosestBoneF
  (for (_array_element _array_index) (LocalVariables|GetBoneSocketName_Local)
    (bind _character (CallFunction|OwningCharacterRefGETF))
    ;[1 1 1] PROOF
    (if (Transformation|DoesSocketExist (Variables|/Script/Engine.Character|GetMesh _character) _array_element)
      _
      (else
        (Development|PrintString (Utilities|String|Append "BPCharacterActionC>AttackMeleeHitResultCloseBoneF==" (Utilities|String|ToString(Name) _array_element)) true true "(R=1.000000,G=0.264731,B=0.000000,A=1.000000)" 22.0)))
    ;[1 1 1] Starting value to compare
    (if (== _array_index 0)
      (LocalVariables|SetShortestDIstanceCurrent_Local (Math|Vector|VectorLength (- (Transformation|GetSocketLocation (Variables|/Script/Engine.Character|GetMesh _character) _array_element) (Variables|HitInfoPrivate|GetHitResultLocation_Private))) :!label _label)
      (LocalVariables|SetBoneSocketCurrent_Local _array_element)
      (LocalVariables|SetBoneSocketIndex_Local _array_index)
      (elif (< (Math|Vector|VectorLength (- (Transformation|GetSocketLocation (Variables|/Script/Engine.Character|GetMesh _character) _array_element) (Variables|HitInfoPrivate|GetHitResultLocation_Private))) (LocalVariables|GetShortestDIstanceCurrent_Local))
        (goto _label))))
  (bind _returnvalue (Utilities|GetDataTableRow "/Game/02CharacterBP/006ActionChar/03HandleDamage/DT_BoneSocketInfo.DT_BoneSocketInfo" (LocalVariables|GetBoneSocketCurrent_Local))
    (:then
      _)
    (:RowNotFound
      (Development|PrintString "BPCharacterActionC>AtttackMeleeHitresultClosestBoneF==GetDataTableRowDTBoneSocketInfo Row Not Found")))
  (return true (LocalVariables|GetBoneSocketCurrent_Local) _returnvalue))