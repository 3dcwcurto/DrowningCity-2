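; Gameplay ability for a normal hit-reaction stun that plays a directional montage and puts the character in the stunned active state.
; On activation it commits, consumes the action input buffer, computes hit direction and broadcasts an interrupt event to end the previous active state.
; A two-direction calculation selects the montage.
; Completion runs the previous-state completion step and ends the ability; montage interruption, cancellation or a later interrupt event also ends it.
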(event Ability|EventActivateAbility
  (bind _returnvalue (Ability|GetOwningActorfromActorInfo))
  ;[1 1 1] Commit
  (|CallParentFunction)
  (Ability|CommitAbility)
  ;[1 1 1] CurrectAction and InputBuffer
  (bind _inputbufferget (CallFunction|ActionInputBufferGETxF))
  (CallFunction|HitLocationDirectionAngleInfoF _inputbufferget)
  (CallFunction|ActionCurrentMoveAbilitySETxF _inputbufferget)
  (CallFunction|ActionInputBufferClearxF)
  ;[1 1 1] StateEvent
  ;;[1 1 1 1 14] Clears/EndsAbility of  all active activeState Abilities. Should only have one active
  (Ability|SendGameplayEventtoActor _returnvalue "(TagName=\"GameplayEvent.StateEvent.PreviousActiveStateInteruptedEvent\")" (Utilities|Struct|MakeGameplayEventData "(TagName=\"\")" _returnvalue))
  ;[1 1 1] HitReactionStunNormal Specifc
  (Utilities|FlowControl|Sequence
    (:then_0
      (CallFunction|SimpleTwoDirectionStyleHitReactionCalculationF -9e+01 9e+01)
      ;[1 1 1] Play Montage
      (bind _animmontage (CallFunction|SimpleTwoDirectionStyleAnimMontageF))
      (Utilities|IsValid _animmontage
        (:Is%20Valid
          _)
        (:Is%20Not%20Valid
          (Development|PrintString "GaHitReactionStun00Parent>EG== Hit animMontage is not valid" true true "(R=1.000000,G=0.516063,B=0.000000,A=1.000000)" 22.0)))
      (|PlayMontageandWaitProxy "None" _animmontage 1.0 "None" true 1.0 0.0
        (:then
          ;[1 1 1] Montage Action
          ;;[1 1 1] Set  ActiveState variable on character
          (CallFunction|ActiveStateSwitchTagSETF "(TagName=\"ActiveState.DisabledAS.StunAS\")")
          ;;[1 1 1] PreviousActiveStateInterupted
          (Ability|Tasks|WaitGameplayEvent "(TagName=\"GameplayEvent.StateEvent.PreviousActiveStateInteruptedEvent\")" 0 true
            (:EventReceived
              (Ability|EndAbility))))
        (:OnCompleted
          ;;[1 1 1] Attacks,Dodges,HitStun,Ect EndAbility when Montage  plays to the end
          ;;;[1 1 1 1 14] ReturnTo  (Loco,Prone,Disabled,ec)
          (CallFunction|ActionPreviousActiveStateCompletexF)
          (Ability|EndAbility))
        (:OnInterrupted
          (Ability|EndAbility :!label _label))
        (:OnCancelled
          (goto _label))))
    (:then_1)))

(event Ability|EventOnEndAbility
  (params (bWasCancelled :type Boolean))
  (|CallParentFunction bWasCancelled) ; This node is disabled and will not be called.\nDrag off pins to build functionality.
)