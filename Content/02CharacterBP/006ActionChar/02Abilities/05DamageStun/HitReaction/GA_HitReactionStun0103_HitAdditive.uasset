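; Gameplay ability that plays an additive hit reaction montage, noted as a jiggle for super armor hits.
; On activation it commits, gathers additive action info, runs hit direction and two-sided angle calculations, then plays the front hit montage and ends when it completes, is interrupted or is cancelled.
; The same montage serves every hit; alternative styles using attacker swing direction or closest hit bone are present but unconnected.
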(event Ability|EventActivateAbility
  (bind _fronthitreactionanimmontage (Variables|Default|GetFrontHitReactionAnimMontage))
  ;[1 1 1] Commit
  (|CallParentFunction)
  (Ability|CommitAbility)
  ;[1 1 1] CurrectAction and InputBuffer
  ;;[1 1 1] Unique variable that stores additive info
  (bind _additive (CallFunction|ActionAdditiveF))
  (CallFunction|HitLocationDirectionAngleInfoF _additive)
  (CallFunction|SimpleTwoDirectionStyleHitReactionCalculationF -9e+01 9e+01)
  ;[1 1 1] Play Montage Additive
  (Utilities|IsValid _fronthitreactionanimmontage
    (:Is%20Valid
      _)
    (:Is%20Not%20Valid
      (Development|PrintString "GaHitReactionStun00Parent>EG== Hit animMontage is not valid" true true "(R=1.000000,G=0.516063,B=0.000000,A=1.000000)" 22.0)))
  (|PlayMontageandWaitProxy "None" _fronthitreactionanimmontage 1.0 "None" true 1.0 0.0
    (:OnCompleted
      _)
    (:OnInterrupted
      _)
    (:OnCancelled
      _))
  ;[1 1 1] Montage Action
  (Ability|EndAbility))

(event Ability|EventOnEndAbility
  (params (bWasCancelled :type Boolean))
  (|CallParentFunction bWasCancelled) ; This node is disabled and will not be called.\nDrag off pins to build functionality.
)