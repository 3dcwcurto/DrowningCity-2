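; Master Gameplay Ability providing shared helpers for character action abilities, with empty activate and end events.
; Helpers use a lazily cached owning Character and interface messages to access state tags, current move, input buffer, tag containers, momentum and gait cap.
; Others snap facing to buffered input relative to control yaw, switch root motion mode and send gameplay events (marked unneeded).
; Directional montage selection and crime reporting are unimplemented stubs.
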(event Ability|EventActivateAbility)

(event Ability|EventOnEndAbility
  (params (bWasCancelled :type Boolean)))

(fn OwningCharacterRefGETF
  (Utilities|IsValid (Variables|Default|GetCharacterRef_Private)
    (:Is%20Valid
      (return (Variables|Default|GetCharacterRef_Private)))
    (:Is%20Not%20Valid
      (bind _ascharacter (Utilities|Casting|CastToCharacter (Ability|GetOwningActorfromActorInfo))
        (:then
          (bind _output_get (Variables|Default|SetCharacterRef_Private _ascharacter)))
        (:CastFailed
          (Development|PrintString "GAAbilityMaster>OwningCharacterGetF== Character cast failed" true true "(R=1.000000,G=0.485480,B=0.000000,A=1.000000)" 22.0)))
      (return _output_get))))

(fn DirectionForwardRightBackLeftF-Todo
  (params (Forward_AnimMontage :type Anim%20Montage%20Object%20Reference) (Right_AnimMontage :type Anim%20Montage%20Object%20Reference) (Back_AnimMontage :type Anim%20Montage%20Object%20Reference) (Left_AnimMontage :type Anim%20Montage%20Object%20Reference)))

(fn ActiveStateSwitchTagSETF
  (params (ActiveState_GameplayTag :type Gameplay%20Tag%20Structure))
  (bind _character (CallFunction|OwningCharacterRefGETF))
  ;[1 1 1] NormalAttack,locomotion,ect
  (Class|BPICharacterActionInterfaceI|CAIActiveStateTagSETI(Message) _character ActiveState_GameplayTag))

(fn ActiveStateSwitchTagGETF
  (bind _character (CallFunction|OwningCharacterRefGETF))
  (bind _activestateswitchtag (Class|BPICharacterActionInterfaceI|CAIActiveStateTagGETI(Message) _character))
  (return _activestateswitchtag _character))

(fn ActionCurrentMoveAbilitySETxF
  (params (ActionCurrentMoveAbility :type S%20Input%20Buffer%20Structure))
  (bind _character (CallFunction|OwningCharacterRefGETF))
  ;[1 1 1] InputBuffer Structure
  (Class|BPICharacterActionInterfaceI|CAIActionCurrentMoveAbilitySETI(Message) _character ActionCurrentMoveAbility))

(fn ActionCurrentMoveAbilityGETxF
  (bind _character (CallFunction|OwningCharacterRefGETF))
  (bind _actioncurrentmoveability (Class|BPICharacterActionInterfaceI|CAIActionCurrentMoveAbilityGETI(Message) _character))
  (return _actioncurrentmoveability _character))

(fn ActionInputBufferGETxF
  (bind _character (CallFunction|OwningCharacterRefGETF))
  (bind _inputbufferget (Class|BPICharacterActionInterfaceI|CAIActionInputBufferGETI(Message) _character))
  (return _inputbufferget))

(fn ActionInputBufferClearxF
  (bind _character (CallFunction|OwningCharacterRefGETF))
  (Class|BPICharacterActionInterfaceI|CAIActionInputBufferClearI(Message) _character)
  (return))

(fn ActionPreviousActiveStateCompletexF
  (bind _character (CallFunction|OwningCharacterRefGETF))
  (Class|BPICharacterActionInterfaceI|CAIActiveStatePreviousCompleteI(Message) _character)
  (return))

(fn ActionContainerTagAddxF
  (params (TagContainerToAdd :type Gameplay%20Tag%20Container%20Structure))
  (bind _character (CallFunction|OwningCharacterRefGETF))
  (Class|BPICharacterActionInterfaceI|CAIAnimNotifyStartAddTagContainerI(Message) _character TagContainerToAdd))

(fn ActionContainerTagRemovexF
  (params (TagContainerToRemove :type Gameplay%20Tag%20Container%20Structure))
  (bind _character (CallFunction|OwningCharacterRefGETF))
  (Class|BPICharacterActionInterfaceI|CAIAnimNotifyEndRemoveTagContainerI(Message) _character TagContainerToRemove))

(fn ActionRotationF
  (bind _actioncurrentmoveability (CallFunction|ActionCurrentMoveAbilityGETxF))
  (bind _character (CallFunction|OwningCharacterRefGETF))
  (if (Math|Vector|NotEqual(Vector) (+ (* (Math|Vector|GetForwardVector (Math|Rotator|MakeRotator 0.0 0.0 (.yaw (Pawn|GetControlRotation _character :!class /Script/Engine.Pawn)))) (.X (Math|Vector|BreakVector (.InputDirection_StartBuffer (Utilities|Struct|BreakS_InputBuffer _actioncurrentmoveability))))) (* (Math|Vector|GetRightVector (Math|Rotator|MakeRotator 0.0 0.0 (.yaw (Pawn|GetControlRotation _character :!class /Script/Engine.Pawn)))) (.Y (Math|Vector|BreakVector (.InputDirection_StartBuffer (Utilities|Struct|BreakS_InputBuffer _actioncurrentmoveability)))))) "0, 0, 0" 0.0001)
    (Transformation|SetActorRotation _character (Math|Rotator|MakeRotator 0.0 0.0 (.Yaw (Math|Rotator|BreakRotator (Math|Conversions|RotationFromXVector (Math|Vector|Normalize (+ (* (Math|Vector|GetForwardVector (Math|Rotator|MakeRotator 0.0 0.0 (.yaw (Pawn|GetControlRotation _character :!class /Script/Engine.Pawn)))) (.X (Math|Vector|BreakVector (.InputDirection_StartBuffer (Utilities|Struct|BreakS_InputBuffer _actioncurrentmoveability))))) (* (Math|Vector|GetRightVector (Math|Rotator|MakeRotator 0.0 0.0 (.yaw (Pawn|GetControlRotation _character :!class /Script/Engine.Pawn)))) (.Y (Math|Vector|BreakVector (.InputDirection_StartBuffer (Utilities|Struct|BreakS_InputBuffer _actioncurrentmoveability))))))))))))))

(fn StopMomentumStopMovementMF
  (bind _character (CallFunction|OwningCharacterRefGETF))
  (Class|BPICharacterLocomotionInterfaceI|CLIStopMovementMomentumI(Message) _character)
  (return))

(fn RoototionResetMF
  (bind _character (CallFunction|OwningCharacterRefGETF))
  (switch Utilities|FlowControl|Switch|SwitchonE_StunRootMotionVsImpulseForce (Variables|Default|GetRootMotionVsImpulseForce_)
    (:NewEnumerator0
      (Development|PrintString "GAhitReactionStun00Parent>RootMotionModeF== RootmotionVsImpulseForce is null" true true "(R=1.000000,G=0.176017,B=0.000000,A=1.000000)" 22.0)
      (return))
    (:NewEnumerator1
      (Class|AnimInstance|SetRootMotionMode (Components|SkeletalMesh|GetAnimInstance (Variables|/Script/Engine.Character|GetMesh _character)) "RootMotionFromMontagesOnly")
      (return))
    (:NewEnumerator2
      (Class|AnimInstance|SetRootMotionMode (Components|SkeletalMesh|GetAnimInstance (Variables|/Script/Engine.Character|GetMesh _character)) "NoRootMotionExtraction")
      (return))))

(fn ActionCurrentMoveAbilityPrivateStartWithinGAF
  (bind _actioncurrentmoveability (CallFunction|ActionCurrentMoveAbilityGETxF))
  ;[1 1 1] Use for timeing inside a GA. Block timing, parry timing,ect
  (Variables|Default|SetActionCurrentMoveAbility_Private _actioncurrentmoveability))

(fn GaitCapSetF
  (bind _character (CallFunction|OwningCharacterRefGETF))
  (Class|BPICharacterLocomotionInterfaceI|CLIGaitCapCurrentI(Message) _character (Variables|Default|GetGaitCapCurrent)))

(fn ActionAdditiveF
  (bind _character (CallFunction|OwningCharacterRefGETF))
  (bind _additive (Class|BPICharacterActionInterfaceI|CAIActionAdditiveGETI(Message) _character))
  (return _additive))

(fn CrimeSystemPingF-todo
  (params (AttackerPerp :type Boolean) (DefenderVictim :type Boolean) (CrimeType-TheftAssultMurderTrophe :type Boolean)))

(fn BTTaskSendCompleteGameplayEventF-dontNeed
  (params (EventTag :type Gameplay%20Tag%20Structure))
  (bind _character (CallFunction|OwningCharacterRefGETF))
  ;[1 1 1] Complete a specific event
  (Ability|SendGameplayEventtoActor 0 EventTag (Utilities|Struct|MakeGameplayEventData "(TagName=\"\")" _character)))

(fn BTTaskSendInteruptGameplayEventF-dontNeed
  (bind _character (CallFunction|OwningCharacterRefGETF))
  ;[1 1 1] Interupt
  (Ability|SendGameplayEventtoActor 0 "(TagName=\"GameplayEvent.StateEvent.PreviousActiveStateInteruptedEvent\")" (Utilities|Struct|MakeGameplayEventData "(TagName=\"\")" _character)))