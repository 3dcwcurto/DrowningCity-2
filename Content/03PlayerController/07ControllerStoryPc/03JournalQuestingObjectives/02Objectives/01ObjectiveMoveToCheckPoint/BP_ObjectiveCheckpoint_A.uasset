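; Checkpoint actor for move-to-checkpoint objectives, identified by a gameplay tag that its TextRender displays.
; Box overlaps, plus characters already inside at BeginPlay when the tag is valid, trigger completion.
; If a required team faction is set, only characters whose preset matches pass; otherwise any overlapping actor does.
; It then notifies player controller 0 by interface message and destroys itself; the marker widget function is unused.
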(event OnComponentBeginOverlap(Box)
  (params (OverlappedComponent :type Primitive%20Component%20Object%20Reference) (OtherActor :type Actor%20Object%20Reference) (OtherComp :type Primitive%20Component%20Object%20Reference) (OtherBodyIndex :type Integer) (bFromSweep :type Boolean) (SweepResult :type Hit%20Result%20Structure%20%28by%20ref%29))
  (CallFunction|ObjectiveCheckpointOverlappedF OtherActor))

(event EventBeginPlay
  ;[0.251 1 0] Beginplay
  (CallFunction|BeginPlayCheckpointOverlapF)
  (CallFunction|ObjectiveTextRenderNameF))

(fn ConstructionScript)

(fn MakerUIF
  (bind _returnvalue (UserInterface|CreateWidget "/Game/03PlayerController/07ControllerStoryPc/03JournalQuestingObjectives/02Objectives/01ObjectiveMoveToCheckPoint/W_ObjectiveCheckpointMarkerUI.W_ObjectiveCheckpointMarkerUI_C" 0 self))
  (UserInterface|Viewport|AddtoViewport _returnvalue 0)
  (Variables|Default|SetWBPObjectiveCHeckpointMarkerUIRef _returnvalue))

(fn ObjectiveCheckpointOverlappedF
  (params (ActorOverlap :type Actor%20Object%20Reference))
  (Utilities|IsValid (Variables|Default|GetTeamFactionRequiredForOverlapp)
    (:Is%20Valid
      (bind _ascharacter (Utilities|Casting|CastToCharacter ActorOverlap))
      (bind _pdacharacterpreset (Class|BPICharacterBaseInterface|CBICharacterPresetPdaGETI(Message) _ascharacter))
      (bind _teamfactionpresetid (Class|BPICharacterPresetInterface|HCPICharacterPresetInfoGETI(Message) _pdacharacterpreset))
      (if (== _teamfactionpresetid (Variables|Default|GetTeamFactionRequiredForOverlapp))
        ;[1 1 1] REmove self from PlayerControllerStory>
        (Class|BPIPlayerControllerStoryInterfaceI|PcSIObjectiveMovetoCheckpointOverlappedI(Message) (Game|GetPlayerController 0) self (Variables|Default|GetObjectiveGameplayTag) :!label _label)
        (Actor|DestroyActor)))
    (:Is%20Not%20Valid
      (goto _label))))

(fn BeginPlayCheckpointOverlapF
  (if (GameplayTags|IsGameplayTagValid (Variables|Default|GetObjectiveGameplayTag))
    (for _array_element (Collision|GetOverlappingActors (Variables|Default|GetBox) "/Script/Engine.Character" :!class /Script/Engine.PrimitiveComponent)
      (CallFunction|ObjectiveCheckpointOverlappedF _array_element))
    (else
      (Development|PrintString "BPObjectiveCheckpointA>EG>Beginplay== objectiveGameplayTag not valid" true true "(R=1.000000,G=0.291373,B=0.000000,A=1.000000)" 22.0))))

(fn ObjectiveTextRenderNameF
  (Rendering|Components|TextRender|SetText (Variables|Default|GetTextRender) (Utilities|Text|ToText(Name) (GameplayTags|GetTagName (Variables|Default|GetObjectiveGameplayTag)))))