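; Base player controller that sets the camera perspective mode, manages the gameplay HUD and handles cursor hover.
; On possess it selects RTS tactics mode, telling the pawn via interface and setting control rotation.
; In isometric and RTS modes, Tick traces under the cursor and sends outline begin/end messages.
; Input and dialogue events toggle HUD widget-switcher menus, while interface getters expose camera, hover and squad-manager data.
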(event EventBeginPlay
  ;[0.251 1 0] BeginPlay
  (|CallParentFunction)
  ;;[1 1 1] UI
  (CallFunction|WidgetHUDGameplayUI)
  ;;;[1 1 1] TodoMoveTo?
  (CallFunction|WidgetHUDPartyUI-todo-MovetoPartySquadPC?))

(event EventTick
  (params (DeltaSeconds :type Float%20%28single-precision%29))
  ;[0.01737 0.4427 0] Tick
  (|CallParentFunction DeltaSeconds)
  (switch Utilities|FlowControl|Switch|SwitchonE_CameraPerspectiveMode-Fps3rdIso (Variables|00PcBase|GetCameraPerspectiveMode)
    (:NewEnumerator3
      _)
    (:NewEnumerator5
      _))
  ;;[1 1 1] HighlightSelection
  (CallFunction|SelectionIsometricHoverHighlightSelectionTickF))

(event EventPossess
  (params (PossessedPawn :type Pawn%20Object%20Reference))
  ;[0 1 0.8984] Possess
  (|CallParentFunction PossessedPawn)
  (CallFunction|CameraCameraPerspectiveModeF "NewEnumerator5" PossessedPawn))

(event EventPcBIDialogueWidgetGameplayUIActiveI
  ;[1 1 1] DialogueConversation UI
  ;;[1 1 1] From playerControllerStory
  (CallFunction|WidgetGameplayMenuUI "NewEnumerator4"))

(event EventPcBIDialogueWidgetGameplayUIDisableI
  ;[1 1 1] DialogueConversation UI
  ;;[1 1 1] Return to default
  (CallFunction|WidgetGameplayMenuUI "NewEnumerator1"))

(event Input|ActionEvents|InputActionMenuJournalI
  (params (Key :type Key%20Structure))
  ;[1 1 1] Questing
  (:Pressed
    (CallFunction|WidgetGameplayMenuUI "NewEnumerator5")))

(event Input|ActionEvents|InputActionMenuStatRosterP
  (params (Key :type Key%20Structure))
  ;[1 1 1] Stat UI
  (:Pressed
    (CallFunction|WidgetGameplayMenuUI "NewEnumerator3")))

(event Input|ActionEvents|InputActionMenuSkillTreeO
  (params (Key :type Key%20Structure))
  ;[1 1 1] SkillTreeUI
  (:Pressed
    (CallFunction|WidgetGameplayMenuUI "NewEnumerator2")))

(fn ConstructionScript)

(fn WidgetHUDGameplayUI
  (Utilities|IsValid (Variables|00PcBase|GetWidget_WBPHudGameplayUI)
    (:Is%20Valid
      (return (Variables|00PcBase|GetWidget_WBPHudGameplayUI)))
    (:Is%20Not%20Valid
      (bind _returnvalue (UserInterface|CreateWidget "/Game/03PlayerController/WBP_HudGameplay_UI.WBP_HudGameplay_UI_C"))
      (bind _output_get (Variables|00PcBase|SetWidget_WBPHudGameplayUI _returnvalue))
      (UserInterface|Viewport|AddtoViewport _output_get 0)
      (return _output_get))))

(fn WidgetHUDPartyUI-todo-MovetoPartySquadPC?
  (bind _widget_wbphudgameplayui (Variables|00PcBase|GetWidget_WBPHudGameplayUI))
  (bind _wbp_partyroster_alwaysvisible (Variables|/Game/03PlayerController/WBP_HudGameplay_UI.WBP_HudGameplay_UI_C|GetWBP_PartyRoster-AlwaysVisible _widget_wbphudgameplayui))
  (Utilities|IsValid (Variables|00PcBase|GetWidget_WBPPartyRosterUI)
    (:Is%20Valid
      (return (Variables|00PcBase|GetWidget_WBPPartyRosterUI)))
    (:Is%20Not%20Valid
      (Utilities|IsValid _wbp_partyroster_alwaysvisible
        (:Is%20Valid
          (bind _output_get (Variables|00PcBase|SetWidget_WBPPartyRosterUI _wbp_partyroster_alwaysvisible))
          (return _output_get))
        (:Is%20Not%20Valid
          (bind _returnvalue (UserInterface|CreateWidget "/Game/xDc03PlayerControllerGame/PlayerIsometricSolo/WBP_PartyRoster00Main_UI.WBP_PartyRoster00Main_UI_C"))
          (bind _output_get_2 (Variables|00PcBase|SetWidget_WBPPartyRosterUI _returnvalue))
          (bind _widget_wbphudgameplayui_2 (CallFunction|WidgetHUDGameplayUI))
          (Widget|Panel|AddChild (Variables|/Game/03PlayerController/WBP_HudGameplay_UI.WBP_HudGameplay_UI_C|GetWidgetSwitcher_Parent _widget_wbphudgameplayui_2) _output_get_2)
          (return _output_get_2))))))

(fn CameraCameraPerspectiveModeF
  (params (Selection :type E_CameraPerspectiveMode-Fps3rdIso%20Enum :default "NewEnumerator0") (PossessedPawn :type Pawn%20Object%20Reference))
  ;[1 1 1] CameraSettings
  (bind _output_get (Variables|00PcBase|SetCameraPerspectiveMode Selection))
  (Class|BPICharacterBaseInterface|CBICameraPerspectiveSetI(Message) PossessedPawn _output_get)
  (switch Utilities|FlowControl|Switch|SwitchonE_CameraPerspectiveMode-Fps3rdIso (Variables|00PcBase|GetCameraPerspectiveMode)
    (:NewEnumerator1
      (Pawn|SetControlRotation (Math|Rotator|MakeRotator 0.0 0.0 0.0)))
    (:NewEnumerator2
      (Pawn|SetControlRotation (Math|Rotator|MakeRotator 0.0 0.0 0.0)))
    (:NewEnumerator3
      (Pawn|SetControlRotation (Math|Rotator|MakeRotator 0.0 -55.0 0.0) :!label _label))
    (:NewEnumerator5
      (goto _label))))

(fn SelectionIsometricHoverHighlightSelectionTickF
  (bind _output_get (LocalVariables|SetHitActor_Local (.HitActor (Collision|BreakHitResult (.HitResult (Class|PlayerController|GetHitResultUnderCursorforObjects (Utilities|Array|MakeArray "ObjectTypeQuery3" "ObjectTypeQuery8") true))))))
  (Utilities|IsValid _output_get
    (:Is%20Valid
      (Utilities|IsValid (Variables|00PcBase|GetSelectable-InteractableActorOrDialogueablePawn)
        (:Is%20Valid
          (if (not (== (Variables|00PcBase|GetSelectable-InteractableActorOrDialogueablePawn) (LocalVariables|GetHitActor_Local)))
            ;[1 1 1] Previous EndHover
            (Class|BPICharacterBaseInterface|CPIOutlineEndHoverActorI(Message) (Variables|00PcBase|GetSelectable-InteractableActorOrDialogueablePawn))
            ;[1 1 1] New BeginHover
            (bind _output_get_2 (Variables|00PcBase|SetSelectable-InteractableActorOrDialogueablePawn (LocalVariables|GetHitActor_Local)))
            (Class|BPICharacterBaseInterface|CPIOutlineBeginHoverActorI(Message) _output_get_2)))
        (:Is%20Not%20Valid
          ;[1 1 1] New BeginHover
          (bind _output_get_3 (Variables|00PcBase|SetSelectable-InteractableActorOrDialogueablePawn (LocalVariables|GetHitActor_Local)))
          (Class|BPICharacterBaseInterface|CPIOutlineBeginHoverActorI(Message) _output_get_3))))
    (:Is%20Not%20Valid
      ;[1 1 1] EndHover
      (Utilities|IsValid (Variables|00PcBase|GetSelectable-InteractableActorOrDialogueablePawn)
        (:Is%20Valid
          (Class|BPICharacterBaseInterface|CPIOutlineEndHoverActorI(Message) (Variables|00PcBase|GetSelectable-InteractableActorOrDialogueablePawn))
          ;;[1 1 1] Clear
          (Variables|00PcBase|SetSelectable-InteractableActorOrDialogueablePawn 0))))))

(fn WidgetGameplayMenuUI
  (params (EWidgetGameplayMenuUI :type E_WidgetGameplayMenuUI%20Enum :default "NewEnumerator0"))
  (bind _widget_wbphudgameplayui (Variables|00PcBase|GetWidget_WBPHudGameplayUI))
  (bind _widget_wbphudgameplayui_2 (Variables|00PcBase|GetWidget_WBPHudGameplayUI))
  (bind _widget_wbphudgameplayui_3 (Variables|00PcBase|GetWidget_WBPHudGameplayUI))
  (bind _widget_wbphudgameplayui_4 (Variables|00PcBase|GetWidget_WBPHudGameplayUI))
  (bind _widget_wbphudgameplayui_5 (Variables|00PcBase|GetWidget_WBPHudGameplayUI))
  (bind _widgetswitcher_parent (Variables|/Game/03PlayerController/WBP_HudGameplay_UI.WBP_HudGameplay_UI_C|GetWidgetSwitcher_Parent _widget_wbphudgameplayui))
  (bind _widgetswitcher_parent_2 (Variables|/Game/03PlayerController/WBP_HudGameplay_UI.WBP_HudGameplay_UI_C|GetWidgetSwitcher_Parent _widget_wbphudgameplayui_2))
  (bind _widgetswitcher_parent_3 (Variables|/Game/03PlayerController/WBP_HudGameplay_UI.WBP_HudGameplay_UI_C|GetWidgetSwitcher_Parent _widget_wbphudgameplayui_3))
  (bind _w_dialogueconversation (Variables|/Game/03PlayerController/WBP_HudGameplay_UI.WBP_HudGameplay_UI_C|GetW_DialogueConversation _widget_wbphudgameplayui_4))
  (bind _w_journalquesting (Variables|/Game/03PlayerController/WBP_HudGameplay_UI.WBP_HudGameplay_UI_C|GetW_JournalQuesting _widget_wbphudgameplayui_5))
  (LocalVariables|SetWidgetUI_Desired_Local EWidgetGameplayMenuUI)
  ;[1 1 1] Current==Desired
  (if (Utilities|Enum|Equal(Enum) (Variables|00PcBase|GetWidgetUI_Current) (LocalVariables|GetWidgetUI_Desired_Local))
    (LocalVariables|SetWidgetUI_Desired_Local "NewEnumerator1"))
  (switch Utilities|FlowControl|Switch|SwitchonE_WidgetGameplayMenuUI (LocalVariables|GetWidgetUI_Desired_Local)
    (:NewEnumerator1
      ;[1 1 1] Default
      (Widget|SetVisibility _widgetswitcher_parent "SelfHitTestInvisible")
      (Class|WidgetSwitcher|SetActiveWidget _widgetswitcher_parent (Variables|/Game/03PlayerController/WBP_HudGameplay_UI.WBP_HudGameplay_UI_C|GetW_Default _widget_wbphudgameplayui))
      (Variables|00PcBase|SetWidgetUI_Current "NewEnumerator1"))
    (:NewEnumerator2
      (Widget|SetVisibility _widgetswitcher_parent_3 "SelfHitTestInvisible")
      ;[1 1 1] StatRoster
      (Class|WidgetSwitcher|SetActiveWidget _widgetswitcher_parent_3 (Variables|/Game/03PlayerController/WBP_HudGameplay_UI.WBP_HudGameplay_UI_C|GetWBP_StatRoster _widget_wbphudgameplayui_3))
      (bind _output_get (Variables|00PcBase|SetWidgetUI_Current "NewEnumerator2")))
    (:NewEnumerator3
      (Widget|SetVisibility _widgetswitcher_parent_2 "SelfHitTestInvisible")
      ;[1 1 1] SkillTreeRoster
      (Class|WidgetSwitcher|SetActiveWidget _widgetswitcher_parent_2 (Variables|/Game/03PlayerController/WBP_HudGameplay_UI.WBP_HudGameplay_UI_C|GetWBP_SkillTree00RosterMain _widget_wbphudgameplayui_2))
      (bind _output_get_2 (Variables|00PcBase|SetWidgetUI_Current "NewEnumerator3")))
    (:NewEnumerator4
      (Widget|SetVisibility _w_dialogueconversation "SelfHitTestInvisible")
      (Class|WidgetSwitcher|SetActiveWidget (Variables|/Game/03PlayerController/WBP_HudGameplay_UI.WBP_HudGameplay_UI_C|GetWidgetSwitcher_Parent _widget_wbphudgameplayui_4) _w_dialogueconversation)
      (bind _output_get_3 (Variables|00PcBase|SetWidgetUI_Current "NewEnumerator4")))
    (:NewEnumerator5
      (Widget|SetVisibility _w_journalquesting "SelfHitTestInvisible")
      (Class|WidgetSwitcher|SetActiveWidget (Variables|/Game/03PlayerController/WBP_HudGameplay_UI.WBP_HudGameplay_UI_C|GetWidgetSwitcher_Parent _widget_wbphudgameplayui_5) _w_journalquesting)
      (bind _output_get_4 (Variables|00PcBase|SetWidgetUI_Current "NewEnumerator5")))))

(fn PcBICameraPerspectiveModeGETI
  (return (Variables|00PcBase|GetCameraPerspectiveMode)))

(fn PcBIHUDGameplayUIGETI-notactualyUsedQ
  (return (Variables|00PcBase|GetWidget_WBPHudGameplayUI)))

(fn PcBIRtsIsoHoverActorGETI
  (return (Variables|00PcBase|GetSelectable-InteractableActorOrDialogueablePawn)))

(fn PcBIRtsIsoMouseCursorActorGETI
  (bind _bp_manager_squadselectioninteractcamera_ac (Variables|Default|GetBP_Manager-SquadSelectionInteractCamera_AC))
  (bind _rtsisomousecursoractor (Variables|/Game/03PlayerController/BP_Manager-SquadSelectionInteractCamera_AC.BP_Manager-SquadSelectionInteractCamera_AC_C|GetRtsIsoMouseCursorActor _bp_manager_squadselectioninteractcamera_ac))
  (Utilities|IsValid _bp_manager_squadselectioninteractcamera_ac
    (:Is%20Valid
      (Utilities|IsValid _rtsisomousecursoractor
        (:Is%20Valid
          (return _rtsisomousecursoractor))
        (:Is%20Not%20Valid
          (Development|PrintString "BPPlayerControllerMasterPC>PCRtsIsoMouseCursorActorGETI==RtsIsoMouseCursorActor is not valid" true true "(R=1.000000,G=0.554357,B=0.000000,A=1.000000)" 22.0))))))

(fn PcBISquadMemberLoadoutCharactersGETI
  (return (Variables|/Game/03PlayerController/BP_Manager-SquadSelectionInteractCamera_AC.BP_Manager-SquadSelectionInteractCamera_AC_C|GetSquadLoadoutCharacters (Variables|Default|GetBP_Manager-SquadSelectionInteractCamera_AC))))

(fn PcBISquadMemeberbyIdNameGETI
  (params (CharacterPresetID :type Primary%20Data%20Asset%20Object%20Reference))
  (return 0 false))