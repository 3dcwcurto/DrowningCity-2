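; Master player controller Blueprint whose BeginPlay, Tick and Possess events only forward to its parent class.
; It retains an old gameplay-menu function, marked as moved, whose only calls here are disconnected.
; That function switches the HUD widget switcher between stat roster, skill tree and dialogue, collapsing it when the current menu is requested again.
; The collapse branch leaves the current-menu state unchanged, as the party roster reset is disconnected.
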(event EventBeginPlay
  (|CallParentFunction))

(event EventTick
  (params (DeltaSeconds :type Float%20%28single-precision%29))
  (|CallParentFunction DeltaSeconds))

(event EventPossess
  (params (PossessedPawn :type Pawn%20Object%20Reference))
  (|CallParentFunction PossessedPawn))

(fn ConstructionScript)

(fn WidgetGameplayMenuUIF-oldMoved
  (params (EWidgetGameplayMenuUI :type E_WidgetGameplayMenuUI%20Enum :default "NewEnumerator0"))
  (bind _widget_wbphudgameplayui (Variables|Default|GetWidget_WBPHudGameplayUI))
  (bind _widgetswitcher_parent (Variables|/Game/03PlayerController/WBP_HudGameplay_UI.WBP_HudGameplay_UI_C|GetWidgetSwitcher_Parent _widget_wbphudgameplayui))
  (bind _w_dialogueconversation (Variables|/Game/03PlayerController/WBP_HudGameplay_UI.WBP_HudGameplay_UI_C|GetW_DialogueConversation _widget_wbphudgameplayui))
  (LocalVariables|SetWidgetUI_Desired_Local EWidgetGameplayMenuUI)
  ;[1 1 1] Current==Desired
  (if (Utilities|Enum|Equal(Enum) (Variables|Default|GetWidgetUI_Current-oldMoved) (LocalVariables|GetWidgetUI_Desired_Local))
    (LocalVariables|SetWidgetUI_Desired_Local "NewEnumerator1"))
  (switch Utilities|FlowControl|Switch|SwitchonE_WidgetGameplayMenuUI (LocalVariables|GetWidgetUI_Desired_Local)
    (:NewEnumerator1
      (Widget|SetVisibility _widgetswitcher_parent "Collapsed"))
    (:NewEnumerator2
      (Widget|SetVisibility _widgetswitcher_parent "SelfHitTestInvisible")
      ;[1 1 1] StatRoster
      (Class|WidgetSwitcher|SetActiveWidget _widgetswitcher_parent (Variables|/Game/03PlayerController/WBP_HudGameplay_UI.WBP_HudGameplay_UI_C|GetWBP_StatRoster _widget_wbphudgameplayui))
      (bind _output_get (Variables|Default|SetWidgetUI_Current-oldMoved "NewEnumerator2"))
      (Development|PrintString (Utilities|String|EnumtoString _output_get) true true "(R=0.000000,G=1.000000,B=0.014685,A=1.000000)"))
    (:NewEnumerator3
      (Widget|SetVisibility _widgetswitcher_parent "SelfHitTestInvisible")
      ;[1 1 1] SkillTreeRoster
      (Class|WidgetSwitcher|SetActiveWidget _widgetswitcher_parent (Variables|/Game/03PlayerController/WBP_HudGameplay_UI.WBP_HudGameplay_UI_C|GetWBP_SkillTree00RosterMain _widget_wbphudgameplayui))
      (bind _output_get_2 (Variables|Default|SetWidgetUI_Current-oldMoved "NewEnumerator3"))
      (Development|PrintString (Utilities|String|EnumtoString _output_get_2) true true "(R=0.000000,G=1.000000,B=0.014685,A=1.000000)"))
    (:NewEnumerator4
      (Widget|SetVisibility _w_dialogueconversation "SelfHitTestInvisible")
      (Class|WidgetSwitcher|SetActiveWidget _widgetswitcher_parent _w_dialogueconversation)
      (Variables|Default|SetWidgetUI_Current-oldMoved "NewEnumerator4"))))