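; Player controller layer that routes stat, skill tree and buff/debuff UI updates to the right party member's widgets.
; On BeginPlay it finds or creates the stat roster and skill tree roster widgets under the gameplay HUD.
; Interface events look up the member's slot via parallel reference arrays, checking the match, then forward data to that widget.
; Skill and knowledge updates also resolve their owning tree; buff updates target party portrait slots.
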(event EventBeginPlay
  ;[0.251 1 0] BeginPlay
  (|CallParentFunction)
  ;;[1 1 1] UI
  (CallFunction|StatRosterWidgetStatRosterMainUICreateF)
  (CallFunction|SkillTreeRosterWidgetTreeRosterMainUICreateF))

(event EventTick
  (params (DeltaSeconds :type Float%20%28single-precision%29))
  (|CallParentFunction DeltaSeconds))

(event EventPCSIStatAdvancedTickUII
  (params (AdvancedPanel :type S%20Advanced%20Stat%2001%20Advanced%20Panel%20Structure) (AdvancedEntry :type S%20Advanced%20Stat%2002%20Advanced%20Entry%20Structure) (Character_PartyMember :type Character%20Object%20Reference))
  ;[0.4247 1 0.4408] AdvancedTick
  (bind _wbpstatrosterslotcharacter (CallFunction|StatRosterWidgetGETF Character_PartyMember))
  (Default|AdvancedStat-Tick-UICE _wbpstatrosterslotcharacter AdvancedPanel AdvancedEntry))

(event EventPCSISkillTree-TREE(VocationUtilitySurivalEct)UpdateUII
  (params (AppliedPanel :type S%20Core%20Stat%2001%20Applied%20Panel%20Structure) (AppliedEntry :type S%20Core%20Stat%2002%20Applied%20Entry%20Structure) (OriginPanel :type S%20Core%20Stat%2003%20Origin%20Panel%20Structure) (OriginEntry :type S%20Core%20Stat%2004%20Origin%20Entry%20Structure) (Character_PartyMember :type Character%20Object%20Reference))
  ;[1 1 1] SkillTree
  ;;[1 1 1] Tree Update
  (bind _wbpskilltreerosterslotcharacter (CallFunction|SkillTreeRosterWidgetGetF Character_PartyMember))
  (Utilities|IsValid _wbpskilltreerosterslotcharacter
    (:Is%20Valid
      (Default|SkillTreeTree(VocationUtilitySurvivalect)Update-UICE _wbpskilltreerosterslotcharacter AppliedPanel AppliedEntry OriginPanel OriginEntry))))

(event EventPCSISkillTree-SKILL(PerkAugFeatEct)UpdateUII
  (params (AppliedPanel :type S%20Core%20Stat%2001%20Applied%20Panel%20Structure) (AppliedEntry :type S%20Core%20Stat%2002%20Applied%20Entry%20Structure) (OriginPanel :type S%20Core%20Stat%2003%20Origin%20Panel%20Structure) (OriginEntry :type S%20Core%20Stat%2004%20Origin%20Entry%20Structure) (Character_PartyMember :type Character%20Object%20Reference))
  (bind (_appliedpanel_treeowner _appliedentry_treeowner) (CallFunction|SkillTreeSKILLGetOwningTreePureF AppliedEntry))
  ;[1 1 1] SkillTree
  ;;[1 1 1] SkillUpdate
  (bind _wbpskilltreerosterslotcharacter (CallFunction|SkillTreeRosterWidgetGetF Character_PartyMember))
  (Utilities|IsValid _wbpskilltreerosterslotcharacter
    (:Is%20Valid
      (Default|SkillTreeSkill(PerkAugFeatEct)UpdateCE _wbpskilltreerosterslotcharacter AppliedPanel AppliedEntry OriginPanel OriginEntry _appliedpanel_treeowner _appliedentry_treeowner))))

(event EventPCSISKillTree-BlankSkillConfigureUII-dontNeed
  (params (AppliedPanel :type S%20Core%20Stat%2001%20Applied%20Panel%20Structure) (AppliedEntry :type S%20Core%20Stat%2002%20Applied%20Entry%20Structure) (OriginPanel :type S%20Core%20Stat%2003%20Origin%20Panel%20Structure) (OriginEntry :type S%20Core%20Stat%2004%20Origin%20Entry%20Structure) (Character_PartyMember :type Character%20Object%20Reference) (Tree_AppliedPanel :type S%20Core%20Stat%2001%20Applied%20Panel%20Structure) (Tree_AppliedEntry :type S%20Core%20Stat%2002%20Applied%20Entry%20Structure))
  ;[1 1 1] SkillTree
  (bind _wbpskilltreerosterslotcharacter (CallFunction|SkillTreeRosterWidgetGetF Character_PartyMember))
  (Default|SkillTreeBlankSkillConfigure-UICE _wbpskilltreerosterslotcharacter AppliedPanel AppliedEntry OriginPanel OriginEntry false Tree_AppliedPanel Tree_AppliedEntry false))

(event EventPCSISkillTree-KnowledgeLearnUII
  (params (AppliedPanel :type S%20Core%20Stat%2001%20Applied%20Panel%20Structure) (AppliedEntry :type S%20Core%20Stat%2002%20Applied%20Entry%20Structure) (OriginPanel :type S%20Core%20Stat%2003%20Origin%20Panel%20Structure) (OriginEntry :type S%20Core%20Stat%2004%20Origin%20Entry%20Structure) (Character_PartyMember :type Character%20Object%20Reference))
  (bind (_appliedpanel_treeowner _appliedentry_treeowner) (CallFunction|SkillTreeSKILLGetOwningTreePureF AppliedEntry))
  ;[1 1 1] SkillTree
  ;;[1 1 1] Knowledge
  (bind _wbpskilltreerosterslotcharacter (CallFunction|SkillTreeRosterWidgetGetF Character_PartyMember))
  (Utilities|IsValid _wbpskilltreerosterslotcharacter
    (:Is%20Valid
      (Default|SkillTreeKnowledgeUpdateCE _wbpskilltreerosterslotcharacter AppliedPanel AppliedEntry OriginPanel OriginEntry _appliedpanel_treeowner _appliedentry_treeowner))))

(event EventPCSISkillTree-BoonAddUII
  (params (AppliedPanel :type S%20Core%20Stat%2001%20Applied%20Panel%20Structure) (AppliedEntry :type S%20Core%20Stat%2002%20Applied%20Entry%20Structure) (OriginPanel :type S%20Core%20Stat%2003%20Origin%20Panel%20Structure) (OriginEntry :type S%20Core%20Stat%2004%20Origin%20Entry%20Structure) (Character_PartyMember :type Character%20Object%20Reference))
  ;[1 1 1] SkillTree
  ;;[1 1 1] Boons&Curses&Ect
  (bind _wbpskilltreerosterslotcharacter (CallFunction|SkillTreeRosterWidgetGetF Character_PartyMember))
  (Utilities|IsValid _wbpskilltreerosterslotcharacter
    (:Is%20Valid
      (Default|BoonsCursesUpdate-UICE _wbpskilltreerosterslotcharacter AppliedPanel AppliedEntry OriginPanel OriginEntry))))

(event EventPCSISkillTree-MemoryLengthUpdateUII
  (params (AppliedPanel :type S%20Core%20Stat%2001%20Applied%20Panel%20Structure) (AppliedEntry :type S%20Core%20Stat%2002%20Applied%20Entry%20Structure) (OriginPanel :type S%20Core%20Stat%2003%20Origin%20Panel%20Structure) (OriginEntry :type S%20Core%20Stat%2004%20Origin%20Entry%20Structure) (Character_PartyMember :type Character%20Object%20Reference))
  ;[1 1 1] SkillTree
  ;;[1 1 1] MemoryLength
  (bind _wbpskilltreerosterslotcharacter (CallFunction|SkillTreeRosterWidgetGetF Character_PartyMember))
  (Utilities|IsValid _wbpskilltreerosterslotcharacter
    (:Is%20Valid
      (Default|MemoryLengthUpdate-UICE _wbpskilltreerosterslotcharacter AppliedPanel AppliedEntry OriginPanel OriginEntry))))

(event EventPCSISkillTree-WeaponArtUpdateUII
  (params (AppliedPanel :type S%20Core%20Stat%2001%20Applied%20Panel%20Structure) (AppliedEntry :type S%20Core%20Stat%2002%20Applied%20Entry%20Structure) (OriginPanel :type S%20Core%20Stat%2003%20Origin%20Panel%20Structure) (OriginEntry :type S%20Core%20Stat%2004%20Origin%20Entry%20Structure) (Character_PartyMember :type Character%20Object%20Reference))
  ;[1 1 1] SkillTree
  (bind _wbpskilltreerosterslotcharacter (CallFunction|SkillTreeRosterWidgetGetF Character_PartyMember))
  (Utilities|IsValid _wbpskilltreerosterslotcharacter
    (:Is%20Valid
      (Default|WeaponArtLength-UICE _wbpskilltreerosterslotcharacter AppliedPanel AppliedEntry OriginPanel OriginEntry))))

(event EventPCSISkillTree-MemoryDragDropUpdateUII
  (params (MemoryEntryP :type S%20Memory%2002%20Entry%20P%20Structure) (MemoryBlockE :type S%20Memory%2003%20Block%20E%20Structure) (Character_PartyMember :type Character%20Object%20Reference) (MemoryResult-ClearVsUpdate :type E_GenericUpdateResult-ClearVsUpdate%20Enum :default "NewEnumerator1"))
  ;[1 1 1] SkillTree
  ;;[1 1 1] MemoryDrop Update
  (bind _wbpskilltreerosterslotcharacter (CallFunction|SkillTreeRosterWidgetGetF Character_PartyMember))
  (Utilities|IsValid _wbpskilltreerosterslotcharacter
    (:Is%20Valid
      (Default|SkillTreeMemoryDragDropUpdate-UICE _wbpskilltreerosterslotcharacter MemoryEntryP MemoryBlockE MemoryResult-ClearVsUpdate))))

(event EventPCSIStatCoreUpdateUII
  (params (01AppliedPanel :type S%20Core%20Stat%2001%20Applied%20Panel%20Structure) (02AppliedCore :type S%20Core%20Stat%2002%20Applied%20Entry%20Structure) (03OriginPanel :type S%20Core%20Stat%2003%20Origin%20Panel%20Structure) (04OriginCore :type S%20Core%20Stat%2004%20Origin%20Entry%20Structure) (Character_PartyMember :type Character%20Object%20Reference))
  ;[1 1 1] StatCore:AppliedEntry
  (bind _wbpstatrosterslotcharacter (CallFunction|StatRosterWidgetGETF Character_PartyMember))
  (Default|StatAppliedCoreUpdateCE _wbpstatrosterslotcharacter 01AppliedPanel 02AppliedCore 03OriginPanel 04OriginCore))

(event EventPossess
  (params (PossessedPawn :type Pawn%20Object%20Reference))
  ;[0.251 1 0] BeginPlay
  (|CallParentFunction PossessedPawn))

(event EventPCSISkillTree-BlankTreeConfigureUII-replaced
  (params (CorePanel :type S%20Core%20Stat%2001%20Applied%20Panel%20Structure) (CoreEntry :type S%20Core%20Stat%2002%20Applied%20Entry%20Structure) (SkillTree_BlankTree :type Boolean) (Character_PartyMember :type Character%20Object%20Reference))
  ;[1 1 1] SkillTree
  (bind _wbpskilltreerosterslotcharacter (CallFunction|SkillTreeRosterWidgetGetF Character_PartyMember))
  (Default|SkillTreeBlankTreeConfigure-UI(CLIENT)CE :self _wbpskilltreerosterslotcharacter :AppliedPanel CorePanel :AppliedEntry CoreEntry))

(event EventPCSIBuffDebuffUpdateStackUII
  (params (AppliedEntryBuff :type S%20Buff%20Core%2001%20Applied%20Entry%20Buff%20Structure) (Character_PartyMember :type Character%20Object%20Reference))
  ;[1 1 1] Buff
  (bind (_wbp_buffdebuffportraitprogress00layout _wbp_partyslot _valid) (CallFunction|PartyRosterWidetGETF-MovetoPartySquadPC? Character_PartyMember))
  (if _valid
    (Default|StatBuffDebuff-UpdateStackCE _wbp_buffdebuffportraitprogress00layout AppliedEntryBuff (Variables|00PcStats|GetBuffDebuffPortriatProgress_DimensionRowMax_RuleSetting))))

(event EventPCSIBuffDebuffTickUpdateUII
  (params (AppliedEntryBuff :type S%20Buff%20Core%2001%20Applied%20Entry%20Buff%20Structure) (CharacterPartyMember :type Character%20Object%20Reference))
  ;[1 1 1] Buff
  (bind (_wbp_buffdebuffportraitprogress00layout _wbp_partyslot _valid) (CallFunction|PartyRosterWidetGETF-MovetoPartySquadPC? CharacterPartyMember))
  (if _valid
    (Default|BuffDebuff-TickUpdateCE _wbp_buffdebuffportraitprogress00layout AppliedEntryBuff)))

(event EventPCSIStatDetailGroupDetailBaseUpdateUII
  (params (1ComboStartPanel :type S%20Detail%20Stat%2001%20Detail%20Panel%20Structure) (2ComboDetailCategory :type S%20Detail%20Stat%2002%20Detail%20Category%20Structure) (3ComboDetailGroup :type S%20Detail%20Stat%2003%20Detail%20Group%20Structure) (4ComboDetailEntry :type S%20Detail%20Stat%2005%20Detail%20Entry%20Structure) (Character_PartyMember :type Character%20Object%20Reference) (6SourcePanel :type S%20Detail%20Stat%2006%20Source%20Panel%20Structure) (7SourceEntry :type S%20Detail%20Stat%2007%20Source%20Entry%20Structure))
  ;[1 1 1] DetailGroup:DetailBase
  (bind _wbpstatrosterslotcharacter (CallFunction|StatRosterWidgetGETF Character_PartyMember))
  (Default|ComboStat-DetailGroupDetailBaseUpdate-UI(CLIENT)CE _wbpstatrosterslotcharacter 1ComboStartPanel 2ComboDetailCategory 3ComboDetailGroup 4ComboDetailEntry 6SourcePanel 7SourceEntry))

(event EventPCSIBuffDebuffDebuggingUII
  (params (01AppliedEntryBuff :type S%20Buff%20Core%2001%20Applied%20Entry%20Buff%20Structure) (02OriginEntryBuff :type S%20Buff%20Core%2002%20Origin%20Entry%20Buff%20Structure) (Character_PartyMember :type Character%20Object%20Reference))
  ;[1 1 1] Buff
  ;;[0.4948 0.4948 0.4948] BuffCoreDebugging
  ;;;[1 1 1 1 12] Note indexes of buffs can accidently overide the index of a statCore
  (bind _wbpstatrosterslotcharacter (CallFunction|StatRosterWidgetGETF Character_PartyMember))
  (Default|BuffDebuffDebuggingCE _wbpstatrosterslotcharacter 01AppliedEntryBuff 02OriginEntryBuff))

(event EventPCSIStatAdvancedUpdateUII
  (params (AdvancedPanel :type S%20Advanced%20Stat%2001%20Advanced%20Panel%20Structure) (AdvancedEntry :type S%20Advanced%20Stat%2002%20Advanced%20Entry%20Structure) (StatisticDetailGroup :type S%20Advanced%20Stat%2003%20Statistic%20Detail%20Group%20Structure) (StatisticDetailEntry :type Boolean) (Character_PartyMember :type Character%20Object%20Reference))
  ;[1 1 1] AdvancedStat
  (bind _wbpstatrosterslotcharacter (CallFunction|StatRosterWidgetGETF Character_PartyMember))
  (Default|AdvancedStat-Update-UICE _wbpstatrosterslotcharacter AdvancedPanel AdvancedEntry StatisticDetailGroup StatisticDetailEntry))

(event EventPCSIStatDetailEntrySupportingNDependentUpdateUII
  (params (1ComboStartPanel :type S%20Detail%20Stat%2001%20Detail%20Panel%20Structure) (2ComboDetailCategory :type S%20Detail%20Stat%2002%20Detail%20Category%20Structure) (3ComboDetailGroup :type S%20Detail%20Stat%2003%20Detail%20Group%20Structure) (4ComboDetailIntermediate :type S%20Detail%20Stat%2004%20Detail%20Intermeidate%20Structure) (5ComboDetailEntry :type S%20Detail%20Stat%2005%20Detail%20Entry%20Structure) (6SourcePanel :type S%20Detail%20Stat%2006%20Source%20Panel%20Structure) (7SourceEntry :type S%20Detail%20Stat%2007%20Source%20Entry%20Structure) (Character_PartyMember :type Character%20Object%20Reference))
  ;[1 1 1] DetailDependent&DetailSupporting
  (bind _wbpstatrosterslotcharacter (CallFunction|StatRosterWidgetGETF Character_PartyMember))
  (Default|ComboStat-DetailSupportingDependentUpdate-UI(CLIENT)CE _wbpstatrosterslotcharacter 1ComboStartPanel 2ComboDetailCategory 3ComboDetailGroup 4ComboDetailIntermediate 5ComboDetailEntry 6SourcePanel 7SourceEntry))

(fn ConstructionScript)

(fn StatRosterWidgetCharacterSlotSelectF-reworktoShowAllatOnce
  (params (CharacterPossessed :type Character%20Object%20Reference%20%28by%20ref%29))
  (bind _wbpstatrosterslotcharacter (CallFunction|StatRosterWidgetGETF CharacterPossessed))
  (Class|WidgetSwitcher|SetActiveWidget (Variables|/Game/02CharacterBP/003StatsChar/01CoreStats/WBP_StatRoster00Main.WBP_StatRoster00Main_C|GetWidgetSwitcher_ParentRoster-old (Variables|00PcStats|GetWidget_WBPStatRoster_UI)) _wbpstatrosterslotcharacter))

(fn StatRosterWidgetStatRosterMainUICreateF
  (bind _widget_wbphudgameplayui (Variables|Default|GetWidget_WBPHudGameplayUI))
  (bind _wbp_statroster (Variables|/Game/03PlayerController/WBP_HudGameplay_UI.WBP_HudGameplay_UI_C|GetWBP_StatRoster _widget_wbphudgameplayui))
  (Utilities|IsValid (Variables|00PcStats|GetWidget_WBPStatRoster_UI)
    (:Is%20Valid
      (return (Variables|00PcStats|GetWidget_WBPStatRoster_UI)))
    (:Is%20Not%20Valid
      (Utilities|IsValid _wbp_statroster
        (:Is%20Valid
          (bind _output_get (Variables|00PcStats|SetWidget_WBPStatRoster_UI _wbp_statroster))
          (return _output_get))
        (:Is%20Not%20Valid
          (bind _returnvalue (UserInterface|CreateWidget "/Game/02CharacterBP/003StatsChar/01CoreStats/WBP_StatRoster00Main.WBP_StatRoster00Main_C"))
          (bind _output_get_2 (Variables|00PcStats|SetWidget_WBPStatRoster_UI _returnvalue))
          (bind _widget_wbphudgameplayui_2 (CallFunction|WidgetHUDGameplayUI))
          (Widget|Panel|AddChild (Variables|/Game/03PlayerController/WBP_HudGameplay_UI.WBP_HudGameplay_UI_C|GetWidgetSwitcher_Parent _widget_wbphudgameplayui_2) _output_get_2)
          (return _output_get_2))))))

(fn SkillTreeRosterWidgetTreeRosterMainUICreateF
  (bind _widget_wbphudgameplayui (Variables|Default|GetWidget_WBPHudGameplayUI))
  (bind _wbp_skilltree00rostermain (Variables|/Game/03PlayerController/WBP_HudGameplay_UI.WBP_HudGameplay_UI_C|GetWBP_SkillTree00RosterMain _widget_wbphudgameplayui))
  (Utilities|IsValid (Variables|00PcStats|GetWidget_WBPSkillTreeRoster_UI)
    (:Is%20Valid
      (return (Variables|00PcStats|GetWidget_WBPSkillTreeRoster_UI)))
    (:Is%20Not%20Valid
      (Utilities|IsValid _wbp_skilltree00rostermain
        (:Is%20Valid
          (bind _output_get (Variables|00PcStats|SetWidget_WBPSkillTreeRoster_UI _wbp_skilltree00rostermain))
          (return _output_get))
        (:Is%20Not%20Valid
          (bind _returnvalue (UserInterface|CreateWidget "/Game/02CharacterBP/003StatsChar/01CoreStats/CoreTree/WBP_SkillTree00RosterMain.WBP_SkillTree00RosterMain_C"))
          (bind _output_get_2 (Variables|00PcStats|SetWidget_WBPSkillTreeRoster_UI _returnvalue))
          (bind _widget_wbphudgameplayui_2 (CallFunction|WidgetHUDGameplayUI))
          (Widget|Panel|AddChild (Variables|/Game/03PlayerController/WBP_HudGameplay_UI.WBP_HudGameplay_UI_C|GetWidgetSwitcher_Parent _widget_wbphudgameplayui_2) _output_get_2)
          (return _output_get_2))))))

(fn PartyRosterWidetGETF-MovetoPartySquadPC?
  (params (character :type Character%20Object%20Reference))
  (bind _widget_wbppartyrosterui (Variables|Default|GetWidget_WBPPartyRosterUI))
  (bind _characterreference_array (Variables|/Game/xDc03PlayerControllerGame/PlayerIsometricSolo/WBP_PartyRoster00Main_UI.WBP_PartyRoster00Main_UI_C|GetCharacterReference_Array _widget_wbppartyrosterui))
  (bind _characterslot_array (Variables|/Game/xDc03PlayerControllerGame/PlayerIsometricSolo/WBP_PartyRoster00Main_UI.WBP_PartyRoster00Main_UI_C|GetCharacterSlot_Array _widget_wbppartyrosterui))
  (bind _returnvalue (Utilities|Array|FindItem _characterreference_array character))
  (bind _output (Utilities|Array|Get(acopy) _characterslot_array _returnvalue))
  (Utilities|IsValid _output
    (:Is%20Valid
      (if (== character (Variables|/Game/xDc03PlayerControllerGame/PlayerIsometricSolo/WBP_PartyRoster01Character_UI.WBP_PartyRoster01Character_UI_C|GetCharacterReference _output))
        (return (Variables|/Game/xDc03PlayerControllerGame/PlayerIsometricSolo/WBP_PartyRoster01Character_UI.WBP_PartyRoster01Character_UI_C|GetWBP_BuffDebuffPortraitProgress00Layout _output) _output true)
        (else
          (Development|PrintString "BPPlayerControlllerStats>GetCharacterRosterSlotF== Slot Index Widget  reference does not match " true true "(R=1.000000,G=0.711823,B=0.000000,A=1.000000)")
          (return 0 0 false))))
    (:Is%20Not%20Valid
      (Development|PrintString "BPPlayerControlllerStats>GetCharacterRosterSlotF== Slot Index Widget is not valid" true true "(R=1.000000,G=0.514614,B=0.000000,A=1.000000)" 22.0)
      (return 0 0 false))))

(fn StatRosterWidgetGETF
  (params (CharacterPartyMember :type Character%20Object%20Reference))
  (bind _widget_wbpstatroster_ui (Variables|00PcStats|GetWidget_WBPStatRoster_UI))
  (bind _characterrostersquadreference_array (Variables|/Game/02CharacterBP/003StatsChar/01CoreStats/WBP_StatRoster00Main.WBP_StatRoster00Main_C|GetCharacterRosterSquadReference_Array _widget_wbpstatroster_ui))
  (bind _statrosterslotcharacter_array (Variables|/Game/02CharacterBP/003StatsChar/01CoreStats/WBP_StatRoster00Main.WBP_StatRoster00Main_C|GetStatRosterSlotCharacter_Array _widget_wbpstatroster_ui))
  (bind _returnvalue (Utilities|Array|FindItem _characterrostersquadreference_array CharacterPartyMember))
  (bind _output (Utilities|Array|Get(acopy) _statrosterslotcharacter_array _returnvalue))
  ;[1 1 1] Proof
  (Utilities|IsValid _output
    (:Is%20Valid
      (if (== CharacterPartyMember (Variables|/Game/02CharacterBP/003StatsChar/01CoreStats/WBP_StatRoster01CharacterSlot.WBP_StatRoster01CharacterSlot_C|GetCharacterReference _output))
        (return _output)
        (else
          (Development|PrintString "BPPlayerControlllerStats>GetStatRosteSlotCharacterF== Slot Index Widget  reference does not match " true true "(R=1.000000,G=0.711823,B=0.000000,A=1.000000)")
          (return 0))))
    (:Is%20Not%20Valid
      (Development|PrintString "BPPlayerControlllerStats>GetStatRosterSlotCharacterF== Slot Index Widget is not valid" true true "(R=1.000000,G=0.514614,B=0.000000,A=1.000000)" 22.0)
      (return 0))))

(fn SkillTreeRosterWidgetGetF
  (params (CharacterPartyMember :type Character%20Object%20Reference%20%28by%20ref%29))
  (bind _widget_wbpskilltreeroster_ui (Variables|00PcStats|GetWidget_WBPSkillTreeRoster_UI))
  (bind _characterreference_array (Variables|/Game/02CharacterBP/003StatsChar/01CoreStats/CoreTree/WBP_SkillTree00RosterMain.WBP_SkillTree00RosterMain_C|GetCharacterReference_Array _widget_wbpskilltreeroster_ui))
  (bind _skilltreeslotcharacter_array (Variables|/Game/02CharacterBP/003StatsChar/01CoreStats/CoreTree/WBP_SkillTree00RosterMain.WBP_SkillTree00RosterMain_C|GetSkillTreeSlotCharacter_Array _widget_wbpskilltreeroster_ui))
  (bind _returnvalue (Utilities|Array|FindItem _characterreference_array CharacterPartyMember))
  (bind _output (Utilities|Array|Get(acopy) _skilltreeslotcharacter_array _returnvalue))
  ;[1 1 1] Proof
  (Utilities|IsValid CharacterPartyMember
    (:Is%20Valid
      (if (== CharacterPartyMember (Variables|/Game/02CharacterBP/003StatsChar/01CoreStats/CoreTree/WBP_SkillTree02SkillBook01LayoutCharaterSlot.WBP_SkillTree02SkillBook01LayoutCharaterSlot_C|GetCharacterReference _output))
        (return _output)
        (else
          (Development|PrintString "BPPlayerControlllerStats>GetSkillTreeSlotCharacterF== Slot Index Widget  reference does not match " true true "(R=1.000000,G=0.711823,B=0.000000,A=1.000000)")
          (return 0))))
    (:Is%20Not%20Valid
      (Development|PrintString "BPPlayerControlllerStats>GetSkillTreeRosterSlotCharacterF== Slot Index Widget is not valid" true true "(R=1.000000,G=0.514614,B=0.000000,A=1.000000)" 22.0)
      (return 0))))

(fn SkillTreeSKILLGetOwningTreePureF
  (params (S_CoreStat02AppliedEntry :type S%20Core%20Stat%2002%20Applied%20Entry%20Structure%20%28by%20ref%29))
  (bind _treeownerruntime (Utilities|Struct|BreakS_CoreStat02AppliedEntry S_CoreStat02AppliedEntry))
  (bind (_appliedpanel _quickindexpanel _appliedentry _quickindexentry) (Utilities|Struct|BreakS_AppliedEntry02TreeOwnerRuntime _treeownerruntime))
  (return (Utilities|Struct|MakeS_CoreStat01AppliedPanel _appliedpanel _quickindexpanel "(())") (Utilities|Struct|MakeS_CoreStat02AppliedEntry _appliedentry _quickindexentry)))