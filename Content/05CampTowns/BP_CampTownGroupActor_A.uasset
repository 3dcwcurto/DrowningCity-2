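; Camp/town actor that groups guards, officers and buildings, registering with the GameState once its preset validates.
; NPC spotted, update and lost-track signals maintain a shared list of targets with last known locations.
; The chasing-NPC list toggles the camp alarm, notifying member AI controllers and the GameMode.
; Work in progress: player-distance activation, building back-references and guard assignment are disconnected or stubbed.
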(event OnComponentBeginOverlap(SpawnActivateTriggerOverlap)
  (params (OverlappedComponent :type Primitive%20Component%20Object%20Reference) (OtherActor :type Actor%20Object%20Reference) (OtherComp :type Primitive%20Component%20Object%20Reference) (OtherBodyIndex :type Integer) (bFromSweep :type Boolean) (SweepResult :type Hit%20Result%20Structure%20%28by%20ref%29))
  ;[1 1 1] BeginOverlap_SpawnTriggerOverlap
)

(event OnComponentEndOverlap(DespawnDeactivateTriggerOverlap)
  (params (OverlappedComponent :type Primitive%20Component%20Object%20Reference) (OtherActor :type Actor%20Object%20Reference) (OtherComp :type Primitive%20Component%20Object%20Reference) (OtherBodyIndex :type Integer))
  ;[1 1 1] EndOverlap_DespawnTriggerOverlap
)

(event Custom|SpawnActivateState_AI_CE
  ;[1 1 1] Activate
)

(event Custom|DeactivateState_AI_CE
  ;[1 1 1] Deactivate
)

(event Custom|AiNpcKilled_CE
  (params (Character :type Character%20Object%20Reference))
  ;[1 0 0.07651] Killed
  (CallFunction|AiNpcKilledF Character))

(event EventCTGIAlertSignalUpdateLocation-CitizenOfCamp-EventSimpleI
  (params (AiNpcWithPerception :type Character%20Object%20Reference) (TargetLockedOn :type Character%20Object%20Reference))
  ;[1 1 1] Events AlertALarmOnOff
  ;;[1 1 1] Update existingTarget
  (AlarmPerception|AlertSignalUpdateLocationGuardtoCampEventF AiNpcWithPerception TargetLockedOn))

(event EventCTGICampTownOfficerDEBUGI
  (params (Debug :type Boolean))
  ;[1 1 1] Debug
  (CallFunction|DebugBillboardIconsF Debug))

(event EventCTGIAlertSignalLostTrack-CitizenOfCamp-EventSimpleI
  (params (AiNpcWithPerception :type Character%20Object%20Reference) (TargetLost :type Character%20Object%20Reference))
  ;[1 1 1] Events AlertALarmOnOff
  (AlarmPerception|AlertSignalLostTrackGuardtoCampEventF AiNpcWithPerception TargetLost))

(event EventBeginPlay
  (bind _camptownpreset (Variables|TownCampPreset|GetCampTownPreset))
  ;[0.2507 1 0] BeginPlay
  (Utilities|IsValid _camptownpreset
    (:Is%20Valid
      (bind _valid (CallFunction|TownCampPresetProofF _camptownpreset))
      (if _valid
        (CallFunction|BeginPlayTownCampGsTFDHFnew)))))

(event EventCTGICampTownCitizenRosterAddI
  (params (Character :type Character%20Object%20Reference))
  ;[1 1 1] CitizenRoster
  (bind _pdacharacterpreset (Class|BPICharacterBaseInterface|CBICharacterPresetPdaGETI(Message) Character)))

(event EventCTGIAlertSignalSpottedEnemy-CizitenOfCamp-EventSimpleI
  (params (AiNpcWithPerception :type Character%20Object%20Reference) (TargetSpotted :type Character%20Object%20Reference))
  ;[1 1 1] Events AlertALarmOnOff
  ;;[1 1 1] New spottedTarget
  ;;;[1 1 1] Todo: check if character is in range of Alarm camp
  (AlarmPerception|AlertSignalSpottedEnemyGuardtoCampEventF AiNpcWithPerception TargetSpotted))

(fn ConstructionScript
  (CallFunction|ConstructBoxExtendF)
  (CallFunction|ConstructNameTextrenderF))

(fn ConstructNameTextrenderF
  (bind _textrender_camptownnameid (Variables|Default|GetTextRender_CampTownNameID))
  (Rendering|Components|TextRender|SetText _textrender_camptownnameid (Utilities|Text|ToText(Name) (GameplayTags|GetTagName (Variables|TownCampPreset|GetCampTownNameID-todoprelace))))
  (Rendering|Components|TextRender|SetTextRenderColor _textrender_camptownnameid (Variables|TownCampPreset|GetCampTownColor-todoprelace)))

(fn ConstructBoxExtendF
  (Components|Box|SetBoxExtent (Variables|Default|GetBox_SpawnAreaZoneVisualization) (Variables|ActivateDeactivateForPerformance|GetSpawnZoneExtent_Default200) true)
  (Components|Sphere|SetSphereRadius (Variables|Default|GetSpawnActivateTriggerOverlap) (Variables|ActivateDeactivateForPerformance|GetSpawnActivateTriggerDistance_Default2000) false)
  (Components|Sphere|SetSphereRadius (Variables|Default|GetDespawnDeactivateTriggerOverlap) (+ (Variables|ActivateDeactivateForPerformance|GetSpawnActivateTriggerDistance_Default2000) (Variables|ActivateDeactivateForPerformance|GetDespawnDeactivateTiggerDistanceTolerance_Default500)) false))

(fn BeginPlaySphereOverlapNstartStateF
  (bind _spawnactivatetriggeroverlap (Variables|Default|GetSpawnActivateTriggerOverlap))
  (bind _returnvalue (Transformation|GetWorldLocation _spawnactivatetriggeroverlap))
  (bind _outhits (Collision|MultiSphereTraceForObjects _returnvalue (+ _returnvalue "0.000000,0.000000,1.000000") (Variables|ActivateDeactivateForPerformance|GetSpawnActivateTriggerDistance_Default2000) (Utilities|Array|MakeArray "ObjectTypeQuery9") false 0 "None" true "(R=1.000000,G=0.000000,B=0.000000,A=1.000000)" "(R=0.000000,G=1.000000,B=0.000000,A=1.000000)" 22.0))
  (for _array_element _outhits
    (Utilities|Array|AddUnique (Variables|ActivateDeactivateForPerformance|GetPlayerCharactersOverlap_Array) (.AsCharacter (Utilities|Casting|CastToCharacter (.HitActor (Collision|BreakHitResult _array_element))))))
  (if (Utilities|Array|IsValidIndex (Variables|ActivateDeactivateForPerformance|GetPlayerCharactersOverlap_Array))
    (Variables|ActivateDeactivateforPerformance|SetCampStatePerformance_ActivateVsDeactive%28PlayerDistance%29 "NewEnumerator1")
    (else
      (CallFunction|DeactivateStateAICE)
      (Variables|ActivateDeactivateforPerformance|SetCampStatePerformance_ActivateVsDeactive%28PlayerDistance%29 "NewEnumerator2")))
  (return))

(fn BeginPlayBuildingsCampTownActorRefSETF
  (Utilities|FlowControl|Sequence
    (:then_1
      (bind _array_element (Utilities|Array|ForEachLoopwithBreak (Variables|Building|GetSpawnZoneActors))
        (:LoopBody
          (Class|BPISpawnZoneQrfLocationIntefaceI|SZQLICampTownActorSETI(Message) _array_element self))))
    (:then_2
      ;[1 1 1] RestingStation
      (bind _array_element_2 (Utilities|Array|ForEachLoopwithBreak (Variables|Building|GetRestingStationActors))
        (:LoopBody
          (Class|BPIRestingStationInterfaceI|RSICampTownActorSETI(Message) _array_element_2 self))))
    (:then_3
      ;[1 1 1] PatrolRoute
      (bind _array_element_3 (Utilities|Array|ForEachLoopwithBreak (Variables|Building|GetPatrolRouteActors))
        (:LoopBody
          (Class|BPIPatrolRouteInterfaceI|PRICampTownActorSETI(Message) _array_element_3 self))))
    (:then_4
      ;[1 1 1] Garrison
      (bind _array_element_4 (Utilities|Array|ForEachLoopwithBreak (Variables|Building|GetGarrisonBarracksActors))
        (:LoopBody
          (Class|BPIGarrisonBarracksInterfaceI|GBICampTownActorSETI(Message) _array_element_4 self))))
    (:then_5
      ;[1 1 1] Assembly
      (bind _array_element_5 (Utilities|Array|ForEachLoopwithBreak (Variables|Building|GetAssemblyFormationActors))
        (:LoopBody
          (Class|BPAssemblyStagingInterfaceI-old|ASICampTownActorSETI(Message) _array_element_5 self))))))

(fn BeginPlayDialyRoutineNLeashF
  (for _array_element (Variables|RosterCitizens|GetAiGuardsAssignedToCamp_Array)
    _))

(fn BeginPlayTownCampGsTFDHFnew
  (Class|BPIGameStateTeamFactionDiplomacyI|GSTFDTeamFactionTownCampAddI(Message) (Game|GetGameState) self))

(fn DissolveEffectDO2FadeOutEffectF-todo)

(fn SpawnInsideZoneCheckF-Oldreplaced
  (LocalVariables|SetPlayerCharacterFound_Local false)
  ;[1 1 1] Todo-checkAllCharacerClasses
  (bind _array_element (Utilities|Array|ForEachLoopwithBreak 0 :!label _label)
    (:LoopBody
      (bind _outactors (Collision|SphereOverlapActors (Transformation|GetWorldLocation (Variables|Default|GetDefaultSceneRoot)) (Variables|ActivateDeactivateForPerformance|GetSpawnActivateTriggerDistance_Default2000) (Utilities|Array|MakeArray "ObjectTypeQuery3") _array_element))
      (if (Utilities|Array|IsValidIndex _outactors)
        (LocalVariables|SetPlayerCharacterFound_Local true)
        (goto _label Break)))
    (:Completed
      (return (LocalVariables|GetPlayerCharacterFound_Local)))))

(fn DespawnInsideZoneCheckF-Oldreplaced
  (LocalVariables|SetPlayerCharacterFound_Local false)
  ;[1 1 1] Todo-checkAllCharacerClasses
  (bind _array_element (Utilities|Array|ForEachLoopwithBreak 0 :!label _label)
    (:LoopBody
      (bind _outactors (Collision|SphereOverlapActors (Transformation|GetWorldLocation (Variables|Default|GetDefaultSceneRoot)) (+ (Variables|ActivateDeactivateForPerformance|GetSpawnActivateTriggerDistance_Default2000) (Variables|ActivateDeactivateForPerformance|GetDespawnDeactivateTiggerDistanceTolerance_Default500)) (Utilities|Array|MakeArray "ObjectTypeQuery3") _array_element))
      (if (Utilities|Array|IsValidIndex _outactors)
        (LocalVariables|SetPlayerCharacterFound_Local true)
        (goto _label Break)))
    (:Completed
      (return (LocalVariables|GetPlayerCharacterFound_Local)))))

(fn DeactivateCampGuardsF
  (bind _array_element (Utilities|Array|ForEachLoopwithBreak (Variables|RosterCitizens|GetAiGuardsAssignedToCamp_Array))
    (:LoopBody
      (Actor|Tick|SetActorTickEnabled _array_element)
      (Collision|SetCollisionEnabled (Variables|/Script/Engine.Character|GetCapsuleComponent _array_element) "NoCollision")
      (AI|Navigation|StopMovement (Pawn|GetController _array_element))
      (CallFunction|DissolveEffectDO2FadeOutEffectF-todo)
      (Rendering|SetVisibility (Variables|/Script/Engine.Character|GetMesh _array_element) false false))))

(fn ActivateCampGuardsF
  (bind _array_element (Utilities|Array|ForEachLoopwithBreak (Variables|RosterCitizens|GetAiGuardsAssignedToCamp_Array))
    (:LoopBody
      (Actor|Tick|SetActorTickEnabled _array_element true)
      (Collision|SetCollisionEnabled (Variables|/Script/Engine.Character|GetCapsuleComponent _array_element) "QueryAndPhysics")
      (CallFunction|DissolveEffectDO2FadeOutEffectF-todo)
      (Rendering|SetVisibility (Variables|/Script/Engine.Character|GetMesh _array_element) true false))))

(fn DeactivateCampCheckF
  ;[1 1 1] Check if Deactivate For Performance
  (if (== (Utilities|Array|Length (Variables|ActivateDeactivateForPerformance|GetPlayerCharactersOverlap_Array)) 0)
    ;;[1 1 1] Cant Deactivate if minions are alive and chasing targets?
    (if (== (Utilities|Array|Length (Variables|ActivateDeactivateForPerformance|GetAINpcWithPerceptionChasingTarget_Array)) 0)
      (if (not (Utilities|Enum|Equal(Enum) (Variables|ActivateDeactivateforPerformance|GetCampStatePerformance_ActivateVsDeactive%28PlayerDistance%29) "NewEnumerator2"))
        ;;[1 1 1] Deactivate
        (CallFunction|DeactivateStateAICE)))))

(fn OverlapEndPlayerCharacterTryDeactivateStateF
  (params (Actor :type Actor%20Object%20Reference))
  (bind _playercharactersoverlap_array (Variables|ActivateDeactivateForPerformance|GetPlayerCharactersOverlap_Array))
  (bind _ascharacter (Utilities|Casting|CastToCharacter Actor))
  (if (Utilities|Array|ContainsItem _playercharactersoverlap_array _ascharacter)
    (Utilities|Array|RemoveItem _playercharactersoverlap_array _ascharacter)
    (if (== (Utilities|Array|Length (Variables|ActivateDeactivateForPerformance|GetPlayerCharactersOverlap_Array)) 0)
      ;[1 1 1] Cant Deactivate if minions are alive and chasing targets?
      (if (== (Utilities|Array|Length (Variables|ActivateDeactivateForPerformance|GetAINpcWithPerceptionChasingTarget_Array)) 0)
        (if (not (Utilities|Enum|Equal(Enum) (Variables|ActivateDeactivateforPerformance|GetCampStatePerformance_ActivateVsDeactive%28PlayerDistance%29) "NewEnumerator2"))
          ;[1 1 1] Deactivate
          (CallFunction|DeactivateStateAICE)
          (Variables|ActivateDeactivateforPerformance|SetCampStatePerformance_ActivateVsDeactive%28PlayerDistance%29 "NewEnumerator2"))))))

(fn OverlapBeginPlayerCharacterTryActivateStateF
  (params (Actor :type Actor%20Object%20Reference))
  (bind _ascharacter (Utilities|Casting|CastToCharacter Actor))
  (Utilities|Array|AddUnique (Variables|ActivateDeactivateForPerformance|GetPlayerCharactersOverlap_Array) _ascharacter)
  (if (Utilities|Array|IsValidIndex (Variables|ActivateDeactivateForPerformance|GetPlayerCharactersOverlap_Array))
    (if (not (Utilities|Enum|Equal(Enum) (Variables|ActivateDeactivateforPerformance|GetCampStatePerformance_ActivateVsDeactive%28PlayerDistance%29) "NewEnumerator1"))
      ;[1 1 1] Activate
      (CallFunction|SpawnActivateStateAICE)
      (Variables|ActivateDeactivateforPerformance|SetCampStatePerformance_ActivateVsDeactive%28PlayerDistance%29 "NewEnumerator1"))))

(fn TargetsSpottedSharedPerceptionADDF
  (params (AiNpcWithPerception :type Character%20Object%20Reference) (TargetSpotted :type Character%20Object%20Reference%20%28by%20ref%29))
  (LocalVariables|SetAiNpcWithPerception_Local AiNpcWithPerception)
  (LocalVariables|SetTargetSpotted_Local TargetSpotted)
  (bind (_array_element _array_index) (Utilities|Array|ForEachLoopwithBreak (Variables|ActivateDeactivateforPerformance|GetTargetsSpottedSharedPerceptionInfo))
    (:LoopBody
      (if (== (.AlarmTargetEnemy (Utilities|Struct|BreakS_CampTownAlarmTargetsSpottedSharedPerception _array_element)) (LocalVariables|GetTargetSpotted_Local))
        (LocalVariables|SetAlreadySpotted_Local (== (.AlarmTargetEnemy (Utilities|Struct|BreakS_CampTownAlarmTargetsSpottedSharedPerception _array_element)) (LocalVariables|GetTargetSpotted_Local)))
        (LocalVariables|SetIndexFound_Local _array_index)
        (LocalVariables|SetIndexInfo_Local _array_element)))
    (:Completed
      (if (LocalVariables|GetAlreadySpotted_Local)
        ;[1 1 1] Existing Entry
        (bind _output_get (LocalVariables|SetNpcsWithPerceptionThatSpottedTarget (.NpcWithPerceptionThatSpottedTarget (Utilities|Struct|BreakS_CampTownAlarmTargetsSpottedSharedPerception (LocalVariables|GetIndexInfo_Local)))))
        (Utilities|Array|AddUnique _output_get (LocalVariables|GetAiNpcWithPerception_Local))
        (Utilities|Array|SetArrayElem (Variables|ActivateDeactivateforPerformance|GetTargetsSpottedSharedPerceptionInfo) (LocalVariables|GetIndexFound_Local) (Utilities|Struct|MakeS_CampTownAlarmTargetsSpottedSharedPerception (LocalVariables|GetNpcsWithPerceptionThatSpottedTarget) (LocalVariables|GetTargetSpotted_Local) (Transformation|GetActorLocation (LocalVariables|GetTargetSpotted_Local)) (Utilities|Time|GetTimeSeconds)) true)
        (else
          ;[1 1 1] New Entry
          (Utilities|Array|Add (Variables|ActivateDeactivateforPerformance|GetTargetsSpottedSharedPerceptionInfo) (Utilities|Struct|MakeS_CampTownAlarmTargetsSpottedSharedPerception (Utilities|Array|MakeArray (LocalVariables|GetAiNpcWithPerception_Local)) (LocalVariables|GetTargetSpotted_Local) (Transformation|GetActorLocation (LocalVariables|GetTargetSpotted_Local)) 0.0)))))))

(fn TargetsLostTrackSharedPerceptionREMOVEF
  (params (AiNpcWithPerception :type Character%20Object%20Reference) (TargetSpotted :type Character%20Object%20Reference%20%28by%20ref%29))
  (LocalVariables|SetAiNpcWithPerception_Local AiNpcWithPerception)
  (LocalVariables|SetTargetSpotted_Local TargetSpotted)
  (bind (_array_element _array_index) (Utilities|Array|ForEachLoopwithBreak (Variables|ActivateDeactivateforPerformance|GetTargetsSpottedSharedPerceptionInfo))
    (:LoopBody
      (if (== (.AlarmTargetEnemy (Utilities|Struct|BreakS_CampTownAlarmTargetsSpottedSharedPerception _array_element)) (LocalVariables|GetTargetSpotted_Local))
        (LocalVariables|SetIndexInfo_Local _array_element)
        (LocalVariables|SetIndexFound_Local _array_index)
        (LocalVariables|SetSpottedFound_Local (== (.AlarmTargetEnemy (Utilities|Struct|BreakS_CampTownAlarmTargetsSpottedSharedPerception _array_element)) (LocalVariables|GetTargetSpotted_Local)))))
    (:Completed
      (if (LocalVariables|GetSpottedFound_Local)
        (LocalVariables|SetNpcsWithPerceptionThatSpottedTarget (.NpcWithPerceptionThatSpottedTarget (Utilities|Struct|BreakS_CampTownAlarmTargetsSpottedSharedPerception (LocalVariables|GetIndexInfo_Local))))
        (bind _returnvalue (Utilities|Array|RemoveItem (LocalVariables|GetNpcsWithPerceptionThatSpottedTarget) (LocalVariables|GetAiNpcWithPerception_Local)))
        (if _returnvalue
          (if (> (Utilities|Array|Length (LocalVariables|GetNpcsWithPerceptionThatSpottedTarget)) 0)
            _
            (else
              ;[1 1 1] All Npcs spotting Target lost track of it. remove target from sharedPerception
              (Utilities|Array|RemoveIndex (Variables|ActivateDeactivateforPerformance|GetTargetsSpottedSharedPerceptionInfo) (LocalVariables|GetIndexFound_Local))
              (return))))
        (return)
        (else
          (return))))))

(fn DebugBillboardIconsF
  (params (Debug :type Boolean))
  (LocalVariables|SetShowDebugVisualizers_Local Debug)
  (Rendering|SetVisibility (Variables|Default|GetSpawnActivateTriggerOverlap) (LocalVariables|GetShowDebugVisualizers_Local) false)
  (Rendering|SetVisibility (Variables|Default|GetBox_SpawnAreaZoneVisualization) (LocalVariables|GetShowDebugVisualizers_Local) false)
  (Rendering|SetVisibility (Variables|Default|GetBillboard) (LocalVariables|GetShowDebugVisualizers_Local) false)
  (Rendering|SetVisibility (Variables|Default|GetDespawnDeactivateTriggerOverlap) (LocalVariables|GetShowDebugVisualizers_Local) false))

(fn AiNpcKilledF
  (params (Character :type Character%20Object%20Reference))
  (bind _aiofficersassignedtocamp_array (Variables|RosterCitizens|GetAiOfficersAssignedtoCamp_Array))
  (bind _ainpcwithperceptionchasingtarget_array (Variables|ActivateDeactivateForPerformance|GetAINpcWithPerceptionChasingTarget_Array))
  (bind _aiguardsassignedtocamp_array (Variables|RosterCitizens|GetAiGuardsAssignedToCamp_Array))
  (if (Utilities|Array|ContainsItem _ainpcwithperceptionchasingtarget_array Character)
    (Utilities|Array|RemoveItem _ainpcwithperceptionchasingtarget_array Character)
    (PerformanceSimulation|DeactivateCampCheckF))
  ;[1 1 1] Remove Assigned character
  (if (Utilities|Array|ContainsItem _aiguardsassignedtocamp_array Character)
    (bind _returnvalue (Utilities|Array|RemoveItem _aiguardsassignedtocamp_array Character))
    (if _returnvalue
      _)
    (elif (Utilities|Array|ContainsItem _aiofficersassignedtocamp_array Character)
      (Utilities|Array|RemoveItem _aiofficersassignedtocamp_array Character))))

(fn AlertSignalUpdateLocationGuardtoCampEventF
  (params (AiNpcWithPerception :type Character%20Object%20Reference) (TargetLockedOn :type Character%20Object%20Reference%20%28by%20ref%29))
  ;[1 1 1] Only need to update existing targets locations
  (AlarmPerception|TargetsSpottedSharedPerceptionADDF AiNpcWithPerception TargetLockedOn))

(fn AlertAlarmSpottedEnemyCamptoGuardEventSimpleF
  ;[1 1 1] Alert Allies Simple
  (for _array_element (Variables|RosterCitizens|GetAiGuardsAssignedToCamp_Array)
    (Class|BPIAIControllerMasterInterfaceI|AICIAlarmonCamptoGuardEventSimpleI(Message) (Pawn|GetController _array_element)))
  (for _array_element_2 (Variables|RosterCitizens|GetAiOfficersAssignedtoCamp_Array)
    (Class|BPIAIControllerMasterInterfaceI|AICIAlarmonCamptoGuardEventSimpleI(Message) (Pawn|GetController _array_element_2)))
  (return))

(fn AlertSignalLostTrackGuardtoCampEventF
  (params (AiNpcWithPerception :type Character%20Object%20Reference) (TargetSpotted :type Character%20Object%20Reference%20%28by%20ref%29))
  (bind _ainpcwithperceptionchasingtarget_array (Variables|ActivateDeactivateForPerformance|GetAINpcWithPerceptionChasingTarget_Array))
  ;[1 1 1] Guards ChaseLost
  (if (Utilities|Array|ContainsItem _ainpcwithperceptionchasingtarget_array AiNpcWithPerception)
    (Utilities|Array|RemoveItem _ainpcwithperceptionchasingtarget_array AiNpcWithPerception))
  (AlarmPerception|TargetsLostTrackSharedPerceptionREMOVEF AiNpcWithPerception TargetSpotted)
  ;[1 1 1] Alarm OnVsOff
  ;;[1 1 1] If guards are chasing cant turnOffALarm
  (if (== (Utilities|Array|Length (Variables|ActivateDeactivateForPerformance|GetAINpcWithPerceptionChasingTarget_Array)) 0)
    (if (not (Utilities|Enum|Equal(Enum) (Variables|ActivateDeactivateforPerformance|GetCampAlarmPerception_OnVsOff%28NpcPerception%29) "NewEnumerator2"))
      (bind _output_get (Variables|ActivateDeactivateforPerformance|SetCampAlarmPerception_OnVsOff%28NpcPerception%29 "NewEnumerator2"))
      (AlarmPerception|AlarmStatusIconUpdateF _output_get)
      ;[1 1 1] AlarmOff blackboard
      (AlarmPerception|AlarmOffBlackboardF)
      ;[1 1 1] Cant DeactivateCamp if guardsOrOfficers are chasing enemies
      (PerformanceSimulation|DeactivateCampCheckF)
      (Class|ZBPIGameplaySpawnDespawnGMI-DontNeedQ|GSDgmAlermAlarmEventTownCampAlarmDeactivatedSimple(Message) (Game|GetGameMode) self))))

(fn AlertSignalSpottedEnemyGuardtoCampEventF
  (params (AiNpcWithPerception :type Character%20Object%20Reference) (TargetSpotted :type Character%20Object%20Reference%20%28by%20ref%29))
  (bind _ainpcwithperceptionchasingtarget_array (Variables|ActivateDeactivateForPerformance|GetAINpcWithPerceptionChasingTarget_Array))
  (if (not (Utilities|Array|ContainsItem _ainpcwithperceptionchasingtarget_array AiNpcWithPerception))
    ;[1 1 1] Guards Chaseing  Enemies
    (Utilities|Array|AddUnique _ainpcwithperceptionchasingtarget_array AiNpcWithPerception))
  (AlarmPerception|TargetsSpottedSharedPerceptionADDF AiNpcWithPerception TargetSpotted)
  ;[1 1 1] Alarm OnVsOff
  ;;[1 1 1] Cant turn on alarm if there are no chasing guards
  (if (Utilities|Array|IsValidIndex (Variables|ActivateDeactivateForPerformance|GetAINpcWithPerceptionChasingTarget_Array))
    (if (not (Utilities|Enum|Equal(Enum) (Variables|ActivateDeactivateforPerformance|GetCampAlarmPerception_OnVsOff%28NpcPerception%29) "NewEnumerator1"))
      (bind _output_get (Variables|ActivateDeactivateforPerformance|SetCampAlarmPerception_OnVsOff%28NpcPerception%29 "NewEnumerator1"))
      ;[1 1 1] Debug AlarmIcon
      (AlarmPerception|AlarmStatusIconUpdateF _output_get)
      ;[1 1 1] Alert On Blackboard
      (AlarmPerception|AlertAlarmSpottedEnemyCamptoGuardEventSimpleF)
      ;[1 1 1] ?
      (Class|ZBPIGameplaySpawnDespawnGMI-DontNeedQ|GSDgmAlertAlarmEventTownCampAlarmActivatedSimple(Message) (Game|GetGameMode) self))))

(fn AlarmOffBlackboardF
  (for _array_element (Variables|RosterCitizens|GetAiGuardsAssignedToCamp_Array)
    (Class|BPIAIControllerMasterInterfaceI|AICIAlarmOffCamptoGuardEventSimpleI(Message) (Pawn|GetController _array_element)))
  (for _array_element_2 (Variables|RosterCitizens|GetAiOfficersAssignedtoCamp_Array)
    (Class|BPIAIControllerMasterInterfaceI|AICIAlarmOffCamptoGuardEventSimpleI(Message) (Pawn|GetController _array_element_2)))
  (return))

(fn RosterCharacterCharacterFindCreateF)

(fn TownCampPresetProofF
  (params (CampTownPreset :type Primary%20Data%20Asset%20Object%20Reference))
  (Utilities|IsValid CampTownPreset
    (:Is%20Valid
      (if (Utilities|DoesObjectImplementInterface CampTownPreset "/Game/05CampTowns/BPI_CampTownPresetInterface_I.BPI_CampTownPresetInterface_I_C")
        (bind _teamfactionpreset (Class|BPICampTownPresetInterfaceI|TownCampPresetInfoGETI(Message) CampTownPreset))
        (Utilities|IsValid _teamfactionpreset
          (:Is%20Valid
            (if (Utilities|DoesObjectImplementInterface _teamfactionpreset "/Game/06GsTeamFactions/TeamFactionPreset/BPI_TeamFactionPresetInterface_I.BPI_TeamFactionPresetInterface_I_C")
              (return true)
              (else
                (Development|PrintString "BPCAmpTownGroupActor>BeginPlayTownCampGsTFDH_F== TeamFactionPreset does not implement TeamFactionInterface" true true "(R=1.000000,G=0.446939,B=0.000000,A=1.000000)" 22.0)
                (return false))))
          (:Is%20Not%20Valid
            (Development|PrintString "BPCAmpTownGroupActor>BeginPlayTownCampGsTFDH_F== TeamFaction is null" true true "(R=1.000000,G=0.446939,B=0.000000,A=1.000000)" 22.0)
            (return false)))
        (else
          (Development|PrintString "BPCAmpTownGroupActor>BeginPlayTownCampGsTFDH_F== CampTownPreset Does not implement Interface" true true "(R=1.000000,G=0.446939,B=0.000000,A=1.000000)" 22.0)
          (return false))))
    (:Is%20Not%20Valid
      (Development|PrintString "BPCAmpTownGroupActor>BeginPlayTownCampGsTFDH_F== CampTownPreset is null" true true "(R=1.000000,G=0.490260,B=0.000000,A=1.000000)" 22.0)
      (return false))))

(fn CancelingInterutionInteractionDialogueLooting-AlarmF-moved
  ;[1 1 1] If alarm already active then ignore?
  (if (Utilities|Enum|Equal(Enum) (Variables|ActivateDeactivateforPerformance|GetCampAlarmPerception_OnVsOff%28NpcPerception%29) "NewEnumerator2")
    _))

(fn AlarmStatusIconUpdateF
  (params (AlarmActive :type E_Generic-OnOpenActiveVsOffClosedDisabled%20Enum :default "NewEnumerator0"))
  (bind _billboard_alarmstatus (Variables|Default|GetBillboard_AlarmStatus))
  (switch Utilities|FlowControl|Switch|SwitchonE_Generic-OnOpenActiveVsOffClosedDisabled AlarmActive
    (:NewEnumerator0
      ;[1 1 1] DebugIcon
      (Rendering|Components|Sprite|SetSprite _billboard_alarmstatus 0 :!label _label)
      (Development|SetHiddeninGame _billboard_alarmstatus true false))
    (:NewEnumerator1
      (Rendering|Components|Sprite|SetSprite _billboard_alarmstatus "/Game/10WidgetUIAssets/PerceptionIconsCustom/Icon_PerceptionIcon_Exclamation.Icon_PerceptionIcon_Exclamation")
      (Development|SetHiddeninGame _billboard_alarmstatus false false))
    (:NewEnumerator2
      (goto _label))))

(fn CTGICampTownAlarmPerceptionGETI
  (return (Variables|ActivateDeactivateforPerformance|GetTargetsSpottedSharedPerceptionInfo) (Variables|ActivateDeactivateforPerformance|GetCampAlarmPerception_OnVsOff%28NpcPerception%29)))

(fn CTGICampTownBuildingsGETI
  (return (Variables|Building|GetPatrolRouteActors) (Variables|Building|GetGarrisonBarracksActors) (Variables|Building|GetAssemblyFormationActors) (Variables|Building|GetRestingStationActors)))

(fn CTGICampTownGuardAssignedSETI
  (params (Character :type Character%20Object%20Reference))
  (Development|PrintString "CampTownGuardAssignedSetI not setup"))

(fn CTGICampTownOfficerAssignedSETI-replacedQ
  (params (Character :type Character%20Object%20Reference))
  (Development|PrintString "CampTownGuardAssignedSet2not setup"))

(fn CTGICampTownPresetPdaGETI
  (return (Variables|TownCampPreset|GetCampTownPreset)))