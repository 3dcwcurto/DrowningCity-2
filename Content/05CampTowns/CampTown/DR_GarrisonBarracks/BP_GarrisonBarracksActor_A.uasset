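; Garrison barracks actor for a camp town that holds two pools of slot locations for garrison assembly and QRF standby.
; Each pool has a reservation-maker array, which interface calls fill by slot index without an occupancy check and release by clearing the caller's first match.
; Interface getters expose both pools and the linked camp town actor.
; BeginPlay only prints a warning if either location array is empty.
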(event EventBeginPlay
  ;[1 1 1] Check if there is alteast one location set in array
  (CallFunction|ProofLocationsSetupCheckF))

(event EventTick
  (params (DeltaSeconds :type Float%20%28single-precision%29)))

(fn ConstructionScript)

(fn GarrisonQrfOnstandbySlotReleaseSETIF
  (params (ReservationReleaser :type Character%20Object%20Reference))
  ;[1 1 1] Start false
  (LocalVariables|SetFound_Local false)
  (bind (_array_element _array_index) (Utilities|Array|ForEachLoopwithBreak (Variables|Default|GetGarrisonQrfOnStandbyReservationMaker) :!label _label)
    (:LoopBody
      (if (== _array_element ReservationReleaser)
        (LocalVariables|SetFoundIndex_Local _array_index)
        (LocalVariables|SetFound_Local true)
        (goto _label Break)))
    (:Completed
      (if (LocalVariables|GetFound_Local)
        ;[1 1 1] Clear
        (Utilities|Array|SetArrayElem (Variables|Default|GetGarrisonQrfOnStandbyReservationMaker) (LocalVariables|GetFoundIndex_Local) 0 true))
      (return (LocalVariables|GetFound_Local)))))

(fn GarrisonAssemblySlotReleaseSETIF
  (params (ReservationReleaser :type Character%20Object%20Reference))
  ;[1 1 1] Start false
  (LocalVariables|SetFound_Local false)
  (bind (_array_element _array_index) (Utilities|Array|ForEachLoopwithBreak (Variables|Default|GetGarrisonAssemblyReservationMaker) :!label _label)
    (:LoopBody
      (if (== _array_element ReservationReleaser)
        (LocalVariables|SetFoundIndex_Local _array_index)
        (LocalVariables|SetFound_Local true)
        (goto _label Break)))
    (:Completed
      (if (LocalVariables|GetFound_Local)
        ;[1 1 1] Clear
        (Utilities|Array|SetArrayElem (Variables|Default|GetGarrisonAssemblyReservationMaker) (LocalVariables|GetFoundIndex_Local) 0 true))
      (return (LocalVariables|GetFound_Local)))))

(fn ProofLocationsSetupCheckF
  ;[0.1596 0 1] Check if there is alteast one slot set for each
  (Utilities|FlowControl|Sequence
    (:then_0
      (if (not (> (Utilities|Array|Length (Variables|Default|GetGarrisonQrfOnstandbySlotLocations)) 0))
        (Development|PrintString "BPGarrisonBarracksActorA>ProofLocationsF== QrfOnStandbySlotLocations== are not setup" true true "(R=1.000000,G=0.446939,B=0.000000,A=1.000000)" 22.0)))
    (:then_1
      (if (not (> (Utilities|Array|Length (Variables|Default|GetGarrisonAssemblySlotLocations)) 0))
        (Development|PrintString "BPGarrisonBarracksActorA>ProofLocationsF== AssemblySlotLocations== are not setup" true true "(R=1.000000,G=0.446939,B=0.000000,A=1.000000)" 22.0)))))

(fn CBIGarrisonAssemblySlotReservationSETI
  (params (SlotIndex :type Integer) (ReservationMaker :type Character%20Object%20Reference))
  (Utilities|Array|SetArrayElem (Variables|Default|GetGarrisonAssemblyReservationMaker) SlotIndex ReservationMaker true)
  (return true))

(fn CBIGarrisonAssemlySlotReleaseSETI
  (params (ReservationReleaser :type Character%20Object%20Reference))
  (bind _found (CallFunction|GarrisonAssemblySlotReleaseSETIF ReservationReleaser))
  (return _found))

(fn CBIGarrisonQrfSlotReleaseSETI
  (params (ReservationReleaser :type Character%20Object%20Reference))
  (bind _found (CallFunction|GarrisonQrfOnstandbySlotReleaseSETIF ReservationReleaser))
  (return _found))

(fn CBIGarrisonQrfSlotReservationSETI
  (params (SlotIndex :type Integer) (ReservationMaker :type Character%20Object%20Reference))
  (Utilities|Array|SetArrayElem (Variables|Default|GetGarrisonQrfOnStandbyReservationMaker) SlotIndex ReservationMaker true)
  (return true))

(fn GBIBuildingBarracksAssemblySETI-old
  (params (GarrissonAssemblyLocationUseageState :type E_GenericUsage-InuseOcupiedVsUnusedUnocupied%20Enum :default "NewEnumerator0") (IndexToUpdate :type Integer)))

(fn GBIBuildingBarracksTrainingSETI-old
  (params (GarrisonTrainingLocationUseageState :type E_GenericUsage-InuseOcupiedVsUnusedUnocupied%20Enum :default "NewEnumerator0") (IndexToUpdate :type Integer)))

(fn GBICampTownActorGETI
  (bind _towncampactor (Variables|Default|GetTownCampActor))
  (Utilities|IsValid _towncampactor
    (:Is%20Valid
      _)
    (:Is%20Not%20Valid
      (Development|PrintString "BPBuildingGarrisonActorA>BGICampTownActorGETI== CampTownActor is not valid" true true "(R=1.000000,G=0.017360,B=0.000000,A=1.000000)")))
  (return _towncampactor))

(fn GBICampTownActorSETI
  (params (CampTownActor :type Actor%20Object%20Reference))
  (bind _output_get (Variables|Default|SetTownCampActor CampTownActor))
  (return (Utilities|IsValid _output_get)))

(fn GBIGarrisonBarracksInfoGETI
  (return (Variables|Default|GetGarrisonQrfOnstandbySlotLocations) (Variables|Default|GetGarrisonQrfOnStandbyReservationMaker) (Variables|Default|GetGarrisonAssemblySlotLocations) (Variables|Default|GetGarrisonAssemblyReservationMaker)))