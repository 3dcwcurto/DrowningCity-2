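; An assembly staging actor, in an old-assets folder, that holds a camp town actor reference and a usage reservation state.
; Interface functions get and set both values, with the camp town getter printing a debug warning when its reference is invalid.
; The staging info getter is an empty stub, and the event graph and construction script do nothing.
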(event EventBeginPlay)

(event Collision|EventActorBeginOverlap
  (params (OtherActor :type Actor%20Object%20Reference)))

(event EventTick
  (params (DeltaSeconds :type Float%20%28single-precision%29)))

(fn ConstructionScript)

(fn ASIAssemblyStatingInfoGETI
  (return))

(fn ASICampTownActorGETI
  (bind _camptownactor (Variables|Default|GetCampTownActor))
  (Utilities|IsValid _camptownactor
    (:Is%20Valid
      _)
    (:Is%20Not%20Valid
      (Development|PrintString "BPAssemblyFormationActor>AFICampTownActorGETI== " true true "(R=1.000000,G=0.622017,B=0.000000,A=1.000000)" 22.0)))
  (return _camptownactor))

(fn ASICampTownActorSETI
  (params (CampTown :type Actor%20Object%20Reference))
  (bind _output_get (Variables|Default|SetCampTownActor CampTown))
  (return (Utilities|IsValid _output_get)))

(fn ASIUsageReservationGETI
  (return (Variables|Default|GetUsageReservation)))

(fn ASIUsageReservationSETI
  (params (UsageReservationUpdate :type E_GenericUsage-InuseOcupiedVsUnusedUnocupied%20Enum :default "NewEnumerator0"))
  (bind _output_get (Variables|Default|SetUsageReservation UsageReservationUpdate))
  (return true))