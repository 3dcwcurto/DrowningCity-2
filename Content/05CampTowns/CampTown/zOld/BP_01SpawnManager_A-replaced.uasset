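; Camp town spawn manager actor, apparently superseded, that spawns AI officers for horde formations.
; On authority, a custom event runs an EQS query over placed location actors, using player 0 as querier, then spawns a Drow officer at the first result and records it in an array.
; The construction script toggles debug visualization on all camp town group actors.
; BeginPlay and Tick are empty, and the test call to spawn is disconnected.
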(event Custom|OnQueryFinished_CE
  (params (QueryInstance :type Env%20Query%20Instance%20Blueprint%20Wrapper%20Object%20Reference) (QueryStatus :type EEnvQueryStatus%20Enum :default "Processing"))
  (bind (_resultlocations _returnvalue) (AI|EQS|GetQueryResultsasLocations QueryInstance))
  (if _returnvalue
    (Development|PrintString "Success")
    (bind _returnvalue_2 (Game|SpawnActorfromClass "/Game/04AiController/BT_BehaviorTrees/Char-old/AINpcOfficer2/BP_CharacterAiNpcOfficer_cccccC.BP_CharacterAiNpcOfficer_cccccC_C" (Math|Transform|MakeTransform (Utilities|Array|Get(acopy) _resultlocations)) "AdjustIfPossibleButAlwaysSpawn" 0 0 0 0 0 0 "/Game/02CharacterBP/003StatsChar/01CoreStats/CoreRaceElfOrcEctStats/BP_Race02Drow_O.BP_Race02Drow_O_C" 0 0 0 0 "/Game/04AiController/BT_BehaviorTrees/BT_AiNpcOfficer_BehaviorTree.BT_AiNpcOfficer_BehaviorTree" 0 0))
    (Utilities|Array|Add (Variables|Default|GetHordeCharacter_OfficersArray) _returnvalue_2)
    (else
      (Development|PrintString "Fail"))))

(event Custom|SpawnCreateHordeFormation_CE
  (Networking|SwitchHasAuthority
    (:Authority
      ;[1 1 1] EQS
      ;;[1 1 1 1 12] Actors: need to manual place 02spawnHordeFormationLocationA actors
      (bind _returnvalue (AI|EQS|RunEQSQuery "/Game/05CampTowns/CampTown/Qrf_SpawnZone/EQS_SpawnQrfOfficerFormation_Actor.EQS_SpawnQrfOfficerFormation_Actor" (Game|GetPlayerCharacter 0) "RandomBest5Pct"))
      (EventDispatchers|BindEventtoOnQueryFinishedEvent _returnvalue (delegate Custom|OnQueryFinished_CE)))))

(event Custom|TimerHandle_CEQ
  ;[0.01737 0.4427 0] Tick
)

(event EventBeginPlay
  ;[0.2507 1 0] BeginPlay
)

(event EventTick
  (params (DeltaSeconds :type Float%20%28single-precision%29))
  ;[0.01737 0.4427 0] Tick
)

(fn ConstructionScript
  (Utilities|FlowControl|Sequence
    (:then_0
      ;[1 1 1] SpawnDespawnOpenWorld
      ;;[1 1 1] SpawnDespawn02ActivateDeactivate_A
      (bind _outactors (Actor|GetAllActorsOfClass "/Game/05CampTowns/BP_CampTownGroupActor_A.BP_CampTownGroupActor_A_C")) ; Visualization for spawn Locations
      (bind _array_element (Utilities|Array|ForEachLoopwithBreak _outactors)
        (:LoopBody
          (Rendering|SetVisibility (Variables|/Game/05CampTowns/BP_CampTownGroupActor_A.BP_CampTownGroupActor_A_C|GetSpawnActivateTriggerOverlap _array_element) (Variables|Default|GetShowDebugs) false)
          (Rendering|SetVisibility (Variables|/Game/05CampTowns/BP_CampTownGroupActor_A.BP_CampTownGroupActor_A_C|GetBox_SpawnAreaZoneVisualization _array_element) (Variables|Default|GetShowDebugs) false)
          (Rendering|SetVisibility (Variables|/Game/05CampTowns/BP_CampTownGroupActor_A.BP_CampTownGroupActor_A_C|GetBillboard _array_element) (Variables|Default|GetShowDebugs) false))))))

(fn CampGroupsPlacedNpcsGETF
  (Actor|GetAllActorsOfClass "/Game/05CampTowns/BP_CampTownGroupActor_A.BP_CampTownGroupActor_A_C"))