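; Placeable location actor that marks a quick reaction force (QRF) spawn zone and links it to a camp town actor.
; The construction script sizes a box visualization from a configurable extent.
; Interface-style getter and setter functions expose the camp town reference, with the setter reporting validity and the getter printing a warning when it is invalid.
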(event EventTick
  (params (DeltaSeconds :type Float%20%28single-precision%29))
  ;[0.01737 0.4427 0] Tick
)

(fn ConstructionScript
  (Components|Box|SetBoxExtent (Variables|Default|GetBox_Visualization) (Variables|Default|GetInBoxExtent) true))

(fn SZQLICampTownActorGETI
  (bind _camptownactor (Variables|Default|GetCampTownActor))
  (Utilities|IsValid _camptownactor
    (:Is%20Valid
      _)
    (:Is%20Not%20Valid
      (Development|PrintString "BPSpawnZoneQrfLocationActorA>SZQLICampTownActorGetI== CampTownACtor is nt valid" true true "(R=1.000000,G=0.166416,B=0.000000,A=1.000000)" 22.0)))
  (return _camptownactor))

(fn SZQLICampTownActorSETI
  (params (CampTown :type Actor%20Object%20Reference))
  (bind _output_get (Variables|Default|SetCampTownActor CampTown))
  (return (Utilities|IsValid _output_get)))