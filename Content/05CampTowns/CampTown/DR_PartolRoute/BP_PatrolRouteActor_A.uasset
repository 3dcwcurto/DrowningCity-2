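; BP_PatrolRouteActor_A is a data actor that describes a patrol route for a camp town.
; Through PRI_ getter and setter functions it stores its owning camp town actor, printing a warning when that reference is invalid on read.
; A further getter returns the patrol paths, the lap completion mode (circle or reverse) and the start direction (forward or backward).
; It contains no movement logic, and its event graph and construction script are empty.
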(fn ConstructionScript)

(fn PRICampTownActorGETI
  (bind _camptownactor (Variables|Default|GetCampTownActor))
  (Utilities|IsValid _camptownactor
    (:Is%20Valid
      _)
    (:Is%20Not%20Valid
      (Development|PrintString "BPPatrolRouteActorA>PRICampTownActorGETI== camptown actor is not valid" true true "(R=1.000000,G=0.222856,B=0.000000,A=1.000000)" 22.0)))
  (return _camptownactor))

(fn PRICampTownActorSETI
  (params (CampTownActor :type Actor%20Object%20Reference))
  (bind _output_get (Variables|Default|SetCampTownActor CampTownActor))
  (return (Utilities|IsValid _output_get)))

(fn PRIPatrolRouteInfoGETI
  (return (Variables|Default|GetPatrolPaths) (Variables|Default|GetPatrolLapCompletion-CircleOrReverse) (Variables|Default|GetPatrolStartDirection-ForwardBackward)))