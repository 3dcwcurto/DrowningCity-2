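; Camera shot pawn that glides to and follows a locked-on actor, supplied by the camera-shot start events or a left-click hover-actor test.
; Tick interpolates location at a distance-dependent speed and zeroes collision component rotation while locked.
; Holding CameraRotateRts enables mouse yaw and clamped spring-arm pitch.
; Desired rotation and shot preset are stored but unapplied: movement, control-rotation interpolation and spring-arm preset calls are disconnected.
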(event Custom|CameraShot_Start_CE
  (params (LockedOnActorFollowDesired :type Actor%20Object%20Reference) (ControlRotationDesired :type Rotator) (CameraSettingDesired :type S%20Camera%20Settings%20Structure))
  (Variables|Default|SetLockedOnActorTrack LockedOnActorFollowDesired)
  (Variables|Default|SetControlRotationDesired ControlRotationDesired)
  (Variables|Default|SetCameraSetting_F-dontneedQ CameraSettingDesired))

(event Custom|PlayerControllerOwning_CE
  ;[0.251 1 0] BeginPlay/EventPossessed
)

(event EventBeginPlay
  ;[0.251 1 0] BeginPlay/EventPossessed
  (|CallParentFunction))

(event EventPossessed
  (params (NewController :type Controller%20Object%20Reference))
  ;[0 1 0.4249] Possessed
  (|CallParentFunction NewController)
  (CallFunction|PossessionPlayerControllerRefF NewController))

(event EventTick
  (params (DeltaSeconds :type Float%20%28single-precision%29))
  ;[0.03766 0.3229 0] Tick
  (CallFunction|LockonFollowMoveTickF)
  ;;[1 1 1 1 14] Controller wont be possesing this pawn?
  (CallFunction|LockonControlRotationTickF))

(event EventCCSCameraShotStartI
  (params (LockedOnActorDesired :type Actor%20Object%20Reference) (ControlRotationDesired :type Rotator :default "0, 0, 0") (ShotPerspectivePresets :type E_CameraShotCameraSettingsPresets-todoDontNeedQ%20Enum :default "NewEnumerator0"))
  (Variables|Default|SetLockedOnActorTrack LockedOnActorDesired)
  (Variables|Default|SetControlRotationDesired ControlRotationDesired)
  (Variables|Default|SetCameraShotSettings ShotPerspectivePresets))

(event Input|ActionEvents|InputActionCameraRotateRts
  (params (Key :type Key%20Structure))
  ;[1 1 1] NoteGame: Disable input
  (:Pressed
    (Variables|Default|SetHoldRotateButton_Var true))
  (:Released
    (Variables|Default|SetHoldRotateButton_Var false)))

(event Input|AxisEvents|InputAxisMoveForward
  (params (AxisValue :type Float%20%28single-precision%29))
  ;[1 1 1] NoteGame: Disable input
)

(event Input|AxisEvents|InputAxisMoveRight
  (params (AxisValue :type Float%20%28single-precision%29))
  ;[1 1 1] NoteGame: Disable input
)

(event Input|AxisEvents|InputAxisTurn
  (params (AxisValue :type Float%20%28single-precision%29))
  ;[1 1 1] NoteGame: Disable input
)

(event Input|AxisEvents|InputAxisLookUp
  (params (AxisValue :type Float%20%28single-precision%29))
  ;[1 1 1] NoteGame: Disable input
)

(event Input|MouseEvents|MouseX
  (params (AxisValue :type Float%20%28single-precision%29))
  ;[1 1 1] NoteGame: Disable input
  (CallFunction|RotateTurn-YawInputBPF AxisValue (Variables|Default|GetCameraRotationSpeed_2Default)))

(event Input|MouseEvents|MouseY
  (params (AxisValue :type Float%20%28single-precision%29))
  ;[1 1 1] NoteGame: Disable input
  (CallFunction|RotateLookup-PitchInputBPF AxisValue (Variables|Default|GetCameraRotationSpeed_2Default) (Variables|Default|GetMin%20Angle%20Pitch%20-89Default) (Variables|Default|GetMaxAnglePitch_-20Default)))

(event Input|KeyboardEvents|LeftAlt
  (params (Key :type Key%20Structure))
  ;[1 1 1] NoteGame: Disable input
  (:Pressed
    (Development|PrintString (Utilities|String|ToString(Rotator) (Pawn|GetControlRotation (Variables|Default|GetControllerReference) :!class /Script/Engine.Controller)) true true "(R=1.000000,G=0.008842,B=0.000000,A=1.000000)" 22.0)))

(event Input|MouseEvents|LeftMouseButton
  (params (Key :type Key%20Structure))
  ;[1 1 1] NoteGame: Disable input
  (:Pressed
    (CallFunction|LockontoActorTestingF)))

(fn ConstructionScript)

(fn CurrentMouseLocationF
  (bind _returnvalue (Game|GetPlayerController 0))
  (bind (_locationx _locationy) (Game|Player|GetMousePosition _returnvalue))
  (return (Math|Vector2D|MakeVector2D _locationx _locationy)))

(fn MoveRightF
  (params (AxisValue :type Float%20%28double-precision%29))
  (Pawn|Input|AddMovementInput self (Math|Vector|GetRightVector (Math|Rotator|MakeRotator 0.0 0.0 (.Yaw (Math|Rotator|BreakRotator (Pawn|GetControlRotation self :!class /Script/Engine.Pawn))))) (+ (/ AxisValue 2.0) (/ (Variables|Default|GetRightEdgeMove_Var) 2.0)) false))

(fn MoveForwardF
  (params (AxisValue :type Float%20%28double-precision%29))
  (Pawn|Input|AddMovementInput self (Math|Vector|GetForwardVector (Math|Rotator|MakeRotator 0.0 0.0 (.Yaw (Math|Rotator|BreakRotator (Pawn|GetControlRotation self :!class /Script/Engine.Pawn))))) (+ (/ AxisValue 2.0) (/ (Variables|Default|GetForwardEdgeMove_Var) 2.0)) false))

(fn RotateLookup-PitchInputBPF
  (params (AxisValue :type Float%20%28double-precision%29) (CameraRotationSpeed :type Float%20%28double-precision%29) (Min :type Float%20%28double-precision%29) (Max :type Float%20%28double-precision%29))
  (if (Variables|Default|GetHoldRotateButton_Var)
    (Transformation|SetRelativeRotation (Variables|Default|GetSpringArm) (Math|Rotator|MakeRotator 0.0 (Math|Float|Clamp(Float) (+ (.pitch (Variables|/Script/Engine.SceneComponent|GetRelativeRotation (Variables|Default|GetSpringArm))) (* AxisValue CameraRotationSpeed)) Min Max) 0.0) false false)))

(fn RotateTurn-YawInputBPF
  (params (AxisValue :type Float%20%28double-precision%29) (B :type Float%20%28double-precision%29))
  (if (Variables|Default|GetHoldRotateButton_Var)
    (Pawn|Input|AddControllerYawInput (* AxisValue B))))

(fn ControllerGETF
  ;[1 1 1] TodoLater: set controller same
  (Utilities|IsValid (Variables|Default|GetControllerReference)
    (:Is%20Valid
      (return (Variables|Default|GetControllerReference)))
    (:Is%20Not%20Valid
      (bind _output_get (Variables|Default|SetControllerReference (Pawn|GetController)))
      (return _output_get))))

(fn CameraPerspectiveSettingsSETF
  (params (TargetArmLength :type Float%20%28double-precision%29) (CameraLagSpeed :type Float%20%28double-precision%29) (SocketOffset :type Vector) (LerpAlhpa :type Float%20%28double-precision%29) (RightShoulder :type Boolean))
  (bind _springarm (Variables|Default|GetSpringArm))
  (Variables|/Script/Engine.SpringArmComponent|SetTargetArmLength _springarm (Math|Float|Lerp (Variables|/Script/Engine.SpringArmComponent|GetTargetArmLength _springarm) TargetArmLength LerpAlhpa))
  (Variables|/Script/Engine.SpringArmComponent|SetCameraLagSpeed _springarm (Math|Float|Lerp (Variables|/Script/Engine.SpringArmComponent|GetCameraLagSpeed _springarm) CameraLagSpeed LerpAlhpa))
  (Variables|/Script/Engine.SpringArmComponent|SetSocketOffset _springarm (Math|Vector|Lerp(Vector) SocketOffset (Math|Vector|MakeVector (.x (Variables|/Script/Engine.SpringArmComponent|GetSocketOffset _springarm)) (* (.y (Variables|/Script/Engine.SpringArmComponent|GetSocketOffset _springarm)) (Math|Float|SelectFloat 1.0 -1.0 RightShoulder)) (.z (Variables|/Script/Engine.SpringArmComponent|GetSocketOffset _springarm))) LerpAlhpa)))

(fn LockonFollowMoveTickF
  (bind _lockedonactortrack (Variables|Default|GetLockedOnActorTrack))
  (Utilities|IsValid _lockedonactortrack
    (:Is%20Valid
      (Transformation|SetActorLocation (Math|Interpolation|VInterpTo (Transformation|GetActorLocation) (Transformation|GetActorLocation _lockedonactortrack) (Utilities|Time|GetWorldDeltaSeconds) (Math|Float|SelectFloat 1e+02 8.0 (> (Math|Vector|Distance(Vector) (Transformation|GetActorLocation) (Transformation|GetActorLocation _lockedonactortrack)) 1e+02))) false false))))

(fn LockonControlRotationTickF
  (Utilities|IsValid (Variables|Default|GetLockedOnActorTrack)
    (:Is%20Valid
      (Transformation|SetWorldRotation (Variables|Default|GetCollisionComponent self) "0, 0, 0" false false))))

(fn LockonCameraSettingTickF
  (Utilities|IsValid (Variables|Default|GetLockedOnActorTrack)
    (:Is%20Valid
      (switch Utilities|FlowControl|Switch|SwitchonE_CameraShotCameraSettingsPresets-todoDontNeedQ (Variables|Default|GetCameraShotSettings)
        (:NewEnumerator0
          (CallFunction|CameraPerspectiveSettingsSETF 525.0 15.0 "55.000000,0.000000,45.000000" 5.0 false :!label _label))
        (:NewEnumerator1
          (goto _label))
        (:NewEnumerator2
          (goto _label))
        (:NewEnumerator3
          (CallFunction|CameraPerspectiveSettingsSETF 1.2e+03 15.0 "55.000000,70.000000,45.000000" 5.0 false :!label _label_2))
        (:NewEnumerator4
          (goto _label_2))
        (:NewEnumerator5
          (goto _label_2))
        (:NewEnumerator6
          (goto _label_2))))))

(fn LockontoActorTestingF
  (bind _controllerget (CallFunction|ControllerGETF))
  (bind _hover_interactableactor (Class|BPIPlayerControllerBaseInterfaceI|PcBIRtsIsoHoverActorGETI(Message) _controllerget))
  (Utilities|IsValid _hover_interactableactor
    (:Is%20Valid
      (Variables|Default|SetLockedOnActorTrack _hover_interactableactor))
    (:Is%20Not%20Valid
      (Variables|Default|SetLockedOnActorTrack 0))))

(fn CameraShotCameraShotSettingsF
  (params (CameraShotSettings :type E_CameraShotCameraSettingsPresets-todoDontNeedQ%20Enum :default "NewEnumerator0"))
  (bind _output_get (Variables|Default|SetCameraShotSettings "NewEnumerator0"))
  (switch Utilities|FlowControl|Switch|SwitchonE_CameraShotCameraSettingsPresets-todoDontNeedQ _output_get
    (:NewEnumerator0
      (CallFunction|CameraPerspectiveSettingsSETF 525.0 15.0 "55.000000,0.000000,45.000000" 5.0 false :!label _label))
    (:NewEnumerator1
      (goto _label))
    (:NewEnumerator2
      (goto _label))
    (:NewEnumerator3
      ;[1 1 1] IsoMetric&Rts
      (CallFunction|CameraPerspectiveSettingsSETF 1.2e+03 15.0 "55.000000,70.000000,45.000000" 5.0 false :!label _label_2))
    (:NewEnumerator4
      (goto _label_2))
    (:NewEnumerator5
      ;[1 0.745 0.0643] TodoLater
      (Development|PrintString "CameraShotPawn>CameraShotSettings== CameraSetttingType not setup yet'" :!label _label_3))
    (:NewEnumerator6
      (goto _label_3)))
  (return))

(fn PossessionPlayerControllerRefF
  (params (ControllerReference :type Controller%20Object%20Reference))
  (Variables|Default|SetControllerReference ControllerReference))

(fn PossessionCameraPerspectiveOF-dontneedQ
  (params (CameraPerspective :type E_CameraPerspectiveMode-Fps3rdIso%20Enum :default "NewEnumerator0"))
  (bind _output_get (Variables|Default|SetCameraPerspective-dontNeedQ CameraPerspective))
  (switch Utilities|FlowControl|Switch|SwitchonE_CameraPerspectiveMode-Fps3rdIso _output_get
    (:NewEnumerator0
      (Development|PrintString "BPCharacterBaseCC>EG== CameraPerspectiveMode is null"))
    (:NewEnumerator1
      (CallFunction|CameraPerspectiveSettingsSETF 525.0 15.0 "55.000000,0.000000,45.000000" 5.0 false :!label _label))
    (:NewEnumerator2
      (goto _label))
    (:NewEnumerator3
      ;[1 1 1] IsoMetric
      (CallFunction|CameraPerspectiveSettingsSETF 1.2e+03 15.0 "55.000000,70.000000,45.000000" 5.0 false :!label _label_2))
    (:NewEnumerator5
      (goto _label_2)))
  (return "NewEnumerator0"))