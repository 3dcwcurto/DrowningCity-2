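; Third-person player controller for squad play, setting camera perspective and default rotation, gait and turn-in-place modes on possession.
; BeginPlay has the squad selection manager component spawn the squad loadout with the roster widgets.
; Inputs route possession, selection of four slots or the whole squad, and follow, Shift-queueable move and hold-ground orders to that manager.
; Possession and selection results update the roster UI; keys 5–7 are placeholders.
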(event EventBeginPlay
  ;[0.2507 1 0] BeginPlay
  (|CallParentFunction)
  (Utilities|IsValid (Pawn|GetControlledPawn)
    (:Is%20Valid
      (Default|SpawnSquadCharacterLoadoutIsometricF (Variables|Default|GetBP_Manager-SquadSelectionInteractCamera_AC) (Variables|Default|GetWidget_WBPPartyRosterUI) (Variables|Default|GetWidget_WBPStatRoster_UI) self (Variables|Default|GetWidget_WBPSkillTreeRoster_UI) (Variables|Default|GetCameraPerspectiveMode)))))

(event EventPossess
  (params (PossessedPawn :type Pawn%20Object%20Reference))
  ;[0 1 0.4249] Possess
  (|CallParentFunction PossessedPawn)
  (CallFunction|CameraCameraPerspectiveModeF "NewEnumerator2" PossessedPawn)
  ;;[1 0.9975 0.4211] todolater: where to set?
  (Class|BPICharacterLocomotionInterfaceI|CLIRotationModeDefaultI(Message) PossessedPawn "NewEnumerator2")
  ;;[0.8629 1 0.3214] todoLater: Move code?
  (Class|BPICharacterLocomotionInterfaceI|CLIGaitCapDefaultI(Message) PossessedPawn "NewEnumerator3")
  (Class|BPICharacterLocomotionInterfaceI|CLITurninPlaceModeDefaultI(Message) PossessedPawn "NewEnumerator1"))

(event Input|ActionEvents|InputActionSelectSlot4Four
  (params (Key :type Key%20Structure :default "None"))
  ;[1 0.8464 0.4983] Todo:move to aparent? use enhancedInput
  ;;[1 1 1] Input Orders
  ;;;[1 1 1] Select squad members
  (:Pressed
    (bind (_squadloadoutcharacter _characterselectindex1) (Default|SelectCharacterIndexIsometricF (Variables|Default|GetBP_Manager-SquadSelectionInteractCamera_AC) 4))
    (Default|PartyRosterCharacterPartySlotSELECTEDUICE (Variables|Default|GetWidget_WBPPartyRosterUI) _squadloadoutcharacter _characterselectindex1 false)))

(event Input|ActionEvents|InputActionSelectSlot1One
  (params (Key :type Key%20Structure :default "None"))
  ;[1 0.8464 0.4983] Todo:move to aparent? use enhancedInput
  ;;[1 1 1] Input Orders
  ;;;[1 1 1] Select squad members
  (:Pressed
    (bind (_squadloadoutcharacter _characterselectindex1) (Default|SelectCharacterIndexIsometricF (Variables|Default|GetBP_Manager-SquadSelectionInteractCamera_AC) 1))
    (Default|PartyRosterCharacterPartySlotSELECTEDUICE (Variables|Default|GetWidget_WBPPartyRosterUI) _squadloadoutcharacter _characterselectindex1 false)))

(event Input|ActionEvents|InputActionPossessSlot1One
  (params (Key :type Key%20Structure :default "None"))
  ;[1 1 1] Input Possess
  (:Pressed
    (bind (_possessionsuccess _characterpossessed) (Default|SelectPossessCharacterIndexF (Variables|Default|GetBP_Manager-SquadSelectionInteractCamera_AC) 1 self))
    (if _possessionsuccess
      (CallFunction|StatRosterWidgetCharacterSlotSelectF-reworktoShowAllatOnce _characterpossessed))))

(event Input|ActionEvents|InputActionPossessSlot3Three
  (params (Key :type Key%20Structure :default "None"))
  ;[1 1 1] Input Possess
  (:Pressed
    (bind (_possessionsuccess _characterpossessed) (Default|SelectPossessCharacterIndexF (Variables|Default|GetBP_Manager-SquadSelectionInteractCamera_AC) 3 self))
    (if _possessionsuccess
      (CallFunction|StatRosterWidgetCharacterSlotSelectF-reworktoShowAllatOnce _characterpossessed))))

(event Input|ActionEvents|InputActionOrderFollowJ
  (params (Key :type Key%20Structure :default "None"))
  ;[1 0.8464 0.4983] Todo:move to aparent? use enhancedInput
  ;;[1 1 1] Input Orders
  ;;;[1 1 1] Follow
  (:Pressed
    (Default|Order04FollowF (Variables|Default|GetBP_Manager-SquadSelectionInteractCamera_AC) "NewEnumerator2" "NewEnumerator1")))

(event Input|ActionEvents|InputActionPossessSlot4Four
  (params (Key :type Key%20Structure :default "None"))
  ;[1 1 1] Input Possess
  (:Pressed
    (bind (_possessionsuccess _characterpossessed) (Default|SelectPossessCharacterIndexF (Variables|Default|GetBP_Manager-SquadSelectionInteractCamera_AC) 4 self))
    (if _possessionsuccess
      (CallFunction|StatRosterWidgetCharacterSlotSelectF-reworktoShowAllatOnce _characterpossessed))))

(event Input|ActionEvents|InputActionOrderMoveToLocationL
  (params (Key :type Key%20Structure :default "None"))
  ;[1 0.8464 0.4983] Todo:move to aparent? use enhancedInput
  ;;[1 1 1] Input Orders
  ;;;[1 1 1] Move
  (:Pressed
    (Default|Order01MovetoIsoF (Variables|Default|GetBP_Manager-SquadSelectionInteractCamera_AC) (Game|Player|IsInputKeyDown "LeftShift") "NewEnumerator1" self)))

(event Input|ActionEvents|InputActionSelectAllSquadPartyMemebers
  (params (Key :type Key%20Structure :default "None"))
  ;[1 0.8464 0.4983] Todo:move to aparent? use enhancedInput
  ;;[1 1 1] Input Orders
  ;;;[1 1 1] Select squad members
  (:Pressed
    (bind _pointmanleader (Default|SelectCharacterSquadIsometricF (Variables|Default|GetBP_Manager-SquadSelectionInteractCamera_AC)))
    (Default|PartyRosterCharacterPartySQUADSELECTALLUICE (Variables|Default|GetWidget_WBPPartyRosterUI) _pointmanleader)))

(event Input|ActionEvents|InputActionSelectSlot3Three
  (params (Key :type Key%20Structure :default "None"))
  ;[1 0.8464 0.4983] Todo:move to aparent? use enhancedInput
  ;;[1 1 1] Input Orders
  ;;;[1 1 1] Select squad members
  (:Pressed
    (bind (_squadloadoutcharacter _characterselectindex1) (Default|SelectCharacterIndexIsometricF (Variables|Default|GetBP_Manager-SquadSelectionInteractCamera_AC) 3))
    (Default|PartyRosterCharacterPartySlotSELECTEDUICE (Variables|Default|GetWidget_WBPPartyRosterUI) _squadloadoutcharacter _characterselectindex1 false)))

(event Input|ActionEvents|InputActionSelectSlot2Two
  (params (Key :type Key%20Structure :default "None"))
  ;[1 0.8464 0.4983] Todo:move to aparent? use enhancedInput
  ;;[1 1 1] Input Orders
  ;;;[1 1 1] Select squad members
  (:Pressed
    (bind (_squadloadoutcharacter _characterselectindex1) (Default|SelectCharacterIndexIsometricF (Variables|Default|GetBP_Manager-SquadSelectionInteractCamera_AC) 2))
    (Default|PartyRosterCharacterPartySlotSELECTEDUICE (Variables|Default|GetWidget_WBPPartyRosterUI) _squadloadoutcharacter _characterselectindex1 false)))

(event Input|ActionEvents|InputActionOrderHoldGroundH
  (params (Key :type Key%20Structure :default "None"))
  (bind _self self)
  (bind _bp_manager_squadselectioninteractcamera_ac (Variables|Default|GetBP_Manager-SquadSelectionInteractCamera_AC))
  ;[1 0.8464 0.4983] Todo:move to aparent? use enhancedInput
  ;;[1 1 1] Input Orders
  ;;;[1 1 1] HoldGround
  (:Pressed
    (Default|Order05HoldGroundAdvancedF _bp_manager_squadselectioninteractcamera_ac true _self))
  (:Released
    (Default|Order05HoldGroundAdvancedF _bp_manager_squadselectioninteractcamera_ac false _self)))

(event Input|ActionEvents|InputActionPossessSlot2Two
  (params (Key :type Key%20Structure :default "None"))
  ;[1 1 1] Input Possess
  (:Pressed
    (bind (_possessionsuccess _characterpossessed) (Default|SelectPossessCharacterIndexF (Variables|Default|GetBP_Manager-SquadSelectionInteractCamera_AC) 2 self))
    (if _possessionsuccess
      (CallFunction|StatRosterWidgetCharacterSlotSelectF-reworktoShowAllatOnce _characterpossessed))))

(event Input|KeyboardEvents|5
  (params (Key :type Key%20Structure :default "None"))
  ;[1 0.8464 0.4983] Todo:move to aparent? use enhancedInput
  ;;[1 1 1] Input Orders
  (:Pressed
    (Development|PrintString "InputNotSetupYet" true true "(R=1.000000,G=0.152452,B=0.000000,A=1.000000)" 22.0)))

(event Input|KeyboardEvents|6
  (params (Key :type Key%20Structure :default "None"))
  ;[1 0.8464 0.4983] Todo:move to aparent? use enhancedInput
  ;;[1 1 1] Input Orders
  (:Pressed
    (Development|PrintString "InputNotSetupYet" true true "(R=1.000000,G=0.152452,B=0.000000,A=1.000000)" 22.0)))

(event Input|KeyboardEvents|7
  (params (Key :type Key%20Structure :default "None"))
  ;[1 0.8464 0.4983] Todo:move to aparent? use enhancedInput
  ;;[1 1 1] Input Orders
  (:Pressed
    (Development|PrintString "InputNotSetupYet" true true "(R=1.000000,G=0.152452,B=0.000000,A=1.000000)" 22.0)))

(fn ConstructionScript)