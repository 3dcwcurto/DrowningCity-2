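; RTS gameplay player controller that handles mouse unit selection and squad move orders.
; Left mouse starts and stops the HUD's selection box, with click and box results arriving through interface events that toggle actor outlines.
; Only box selection fills the squad array, which deselection never clears.
; Right click sends that squad to the cursor hit location via ACManagerSquadOrders, with Left Shift queuing.
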(event Custom|PlaySound2d_CE
  (params (Todo-2dSoundEnum :type E_SoundsPlayerController%20Enum :default "NewEnumerator0"))
  ;[1 1 1] 2DSound
  (Audio|PlaySound2D "/Game/09SfxAsset/ActionRPGbyUnreal/A_Character_Step01.A_Character_Step01" 0.5 1.0 0.0 0 0))

(event EventPcBIRtsSelectionBoxAddActorI
  (params (SelectedActors :type Array%20of%20Actor%20Object%20References) (InputModifier-CombinePrevious :type Boolean))
  ;[1 1 1] SelectionSingle&Drag
  ;;[1 1 1] SelectActor
  (CallFunction|SelectionBoxAddActorF SelectedActors InputModifier-CombinePrevious))

(event EventPcBIRtsSelectionClickAddActorI
  (params (SelectedActor :type Actor%20Object%20Reference) (InputModifier-CombinePrevious :type Boolean))
  ;[1 1 1] SelectionSingle&Drag
  ;;[1 1 1] SelectActor
  (CallFunction|SelectionClickAddActorF SelectedActor InputModifier-CombinePrevious))

(event EventBeginPlay
  ;[0.2507 1 0] BeginPlay
  ;;[1 1 1 1 14] Remove all viewport widgets
  (Viewport|RemoveAllWidgets))

(event Input|MouseEvents|LeftMouseButton
  (params (Key :type Key%20Structure))
  ;[1 1 1] SelectionSingle&Drag
  ;;[1 1 1] SelectionBox
  (:Pressed
    ;;;[0.8276 1 0.5153] SelectionBox
    (Input|SetInputModeGameandUI self 0 "LockAlways" true)
    (Variables|Default|SetbShowMouseCursor true)
    ;;;;[1 1 1] HudClass is RTSTemplate Asset
    (Class|BPIRtsHUDInterfaceI|RHIRtsSelectionIsDrawingStartI(Message) (CallFunction|SetupHUD-HUDGameplayRtsF)))
  (:Released
    (Class|BPIRtsHUDInterfaceI|RHIRtsSelectionIsDrawingStopI(Message) (CallFunction|SetupHUD-HUDGameplayRtsF))))

(event Input|MouseEvents|RightMouseButton
  (params (Key :type Key%20Structure))
  (bind _hitresult (Game|Player|GetHitResultUnderCursorbyChannel "TraceTypeQuery1" false))
  (bind _selectedactors_squad (Variables|Default|GetSelectedActors_Squad))
  (bind (_bblockinghit _binitialoverlap _time _distance _location _impactpoint _normal _impactnormal _physmat _hitactor) (Collision|BreakHitResult _hitresult))
  (:Pressed
    (if (> (Utilities|Array|Length _selectedactors_squad) 0)
      (Utilities|IsValid _hitactor
        (:Is%20Valid
          (Default|Order01MovetoRtsF (Variables|Default|GetAC_Manager-SquadOrders) _selectedactors_squad _location (Game|Player|IsInputKeyDown self "LeftShift") "NewEnumerator4"))))))

(fn ConstructionScript)

(fn SetupWidget-WBPGameplayUIF
  (bind _returnvalue (UserInterface|CreateWidget "/Game/03PlayerController/WBP_HudGameplay_UI.WBP_HudGameplay_UI_C"))
  (bind _output_get (Variables|Default|SetWBP_PlayerGameplayUI _returnvalue))
  (UserInterface|Viewport|AddtoViewport _output_get 0)
  (Variables|Default|SetWBP_RtsSelectionSquareUI (Variables|/Game/03PlayerController/WBP_HudGameplay_UI.WBP_HudGameplay_UI_C|GetWBP_RtsSelectionSquare_UMG _output_get)))

(fn SelectionClickorBoxStartF
  (Class|BPIRtsHUDInterfaceI|RHIRtsSelectionIsDrawingStartI(Message) (CallFunction|SetupHUD-HUDGameplayRtsF)))

(fn SelectionClickorBoxStopF)

(fn DeselectActorsF
  (for _array_element (Variables|Default|GetSelectedActors_Squad)
    (Class|BPICharacterBaseInterface|CPIOutlineDeselectActorxI(Message) _array_element)))

(fn SelectionBoxAddActorF
  (params (SelectedActors :type Array%20of%20Actor%20Object%20References) (InputModifier-CombinePrevious :type Boolean))
  (if InputModifier-CombinePrevious
    _
    (else
      (CallFunction|DeselectActorsF)))
  (for _array_element SelectedActors
    (if (Utilities|DoesObjectImplementInterface _array_element "/Game/02CharacterBP/BPI_CharacterMasterInterface_I.BPI_CharacterMasterInterface_I_C")
      (Utilities|Array|Add (Variables|Default|GetSelectedActors_Squad) _array_element)
      ;[1 1 1] selection Outline +
      (Class|BPICharacterBaseInterface|CPIOutlineSelectActorxI(Message) _array_element))))

(fn SetupHUD-HUDGameplayRtsF
  (bind _output_get (Variables|Default|SetHUDRef (HUD|GetHUD)))
  (return _output_get))

(fn SelectionClickAddActorF
  (params (SelectedActor :type Actor%20Object%20Reference) (InputModifier-CombinePrevious :type Boolean))
  (if InputModifier-CombinePrevious
    _
    (else
      (CallFunction|DeselectActorsF)))
  (if (Utilities|DoesObjectImplementInterface SelectedActor "/Game/03PlayerController/01ControllerBase/BPI_PlayerControllerBaseInterface_I.BPI_PlayerControllerBaseInterface_I_C")
    ;[1 1 1] selection Outline +
    (Class|BPICharacterBaseInterface|CPIOutlineSelectActorxI(Message) SelectedActor)
    ;[1 1 1] SelectionSound
    (CallFunction|PlaySound2dCE "NewEnumerator1")))

(fn PcBICameraPerspectiveModeGETI
  (return "NewEnumerator0"))

(fn PcBIHUDGameplayUIGETI-notactualyUsedQ
  (return 0))

(fn PcBIRtsIsoHoverActorGETI
  (return 0))

(fn PcBIRtsIsoMouseCursorActorGETI
  (return 0))

(fn PcBISquadMemberLoadoutCharactersGETI
  (return 0))

(fn PcBISquadMemeberbyIdNameGETI
  (params (CharacterPresetID :type Primary%20Data%20Asset%20Object%20Reference))
  (return 0 false))