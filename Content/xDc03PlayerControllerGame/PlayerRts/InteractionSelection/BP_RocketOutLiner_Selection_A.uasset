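; Selectable RTS actor that changes its outline stencil group when hovered or selected.
; Its StaticMesh renders custom depth and switches stencil values between idle, hovered and selected groups.
; Cursor-over events drive hover, and select/deselect interface events drive selection.
; No selection state is tracked, so hover changes overwrite the selected stencil; player-controller interface functions are empty or default stubs.
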(event OnBeginCursorOver(StaticMesh)
  (params (TouchedComponent :type Primitive%20Component%20Object%20Reference))
  (CallFunction|OnHoveredCE))

(event OnEndCursorOver(StaticMesh)
  (params (TouchedComponent :type Primitive%20Component%20Object%20Reference))
  (CallFunction|OnUnhoveredCE))

(event Custom|OnUnhovered_CE
  (Rendering|SetCustomDepthStencilValue (Variables|Default|GetStaticMesh) (Variables|Default|GetIdleStateGroup)))

(event Custom|OnSelected
  (Rendering|SetCustomDepthStencilValue (Variables|Default|GetStaticMesh) (Variables|Default|GetSelectedStateGroup)))

(event Custom|OnUnselected
  (Rendering|SetCustomDepthStencilValue (Variables|Default|GetStaticMesh) (Variables|Default|GetIdleStateGroup)))

(event Custom|OnHovered_CE
  (Development|PrintString "Selection")
  (Rendering|SetCustomDepthStencilValue (Variables|Default|GetStaticMesh) (Variables|Default|GetHoveredStateGroup)))

(event EventBeginPlay
  (Rendering|SetCustomDepthStencilValue (Variables|Default|GetStaticMesh) (Variables|Default|GetIdleStateGroup))
  (Rendering|SetRenderCustomDepth (Variables|Default|GetStaticMesh) true)
  (Rendering|SetRenderCustomDepth (Variables|Default|GetStaticMesh) true))

(event EventLSISelectActorI
  (params (PlayerSelecting-dontNeedQ :type Player%20Controller%20Object%20Reference))
  (CallFunction|OnSelected))

(event EventLSIDeselectActorI
  (params (PlayerDeselecting :type Player%20Controller%20Object%20Reference))
  (CallFunction|OnUnselected))

(fn ConstructionScript)

(fn PcBICameraPerspectiveModeGETI
  (return "NewEnumerator0"))

(fn PcBIHUDGameplayUIGETI-notactualyUsedQ
  (return 0))

(fn PcBIRtsIsoHoverActorGETI
  (return 0))

(fn PcBIRtsIsoMouseCursorActorGETI
  (return 0))

(fn PcBISquadMemberLoadoutCharactersGETI
  (return 0))

(fn PcBISquadMemeberbyIdNameGETI
  (params (CharacterPresetID :type Primary%20Data%20Asset%20Object%20Reference))
  (return 0 false))