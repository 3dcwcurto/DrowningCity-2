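; Player controller for take recording that triggers character animations on demand from input.
; On possess it sets a camera perspective mode, and the slot inputs stop the current montage or play talk, wave and think montages on the controlled character's anim instance.
; The T key flip-flops the locomotion character's turn-in-place mode.
; Draw/sheath, spell and dialogue action calls are present but never run.
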(event EventBeginPlay
  ;[0.2507 1 0] BeginPlay
  (|CallParentFunction))

(event EventTick
  (params (DeltaSeconds :type Float%20%28single-precision%29))
  (|CallParentFunction DeltaSeconds) ; This node is disabled and will not be called.\nDrag off pins to build functionality.
)

(event EventPossess
  (params (PossessedPawn :type Pawn%20Object%20Reference))
  ;[0 1 0.4249] Possess
  (|CallParentFunction PossessedPawn)
  (CallFunction|CameraCameraPerspectiveModeF "NewEnumerator2" PossessedPawn))

(event Input|ActionEvents|InputActionSelectSlot4Four
  (params (Key :type Key%20Structure))
  ;[1 1 1] AnimMontages
  (:Pressed
    (bind _returnvalue (CallFunction|OwnedCharacterAnimInstanceF))
    ;;[1 1 1] Think
    (Animation|Montage|MontagePlay _returnvalue "/Game/01AnimationAssets/NpcGeneric/Anim_Thinking_Montage.Anim_Thinking_Montage" 1.0 "MontageLength" 0.0 true)))

(event Input|ActionEvents|InputActionSelectSlot1One
  (params (Key :type Key%20Structure))
  ;[1 1 1] AnimMontages
  (:Pressed
    (bind _returnvalue (CallFunction|OwnedCharacterAnimInstanceF))
    ;;[1 1 1] Cancel
    (Animation|Montage|MontageStop _returnvalue 0.1 0)))

(event Input|ActionEvents|InputActionSelectSlot3Three
  (params (Key :type Key%20Structure))
  ;[1 1 1] AnimMontages
  (:Pressed
    (bind _returnvalue (CallFunction|OwnedCharacterAnimInstanceF))
    ;;[1 1 1] Wave
    (Animation|Montage|MontagePlay _returnvalue "/Game/01AnimationAssets/NpcGeneric/Anim_Wave_1_Montage.Anim_Wave_1_Montage" 1.0 "MontageLength" 0.0 true)))

(event Input|ActionEvents|InputActionSelectSlot2Two
  (params (Key :type Key%20Structure))
  ;[1 1 1] AnimMontages
  (:Pressed
    (Development|PrintString "TakeRecovereasdasdas")
    (bind _returnvalue (CallFunction|OwnedCharacterAnimInstanceF))
    ;;[1 1 1] Talkv3
    (Animation|Montage|MontagePlay _returnvalue "/Game/01AnimationAssets/NpcGeneric/Anim_Talking_3_Montage.Anim_Talking_3_Montage" 1.0 "MontageLength" 0.0 true)))

(event Input|KeyboardEvents|T
  (params (Key :type Key%20Structure))
  ;[1 1 1] TurnInPlace ToggleMontage
  (:Pressed
    (bind _ascharacter (Utilities|Casting|CastToCharacter (Pawn|GetControlledPawn)))
    (bind _asbp_character_locomotion_c_c (Utilities|Casting|CastToBP_CharacterLocomotion_cC _ascharacter))
    (Utilities|FlowControl|FlipFlop
      (:A
        (Default|Loco:TurninPlaceModeAnimBpUPDATEF _asbp_character_locomotion_c_c "NewEnumerator0"))
      (:B
        (Default|Loco:TurninPlaceModeAnimBpUPDATEF _asbp_character_locomotion_c_c "NewEnumerator1")))))

(fn ConstructionScript
  (|CallParentFunction))

(fn OwnedCharacterAnimInstanceF
  (bind _ascharacter (Utilities|Casting|CastToCharacter (Pawn|GetControlledPawn)))
  (return (Components|SkeletalMesh|GetAnimInstance (Variables|/Script/Engine.Character|GetMesh _ascharacter))))