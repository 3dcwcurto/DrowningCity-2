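; Game State that acts as the central registry for team factions, covering hierarchy rosters and diplomacy alignment.
; Each faction preset maps to an index shared with the GameInstance's save data, which registers missing factions.
; That index selects a lazily created BP_TeamFactionManagementSystem_O per faction, which receives roster additions and war declarations and supplies getter data.
; Town-camp registration is unhooked, its lookup is stubbed, and the war-declaration event is marked DontUse.
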(event EventGSTFDTeamFactionHierarchyRosterDispatcherI
  (params (Character :type Character%20Object%20Reference))
  ;[1 1 1] HierachyRoster
  (CallFunction|HierarchyRosterAddF-newx Character))

(event EventTick
  (params (DeltaSeconds :type Float%20%28single-precision%29)))

(event EventGSTFDTeamFactionTownCampAddI
  (params (TownCampSceneActor :type Actor%20Object%20Reference))
  ;[0 1 0.3728] TownCamp
)

(event EventGSTFDDeclareWarHostileUnconfirmedI-notNeeded
  (params (TeamFactionPresetID-Delcaring :type Primary%20Data%20Asset%20Object%20Reference) (TeamFactionPresetID-Target :type Primary%20Data%20Asset%20Object%20Reference))
  ;[0 0 0] DontUse: Dont want characters far away know right away to attack player who commited a crime.
  (CallFunction|GSTFDDeclareWarHostileUnconfrimedF TeamFactionPresetID-Delcaring TeamFactionPresetID-Target))

(event EventGSTFDCrimeReport-HiddenSharedTeamOrganizerI
  (params (CrimeInfo :type S%20Record%20Crime%20Assistance%2002%20Structure)))

(event EventBeginPlay)

(fn ConstructionScript)

(fn LoadSaveTeamFactionF
  (params (TeamFactionPresetIDFind :type Primary%20Data%20Asset%20Object%20Reference))
  (bind _output_get (LocalVariables|SetTeamFactionPresetID_Local TeamFactionPresetIDFind))
  (Utilities|IsValid _output_get
    (:Is%20Valid
      (bind _savegamedata (Class|BPIGameInstanceInterfaceI|GIISaveGameDataCurrentGetI(Message) (Game|GetGameInstance)))
      (Utilities|IsValid _savegamedata
        (:Is%20Valid
          (bind _teamfactionpresetid_logindexerx (Class|BPISaveGameDataInterfaceI|SGDISaveGameDataInfoGETI(Message) _savegamedata))
          (if (Utilities|Array|ContainsItem _teamfactionpresetid_logindexerx (LocalVariables|GetTeamFactionPresetID_Local))
            (Utilities|Array|SetArrayElem (Variables|Default|GetTeamFactionPreset-IDLogIndexer) (Utilities|Array|FindItem _teamfactionpresetid_logindexerx (LocalVariables|GetTeamFactionPresetID_Local)) (LocalVariables|GetTeamFactionPresetID_Local) true)
            (return (Utilities|Array|FindItem _teamfactionpresetid_logindexerx (LocalVariables|GetTeamFactionPresetID_Local)))
            (else
              (bind _index (Class|BPISaveGameDataInterfaceI|SGDISaveGameDataInfoADDMissingTeamFactionI(Message) _savegamedata (LocalVariables|GetTeamFactionPresetID_Local)))
              (Development|PrintString (Utilities|String|Append (Utilities|GetDisplayName (LocalVariables|GetTeamFactionPresetID_Local)) ":  SaveGameData missing tamefaction"))
              (Utilities|Array|SetArrayElem (Variables|Default|GetTeamFactionPreset-IDLogIndexer) _index (LocalVariables|GetTeamFactionPresetID_Local) true)
              (return _index))))
        (:Is%20Not%20Valid
          (Development|PrintString "SaveGameDataNot Valid. Check if gameinstance is valid")
          ;[1 0.9415 0.2285] TodoLater:setup fallback system?
          (return 0))))
    (:Is%20Not%20Valid
      (return 0))))

(fn LoadSavedGameDataFx
  (bind _returnvalue (Game|GetGameInstance))
  (Utilities|IsValid _returnvalue
    (:Is%20Valid
      (bind _savegamedata (Class|BPIGameInstanceInterfaceI|GIISaveGameDataCurrentGetI(Message) _returnvalue))
      (Utilities|IsValid _savegamedata
        (:Is%20Valid
          (bind _teamfactionpresetid_logindexerx (Class|BPISaveGameDataInterfaceI|SGDISaveGameDataInfoGETI(Message) _savegamedata))
          (Variables|Default|SetTeamFactionPreset-IDLogIndexer _teamfactionpresetid_logindexerx))))))

(fn ManagementSystem-FindCreatePureF-newx
  (params (TeamFactionIdIndexer :type Integer) (TeamFactionPresetID :type Primary%20Data%20Asset%20Object%20Reference))
  (bind _teamfactionmanagementsystem (Variables|Default|GetTeamFactionManagementSystem))
  (bind _output (Utilities|Array|Get(acopy) _teamfactionmanagementsystem TeamFactionIdIndexer))
  (Utilities|IsValid _output
    (:Is%20Valid
      ;[1 1 1] Found
      (return _output ""))
    (:Is%20Not%20Valid
      ;[1 1 1] Create
      (bind _returnvalue (Game|AddComponentbyClass "/Game/06GsTeamFactions/TeamFactionPreset/BP_TeamFactionManagementSystem_O.BP_TeamFactionManagementSystem_O_C"))
      (Utilities|Array|SetArrayElem (Variables|Default|GetTeamFactionManagementSystem) TeamFactionIdIndexer _returnvalue true)
      (Default|TeamFactionManagementSystemSetupCE _returnvalue TeamFactionPresetID)
      (return _returnvalue ""))))

(fn TeamFactionPresetIDLogIndex-FindCreatePureFv2x
  (params (TeamFactionPreset :type Primary%20Data%20Asset%20Object%20Reference) (DebugLocation:TownCampVsTownHierachyVsDiplomacyAlignment :type Name))
  (bind _teamfactionpreset_idlogindexer (Variables|Default|GetTeamFactionPreset-IDLogIndexer))
  (LocalVariables|SetDebugLocation:TownCampVsTownHierachyVsDiplomacyAlignment_Local DebugLocation:TownCampVsTownHierachyVsDiplomacyAlignment)
  (bind _output_get (LocalVariables|SetTeamFactionPresetID_Local TeamFactionPreset))
  (if (Utilities|Array|ContainsItem _teamfactionpreset_idlogindexer _output_get)
    (return (Utilities|Array|FindItem _teamfactionpreset_idlogindexer _output_get) true)
    (else
      ;[1 1 1] GameInstance SavedData
      (bind _newindex (CallFunction|LoadSaveTeamFactionF (LocalVariables|GetTeamFactionPresetID_Local)))
      (return _newindex true))))

(fn TownCampLoadSaveFindCreateF-old
  (for _array_element 0
    _))

(fn TownCampAddF-replaced-old
  (params (TownCampSceneActor :type Actor%20Object%20Reference)))

(fn TownCampFindCreateFv2-old
  (params (TownCampPresetID :type Primary%20Data%20Asset%20Object%20Reference) (TeamFactionPresetID :type Primary%20Data%20Asset%20Object%20Reference)))

(fn TownCampFindCreateF-replaced-old
  (params (TownCampNameID :type Gameplay%20Tag%20Structure) (TeamFaction :type Gameplay%20Tag%20Structure)))

(fn CharacterPresetIDLogIndexerFindCreatePureF-old
  (params (CharacterPresetLogIndexer :type Array%20of%20Primary%20Data%20Asset%20Object%20References) (CharacterPresetID :type Primary%20Data%20Asset%20Object%20Reference) (TeamFaction :type Primary%20Data%20Asset%20Object%20Reference))
  (if (Utilities|Array|ContainsItem CharacterPresetLogIndexer CharacterPresetID)
    (return CharacterPresetLogIndexer true (Utilities|Array|FindItem CharacterPresetLogIndexer CharacterPresetID))
    (else
      (bind _hierarchyrosterdefault (Class|BPITeamFactionPresetInterfaceI|TFPITeamFactionPresetInfoGETI(Message) TeamFaction))
      (if (Utilities|Array|ContainsItem _hierarchyrosterdefault CharacterPresetID)
        (return _hierarchyrosterdefault (Utilities|Array|ContainsItem _hierarchyrosterdefault CharacterPresetID) (Utilities|Array|FindItem _hierarchyrosterdefault CharacterPresetID))
        (else
          (Development|PrintString "BPGameStateTeamDiplomacyGS>CharacterPersetIDLogIndexerFIndCreatePureF== not contained " true true "(R=1.000000,G=0.368925,B=0.000000,A=1.000000)" 22.0)
          (return 0 false 0))))))

(fn HierarchyRosterAddFv2-old
  (params (Character :type Character%20Object%20Reference)))

(fn HierarchyRosterAddF-newx
  (params (Character :type Character%20Object%20Reference))
  (bind _output_get (LocalVariables|SetCharacterRuntime_Local Character))
  (bind _pdacharacterpreset (Class|BPICharacterBaseInterface|CBICharacterPresetPdaGETI(Message) _output_get))
  (bind _output_get_2 (LocalVariables|SetCharacterPresetID_Local _pdacharacterpreset))
  (bind _teamfactionpresetid (Class|BPICharacterPresetInterface|HCPICharacterPresetInfoGETI(Message) _output_get_2))
  (bind _output_get_3 (LocalVariables|SetTeamFactionPresetID_Local _teamfactionpresetid))
  (Utilities|IsValid (.TeamFactionManagementSystem (CallFunction|ManagementSystem-FindCreatePureF-newx (.TeamFactionIdIndexer (CallFunction|TeamFactionPresetIDLogIndex-FindCreatePureFv2x _teamfactionpresetid "CharacterHieracyh")) _output_get_3))
    (:Is%20Valid
      (Default|TeamFactionManagementSetup-HeirarchyRosterAddCE (.TeamFactionManagementSystem (CallFunction|ManagementSystem-FindCreatePureF-newx (.TeamFactionIdIndexer (CallFunction|TeamFactionPresetIDLogIndex-FindCreatePureFv2x _teamfactionpresetid "CharacterHieracyh")) _output_get_3)) (LocalVariables|GetCharacterRuntime_Local)))))

(fn TownCampAddFv2
  (params (TownCampSceneActor :type Actor%20Object%20Reference))
  ;[1 1 1] Actor
  (bind _output_get (LocalVariables|SetCampTownActorRuntime_Local TownCampSceneActor))
  (bind _camptownpresetid (Class|BPICampTownActorInterfaceI|CTGICampTownPresetPdaGETI(Message) _output_get))
  ;[1 1 1] Preset
  (bind _output_get_2 (LocalVariables|SetTownCampPresetID_Local _camptownpresetid))
  (bind _teamfactionpreset (Class|BPICampTownPresetInterfaceI|TownCampPresetInfoGETI(Message) _output_get_2))
  (bind _output_get_3 (LocalVariables|SetTeamFactionPresetID_Local _teamfactionpreset))
  (Default|TeamFactionManagementSystem-TownCampAddCE (.TeamFactionManagementSystem (CallFunction|ManagementSystem-FindCreatePureF-newx (.TeamFactionIdIndexer (CallFunction|TeamFactionPresetIDLogIndex-FindCreatePureFv2x _output_get_3 "TownCamp")) (LocalVariables|GetTeamFactionPresetID_Local))) (LocalVariables|GetCampTownActorRuntime_Local)))

(fn GSTFDDeclareWarHostileUnconfrimedF
  (params (TeamFactionPresetID-Declaring :type Primary%20Data%20Asset%20Object%20Reference) (TeamFactionPresetID-Target :type Primary%20Data%20Asset%20Object%20Reference))
  (bind (_teamfactionidindexer _valid_dontneed) (CallFunction|TeamFactionPresetIDLogIndex-FindCreatePureFv2x TeamFactionPresetID-Declaring "None"))
  (if _valid_dontneed
    (Utilities|IsValid (.TeamFactionManagementSystem (CallFunction|ManagementSystem-FindCreatePureF-newx _teamfactionidindexer TeamFactionPresetID-Target))
      (:Is%20Valid
        (Default|ManagerSystem-DeclareWarHostileUnconfirmedCE (Utilities|Array|Get(acopy) (Variables|Default|GetTeamFactionManagementSystem) _teamfactionidindexer) TeamFactionPresetID-Target)))))

(fn GSTFDLeaderPlayerControllerGETI
  (return (Variables|Default|GetQuestLeader-PlayerController) (Variables|Default|GetDialogueLeader-PlayerController)))

(fn GSTFDTeamFactionDiplomacyAlignmentGETI
  (params (TeamFactionPresetID :type Primary%20Data%20Asset%20Object%20Reference))
  (return (.DiplomacyAlignment (CallFunction|ManagementSystem-FindCreatePureF-newx (.TeamFactionIdIndexer (CallFunction|TeamFactionPresetIDLogIndex-FindCreatePureFv2x TeamFactionPresetID "DiplomacyAlignmnet")) TeamFactionPresetID))))

(fn GSTFDTeamFactionHierachyRosterGETI
  (params (CharacterPresetID-_ :type Primary%20Data%20Asset%20Object%20Reference))
  (bind _output_get (LocalVariables|SetCharacterPresetID_Local CharacterPresetID-_))
  (bind _teamfactionpresetid (Class|BPICharacterPresetInterface|HCPICharacterPresetInfoGETI(Message) _output_get))
  (Utilities|IsValid _teamfactionpresetid
    (:Is%20Valid
      (Utilities|IsValid (Utilities|Array|Get(acopy) (Variables|Default|GetTeamFactionManagementSystem) (.TeamFactionIdIndexer (CallFunction|TeamFactionPresetIDLogIndex-FindCreatePureFv2x _teamfactionpresetid "None")))
        (:Is%20Valid
          (Utilities|IsValid (.CharacterRuntime (Utilities|Struct|BreakS_HierarchyRoster02CharactersRoster (Utilities|Array|Get(acopy) (Variables|/Game/06GsTeamFactions/TeamFactionPreset/BP_TeamFactionManagementSystem_O.BP_TeamFactionManagementSystem_O_C|GetHierarchyRosterInfoArray (Utilities|Array|Get(acopy) (Variables|Default|GetTeamFactionManagementSystem) (.TeamFactionIdIndexer (CallFunction|TeamFactionPresetIDLogIndex-FindCreatePureFv2x _teamfactionpresetid "None")))) (Utilities|Array|FindItem (Variables|/Game/06GsTeamFactions/TeamFactionPreset/BP_TeamFactionManagementSystem_O.BP_TeamFactionManagementSystem_O_C|GetHierarchyRosterPresetID-LogIndexer (Utilities|Array|Get(acopy) (Variables|Default|GetTeamFactionManagementSystem) (.TeamFactionIdIndexer (CallFunction|TeamFactionPresetIDLogIndex-FindCreatePureFv2x _teamfactionpresetid "None")))) (LocalVariables|GetCharacterPresetID_Local)))))
            (:Is%20Valid
              (return (.CharacterRuntime (Utilities|Struct|BreakS_HierarchyRoster02CharactersRoster (Utilities|Array|Get(acopy) (Variables|/Game/06GsTeamFactions/TeamFactionPreset/BP_TeamFactionManagementSystem_O.BP_TeamFactionManagementSystem_O_C|GetHierarchyRosterInfoArray (Utilities|Array|Get(acopy) (Variables|Default|GetTeamFactionManagementSystem) (.TeamFactionIdIndexer (CallFunction|TeamFactionPresetIDLogIndex-FindCreatePureFv2x _teamfactionpresetid "None")))) (Utilities|Array|FindItem (Variables|/Game/06GsTeamFactions/TeamFactionPreset/BP_TeamFactionManagementSystem_O.BP_TeamFactionManagementSystem_O_C|GetHierarchyRosterPresetID-LogIndexer (Utilities|Array|Get(acopy) (Variables|Default|GetTeamFactionManagementSystem) (.TeamFactionIdIndexer (CallFunction|TeamFactionPresetIDLogIndex-FindCreatePureFv2x _teamfactionpresetid "None")))) (LocalVariables|GetCharacterPresetID_Local)))))))
            (:Is%20Not%20Valid
              (Development|PrintString "GameStateTeamDiplomacy>TeamFactionHiearchyRosterGET== TeamFaction Character is not valid" true true "(R=1.000000,G=0.868055,B=0.000000,A=1.000000)" 22.0)
              (return 0))))
        (:Is%20Not%20Valid
          (Development|PrintString "GameStateTeamDiplomacy>TeamFactionHiearchyRosterGET== TeamFactionOBJECT not valid" true true "(R=1.000000,G=0.868055,B=0.000000,A=1.000000)" 22.0)
          (return 0))))
    (:Is%20Not%20Valid
      (Development|PrintString "GameStateTeamDiplomacy>TeamFactionHiearchyRosterGET== TeamFactionPresetID not valid" true true "(R=1.000000,G=0.608595,B=0.000000,A=1.000000)" 22.0)
      (return 0))))

(fn GSTFDTeamFactionTownCampFindCreateI
  (params (TeamFactionID :type Gameplay%20Tag%20Structure) (TownCampNameID :type Gameplay%20Tag%20Structure) (TeamFactionPresetID :type Primary%20Data%20Asset%20Object%20Reference) (TowncampPresetID :type Primary%20Data%20Asset%20Object%20Reference))
  (bind _towncampactor (old|TownCampFindCreateFv2-old TeamFactionPresetID TowncampPresetID))
  (return _towncampactor))