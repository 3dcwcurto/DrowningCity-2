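; Retired team-faction diplomacy component, in a "replaced" folder, for telling how other characters' factions relate to its own.
; It fetches diplomacy from the GameState through an interface message and caches it.
; The main compare searches neutral, allied, then enemy lists, defaulting to the neutral result, but passes a class while the helper matches preset IDs.
; Enemy filters for perceived actors and hit results are disconnected, so they never add enemies.
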(event EventBeginPlay)

(event EventTick
  (params (DeltaSeconds :type Float%20%28single-precision%29)))

(fn TeamFactionEnemyCheckActorsF-todo-Replaced
  (params (PercievedActors :type Array%20of%20Actor%20Object%20References))
  (if (> (Utilities|Array|Length (.Enemy_FactionsHated_War (Utilities|Struct|BreakS_DiplomacyAlignment01 (Variables|00TeamFaction|GetTeamFactionDiplomacyOfSelf)))) 0)
    (for _array_element PercievedActors
      _)
    (else
      (Development|PrintString (Utilities|String|Append "ACTeamsFactions>CheckIfHitResultAreEnemies " (Utilities|GetClassDisplayName (Variables|00TeamFaction|GetTeamFactionClass)) "TeamFaction does not have enemies") true true "(R=1.000000,G=0.000000,B=0.044178,A=1.000000)")))
  (return (LocalVariables|GetEnemiesConfirmed_Local)))

(fn TeamFactionEnemyCheckHitResultF-todo-Replaced
  (params (HitResult :type Array%20of%20Hit%20Result%20Structures))
  ;[1 1 1] TodoLater: get diplomacy info on beingplay? then update when there are diplomacy changes??? or always get when needing to do teamchecks?
  (bind _teamfactiondiplomacyofself (CallFunction|TeamFactionDiplomacyInfoGETF-Replaced))
  (if (> (Utilities|Array|Length (.Enemy_FactionsHated_War (Utilities|Struct|BreakS_DiplomacyAlignment01 _teamfactiondiplomacyofself))) 0)
    (for _array_element HitResult
      (Utilities|Casting|CastToCharacter (.HitActor (Collision|BreakHitResult _array_element))))
    (else
      (Development|PrintString (Utilities|String|Append "BPInfoTeamsFactionsHierachyLeadership>TeamFactionCheckIfHitResultF==" (Utilities|GetClassDisplayName (Variables|00TeamFaction|GetTeamFactionClass)) "TeamFaction does not have enemies") true true "(R=1.000000,G=0.000000,B=0.044178,A=1.000000)")))
  (return (LocalVariables|GetHitResultEnemyConfirmed_Local)))

(fn TeamFactionDiplomacyInfoGETF-Replaced
  (params (TeamFactionPresetID :type Primary%20Data%20Asset%20Object%20Reference))
  (bind _teamfactiondiplomacy (Class|BPIGameStateTeamFactionDiplomacyI|GSTFDTeamFactionDiplomacyAlignmentGETI(Message) (Game|GetGameState) TeamFactionPresetID))
  (bind _output_get (Variables|00TeamFaction|SetTeamFactionDiplomacyOfSelf _teamfactiondiplomacy))
  (return _output_get))

(fn EnemyClosestF-todoQ-Replaced)

(fn TeamFactionEnemiesGETF-Old-Replaced)

(fn TeamFactionInfoF-Old-oReplaced
  (bind _teamfactionclass (Variables|00TeamFaction|GetTeamFactionClass))
  (if (Utilities|IsValidClass _teamfactionclass)
    (return _teamfactionclass)
    (else
      (Development|PrintString "ACTeamFaction>TeamValidCheck== Team not Valid" true true "(R=1.000000,G=0.287168,B=0.000000,A=1.000000)" 22.0)
      ;[1 1 1] FallBack Nuetral
      (return 0))))

(fn TeamFactionCompareF-Replaced
  (params (TeamFactionDiplomacy :type Array%20of%20S%20Diplomacy%20Alignment%2002%20Amity%20Hate%20Structures) (TeamFactionOfOtherCharaterToCompareClass :type BP%20Team%20Faction%20Preset%2000%20Parent%20O%20Class%20Reference) (TeamFactionOfOtherCharaterToComparePda :type Primary%20Data%20Asset%20Object%20Reference))
  (LocalVariables|SetFoundValid_Local false)
  (bind _array_element (Utilities|Array|ForEachLoopwithBreak TeamFactionDiplomacy :!label _label)
    (:LoopBody
      (if (== (.TeamFactionPresetID (Utilities|Struct|BreakS_DiplomacyAlignment02AmityHate _array_element)) TeamFactionOfOtherCharaterToComparePda)
        (LocalVariables|SetFoundValid_Local true)
        (goto _label Break)))
    (:Completed
      (return (LocalVariables|GetFoundValid_Local)))))

(fn TeamFactionCompareMainF-Replaced
  (params (TeamFactionOfOtherCharaterToCompare :type BP%20Team%20Faction%20Preset%2000%20Parent%20O%20Class%20Reference))
  (LocalVariables|SetTeamFactionOfOtherCharacterToCompare_Local TeamFactionOfOtherCharaterToCompare)
  (bind _teamfactiondiplomacyofself (CallFunction|TeamFactionDiplomacyInfoGETF-Replaced))
  (bind _foundvalid (CallFunction|TeamFactionCompareF-Replaced (.NUetral_Factions (Utilities|Struct|BreakS_DiplomacyAlignment01 _teamfactiondiplomacyofself)) (LocalVariables|GetTeamFactionOfOtherCharacterToCompare_Local)))
  (if _foundvalid
    (LocalVariables|SetTeamFactionRelationshipAlignment_Local "NewEnumerator2")
    (else
      (bind _foundvalid_2 (CallFunction|TeamFactionCompareF-Replaced (.Allied_FactionsLiked_Alliance (Utilities|Struct|BreakS_DiplomacyAlignment01 _teamfactiondiplomacyofself)) (LocalVariables|GetTeamFactionOfOtherCharacterToCompare_Local)))
      (if _foundvalid_2
        (LocalVariables|SetTeamFactionRelationshipAlignment_Local "NewEnumerator1")
        (else
          (bind _foundvalid_3 (CallFunction|TeamFactionCompareF-Replaced (.Enemy_FactionsHated_War (Utilities|Struct|BreakS_DiplomacyAlignment01 _teamfactiondiplomacyofself)) (LocalVariables|GetTeamFactionOfOtherCharacterToCompare_Local)))
          (if _foundvalid_3
            (LocalVariables|SetTeamFactionRelationshipAlignment_Local "NewEnumerator3")
            (else
              (Development|PrintString "BPinfoTeamFactionHierarchyLeadershipAC>TeamFactionCompareMainF--  Faction not found in DiplomacyOfSelf" true true "(R=1.000000,G=0.426837,B=0.000000,A=1.000000)" 22.0)
              (LocalVariables|SetTeamFactionRelationshipAlignment_Local "NewEnumerator2")))))))
  (return (LocalVariables|GetTeamFactionRelationshipAlignment_Local)))

(fn TeamFactionPlayerTeamOfSelfF-Replaced
  (return (== (Variables|00TeamFaction|GetTeamFactionClass) 0)))

(fn TeamFactionPlayerTeamOtherCharacterF-Replaced
  (params (TeamFactionOfOtherCharacter :type BP%20Team%20Faction%20Preset%2000%20Parent%20O%20Class%20Reference))
  (return (== (Variables|00TeamFaction|GetTeamFactionClass) TeamFactionOfOtherCharacter)))