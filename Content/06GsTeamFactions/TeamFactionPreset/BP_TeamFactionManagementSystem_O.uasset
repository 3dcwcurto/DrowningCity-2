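; Per-faction management system that tracks one team faction's character roster, town camps and diplomatic standing.
; Setup seeds ally, neutral and enemy lists from the faction preset, using preset-ID arrays as indexes into parallel struct arrays.
; Find-or-create functions register runtime characters and camps, though new camps only gain an index entry because their struct write is unconnected.
; Unconfirmed-hostile war declaration is marked DontUse; save loading and witness reports are stubs.
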(event Custom|TeamFactionManagementSystemLoadFile_CE
  (params (TeamFactionPreset :type Primary%20Data%20Asset%20Object%20Reference) (AlliesEnemiesNeutralLoadedSave-todo :type Boolean)))

(event Custom|TeamFactionManagementSystem-TownCampAdd_CE
  (params (TownCampActor :type Actor%20Object%20Reference))
  ;[1 1 1] TownCampActorAdd
  (CallFunction|ManagementSystem-TownCamp-FindCreateF TownCampActor))

(event Custom|TeamFactionManagementSetup-HeirarchyRosterAdd_CE
  (params (Character :type Character%20Object%20Reference))
  ;[1 1 1] HeirarchyRosterCharacterAdd
  (CallFunction|ManagementSystem-HeirarchyRosterFindCreateF Character))

(event Custom|TeamFactionManagementSystemSetup_CE
  (params (TeamFactionPreset :type Primary%20Data%20Asset%20Object%20Reference))
  (CallFunction|ManagementSystem-SetupF TeamFactionPreset))

(event Custom|ManagerSystem-DeclareWarHostileUnconfirmed_CE
  (params (TeamFactionPresetID-Target :type Primary%20Data%20Asset%20Object%20Reference))
  ;[0.05729 0.05729 0.05729] DontUse: Dont want characters far away know right away to attack player who commited a crime.
  (CallFunction|ManagementSystem-DeclareWarHostileUnconfirmedF TeamFactionPresetID-Target))

(event Custom|ManagerSystem-DiplomacyAlignmentWitnessReport_CE)

(event EventBeginPlay)

(event EventTick
  (params (DeltaSeconds :type Float%20%28single-precision%29)))

(fn ManagementSystem-SetupF
  (params (TeamFactionPreset :type Primary%20Data%20Asset%20Object%20Reference))
  (bind _output_get (Variables|Default|SetTeamFactionPresetIDOfSelf TeamFactionPreset))
  (bind (_towncamps _hierarchyrosterdefault _diplomaticalignment_enemiesstartdefault _diplomaticalignment_alliesstartdefault _diplomaticalignment_nuetralstartdefault) (Class|BPITeamFactionPresetInterfaceI|TFPITeamFactionPresetInfoGETI(Message) _output_get))
  (Variables|Default|SetTowncampPresetID-LogIndexer _towncamps)
  (Variables|Default|SetHierarchyRosterPresetID-LogIndexer _hierarchyrosterdefault)
  (bind _output_get_2 (Variables|DiplomaticAlignment|SetDiplomaticAlignment-Enemy-LogIndexer _diplomaticalignment_enemiesstartdefault))
  (CallFunction|ManagementSystem-DiplomacyAlignment-DefaultSetupF _output_get_2 "NewEnumerator3")
  (bind _output_get_3 (Variables|DiplomaticAlignment|SetDiplomaticAlignment-Ally-LogIndexer _diplomaticalignment_alliesstartdefault))
  (CallFunction|ManagementSystem-DiplomacyAlignment-DefaultSetupF _output_get_3 "NewEnumerator1")
  (bind _output_get_4 (Variables|DiplomaticAlignment|SetDiplomaticAlignment-Nuetral-LogIndexer _diplomaticalignment_nuetralstartdefault))
  (CallFunction|ManagementSystem-DiplomacyAlignment-DefaultSetupF _output_get_4 "NewEnumerator2"))

(fn ManagementSystem-HeirarchyRosterFindCreateF
  (params (Character :type Character%20Object%20Reference))
  (bind _hierarchyrosterpresetid_logindexer (Variables|Default|GetHierarchyRosterPresetID-LogIndexer))
  (bind _output_get (LocalVariables|SetCharacterRuntime_Local Character))
  (Utilities|IsValid _output_get
    (:Is%20Valid
      (bind _pdacharacterpreset (Class|BPICharacterBaseInterface|CBICharacterPresetPdaGETI(Message) _output_get))
      (Utilities|IsValid _pdacharacterpreset
        (:Is%20Valid
          (if (Utilities|Array|ContainsItem _hierarchyrosterpresetid_logindexer _pdacharacterpreset)
            (LocalVariables|SetCharacterInfo_Local (Utilities|Array|Get(acopy) (Variables|Default|GetHierarchyRosterInfoArray) (Utilities|Array|FindItem _hierarchyrosterpresetid_logindexer _pdacharacterpreset)))
            (bind _bisalive (Class|BPCharacterStatsInterfaceI|CSIAliveGETCheckI(Message) (LocalVariables|GetCharacterRuntime_Local)))
            (bind _structout (Utilities|Struct|SetmembersinS_HierarchyRoster02CharactersRoster (LocalVariables|GetCharacterInfo_Local) (LocalVariables|GetCharacterRuntime_Local) _bisalive))
            (LocalVariables|SetCharacterInfo_Local _structout)
            (Utilities|Array|SetArrayElem (Variables|Default|GetHierarchyRosterInfoArray) (Utilities|Array|FindItem _hierarchyrosterpresetid_logindexer _pdacharacterpreset) (LocalVariables|GetCharacterInfo_Local) true)
            (else
              (Development|PrintString "BPTeamFactionManagementSystemAC>HierarchyRosterAddF== characterPresetID is not in HierarchyRosterlogIndexer" true true "(R=1.000000,G=0.206790,B=0.000000,A=1.000000)" 22.0)
              (Development|PrintString (Utilities|String|Append "(Character==" (Utilities|GetDisplayName _pdacharacterpreset) ") ( Team== " (Utilities|GetDisplayName (Variables|Default|GetTeamFactionPresetIDOfSelf)) ")") true true "(R=1.000000,G=0.206790,B=0.000000,A=1.000000)" 22.0)
              (bind _returnvalue (Utilities|Array|Add (Variables|Default|GetHierarchyRosterPresetID-LogIndexer) _pdacharacterpreset))
              (bind _bisalive_2 (Class|BPCharacterStatsInterfaceI|CSIAliveGETCheckI(Message) (LocalVariables|GetCharacterRuntime_Local)))
              (Utilities|Array|SetArrayElem (Variables|Default|GetHierarchyRosterInfoArray) _returnvalue (Utilities|Struct|MakeS_HierarchyRoster02CharactersRoster (LocalVariables|GetCharacterRuntime_Local) _bisalive_2) true))))))))

(fn ManagementSystem-TownCamp-FindCreateF
  (params (TownCampActor :type Actor%20Object%20Reference))
  (bind _towncamppresetid_logindexer (Variables|Default|GetTowncampPresetID-LogIndexer))
  (bind _output_get (LocalVariables|SetTownCampActor_Local TownCampActor))
  (Utilities|IsValid _output_get
    (:Is%20Valid
      (bind _teamfactionpreset (Class|BPICampTownPresetInterfaceI|TownCampPresetInfoGETI(Message) _output_get))
      (Utilities|IsValid _teamfactionpreset
        (:Is%20Valid
          (if (Utilities|Array|ContainsItem _towncamppresetid_logindexer _teamfactionpreset)
            (LocalVariables|SetCampTownInfo_Local (Utilities|Array|Get(acopy) (Variables|Default|GetTownCampsInfoArray) (Utilities|Array|FindItem _towncamppresetid_logindexer _teamfactionpreset)))
            (bind _structout (Utilities|Struct|SetmembersinS_CampTown02TownManagement (LocalVariables|GetCampTownInfo_Local) (LocalVariables|GetTownCampActor_Local) "NewEnumerator0"))
            (LocalVariables|SetCampTownInfo_Local _structout)
            (Utilities|Array|SetArrayElem (Variables|Default|GetTownCampsInfoArray) (Utilities|Array|FindItem _towncamppresetid_logindexer _teamfactionpreset) (LocalVariables|GetCampTownInfo_Local) true)
            (else
              (bind _returnvalue (Utilities|Array|Add (Variables|Default|GetTowncampPresetID-LogIndexer) _teamfactionpreset)))))))))

(fn ManagementSystem-DiplomacyAlignment-DefaultSetupF
  (params (DiplomaticAlignment :type Array%20of%20Primary%20Data%20Asset%20Object%20References) (Alignment :type E_TeamFactionDiplomacyAlignment%20Enum :default "NewEnumerator0"))
  (switch Utilities|FlowControl|Switch|SwitchonE_TeamFactionDiplomacyAlignment Alignment
    (:NewEnumerator1
      (for (_array_element _array_index) DiplomaticAlignment
        (Utilities|Array|SetArrayElem (Variables|DiplomaticAlignment|GetDiplomaticAlignment-Ally) _array_index (Utilities|Struct|MakeS_DiplomacyAlignment02AmityHate _array_element "NewEnumerator0") true)))
    (:NewEnumerator2
      (for (_array_element_2 _array_index_2) DiplomaticAlignment
        (Utilities|Array|SetArrayElem (Variables|DiplomaticAlignment|GetDiplomaticAlignment-Nuetral) _array_index_2 (Utilities|Struct|MakeS_DiplomacyAlignment02AmityHate _array_element_2 "NewEnumerator0") true)))
    (:NewEnumerator3
      (for (_array_element_3 _array_index_3) DiplomaticAlignment
        (Utilities|Array|SetArrayElem (Variables|DiplomaticAlignment|GetDiplomaticAlignment-Enemy) _array_index_3 (Utilities|Struct|MakeS_DiplomacyAlignment02AmityHate _array_element_3 "NewEnumerator0") true)))))

(fn ManagementSystem-DeclareWarHostileUnconfirmedF
  (params (TeamFactionPresetID-Target :type Primary%20Data%20Asset%20Object%20Reference))
  (bind _diplomaticalignment_unconfirmedhostile_logindexer (Variables|DiplomaticAlignment|GetDiplomaticAlignment-UnconfirmedHostile-LogIndexer))
  (bind _output_get (LocalVariables|SetTeamFactionPresetID_Local TeamFactionPresetID-Target))
  (if (Utilities|Array|ContainsItem _diplomaticalignment_unconfirmedhostile_logindexer _output_get)
    (LocalVariables|SetDiplomacyAlignment_Local (Utilities|Array|Get(acopy) (Variables|DiplomaticAlignment|GetDiplomaticAlignment-UnconfirmedHostile) (Utilities|Array|FindItem _diplomaticalignment_unconfirmedhostile_logindexer _output_get)))
    (bind _structout (Utilities|Struct|SetmembersinS_DiplomacyAlignment02AmityHate (LocalVariables|GetDiplomacyAlignment_Local) (LocalVariables|GetTeamFactionPresetID_Local)))
    (bind _output_get_2 (LocalVariables|SetDiplomacyAlignment_Local _structout))
    (Utilities|Array|SetArrayElem (Variables|DiplomaticAlignment|GetDiplomaticAlignment-UnconfirmedHostile) (Utilities|Array|FindItem _diplomaticalignment_unconfirmedhostile_logindexer _output_get) _output_get_2 true)
    (else
      (bind _returnvalue (Utilities|Array|Add _diplomaticalignment_unconfirmedhostile_logindexer _output_get))
      (Utilities|Array|SetArrayElem (Variables|DiplomaticAlignment|GetDiplomaticAlignment-UnconfirmedHostile) _returnvalue (Utilities|Struct|MakeS_DiplomacyAlignment02AmityHate _output_get "NewEnumerator0") true))))